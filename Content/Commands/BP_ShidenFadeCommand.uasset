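; Shiden scenario command that fades a named screen layer in or out to a target color with configurable easing, duration and Z order.
; PreProcessCommand starts the fade on the widget, and ProcessCommand optionally waits for completion, then saves the layer's color and Z order as scenario properties, encoding fade-out as alpha 1.
; RestoreFromSaveData replays saved fade-outs instantly, and PreviewCommand zeroes the duration for non-current commands.
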(fn `ConvertToEasingFunc`
  (params (EasingFunc :type String))
  (returns (EnumValue :type "EEasingFunc Enum") (Success :type Boolean))
  (switch `string` EasingFunc
    (:`Default`
      (return "Linear" false))
    (:`Linear`
      (return "Linear" true))
    (:`Step`
      (return "Step" true))
    (:`Sinusoidal in`
      (return "SinusoidalIn" true))
    (:`Sinusoidal out`
      (return "SinusoidalOut" true))
    (:`Sinusoidal in out`
      (return "SinusoidalInOut" true))
    (:`Ease in`
      (return "EaseIn" true))
    (:`Ease out`
      (return "EaseOut" true))
    (:`Ease in out`
      (return "EaseInOut" true))
    (:`Expo in`
      (return "ExpoIn" true))
    (:`Expo out`
      (return "ExpoOut" true))
    (:`Expo in out`
      (return "ExpoInOut" true))
    (:`Circular in`
      (return "CircularIn" true))
    (:`Circular out`
      (return "CircularOut" true))
    (:`Circular in out`
      (return "CircularInOut" true))))

(fn `GetFadeInfo`
  (params (FadeType :type String))
  (returns (IsFadeOut :type Boolean))
  (switch `string` FadeType
    (:`FadeOut`
      (return true))
    (:`FadeIn`
      (return false))))

(fn `PreProcessCommand`
  (params (ProcessName :type String) (Command :type "ShidenCommand Structure") (Widget :type "ShidenWidget Object Reference") (ScenarioManager :type "ShidenScenarioManagerInterface Interface (by ref)") (CallerObject :type "Object Object Reference"))
  (returns (Status :type "EShidenPreProcessStatus Enum") (ErrorMessage :type String))
  (bind (_success _errormessage) (`self.StartFade` Command Widget ProcessName))
  (if _success
    (return "Complete" "")
    (else
      (return "Error" _errormessage))))

(fn `PreviewCommand`
  (params (Command :type "ShidenCommand Structure (by ref)") (Widget :type "ShidenWidget Object Reference") (ScenarioManager :type "ShidenScenarioManagerInterface Interface (by ref)") (bIsCurrentCommand :type Boolean))
  (returns (Status :type "EShidenPreviewStatus Enum") (ErrorMessage :type String))
  (locals (TempCommand :type "ShidenCommand Structure"))
  (if bIsCurrentCommand
    (bind (_success _errormessage) (`self.StartFade` Command Widget "Default"))
    (if _success
      (return "Complete" "")
      (else
        (return "Error" _errormessage)))
    (else
      (`BlueprintMapLibrary.Map_Add` (`.Args` (break `ShidenCommand` Command)) "FadeDuration" "0.0")
      (bind (_success_2 _errormessage_2) (`self.StartFade` Command Widget "Default"))
      (if _success_2
        (return "Complete" "")
        (else
          (return "Error" _errormessage_2))))))

(fn `ProcessCommand`
  (params (ProcessName :type String) (Command :type "ShidenCommand Structure") (Widget :type "ShidenWidget Object Reference") (ScenarioManager :type "ShidenScenarioManagerInterface Interface (by ref)") (DeltaTime :type "Float (single-precision)") (CallerObject :type "Object Object Reference"))
  (returns (Status :type "EShidenProcessStatus Enum") (BreakReason :type String) (NextScenarioName :type String) (ErrorMessage :type String))
  (bind (_commandid _benabled _commandname) (break `ShidenCommand` Command))
  (bind (_layername _fadetype _fadeduration _fadefunction _targetcolor _steps _blendexp _waitforcompletion _zorder) (`|GetCommandArguments` "/Shiden/Commands/DA_ShidenPrimaryCommandDefinitions.DA_ShidenPrimaryCommandDefinitions" "Fade" Command))
  (bind _outconvertedvector (`KismetStringLibrary.Conv_StringToVector` _targetcolor))
  (if (`KismetStringLibrary.EqualEqual_StrStr` _waitforcompletion "true")
    (if (`ShidenWidget.IsFadeCompleted` Widget _layername)
      _
      (else
        (return "DelayUntilNextTick" "" "" ""))))
  (`ShidenCommandFunctionLibrary.RegisterScenarioProperty` _commandname (`KismetStringLibrary.Concat_StrStr` _layername "::Color") (`KismetStringLibrary.Conv_ColorToString` (`KismetMathLibrary.MakeColor` (.x _outconvertedvector) (.y _outconvertedvector) (.z _outconvertedvector) (`KismetMathLibrary.SelectFloat` 1.0 0.0 (`self.GetFadeInfo` _fadetype)))))
  (`ShidenCommandFunctionLibrary.RegisterScenarioProperty` _commandname (`KismetStringLibrary.Concat_StrStr` _layername "::ZOrder") _zorder)
  (return "Next" "" "" ""))

(fn `RestoreFromSaveData`
  (params (ScenarioProperties :type "Map of String to String (by ref)") (Widget :type "ShidenWidget Object Reference") (ScenarioManager :type "ShidenScenarioManagerInterface Interface (by ref)") (CallerObject :type "Object Object Reference"))
  (returns (Status :type "EShidenInitFromSaveDataStatus Enum") (ErrorMessage :type String))
  (bind _keys (`BlueprintMapLibrary.Map_Keys` ScenarioProperties))
  (for _array_element _keys
    (bind (_lefts _rights) (`KismetStringLibrary.Split` _array_element "::"))
    (if (`KismetStringLibrary.EqualEqual_StrStr` _rights "Color")
      (bind _value (`BlueprintMapLibrary.Map_Find` ScenarioProperties _array_element))
      (bind (_outconvertedcolor _outisvalid) (`KismetStringLibrary.Conv_StringToColor` _value))
      (if _outisvalid
        (if (== (`.A` (`KismetMathLibrary.BreakColor` _outconvertedcolor)) 1.0)
          (bind (_success _errormessage) (`self.StartFade` (make `ShidenCommand` "00000000000000000000000000000000" true "Fade" "" (`|MakeMap` "LayerName" _lefts "FadeType" "FadeOut" "FadeDuration" "0.0" "FadeFunction" "Linear" "TargetColor" _value "Steps" "2" "BlendExp" "2.0" "WaitForCompletion" "true" "ZOrder" (`BlueprintMapLibrary.Map_Find` ScenarioProperties (`KismetStringLibrary.Concat_StrStr` _lefts "::ZOrder")))) Widget "Default"))
          (if (not _success)
            (return "Error" _errormessage)))
        (else
          (return "Error" (`KismetStringLibrary.Concat_StrStr` "BrushColor \"" _value "\" is invalid"))))))
  (return "Complete" ""))

(fn `StartFade`
  (params (Command :type "ShidenCommand Structure (by ref)") (Widget :type "ShidenWidget Object Reference") (OwnerProcessName :type String))
  (returns (Success :type Boolean) (ErrorMessage :type String))
  (locals (NewLocalVar :type "Vector Structure" :default (0.0 0.0 0.0)))
  (bind (_layername _fadetype _fadeduration _fadefunction _targetcolor _steps _blendexp _waitforcompletion _zorder) (`|GetCommandArguments` "/Shiden/Commands/DA_ShidenPrimaryCommandDefinitions.DA_ShidenPrimaryCommandDefinitions" "Fade" Command))
  (bind _outconvertedvector (`KismetStringLibrary.Conv_StringToVector` _targetcolor))
  (bind (_enumvalue _success) (`self.ConvertToEasingFunc` _fadefunction))
  (if _success
    (bind (_success_2 _errormessage) (`ShidenWidget.StartFade` Widget _layername _enumvalue (`KismetStringLibrary.Conv_StringToDouble` _fadeduration) (`KismetMathLibrary.MakeColor` (.x _outconvertedvector) (.y _outconvertedvector) (.z _outconvertedvector)) (`self.GetFadeInfo` _fadetype) (`KismetStringLibrary.Conv_StringToDouble` _blendexp) (`KismetStringLibrary.Conv_StringToInt` _steps) OwnerProcessName (`KismetStringLibrary.Conv_StringToInt` _zorder)))
    (return _success_2 _errormessage)
    (else
      (return false "Invalid ease func"))))