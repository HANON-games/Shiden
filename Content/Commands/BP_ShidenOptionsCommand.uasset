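; Shiden scenario command that shows up to five choices to the player and stores the selected index in an integer variable.
; Pre-process fills the choices, shows OptionLayer, optionally collapses TextLayer and switches input to option selection.
; Processing waits each tick for a selection, then writes the variable, restores input, hides the options and logs to the backlog.
; Preview mirrors the layout without registering scenario properties and reports variable errors.
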(fn `PreProcessCommand`
  (params (ProcessName :type String) (Command :type "ShidenCommand Structure") (Widget :type "ShidenWidget Object Reference") (ScenarioManager :type "ShidenScenarioManagerInterface Interface (by ref)") (CallerObject :type "Object Object Reference"))
  (returns (Status :type "EShidenPreProcessStatus Enum") (ErrorMessage :type String))
  (`self.SetOptions` Command Widget)
  (`self.SetLayerVisibility` Command Widget true)
  (`ShidenWidget.SetInputModeOptionSelection` Widget)
  (return "Complete" ""))

(fn `PreviewCommand`
  (params (Command :type "ShidenCommand Structure (by ref)") (Widget :type "ShidenWidget Object Reference") (ScenarioManager :type "ShidenScenarioManagerInterface Interface (by ref)") (bIsCurrentCommand :type Boolean))
  (returns (Status :type "EShidenPreviewStatus Enum") (ErrorMessage :type String))
  (bind (_choice_1 _choice_2 _choice_3 _choice_4 _choice_5 _destinationvariablekind _destinationvariablename _hidetextlayer) (`|GetCommandArguments` "/Shiden/Commands/DA_ShidenPrimaryCommandDefinitions.DA_ShidenPrimaryCommandDefinitions" "Options" Command))
  (bind (_result _bsuccess) (`ShidenVariableFunctionLibrary.ConvertToVariableKind` _destinationvariablekind))
  (if bIsCurrentCommand
    (`self.SetLayerVisibility` Command Widget)
    (`self.SetOptions` Command Widget)
    (elif (`ShidenCommandFunctionLibrary.IsTrue` _hidetextlayer)
      (`ShidenWidget.SetVisibilityByName` Widget "TextLayer" "Collapsed" false)))
  (if _bsuccess
    (bind (_bsuccess_2 _errormessage) (`ShidenVariableFunctionLibrary.UpdateVariable` "Default" _result "Integer" _destinationvariablename))
    (if _bsuccess_2
      (return "Complete" "")
      (else
        (return "Error" _errormessage)))
    (else
      (return "Error" (`KismetStringLibrary.Concat_StrStr` "Variable kind \"" _destinationvariablekind "\" is invalid")))))

(fn `ProcessCommand`
  (params (ProcessName :type String) (Command :type "ShidenCommand Structure") (Widget :type "ShidenWidget Object Reference") (ScenarioManager :type "ShidenScenarioManagerInterface Interface (by ref)") (DeltaTime :type "Float (single-precision)") (CallerObject :type "Object Object Reference"))
  (returns (Status :type "EShidenProcessStatus Enum") (BreakReason :type String) (NextScenarioName :type String) (ErrorMessage :type String))
  (bind (_choice_1 _choice_2 _choice_3 _choice_4 _choice_5 _destinationvariablekind _destinationvariablename) (`|GetCommandArguments` "/Shiden/Commands/DA_ShidenPrimaryCommandDefinitions.DA_ShidenPrimaryCommandDefinitions" "Options" Command))
  (bind (_result _bsuccess) (`ShidenVariableFunctionLibrary.ConvertToVariableKind` _destinationvariablekind))
  (if (`ShidenWidget.IsOptionSelected` Widget)
    (if _bsuccess
      (bind (_bsuccess_2 _errormessage) (`ShidenVariableFunctionLibrary.UpdateVariable` ProcessName _result "Integer" _destinationvariablename false "" (`ShidenWidget.GetSelectedOption` Widget)))
      (if _bsuccess_2
        (`ShidenWidget.SetInputModeGameAndUI` (`local.Widget`))
        (`ShidenWidget.SetVisibilityByName` (`local.Widget`) "OptionLayer" "Collapsed" true)
        (`ShidenCoreFunctionLibrary.AddBacklogItem` (`local.Command`) (`|MakeMap` "SelectedOption" (`KismetStringLibrary.Conv_IntToString` (`ShidenWidget.GetSelectedOption` (`local.Widget`)))))
        (return "Next" "" "" "")
        (else
          (return "Error" "" "" _errormessage)))
      (else
        (return "Error" "" "" (`KismetStringLibrary.Concat_StrStr` "Variable kind \"" _destinationvariablekind "\" is invalid"))))
    (else
      (return "DelayUntilNextTick" "" "" ""))))

(fn `SetLayerVisibility`
  (params (Command :type "ShidenCommand Structure") (Widget :type "ShidenWidget Object Reference") (bShouldRegisterScenarioProperty :type Boolean))
  (`ShidenWidget.SetVisibilityByName` Widget "OptionLayer" "SelfHitTestInvisible" bShouldRegisterScenarioProperty)
  (if (`ShidenCommandFunctionLibrary.IsTrue` (`.HideTextLayer` (`|GetCommandArguments` "/Shiden/Commands/DA_ShidenPrimaryCommandDefinitions.DA_ShidenPrimaryCommandDefinitions" "Options" Command)))
    (`ShidenWidget.SetVisibilityByName` Widget "TextLayer" "Collapsed" bShouldRegisterScenarioProperty)))

(fn `SetOptions`
  (params (Command :type "ShidenCommand Structure (by ref)") (Widget :type "ShidenWidget Object Reference"))
  (bind (_choice_1 _choice_2 _choice_3 _choice_4 _choice_5) (`|GetCommandArguments` "/Shiden/Commands/DA_ShidenPrimaryCommandDefinitions.DA_ShidenPrimaryCommandDefinitions" "Options" Command))
  (`ShidenWidget.SetOptions` Widget (`|MakeArray` _choice_1 _choice_2 _choice_3 _choice_4 _choice_5)))