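; BP_ShidenDelayCommand is the Shiden scenario command "Delay", which holds the scenario for the time given in its command arguments.
; PreProcessCommand resets the elapsed time, and ProcessCommand adds delta time each tick, returning DelayUntilNextTick until the duration is exceeded, then Next.
; While the IA_ShidenSkip input is active and skipping is allowed, delta time is multiplied by the skip speed rate to shorten the wait.
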(fn `PreProcessCommand`
  (params (ProcessName :type String) (Command :type "ShidenCommand Structure") (Widget :type "ShidenWidget Object Reference") (ScenarioManager :type "ShidenScenarioManagerInterface Interface (by ref)") (CallerObject :type "Object Object Reference"))
  (returns (Status :type "EShidenPreProcessStatus Enum") (ErrorMessage :type String))
  (set `self.ElaspedTime` 0.0)
  (return "Complete" ""))

(fn `ProcessCommand`
  (params (ProcessName :type String) (Command :type "ShidenCommand Structure") (Widget :type "ShidenWidget Object Reference") (ScenarioManager :type "ShidenScenarioManagerInterface Interface (by ref)") (DeltaTime :type "Float (single-precision)") (CallerObject :type "Object Object Reference"))
  (returns (Status :type "EShidenProcessStatus Enum") (BreakReason :type String) (NextScenarioName :type String) (ErrorMessage :type String))
  (locals (SkipButton :type "InputAction Object Reference" :default "/Script/EnhancedInput.InputAction'/Shiden/Misc/EnhancedInput/IA_ShidenSkip.IA_ShidenSkip'"))
  (bind _bvalue (`ShidenScenarioManagerInterface.FindShidenDigitalInput` ScenarioManager "/Shiden/Misc/EnhancedInput/IA_ShidenSkip.IA_ShidenSkip"))
  (bind _output_get (set `self.ElaspedTime` (+ (`self.ElaspedTime`) (`KismetMathLibrary.SelectFloat` (* (`ShidenVariableFunctionLibrary.GetSkipSpeedRate`) DeltaTime) DeltaTime (and _bvalue (`ShidenScenarioFunctionLibrary.CanSkipCommand`))))))
  (if (> _output_get (`|GetCommandArguments` "/Shiden/Commands/DA_ShidenPrimaryCommandDefinitions.DA_ShidenPrimaryCommandDefinitions" "Delay" Command))
    (return "Next" "" "" "")
    (else
      (return "DelayUntilNextTick" "" "" ""))))