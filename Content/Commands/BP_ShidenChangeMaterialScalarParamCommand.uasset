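; Shiden scenario command that eases a material scalar parameter on a named widget Image or RetainerBox, as an absolute or additive change.
; PreProcess starts the widget-side change; additive changes build on any tracked end value, else the material's current value.
; Process optionally waits (both targets poll the RetainerBox completion check), then saves the end value under an escaped composite key.
; RestoreFromSaveData replays saved values as zero-duration changes.
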(fn `ConvertToEasingFunc`
  (params (EasingFunc :type String))
  (returns (EnumValue :type "EEasingFunc Enum") (Success :type Boolean))
  (switch `string` EasingFunc
    (:`Default`
      (return "Linear" false))
    (:`Linear`
      (return "Linear" true))
    (:`Step`
      (return "Step" true))
    (:`Sinusoidal in`
      (return "SinusoidalIn" true))
    (:`Sinusoidal out`
      (return "SinusoidalOut" true))
    (:`Sinusoidal in out`
      (return "SinusoidalInOut" true))
    (:`Ease in`
      (return "EaseIn" true))
    (:`Ease out`
      (return "EaseOut" true))
    (:`Ease in out`
      (return "EaseInOut" true))
    (:`Expo in`
      (return "ExpoIn" true))
    (:`Expo out`
      (return "ExpoOut" true))
    (:`Expo in out`
      (return "ExpoInOut" true))
    (:`Circular in`
      (return "CircularIn" true))
    (:`Circular out`
      (return "CircularOut" true))
    (:`Circular in out`
      (return "CircularInOut" true))))

(fn `GetEndValueFromImageMaterialParams`
  (params (Widget :type "ShidenWidget Object Reference") (Command :type "ShidenCommand Structure (by ref)"))
  (returns (EndValue :type "Float (double-precision)") (Found :type Boolean))
  (bind (_target _targetname _parametername) (`|GetCommandArguments` "/Shiden/Commands/DA_ShidenPrimaryCommandDefinitions.DA_ShidenPrimaryCommandDefinitions" "ChangeMaterialScalarParameter" Command))
  (bind (_value _bsuccess) (`ShidenWidget.FindImageMaterialScalarParams` Widget (`ShidenWidget.MakeMaterialParamsKey` Widget _targetname _parametername)))
  (return (`.EndValue` (break `ShidenImageMaterialScalarParams` _value)) _bsuccess))

(fn `GetEndValueFromRetainerMaterialParams`
  (params (Widget :type "ShidenWidget Object Reference") (Command :type "ShidenCommand Structure (by ref)"))
  (returns (EndValue :type "Float (double-precision)") (Found :type Boolean))
  (bind (_target _targetname _parametername) (`|GetCommandArguments` "/Shiden/Commands/DA_ShidenPrimaryCommandDefinitions.DA_ShidenPrimaryCommandDefinitions" "ChangeMaterialScalarParameter" Command))
  (bind (_value _bsuccess) (`ShidenWidget.FindRetainerBoxMaterialScalarParams` Widget (`ShidenWidget.MakeMaterialParamsKey` Widget _targetname _parametername)))
  (return (`.EndValue` (break `ShidenRetainerBoxMaterialScalarParams` _value)) _bsuccess))

(fn `MakeCurrentKey`
  (params (TargetType :type String) (TargetName :type String) (ParameterName :type String))
  (returns (ReturnValue :type String))
  (return (`KismetStringLibrary.Concat_StrStr` (`KismetStringLibrary.Replace` TargetType ":" "\\:") "::" (`KismetStringLibrary.Replace` TargetName ":" "\\:") "::" (`KismetStringLibrary.Replace` ParameterName ":" "\\:"))))

(fn `ParseCurrentKey`
  (params (Key :type String))
  (returns (TargetType :type String) (TargetName :type String) (ParameterName :type String))
  (bind (_lefts _rights) (`KismetStringLibrary.Split` Key "::"))
  (bind (_lefts_2 _rights_2) (`KismetStringLibrary.Split` _rights "::"))
  (return (`KismetStringLibrary.Replace` _lefts "\\:" ":") (`KismetStringLibrary.Replace` _lefts_2 "\\:" ":") (`KismetStringLibrary.Replace` _rights_2 "\\:" ":")))

(fn `PreProcessCommand`
  (params (ProcessName :type String) (Command :type "ShidenCommand Structure") (Widget :type "ShidenWidget Object Reference") (ScenarioManager :type "ShidenScenarioManagerInterface Interface (by ref)") (CallerObject :type "Object Object Reference"))
  (returns (Status :type "EShidenPreProcessStatus Enum") (ErrorMessage :type String))
  (bind (_success _errormessage) (`self.StartChangeParameter` Command Widget ProcessName))
  (if _success
    (return "Complete" "")
    (else
      (return "Error" _errormessage))))

(fn `PreviewCommand`
  (params (Command :type "ShidenCommand Structure (by ref)") (Widget :type "ShidenWidget Object Reference") (ScenarioManager :type "ShidenScenarioManagerInterface Interface (by ref)") (bIsCurrentCommand :type Boolean))
  (returns (Status :type "EShidenPreviewStatus Enum") (ErrorMessage :type String))
  (if true
    (bind (_success _errormessage) (`self.StartChangeParameter` Command Widget "Default"))
    (if _success
      (return "Complete" "")
      (else
        (return "Error" _errormessage)))
    (else
      (`BlueprintMapLibrary.Map_Add` (`.Args` (break `ShidenCommand` Command)) "Duration" "0.0")
      (bind (_success_2 _errormessage_2) (`self.StartChangeParameter` Command Widget "Default"))
      (if _success_2
        (return "Complete" "")
        (else
          (return "Error" _errormessage_2))))))

(fn `ProcessCommand`
  (params (ProcessName :type String) (Command :type "ShidenCommand Structure") (Widget :type "ShidenWidget Object Reference") (ScenarioManager :type "ShidenScenarioManagerInterface Interface (by ref)") (DeltaTime :type "Float (single-precision)") (CallerObject :type "Object Object Reference"))
  (returns (Status :type "EShidenProcessStatus Enum") (BreakReason :type String) (NextScenarioName :type String) (ErrorMessage :type String))
  (bind (_target _targetname _parametername _easingfunction _duration _changetype _endvalue _steps _blendexp _waitforcompletion) (`|GetCommandArguments` "/Shiden/Commands/DA_ShidenPrimaryCommandDefinitions.DA_ShidenPrimaryCommandDefinitions" "ChangeMaterialScalarParameter" Command))
  (if (`KismetStringLibrary.EqualEqual_StrStr` _waitforcompletion "true")
    (if (`KismetStringLibrary.EqualEqual_StrStr` _target "RetainerBox")
      (if (`ShidenWidget.IsRetainerBoxMaterialParameterChangeCompleted` Widget _targetname _parametername)
        _
        (else
          (return "DelayUntilNextTick" "" "" "")))
      (elif (`ShidenWidget.IsRetainerBoxMaterialParameterChangeCompleted` Widget _targetname _parametername)
        _
        (else
          (return "DelayUntilNextTick" "" "" "")))))
  (`ShidenCommandFunctionLibrary.RegisterScenarioProperty` (`.CommandName` (break `ShidenCommand` (`local.Command`))) (`self.MakeCurrentKey` _target _targetname _parametername) (`KismetStringLibrary.Conv_DoubleToString` (`self.EndValue`)))
  (return "Next" "" "" ""))

(fn `RestoreFromSaveData`
  (params (ScenarioProperties :type "Map of String to String (by ref)") (Widget :type "ShidenWidget Object Reference") (ScenarioManager :type "ShidenScenarioManagerInterface Interface (by ref)") (CallerObject :type "Object Object Reference"))
  (returns (Status :type "EShidenInitFromSaveDataStatus Enum") (ErrorMessage :type String))
  (bind _keys (`BlueprintMapLibrary.Map_Keys` ScenarioProperties))
  (for _array_element _keys
    (bind (_targettype _targetname _parametername) (`self.ParseCurrentKey` _array_element))
    (bind (_success _errormessage) (`self.StartChangeParameter` (make `ShidenCommand` "00000000000000000000000000000000" true "ChangeMaterialScalarParameter" "" (`|MakeMap` "Target" _targettype "TargetName" _targetname "ParameterName" _parametername "EasingFunction" "Linear" "Duration" "0.0" "ChangeType" "AbsoluteValue" "EndValue" (`BlueprintMapLibrary.Map_Find` ScenarioProperties _array_element) "Steps" "" "BlendExp" "" "WaitForCompletion")) Widget "Default"))
    (if (not _success)
      (return "Error" _errormessage)))
  (return "Complete" ""))

(fn `StartChangeParameter`
  (params (Command :type "ShidenCommand Structure (by ref)") (Widget :type "ShidenWidget Object Reference") (OwnerProcessName :type String))
  (returns (Success :type Boolean) (ErrorMessage :type String))
  (bind (_target _targetname) (`|GetCommandArguments` "/Shiden/Commands/DA_ShidenPrimaryCommandDefinitions.DA_ShidenPrimaryCommandDefinitions" "ChangeMaterialScalarParameter" Command))
  (bind (_image _bresult) (`ShidenWidget.FindImage` (`local.Widget`) _targetname))
  (bind (_retainerbox _bresult_2) (`ShidenWidget.FindRetainerBox` (`local.Widget`) (`.TargetName` (`|GetCommandArguments` "/Shiden/Commands/DA_ShidenPrimaryCommandDefinitions.DA_ShidenPrimaryCommandDefinitions" "ChangeMaterialScalarParameter" (`local.Command`)))))
  (bind (_enumvalue _success) (`self.ConvertToEasingFunc` (`.EasingFunction` (`|GetCommandArguments` "/Shiden/Commands/DA_ShidenPrimaryCommandDefinitions.DA_ShidenPrimaryCommandDefinitions" "ChangeMaterialScalarParameter" (`local.Command`)))))
  (bind (_enumvalue_2 _success_2) (`self.ConvertToEasingFunc` (`.EasingFunction` (`|GetCommandArguments` "/Shiden/Commands/DA_ShidenPrimaryCommandDefinitions.DA_ShidenPrimaryCommandDefinitions" "ChangeMaterialScalarParameter" (`local.Command`)))))
  (if (== _target "RetainerBox")
    (if _bresult_2
      (if _success_2
        (bind (_success_3 _errormessage) (`self.StartRetainerMaterialChange` Command (`local.Widget`) _retainerbox _enumvalue_2 (`local.OwnerProcessName`)))
        (return _success_3 _errormessage)
        (else
          (return false "Invalid ease func")))
      (else
        (return false "Retainer Box not found")))
    (elif _bresult
      (if _success
        (bind (_success_4 _errormessage_2) (`self.StartImageMaterialChange` (`local.Command`) (`local.Widget`) _image _enumvalue (`local.OwnerProcessName`)))
        (return _success_4 _errormessage_2)
        (else
          (return false "Invalid ease func")))
      (else
        (return false "Image not found")))))

(fn `StartImageMaterialChange`
  (params (Command :type "ShidenCommand Structure (by ref)") (Widget :type "ShidenWidget Object Reference") (Image :type "Image Object Reference") (EasingFunction :type "EEasingFunc Enum" :default "Linear") (OwnerProcessName :type String))
  (returns (Success :type Boolean) (ErrorMessage :type String))
  (bind (_endvalue _found) (`self.GetEndValueFromImageMaterialParams` Widget Command))
  (bind (_target _targetname _parametername) (`|GetCommandArguments` "/Shiden/Commands/DA_ShidenPrimaryCommandDefinitions.DA_ShidenPrimaryCommandDefinitions" "ChangeMaterialScalarParameter" Command))
  (bind (_target_2 _targetname_2 _parametername_2 _easingfunction _duration _changetype _endvalue_2) (`|GetCommandArguments` "/Shiden/Commands/DA_ShidenPrimaryCommandDefinitions.DA_ShidenPrimaryCommandDefinitions" "ChangeMaterialScalarParameter" (`local.Command`)))
  (bind (_target_3 _targetname_3 _parametername_3 _easingfunction_2 _duration_2 _changetype_2 _endvalue_3 _steps _blendexp) (`|GetCommandArguments` "/Shiden/Commands/DA_ShidenPrimaryCommandDefinitions.DA_ShidenPrimaryCommandDefinitions" "ChangeMaterialScalarParameter" (`local.Command`)))
  (bind _returnvalue (`KismetStringLibrary.Conv_StringToDouble` _endvalue_2))
  (bind _returnvalue_2 (`MaterialInstanceDynamic.K2_GetScalarParameterValue` (`WidgetBlueprintLibrary.GetDynamicMaterial` (`Image.Brush` (`ShidenWidget.FindImage` (`local.Widget`) _targetname))) (`KismetStringLibrary.Conv_StringToName` _parametername)))
  (bind _returnvalue_3 (`KismetMathLibrary.SelectFloat` (+ _returnvalue (`KismetMathLibrary.SelectFloat` _endvalue _returnvalue_2 _found)) _returnvalue (`KismetStringLibrary.EqualEqual_StrStr` _changetype "AddToCurrent")))
  (bind (_success _errormessage) (`ShidenWidget.StartImageMaterialScalarChange` (`local.Widget`) _targetname_3 (`local.Image`) (`KismetStringLibrary.Conv_StringToName` _parametername_3) (`local.EasingFunction`) (`KismetStringLibrary.Conv_StringToDouble` _duration_2) _returnvalue_3 (`KismetStringLibrary.Conv_StringToDouble` _blendexp) (`KismetStringLibrary.Conv_StringToInt` _steps) (`local.OwnerProcessName`)))
  (if _success
    (set `self.EndValue` _returnvalue_3)
    (return true "")
    (else
      (return false _errormessage))))

(fn `StartRetainerMaterialChange`
  (params (Command :type "ShidenCommand Structure (by ref)") (Widget :type "ShidenWidget Object Reference") (RetainerBox :type "RetainerBox Object Reference") (EasingFunction :type "EEasingFunc Enum" :default "Linear") (`Owner Process Name` :type String))
  (returns (Success :type Boolean) (ErrorMessage :type String))
  (bind (_endvalue _found) (`self.GetEndValueFromRetainerMaterialParams` Widget Command))
  (bind (_target _targetname _parametername) (`|GetCommandArguments` "/Shiden/Commands/DA_ShidenPrimaryCommandDefinitions.DA_ShidenPrimaryCommandDefinitions" "ChangeMaterialScalarParameter" Command))
  (bind (_target_2 _targetname_2 _parametername_2 _easingfunction _duration _changetype _endvalue_2 _steps _blendexp) (`|GetCommandArguments` "/Shiden/Commands/DA_ShidenPrimaryCommandDefinitions.DA_ShidenPrimaryCommandDefinitions" "ChangeMaterialScalarParameter" (`local.Command`)))
  (bind (_target_3 _targetname_3 _parametername_3 _easingfunction_2 _duration_2 _changetype_2 _endvalue_3) (`|GetCommandArguments` "/Shiden/Commands/DA_ShidenPrimaryCommandDefinitions.DA_ShidenPrimaryCommandDefinitions" "ChangeMaterialScalarParameter" (`local.Command`)))
  (bind _returnvalue (`KismetStringLibrary.Conv_StringToDouble` _endvalue_3))
  (bind _returnvalue_2 (`MaterialInstanceDynamic.K2_GetScalarParameterValue` (`RetainerBox.GetEffectMaterial` (`ShidenWidget.FindRetainerBox` (`local.Widget`) _targetname)) (`KismetStringLibrary.Conv_StringToName` _parametername)))
  (bind _returnvalue_3 (`KismetMathLibrary.SelectFloat` (+ _returnvalue (`KismetMathLibrary.SelectFloat` _endvalue _returnvalue_2 _found)) _returnvalue (`KismetStringLibrary.EqualEqual_StrStr` _changetype_2 "AddToCurrent")))
  (bind (_success _errormessage) (`ShidenWidget.StartRetainerBoxMaterialScalarChange` (`local.Widget`) _targetname_2 (`local.RetainerBox`) (`KismetStringLibrary.Conv_StringToName` _parametername_2) (`local.EasingFunction`) (`KismetStringLibrary.Conv_StringToDouble` _duration) _returnvalue_3 (`KismetStringLibrary.Conv_StringToDouble` _blendexp) (`KismetStringLibrary.Conv_StringToInt` _steps) (`local.Owner Process Name`)))
  (if _success
    (set `self.EndValue` _returnvalue_3)
    (return true "")
    (else
      (return false _errormessage))))