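; Shiden scenario command that shows a single- or multi-line text input and stores the player's entry in a user, local or system string variable.
; PreProcess shows and initializes the input layer, optionally hiding the text layer.
; Process waits each tick for submission, then collapses the input, saves the text and adds it to the backlog; predefined system variables are rejected.
; Preview mirrors the layout and writes the default text, or "Sample", instead.
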(fn `GetAssetPaths`
  (params (Command :type "ShidenCommand Structure") (CallerObject :type "Object Object Reference"))
  (returns (AssetObjectPaths :type "Set of String"))
  (return))

(fn `PreProcessCommand`
  (params (ProcessName :type String) (Command :type "ShidenCommand Structure") (Widget :type "ShidenWidget Object Reference") (ScenarioManager :type "ShidenScenarioManagerInterface Interface (by ref)") (CallerObject :type "Object Object Reference"))
  (returns (Status :type "EShidenPreProcessStatus Enum") (ErrorMessage :type String))
  (bind (_ismultiline _maxlinecount _defaulttext _hinttext) (`|GetCommandArguments` "/Shiden/Commands/DA_ShidenPrimaryCommandDefinitions.DA_ShidenPrimaryCommandDefinitions" "TextInput" Command))
  (bind _returnvalue (`KismetTextLibrary.Conv_StringToText` _defaulttext))
  (bind _returnvalue_2 (`KismetTextLibrary.Conv_StringToText` _hinttext))
  (`self.SetLayerVisibility` Command Widget true)
  (if (== _ismultiline "true")
    (`ShidenWidget.InitMultiLineTextInput` Widget _returnvalue _returnvalue_2 (`KismetStringLibrary.Conv_StringToInt` _maxlinecount))
    (`ShidenWidget.SetInputModeMultiLineTextInput` Widget)
    (else
      (`ShidenWidget.InitSingleLineTextInput` Widget _returnvalue _returnvalue_2)
      (`ShidenWidget.SetInputModeSingleLineTextInput` Widget)))
  (return "Complete" ""))

(fn `PreviewCommand`
  (params (Command :type "ShidenCommand Structure (by ref)") (Widget :type "ShidenWidget Object Reference") (ScenarioManager :type "ShidenScenarioManagerInterface Interface (by ref)") (bIsCurrentCommand :type Boolean))
  (returns (Status :type "EShidenPreviewStatus Enum") (ErrorMessage :type String))
  (bind (_ismultiline _maxlinecount _defaulttext _hinttext _destinationvariablekind _destinationvariablename) (`|GetCommandArguments` "/Shiden/Commands/DA_ShidenPrimaryCommandDefinitions.DA_ShidenPrimaryCommandDefinitions" "TextInput" Command))
  (bind (_ismultiline_2 _maxlinecount_2 _defaulttext_2 _hinttext_2) (`|GetCommandArguments` "/Shiden/Commands/DA_ShidenPrimaryCommandDefinitions.DA_ShidenPrimaryCommandDefinitions" "TextInput" Command))
  (bind _returnvalue (`KismetTextLibrary.Conv_StringToText` _defaulttext_2))
  (bind _returnvalue_2 (`KismetTextLibrary.Conv_StringToText` _hinttext_2))
  (bind _returnvalue_3 (`KismetMathLibrary.SelectString` "Sample" _defaulttext_2 (`KismetStringLibrary.IsEmpty` _defaulttext_2)))
  (if bIsCurrentCommand
    (`self.SetLayerVisibility` Command Widget)
    (if (== _ismultiline_2 "true")
      (`ShidenWidget.InitMultiLineTextInput` Widget _returnvalue _returnvalue_2 (`KismetStringLibrary.Conv_StringToInt` _maxlinecount_2))
      (else
        (`ShidenWidget.InitSingleLineTextInput` Widget _returnvalue _returnvalue_2)))
    (elif (== (`.HideTextLayer` (`|GetCommandArguments` "/Shiden/Commands/DA_ShidenPrimaryCommandDefinitions.DA_ShidenPrimaryCommandDefinitions" "TextInput" Command)) "true")
      (`ShidenWidget.SetVisibilityByName` Widget "TextLayer" "Collapsed" false)))
  (switch `EShidenVariableKind` (`ShidenVariableFunctionLibrary.ConvertToVariableKind` _destinationvariablekind)
    (:`UserVariable`
      (`ShidenVariableFunctionLibrary.AddUserString` _destinationvariablename _returnvalue_3))
    (:`LocalVariable`
      (`ShidenVariableFunctionLibrary.AddLocalString` "Default" _destinationvariablename _returnvalue_3))
    (:`SystemVariable`
      (`ShidenVariableFunctionLibrary.AddSystemString` _destinationvariablename _returnvalue_3))
    (:`PredefinedSystemVariable`
      (return "Error" (`KismetStringLibrary.Concat_StrStr` "Variable kind \"" _destinationvariablekind "\" is invalid"))))
  (return "Complete" ""))

(fn `ProcessCommand`
  (params (ProcessName :type String) (Command :type "ShidenCommand Structure") (Widget :type "ShidenWidget Object Reference") (ScenarioManager :type "ShidenScenarioManagerInterface Interface (by ref)") (DeltaTime :type "Float (single-precision)") (CallerObject :type "Object Object Reference"))
  (returns (Status :type "EShidenProcessStatus Enum") (BreakReason :type String) (NextScenarioName :type String) (ErrorMessage :type String))
  (bind (_ismultiline _maxlinecount _defaulttext _hinttext _destinationvariablekind _destinationvariablename) (`|GetCommandArguments` "/Shiden/Commands/DA_ShidenPrimaryCommandDefinitions.DA_ShidenPrimaryCommandDefinitions" "TextInput" Command))
  (bind _returnvalue (`KismetMathLibrary.SelectString` (`KismetTextLibrary.Conv_TextToString` (`ShidenWidget.GetMultiLineTextInput` Widget)) (`KismetTextLibrary.Conv_TextToString` (`ShidenWidget.GetSingleLineTextInput` Widget)) (== _ismultiline "true")))
  (if (== _ismultiline "true")
    (if (`ShidenWidget.bIsMultiLineTextSubmitted` Widget)
      (`ShidenWidget.SetVisibilityByName` Widget "MultiLineTextInputLayer" "Collapsed" true)
      (switch `EShidenVariableKind` (`ShidenVariableFunctionLibrary.ConvertToVariableKind` _destinationvariablekind) :!label _label
        (:`UserVariable`
          (`ShidenVariableFunctionLibrary.AddUserString` _destinationvariablename _returnvalue))
        (:`LocalVariable`
          (`ShidenVariableFunctionLibrary.AddLocalString` ProcessName _destinationvariablename _returnvalue))
        (:`SystemVariable`
          (`ShidenVariableFunctionLibrary.AddSystemString` _destinationvariablename _returnvalue))
        (:`PredefinedSystemVariable`
          (return "Error" "" "" (`KismetStringLibrary.Concat_StrStr` "Variable kind \"" (`.DestinationVariableKind` (`|GetCommandArguments` "/Shiden/Commands/DA_ShidenPrimaryCommandDefinitions.DA_ShidenPrimaryCommandDefinitions" "TextInput" Command)) "\" is invalid"))))
      (`ShidenWidget.SetInputModeGameAndUI` Widget)
      (`ShidenCoreFunctionLibrary.AddBacklogItem` (`local.Command`) (`|MakeMap` "InputText" _returnvalue))
      (return "Next" "" "" "")
      (else
        _))
    (elif (`ShidenWidget.bIsSingleLineTextSubmitted` Widget)
      (`ShidenWidget.SetVisibilityByName` Widget "TextInputLayer" "Collapsed" true)
      (goto _label)
      (else
        _)))
  (return "DelayUntilNextTick" "" "" ""))

(fn `SetLayerVisibility`
  (params (Command :type "ShidenCommand Structure") (Widget :type "ShidenWidget Object Reference") (ShouldRegisterScenarioProperty :type Boolean))
  (if (== (`|GetCommandArguments` "/Shiden/Commands/DA_ShidenPrimaryCommandDefinitions.DA_ShidenPrimaryCommandDefinitions" "TextInput" Command) "true")
    (`ShidenWidget.SetVisibilityByName` Widget "MultiLineTextInputLayer" "Visible" ShouldRegisterScenarioProperty)
    (else
      (`ShidenWidget.SetVisibilityByName` Widget "TextInputLayer" "Visible" ShouldRegisterScenarioProperty)))
  (if (== (`.HideTextLayer` (`|GetCommandArguments` "/Shiden/Commands/DA_ShidenPrimaryCommandDefinitions.DA_ShidenPrimaryCommandDefinitions" "TextInput" Command)) "true")
    (`ShidenWidget.SetVisibilityByName` Widget "TextLayer" "Collapsed" ShouldRegisterScenarioProperty)))