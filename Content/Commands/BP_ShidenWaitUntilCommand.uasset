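; Shiden scenario command "WaitUntil" that holds a scenario until a variable satisfies a comparison.
; ProcessCommand reads the variable kind, name, operator and right-hand value from the command arguments, finds the variable, and compares it with the value converted from text.
; A true result advances to the next command, while a false one delays until the next tick to poll again.
; An invalid kind, missing variable or failed evaluation returns an error.
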(fn `ProcessCommand`
  (params (ProcessName :type String) (Command :type "ShidenCommand Structure") (Widget :type "ShidenWidget Object Reference") (ScenarioManager :type "ShidenScenarioManagerInterface Interface (by ref)") (DeltaTime :type "Float (single-precision)") (CallerObject :type "Object Object Reference"))
  (returns (Status :type "EShidenProcessStatus Enum") (BreakReason :type String) (NextScenarioName :type String) (ErrorMessage :type String))
  (bind (_variablekind _variablename _operator _righthandvalue) (`|GetCommandArguments` "/Shiden/Commands/DA_ShidenPrimaryCommandDefinitions.DA_ShidenPrimaryCommandDefinitions" "WaitUntil" Command))
  (bind (_result _bsuccess) (`ShidenVariableFunctionLibrary.ConvertToVariableKind` _variablekind))
  (if _bsuccess
    (bind (_variabletype _bbooleanvalue _stringvalue _integervalue _floatvalue _vector2value _vector3value _breturnvalue) (`ShidenVariableFunctionLibrary.FindVariable` ProcessName _result _variablename))
    (if _breturnvalue
      (bind (_bresult _bsuccess_2 _errormessage) (`ShidenVariableFunctionLibrary.EvaluateCondition` _variabletype _operator _bbooleanvalue _stringvalue _integervalue _floatvalue _vector2value _vector3value (== _righthandvalue "true") _righthandvalue (`KismetStringLibrary.Conv_StringToInt` _righthandvalue) (`KismetStringLibrary.Conv_StringToDouble` _righthandvalue) (`KismetStringLibrary.Conv_StringToVector2D` _righthandvalue) (`KismetStringLibrary.Conv_StringToVector` _righthandvalue)))
      (if _bsuccess_2
        (if _bresult
          (return "Next" "" "" "")
          (else
            (return "DelayUntilNextTick" "" "" "")))
        (else
          (return "Error" "" "" _errormessage)))
      (else
        (return "Error" "" "" "Variable not found")))
    (else
      (return "Error" "" "" "Invalid variable kind"))))