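; Shiden scenario command that shows or hides the text window by switching the widget's window mode between Texts and None.
; Processing and preview share SetVisibility, which reads a "true"/"false" string from Arg1, switches only when needed, and registers the change as a current property.
; InitFromSaveData restores the saved visibility without re-registering it, returning an error if the value is missing.
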(fn `InitFromSaveData`
  (params (ScenarioProperties :type "Map of String to String (by ref)") (Widget :type "ShidenWidget Object Reference") (ScenarioManager :type "ShidenScenarioManagerInterface Interface (by ref)"))
  (returns (Status :type "EShidenInitFromSaveDataStatus Enum") (ErrorMessage :type String))
  (bind (_value _returnvalue) (`BlueprintMapLibrary.Map_Find` ScenarioProperties "ChangeTextWindowVisibility"))
  (if _returnvalue
    (switch `string` _value
      (:`Default`
        (`ShidenWidget.ChangeWindowMode` Widget "None" false :!label _label))
      (:`true`
        (`ShidenWidget.ChangeWindowMode` Widget "Texts" false))
      (:`false`
        (goto _label)))
    (return "Completed" "")
    (else
      (return "Error" "Value not found"))))

(fn `PreviewCommmand`
  (params (Command :type "ShidenCommand Structure (by ref)") (Widget :type "ShidenWidget Object Reference") (ScenarioManager :type "ShidenScenarioManagerInterface Interface (by ref)") (bIsCurrentCommand :type Boolean))
  (returns (Status :type "EShidenPreviewStatus Enum") (ErrorMessage :type String))
  (`self.SetVisibility` (`.Arg1` (break `ShidenCommand` Command)) Widget)
  (return "Completed" ""))

(fn `ProcessCommmand`
  (params (ProcessName :type String) (Command :type "ShidenCommand Structure") (Widget :type "ShidenWidget Object Reference") (ScenarioManager :type "ShidenScenarioManagerInterface Interface (by ref)") (DeltaTime :type "Float (single-precision)") (HookedObject :type "Object Object Reference"))
  (returns (Status :type "EShidenProcessStatus Enum") (BreakReason :type String) (NextScenarioName :type String) (ErrorMessage :type String))
  (`self.SetVisibility` (`.Arg1` (break `ShidenCommand` Command)) Widget)
  (return "Next" "" "" ""))

(fn `SetVisibility`
  (params (Visible :type String) (Widget :type "ShidenWidget Object Reference"))
  (if (and (== Visible "true") (`|EnumEquality` (`ShidenWidget.GetWindowMode` Widget)))
    (`ShidenWidget.ChangeWindowMode` Widget "Texts" true)
    (elif (and (== Visible "false") (`|EnumInequality` (`ShidenWidget.GetWindowMode` Widget)))
      (`ShidenWidget.ChangeWindowMode` Widget "None" true)))
  (return))