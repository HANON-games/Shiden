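; Shiden scenario command "Calculation" that applies a compound operator to a stored variable and saves the result.
; CalculationVariable takes the right operand from a literal or a second variable of matching type, then dispatches by type to per-type Calc helpers.
; Strings are always appended, Booleans are rejected, and vectors have no modulo.
; ProcessCommand and PreviewCommand share this logic, with preview using the "Default" process.
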(event `AddFloat`
  (params (VariableKind :type String) (Key :type String) (NewParam :type String)))

(fn `CalcFloat`
  (params (Operator :type String) (A :type "Float (double-precision)") (B :type "Float (double-precision)"))
  (returns (ReturnValue :type "Float (double-precision)") (Success :type Boolean))
  (switch `string` Operator
    (:`Default`
      (return 0.0 false))
    (:`+=`
      (return (+ A B) true))
    (:`-=`
      (return (- A B) true))
    (:`*=`
      (return (* A B) true))
    (:`/=`
      (return (/ A B) true))
    (:`%=`
      (return (mod A B) true))))

(fn `CalcInteger`
  (params (A :type Integer) (B :type Integer) (operator :type String))
  (returns (ReturnValue :type Integer) (Success :type Boolean))
  (switch `string` operator
    (:`Default`
      (return 0 false))
    (:`+=`
      (return (+ A B) true))
    (:`-=`
      (return (- A B) true))
    (:`*=`
      (return (* A B) true))
    (:`/=`
      (return (/ A B) true))
    (:`%=`
      (return (mod A B) true))))

(fn `CalculationVariable`
  (params (ProcessName :type String) (Command :type "ShidenCommand Structure"))
  (returns (Success :type Boolean) (ErrorMessage :type String))
  (locals (IsRVariable :type Boolean))
  (bind (_variablekind _variabletype _variablename _operator _value) (`|GetCommandArguments` "/Shiden/Commands/DA_ShidenPrimaryCommandDefinitions.DA_ShidenPrimaryCommandDefinitions" "Calculation" Command))
  (bind (_result _bsuccess) (`ShidenVariableFunctionLibrary.ConvertToVariableKind` _variablekind))
  (bind (_result_2 _bsuccess_2) (`ShidenVariableFunctionLibrary.ConvertToVariableType` _variabletype))
  (bind (_result_3 _bsuccess_3) (`ShidenVariableFunctionLibrary.ConvertToVariableKind` _variabletype))
  (if _bsuccess
    (bind (_variabletype_2 _bbooleanvalue _stringvalue _integervalue _floatvalue _vector2value _vector3value _breturnvalue) (`ShidenVariableFunctionLibrary.FindVariable` ProcessName _result _variablename))
    (if _breturnvalue
      (if _bsuccess_2
        (if (`|EnumEquality` _result_2 _variabletype_2)
          (set `local.IsRVariable` false)
          (else
            (return false "Variable type is not match")))
        (elif (or (and (`|EnumEquality` _variabletype_2 "Boolean") (`KismetStringLibrary.EqualEqual_StrStr` _operator "+=")) (and (or (`|EnumEquality` _variabletype_2 "Boolean") (`|EnumEquality` _variabletype_2 "Boolean")) (`KismetStringLibrary.NotEqual_StrStr` _operator "%=")))
          (if _bsuccess_3
            (bind (_variabletype_3 _bbooleanvalue_2 _stringvalue_2 _integervalue_2 _floatvalue_2 _vector2value_2 _vector3value_2 _breturnvalue_2) (`ShidenVariableFunctionLibrary.FindVariable` (`local.ProcessName`) _result_3 _value))
            (if _breturnvalue_2
              (if (`|EnumEquality` _variabletype_2 _variabletype_3)
                (set `local.IsRVariable` true)
                (else
                  (return false "Variable type is not match")))
              (else
                (return false "Variable not found")))
            (else
              (return false "Invalid variable type")))
          (else
            (return false "Invalid operator"))))
      (switch `EShidenVariableType` _variabletype_2
        (:`Boolean`
          (return false "Boolean is not supported"))
        (:`String`
          (bind (_bsuccess_4 _errormessage) (`ShidenVariableFunctionLibrary.AddVariable` (`local.ProcessName`) _result _variabletype_2 _variablename false (`KismetStringLibrary.Concat_StrStr` _stringvalue (`KismetMathLibrary.SelectString` _stringvalue_2 _value (`local.IsRVariable`)))))
          (return _bsuccess_4 _errormessage))
        (:`Integer`
          (bind (_returnvalue _success) (`self.CalcInteger` _integervalue (`KismetMathLibrary.SelectInt` _integervalue_2 (`KismetStringLibrary.Conv_StringToInt` _value) (`local.IsRVariable`)) _operator))
          (if _success
            (bind (_bsuccess_5 _errormessage_2) (`ShidenVariableFunctionLibrary.AddVariable` (`local.ProcessName`) _result _variabletype_2 _variablename false "" _returnvalue))
            (return _bsuccess_5 _errormessage_2)
            (else
              (return false "Calculation failed"))))
        (:`Float`
          (bind (_returnvalue_2 _success_2) (`self.CalcFloat` _operator _floatvalue (`KismetMathLibrary.SelectFloat` _floatvalue_2 (`KismetStringLibrary.Conv_StringToDouble` _value) (`local.IsRVariable`))))
          (if _success_2
            (bind (_bsuccess_6 _errormessage_3) (`ShidenVariableFunctionLibrary.AddVariable` (`local.ProcessName`) _result _variabletype_2 _variablename false "" 0 _returnvalue_2))
            (return _bsuccess_6 _errormessage_3)
            (else
              (return false "Calculation failed"))))
        (:`Vector2`
          (bind (_returnvalue_3 _success_3) (`self.CalcVector2` _operator _vector2value (select `bool` (`local.IsRVariable`) :`false` (`KismetStringLibrary.Conv_StringToVector2D` _value) :`true` _vector2value_2)))
          (if _success_3
            (bind (_bsuccess_7 _errormessage_4) (`ShidenVariableFunctionLibrary.AddVariable` (`local.ProcessName`) _result _variabletype_2 _variablename false "" 0 0.0 _returnvalue_3))
            (return _bsuccess_7 _errormessage_4)
            (else
              (return false "Calculation failed"))))
        (:`Vector3`
          (bind (_returnvalue_4 _success_4) (`self.CalcVector3` _operator _vector3value (`KismetMathLibrary.SelectVector` _vector3value_2 (`KismetStringLibrary.Conv_StringToVector` _value) (`local.IsRVariable`))))
          (if _success_4
            (bind (_bsuccess_8 _errormessage_5) (`ShidenVariableFunctionLibrary.AddVariable` (`local.ProcessName`) _result _variabletype_2 _variablename false "" 0 0.0 (0.0 0.0) _returnvalue_4))
            (return _bsuccess_8 _errormessage_5)
            (else
              (return false "Calculation failed")))))
      (else
        (return false "Variable not found")))
    (else
      (return false "Invalid variable kind"))))

(fn `CalcVector2`
  (params (Operator :type String) (A :type "Vector2D Structure") (B :type "Vector2D Structure"))
  (returns (ReturnValue :type "Vector2D Structure") (Success :type Boolean))
  (switch `string` Operator
    (:`Default`
      (return (0.0 0.0) false))
    (:`+=`
      (return (+ A B) true))
    (:`-=`
      (return (- A B) true))
    (:`*=`
      (return (* A B) true))
    (:`/=`
      (return (/ A B) true))))

(fn `CalcVector3`
  (params (Operator :type String) (A :type "Vector Structure") (B :type "Vector Structure"))
  (returns (ReturnValue :type "Vector Structure") (Success :type Boolean))
  (switch `string` Operator
    (:`Default`
      (return (0.0 0.0 0.0) false))
    (:`+=`
      (return (+ A B) true))
    (:`-=`
      (return (- A B) true))
    (:`*=`
      (return (* A B) true))
    (:`/=`
      (return (/ A B) true))))

(fn `PreviewCommand`
  (params (Command :type "ShidenCommand Structure (by ref)") (Widget :type "ShidenWidget Object Reference") (ScenarioManager :type "ShidenScenarioManagerInterface Interface (by ref)") (bIsCurrentCommand :type Boolean))
  (returns (Status :type "EShidenPreviewStatus Enum") (ErrorMessage :type String))
  (bind (_success _errormessage) (`self.CalculationVariable` "Default" Command))
  (if _success
    (return "Complete" "")
    (else
      (return "Error" _errormessage))))

(fn `ProcessCommand`
  (params (ProcessName :type String) (Command :type "ShidenCommand Structure") (Widget :type "ShidenWidget Object Reference") (ScenarioManager :type "ShidenScenarioManagerInterface Interface (by ref)") (DeltaTime :type "Float (single-precision)") (CallerObject :type "Object Object Reference"))
  (returns (Status :type "EShidenProcessStatus Enum") (BreakReason :type String) (NextScenarioName :type String) (ErrorMessage :type String))
  (bind (_success _errormessage) (`self.CalculationVariable` ProcessName Command))
  (if _success
    (return "Next" "" "" "")
    (else
      (return "Error" "" "" _errormessage))))