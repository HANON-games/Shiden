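; Shiden scenario command that plays a named animation on the scenario widget, with start time, loop count, play mode, speed and restore state taken from command arguments.
; An optional wait flag binds the finish event, delaying the scenario each tick until the animation ends.
; On completion it registers the animation name as a scenario property, so loading save data replays it from its end time.
; Preview starts the animation only for the current command.
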(event `Bind to Animation Finished`
  (params (Widget :type "UserWidget Object Reference") (Animation :type "WidgetAnimation Object Reference"))
  (`UserWidget.BindToAnimationFinished` Widget Animation (delegate `OnAnimationFinished`)))

(event `OnAnimationFinished`
  (set `self.IsAnimationEnd` true))

(fn `ConvertToPlayMode`
  (params (PlayMode :type String))
  (returns (Result :type "EUMGSequencePlayMode Enum") (Success :type Boolean))
  (switch `string` PlayMode
    (:`Default`
      (return "Forward" false))
    (:`Forward`
      (return "Forward" true))
    (:`Reverse`
      (return "Reverse" true))
    (:`Ping Pong`
      (return "PingPong" true))))

(fn `InitFromSaveData`
  (params (ScenarioProperties :type "Map of String to String (by ref)") (Widget :type "ShidenWidget Object Reference") (ScenarioManager :type "ShidenScenarioManagerInterface Interface (by ref)"))
  (returns (Status :type "EShidenInitFromSaveDataStatus Enum") (ErrorMessage :type String))
  (bind _keys (`BlueprintMapLibrary.Map_Keys` ScenarioProperties))
  (for _array_element _keys
    (bind (_value _returnvalue) (`BlueprintMapLibrary.Map_Find` (`ShidenWidget.GetAnimations` Widget) _array_element))
    (if _returnvalue
      (`UserWidget.PlayAnimation` Widget _value (`WidgetAnimation.GetEndTime` _value) 1 "Forward" 1.0 false)
      (else
        (return "Error" (`KismetStringLibrary.Concat_StrStr` "Animation \"" _array_element "\" is not found")))))
  (return "Completed" ""))

(fn `PreProcessCommmand`
  (params (ProcessName :type String) (Command :type "ShidenCommand Structure") (Widget :type "ShidenWidget Object Reference") (ScenarioManager :type "ShidenScenarioManagerInterface Interface (by ref)") (HookedObject :type "Object Object Reference"))
  (returns (Status :type "EShidenPreProcessStatus Enum") (ErrorMessage :type String))
  (bind _result (`self.StartAnimation` Command Widget))
  (if _result
    (return "Completed" "")
    (else
      (return "Completed" "Animation not found"))))

(fn `PreviewCommmand`
  (params (Command :type "ShidenCommand Structure (by ref)") (Widget :type "ShidenWidget Object Reference") (ScenarioManager :type "ShidenScenarioManagerInterface Interface (by ref)") (bIsCurrentCommand :type Boolean))
  (returns (Status :type "EShidenPreviewStatus Enum") (ErrorMessage :type String))
  (if bIsCurrentCommand
    (bind _result (`self.StartAnimation` Command Widget))
    (if _result
      (return "Completed" "")
      (else
        (return "Error" "Animation not found")))
    (else
      (return "Completed" ""))))

(fn `ProcessCommmand`
  (params (ProcessName :type String) (Command :type "ShidenCommand Structure") (Widget :type "ShidenWidget Object Reference") (ScenarioManager :type "ShidenScenarioManagerInterface Interface (by ref)") (DeltaTime :type "Float (single-precision)") (HookedObject :type "Object Object Reference"))
  (returns (Status :type "EShidenProcessStatus Enum") (BreakReason :type String) (NextScenarioName :type String) (ErrorMessage :type String))
  (bind (_commandname _presetname _arg1) (break `ShidenCommand` Command))
  (if (`self.IsAnimationEnd`)
    (`ShidenCommandFunctionLibrary.RegisterCurrentScenarioProperty` _commandname _arg1 "EMPTY")
    (return "Next" "" "" "")
    (else
      (return "DelayUntilNextTick" "" "" ""))))

(fn `StartAnimation`
  (params (Command :type "ShidenCommand Structure (by ref)") (ScenarioWidget :type "ShidenWidget Object Reference"))
  (returns (Result :type Boolean))
  (bind (_commandname _presetname _arg1 _arg2 _arg3 _arg4 _arg5 _arg6 _arg7) (break `ShidenCommand` Command))
  (bind (_result _success) (`self.ConvertToPlayMode` _arg4))
  (bind (_value _returnvalue) (`BlueprintMapLibrary.Map_Find` (`ShidenWidget.GetAnimations` ScenarioWidget) _arg1))
  (if _returnvalue
    (switch `string` _arg7
      (:`Default`
        (set `self.IsAnimationEnd` true :!label _label))
      (:`true`
        (set `self.IsAnimationEnd` false)
        (`self.Bind to Animation Finished` (`local.ScenarioWidget`) _value))
      (:`false`
        (goto _label)))
    (if _success
      (`UserWidget.PlayAnimation` (`local.ScenarioWidget`) _value (`KismetStringLibrary.Conv_StringToDouble` _arg2) (`KismetStringLibrary.Conv_StringToInt` _arg3) _result (`KismetStringLibrary.Conv_StringToDouble` _arg5) (== _arg6 "true"))
      (return true)
      (else
        (return false)))
    (else
      (return false))))