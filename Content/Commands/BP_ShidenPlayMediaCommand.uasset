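; Shiden scenario command that plays a media source as a movie through the widget.
; PreProcessCommand reads the source path, pause-menu permission and Z-order from the primary command definitions, starts playback, and reports an error if it fails.
; ProcessCommand waits tick by tick until the widget reports completion, then collapses the media and advances to the next command.
; GetAssetPaths exposes the media source as the command's asset dependency.
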(fn `GetAssetPaths`
  (params (Command :type "ShidenCommand Structure") (CallerObject :type "Object Object Reference"))
  (returns (AssetObjectPaths :type "Set of String"))
  (return (`|MakeSet` (`|GetCommandArguments` "/Shiden/Commands/DA_ShidenPrimaryCommandDefinitions.DA_ShidenPrimaryCommandDefinitions" "PlayMedia" Command))))

(fn `PreProcessCommand`
  (params (ProcessName :type String) (Command :type "ShidenCommand Structure") (Widget :type "ShidenWidget Object Reference") (ScenarioManager :type "ShidenScenarioManagerInterface Interface (by ref)") (CallerObject :type "Object Object Reference"))
  (returns (Status :type "EShidenPreProcessStatus Enum") (ErrorMessage :type String))
  (bind (_mediasource _canopenpausemenu _mediazorder) (`|GetCommandArguments` "/Shiden/Commands/DA_ShidenPrimaryCommandDefinitions.DA_ShidenPrimaryCommandDefinitions" "PlayMedia" Command))
  (bind _bsuccess (`ShidenWidget.PlayMedia` Widget _mediasource (== _canopenpausemenu "true") (`KismetStringLibrary.Conv_StringToInt` _mediazorder)))
  (if _bsuccess
    (return "Complete" "")
    (else
      (return "Error" "Playing movie failed"))))

(fn `ProcessCommand`
  (params (ProcessName :type String) (Command :type "ShidenCommand Structure") (Widget :type "ShidenWidget Object Reference") (ScenarioManager :type "ShidenScenarioManagerInterface Interface (by ref)") (DeltaTime :type "Float (single-precision)") (CallerObject :type "Object Object Reference"))
  (returns (Status :type "EShidenProcessStatus Enum") (BreakReason :type String) (NextScenarioName :type String) (ErrorMessage :type String))
  (if (`ShidenWidget.IsMediaCompleted` Widget)
    (`ShidenWidget.CollapseMedia` Widget)
    (return "Next" "" "" "")
    (else
      (return "DelayUntilNextTick" "" "" ""))))