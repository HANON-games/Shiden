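; Shiden scenario command that runs another scenario as a macro, found by ID or object path.
; Up to five typed arguments become local variables, using the macro's defaults where values are empty.
; Processing pushes the macro and resets its index so the scenario continues inside it.
; Preview runs macro-callable commands inline, skipping If-block contents without evaluating conditions, and errors on disallowed, undefined or failed commands.
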(fn `GetAssetPaths`
  (params (Command :type "ShidenCommand Structure") (CallerObject :type "Object Object Reference"))
  (returns (AssetObjectPaths :type "Set of String"))
  (return))

(fn `PreviewCommmand`
  (params (Command :type "ShidenCommand Structure (by ref)") (Widget :type "ShidenWidget Object Reference") (ScenarioManager :type "ShidenScenarioManagerInterface Interface (by ref)") (bIsCurrentCommand :type Boolean))
  (returns (Status :type "EShidenPreviewStatus Enum") (ErrorMessage :type String))
  (locals (IsInIfBracket :type Boolean) (CurrentBgm :type "ShidenSoundInfo Structure"))
  (bind (_commandname _presetname _arg1) (break `ShidenCommand` Command))
  (bind (_commandname_2 _presetname_2 _arg1_2 _arg2 _arg3 _arg4 _arg5 _arg6) (break `ShidenCommand` Command))
  (bind (_scenarioid _scenario _bsuccess) (`ShidenScenarioFunctionLibrary.GetScenarioByIdOrObjectPath` _arg1))
  (if _bsuccess
    (`ShidenScenarioFunctionLibrary.PushScenario` _arg1_2 _scenario)
    (`self.SetMacroArguments` _arg1_2 _scenario _arg2 _arg3 _arg4 _arg5 _arg6)
    (set `local.IsInIfBracket` false)
    (for (_array_element _array_index) (`ShidenScenario.Commands` _scenario)
      (bind _command (`ShidenScenarioFunctionLibrary.ConstructCommand` "Default" _array_element))
      (bind (_commandname_3 _presetname_3 _arg1_3 _arg2_2 _arg3_2 _arg4_2 _arg5_2 _arg6_2 _arg7 _arg8 _arg9 _arg10 _commandid _benabled) (break `ShidenCommand` _command))
      (if _benabled
        (switch `string` _commandname_3
          (:`Default`
            (bind (_value _returnvalue) (`BlueprintMapLibrary.Map_Find` (`ShidenSubsystem.CommandDefinitionCache` (subsystem `ShidenSubsystem`)) _commandname_3))
            (if _returnvalue
              (bind (_note _fontcolor _itemnormalcolor _itemhoveredcolor _itempressedcolor _bcancallinmacro _commandblueprint) (break `ShidenCommandDefinition` _value))
              (if _bcancallinmacro
                (if (not (`local.IsInIfBracket`))
                  (bind _command_2 (`ShidenScenarioFunctionLibrary.GetCommandFromCache` self "Default" _commandblueprint))
                  (bind (_status _errormessage) (`self.PreviewCommmand` _command_2 _command (`local.Widget`) (`local.ScenarioManager`) (`local.bIsCurrentCommand`)))
                  (if (not (`|EnumEquality` _status "Completed"))
                    (return "Error" (`ShidenCoreFunctionLibrary.MakeErrorMessage` _scenarioid _array_index _commandname_3 _errormessage))))
                (else
                  (return "Error" (`ShidenCoreFunctionLibrary.MakeErrorMessage` _scenarioid _array_index _commandname_3 "this command cannot call in macro"))))
              (else
                (return "Error" (`ShidenCoreFunctionLibrary.MakeErrorMessage` _scenarioid _array_index _commandname_3 "command definition not found")))))
          (:`If`
            (set `local.IsInIfBracket` true :!label _label))
          (:`ElseIf`
            (goto _label))
          (:`Else`
            (goto _label))
          (:`EndIf`
            (set `local.IsInIfBracket` false)))))
    (`ShidenScenarioFunctionLibrary.PopScenario` "Default")
    (return "Completed" "")
    (else
      (return "Error" (`KismetStringLibrary.Concat_StrStr` "Macro \"" _arg1 "\" was not found")))))

(fn `ProcessCommmand`
  (params (ProcessName :type String) (Command :type "ShidenCommand Structure") (Widget :type "ShidenWidget Object Reference") (ScenarioManager :type "ShidenScenarioManagerInterface Interface (by ref)") (DeltaTime :type "Float (single-precision)") (CallerObject :type "Object Object Reference"))
  (returns (Status :type "EShidenProcessStatus Enum") (BreakReason :type String) (NextScenarioName :type String) (ErrorMessage :type String))
  (bind (_commandname _presetname _arg1) (break `ShidenCommand` Command))
  (bind (_commandname_2 _presetname_2 _arg1_2 _arg2 _arg3 _arg4 _arg5 _arg6) (break `ShidenCommand` Command))
  (bind (_scenarioid _scenario _bsuccess) (`ShidenScenarioFunctionLibrary.GetScenarioByIdOrObjectPath` _arg1))
  (if _bsuccess
    (`ShidenScenarioFunctionLibrary.PushScenario` ProcessName _scenario)
    (`ShidenScenarioFunctionLibrary.SetCurrentScenarioIndex` ProcessName -1)
    (`self.SetMacroArguments` _arg1_2 _scenario _arg2 _arg3 _arg4 _arg5 _arg6)
    (return "Next" "" "" "")
    (else
      (return "Error" "" "" (`KismetStringLibrary.Concat_StrStr` "Macro \"" _arg1 "\" is not found.")))))

(fn `SetMacroArguments`
  (params (ProcessName :type String) (ShidenScenario :type "ShidenScenario Object Reference") (Arg1Value :type String) (Arg2Value :type String) (Arg3Value :type String) (Arg4Value :type String) (Arg5Value :type String))
  (bind _processname (`local.ProcessName`))
  (for _index (range 5)
    (bind _returnvalue (select `int` _index :`0` (`ShidenScenario.Arg1Name` ShidenScenario) :`1` (`ShidenScenario.Arg2Name` ShidenScenario) :`2` (`ShidenScenario.Arg3Name` ShidenScenario) :`3` (`ShidenScenario.Arg4Name` ShidenScenario) :`4` (`ShidenScenario.Arg5Name` ShidenScenario)))
    (if (not (`KismetStringLibrary.IsEmpty` _returnvalue))
      (switch `EShidenVariableType` (select `int` _index :`0` (`ShidenScenario.Arg1Type` ShidenScenario) :`1` (`ShidenScenario.Arg2Type` ShidenScenario) :`2` (`ShidenScenario.Arg3Type` ShidenScenario) :`3` (`ShidenScenario.Arg4Type` ShidenScenario) :`4` (`ShidenScenario.Arg5Type` ShidenScenario))
        (:`Boolean`
          (bind _returnvalue_2 (select `int` _index :`0` Arg1Value :`1` Arg2Value :`2` Arg3Value :`3` Arg4Value :`4` Arg5Value))
          (bind _returnvalue_3 (`KismetMathLibrary.SelectString` (select `int` _index :`0` (`ShidenScenario.Arg1DefaultValue` ShidenScenario) :`1` (`ShidenScenario.Arg2DefaultValue` ShidenScenario) :`2` (`ShidenScenario.Arg3DefaultValue` ShidenScenario) :`3` (`ShidenScenario.Arg4DefaultValue` ShidenScenario) :`4` (`ShidenScenario.Arg5DefaultValue` ShidenScenario)) _returnvalue_2 (`KismetStringLibrary.IsEmpty` _returnvalue_2)))
          (`ShidenVariableFunctionLibrary.AddLocalBoolean` _processname _returnvalue (== _returnvalue_3 "true")))
        (:`String`
          (`ShidenVariableFunctionLibrary.AddLocalString` _processname _returnvalue _returnvalue_3))
        (:`Integer`
          (`ShidenVariableFunctionLibrary.AddLocalInteger` _processname _returnvalue (`KismetStringLibrary.Conv_StringToInt` _returnvalue_3)))
        (:`Float`
          (`ShidenVariableFunctionLibrary.AddLocalFloat` _processname _returnvalue (`KismetStringLibrary.Conv_StringToDouble` _returnvalue_3)))
        (:`Vector2`
          (`ShidenVariableFunctionLibrary.AddLocalVector2` _processname _returnvalue (`KismetStringLibrary.Conv_StringToVector2D` _returnvalue_3)))
        (:`Vector3`
          (`ShidenVariableFunctionLibrary.AddLocalVector3` _processname _returnvalue (`KismetStringLibrary.Conv_StringToVector` _returnvalue_3))))
      (else
        (break))))
  (return))