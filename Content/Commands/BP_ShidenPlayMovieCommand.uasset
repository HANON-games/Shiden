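; Shiden scenario command that plays a movie from a media source path given in the command arguments.
; Pre-processing starts playback on the widget, passing a pause-menu flag and Z-orders for the movie and pause menu, and reports an error on failure.
; Processing waits tick by tick until the movie completes, then collapses it and advances to the next command.
; The media path is also reported as the command's asset dependency.
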(fn `GetAssetPaths`
  (params (Command :type "ShidenCommand Structure"))
  (returns (AssetObjectPaths :type "Set of String"))
  (return (`|MakeSet` (`.Arg1` (break `ShidenCommand` Command)))))

(fn `PreProcessCommmand`
  (params (ProcessName :type String) (Command :type "ShidenCommand Structure") (Widget :type "ShidenWidget Object Reference") (ScenarioManager :type "ShidenScenarioManagerInterface Interface (by ref)") (HookedObject :type "Object Object Reference"))
  (returns (Status :type "EShidenPreProcessStatus Enum") (ErrorMessage :type String))
  (bind (_commandname _presetname _arg1 _arg2 _arg3 _arg4) (break `ShidenCommand` Command))
  (bind _bsuccess (`ShidenWidget.PlayMovie` Widget _arg1 (== _arg2 "true") (`KismetStringLibrary.Conv_StringToInt` _arg3) (`KismetStringLibrary.Conv_StringToInt` _arg4)))
  (if _bsuccess
    (return "Completed" "")
    (else
      (return "Error" "Playing movie failed"))))

(fn `ProcessCommmand`
  (params (ProcessName :type String) (Command :type "ShidenCommand Structure") (Widget :type "ShidenWidget Object Reference") (ScenarioManager :type "ShidenScenarioManagerInterface Interface (by ref)") (DeltaTime :type "Float (single-precision)") (HookedObject :type "Object Object Reference"))
  (returns (Status :type "EShidenProcessStatus Enum") (BreakReason :type String) (NextScenarioName :type String) (ErrorMessage :type String))
  (if (`ShidenWidget.IsMovieCompleted` Widget)
    (`ShidenWidget.CollapseMovie` Widget)
    (return "Next" "" "" "")
    (else
      (return "DelayUntilNextTick" "" "" ""))))