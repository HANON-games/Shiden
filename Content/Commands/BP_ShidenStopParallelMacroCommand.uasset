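; Shiden scenario command that stops a parallel macro by requesting cancellation of the process named in the command.
; Pre-processing passes the reason and cancel type (immediate or on current command end) to RequestCancelScenario, returning an error for any other type.
; When the ensure-cancel argument is true, processing delays each tick until that process leaves the subsystem's scenario progress stack, then advances.
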(fn `PreProcessCommmand`
  (params (ProcessName :type String) (Command :type "ShidenCommand Structure") (Widget :type "ShidenWidget Object Reference") (ScenarioManager :type "ShidenScenarioManagerInterface Interface (by ref)") (HookedObject :type "Object Object Reference"))
  (returns (Status :type "EShidenPreProcessStatus Enum") (ErrorMessage :type String))
  (bind (_commandname _presetname _arg1 _arg2 _arg3) (break `ShidenCommand` Command))
  (switch `string` _arg3
    (:`Default`
      (return "Error" "Invalid Cancel Type"))
    (:`Immediately`
      (`ShidenScenarioFunctionLibrary.RequestCancelScenario` _arg1 _arg2 "Immediately"))
    (:`OnCurrentCommandEnd`
      (`ShidenScenarioFunctionLibrary.RequestCancelScenario` _arg1 _arg2 "OnCurrentCommandEnd")))
  (return "Completed" ""))

(fn `ProcessCommmand`
  (params (ProcessName :type String) (Command :type "ShidenCommand Structure") (Widget :type "ShidenWidget Object Reference") (ScenarioManager :type "ShidenScenarioManagerInterface Interface (by ref)") (DeltaTime :type "Float (single-precision)") (HookedObject :type "Object Object Reference"))
  (returns (Status :type "EShidenProcessStatus Enum") (BreakReason :type String) (NextScenarioName :type String) (ErrorMessage :type String))
  (bind (_commandname _presetname _arg1 _arg2 _arg3 _arg4) (break `ShidenCommand` Command))
  (if (== _arg4 "true")
    (if (`.ReturnValue` (`BlueprintMapLibrary.Map_Find` (`ShidenSubsystem.ScenarioProgressStack` (subsystem `ShidenSubsystem`)) _arg1))
      (return "DelayUntilNextTick" "" "" "")
      (else
        _)))
  (return "Next" "" "" ""))