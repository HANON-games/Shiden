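; Shiden scenario command for End Loop While, which closes a while loop by deciding whether the scenario repeats it.
; It scans backward from the current command to the matching Loop While, recursively skipping nested loop pairs without evaluating their conditions.
; It then checks that loop's variable type and comparison, moving the scenario index back to the Loop While when true.
; Failed lookups or checks return an error.
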(fn `CheckCondition`
  (params (ProcessName :type String) (Kind :type "EShidenVariableKind Enum" :default "UserVariable") (Type :type "EShidenVariableType Enum" :default "Boolean") (Key :type String) (Operator :type String) (Value :type String))
  (returns (Result :type Boolean) (Success :type Boolean) (ErrorMessage :type String))
  (bind (_variabletype _bbooleanvalue _stringvalue _integervalue _floatvalue _vector2value _vector3value _breturnvalue) (`ShidenVariableFunctionLibrary.FindVariable` ProcessName Kind Key))
  (if _breturnvalue
    (if (`|EnumEquality` _variabletype Type)
      (bind (_bresult _bsuccess _errormessage) (`ShidenVariableFunctionLibrary.EvaluateCondition` Type Operator _bbooleanvalue _stringvalue _integervalue _floatvalue _vector2value _vector3value (== Value "true") Value (`KismetStringLibrary.Conv_StringToInt` Value) (`KismetStringLibrary.Conv_StringToDouble` Value) (`KismetStringLibrary.Conv_StringToVector2D` Value) (`KismetStringLibrary.Conv_StringToVector` Value)))
      (return _bresult _bsuccess _errormessage)
      (else
        (return false false "Variable type not match")))
    (else
      (return false false "Variable not found"))))

(fn `FindLoopWhileIndex`
  (params (ProcessName :type String) (CurrentIndex :type Integer) (Commands :type "Array of ShidenCommand Structure"))
  (returns (Success :type Boolean) (ErrorMessage :type String))
  (locals (TargetCommandNames :type "Array of String"))
  (for _index (range 1 (+ CurrentIndex 1))
    (bind _returnvalue (- CurrentIndex _index))
    (bind _output (`|GetArrayItem` Commands _returnvalue))
    (switch `string` (`.CommandName` (break `ShidenCommand` _output))
      (:`EndLoopWhile`
        (bind (_index_2 _success _errormessage) (`self.FindLoopWhileIndexWithoutCheckCondition` (`local.ProcessName`) _returnvalue (`local.Commands`)))
        (if _success
          (bind (_success_2 _errormessage_2) (`self.FindLoopWhileIndex` (`local.ProcessName`) _index_2 (`local.Commands`)))
          (return _success_2 _errormessage_2)
          (else
            (return false _errormessage))))
      (:`LoopWhile`
        (bind (_variablekind _variablename _operator _righthandvalue) (`|GetCommandArguments` "/Shiden/Commands/DA_ShidenPrimaryCommandDefinitions.DA_ShidenPrimaryCommandDefinitions" "LoopWhile" _output))
        (bind _result (`ShidenVariableFunctionLibrary.ConvertToVariableKind` _variablekind))
        (bind (_definition _bsuccess _errormessage_3) (`ShidenVariableFunctionLibrary.GetVariableDefinition` ProcessName _result _variablename))
        (if _bsuccess
          (bind (_result_2 _success_3 _errormessage_4) (`self.CheckCondition` (`local.ProcessName`) _result (`.Type` (break `ShidenVariableDefinition` _definition)) _variablename _operator _righthandvalue))
          (if _success_3
            (if _result_2
              (`ShidenScenarioFunctionLibrary.SetCurrentScenarioIndex` (`local.ProcessName`) _returnvalue))
            (return true "")
            (else
              (return false _errormessage_4)))
          (else
            (return false _errormessage_3))))))
  (return false "Not Found EndIf"))

(fn `FindLoopWhileIndexWithoutCheckCondition`
  (params (ProcessName :type String) (CurrentIndex :type Integer) (Commands :type "Array of ShidenCommand Structure"))
  (returns (Index :type Integer) (Success :type Boolean) (ErrorMessage :type String))
  (locals (TargetCommandNames :type "Array of String"))
  (for _index (range 1 (+ CurrentIndex 1))
    (bind _returnvalue (- CurrentIndex _index))
    (switch `string` (`.CommandName` (break `ShidenCommand` (`|GetArrayItem` Commands _returnvalue)))
      (:`EndLoopWhile`
        (bind (_index_2 _success _errormessage) (`self.FindLoopWhileIndexWithoutCheckCondition` (`local.ProcessName`) _returnvalue (`local.Commands`)))
        (if _success
          (bind (_index_3 _success_2 _errormessage_2) (`self.FindLoopWhileIndexWithoutCheckCondition` (`local.ProcessName`) _index_2 (`local.Commands`)))
          (return _index_3 _success_2 _errormessage_2)
          (else
            (return 0 false _errormessage))))
      (:`LoopWhile`
        (return _returnvalue true ""))))
  (return 0 false "Not Found EndIf"))

(fn `ProcessCommand`
  (params (ProcessName :type String) (Command :type "ShidenCommand Structure") (Widget :type "ShidenWidget Object Reference") (ScenarioManager :type "ShidenScenarioManagerInterface Interface (by ref)") (DeltaTime :type "Float (single-precision)") (CallerObject :type "Object Object Reference"))
  (returns (Status :type "EShidenProcessStatus Enum") (BreakReason :type String) (NextScenarioName :type String) (ErrorMessage :type String))
  (bind _scenarioprogress (`ShidenScenarioFunctionLibrary.PeekScenario` "Default"))
  (bind _scenario (`ShidenScenarioFunctionLibrary.GetScenarioFromCache` (break `ShidenScenarioProgress` _scenarioprogress)))
  (bind (_success _errormessage) (`self.FindLoopWhileIndex` ProcessName (`.CurrentIndex` (break `ShidenScenarioProgress` _scenarioprogress)) (`ShidenScenario.Commands` _scenario)))
  (if _success
    (return "Next" "" "" "")
    (else
      (return "Error" "" "" _errormessage))))