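; Shiden scenario command "ChangeVisibility" that sets the visibility of a named widget from the command's Name and Visibility arguments.
; Processing applies the change through SetVisibilityByName and registers it as a scenario property, while preview applies it without registering.
; Restoring from save data replays each stored name and visibility pair without re-registering.
; A helper maps the visibility text to the widget visibility enum, and a missing widget returns an error.
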(fn `ConvertToVisibility`
  (params (Visibility :type String))
  (returns (Result :type "ESlateVisibility Enum"))
  (switch `string` Visibility
    (:`Visible`
      (return "Visible"))
    (:`Collapsed`
      (return "Collapsed"))
    (:`Hidden`
      (return "Hidden"))
    (:`Not Hit-Testable (Self & All Children)`
      (return "HitTestInvisible"))
    (:`Not Hit-Testable (Self Only)`
      (return "SelfHitTestInvisible"))))

(fn `PreviewCommand`
  (params (Command :type "ShidenCommand Structure (by ref)") (Widget :type "ShidenWidget Object Reference") (ScenarioManager :type "ShidenScenarioManagerInterface Interface (by ref)") (bIsCurrentCommand :type Boolean))
  (returns (Status :type "EShidenPreviewStatus Enum") (ErrorMessage :type String))
  (bind (_name _visibility) (`|GetCommandArguments` "/Shiden/Commands/DA_ShidenPrimaryCommandDefinitions.DA_ShidenPrimaryCommandDefinitions" "ChangeVisibility" Command))
  (bind _bsuccess (`ShidenWidget.SetVisibilityByName` Widget _name (`self.ConvertToVisibility` _visibility) false))
  (if _bsuccess
    (return "Complete" "")
    (else
      (return "Error" (`KismetStringLibrary.Concat_StrStr` "Widget \"" _name "\" is not found.")))))

(fn `ProcessCommand`
  (params (ProcessName :type String) (Command :type "ShidenCommand Structure") (Widget :type "ShidenWidget Object Reference") (ScenarioManager :type "ShidenScenarioManagerInterface Interface (by ref)") (DeltaTime :type "Float (single-precision)") (CallerObject :type "Object Object Reference"))
  (returns (Status :type "EShidenProcessStatus Enum") (BreakReason :type String) (NextScenarioName :type String) (ErrorMessage :type String))
  (bind (_name _visibility) (`|GetCommandArguments` "/Shiden/Commands/DA_ShidenPrimaryCommandDefinitions.DA_ShidenPrimaryCommandDefinitions" "ChangeVisibility" Command))
  (bind _bsuccess (`ShidenWidget.SetVisibilityByName` Widget _name (`self.ConvertToVisibility` _visibility) true))
  (if _bsuccess
    (return "Next" "" "" "")
    (else
      (return "Error" "" "" (`KismetStringLibrary.Concat_StrStr` "Widget \"" _name "\" is not found.")))))

(fn `RestoreFromSaveData`
  (params (ScenarioProperties :type "Map of String to String (by ref)") (Widget :type "ShidenWidget Object Reference") (ScenarioManager :type "ShidenScenarioManagerInterface Interface (by ref)") (CallerObject :type "Object Object Reference"))
  (returns (Status :type "EShidenInitFromSaveDataStatus Enum") (ErrorMessage :type String))
  (bind _keys (`BlueprintMapLibrary.Map_Keys` ScenarioProperties))
  (for _array_element _keys
    (bind _bsuccess (`ShidenWidget.SetVisibilityByName` Widget _array_element (`self.ConvertToVisibility` (`BlueprintMapLibrary.Map_Find` ScenarioProperties _array_element)) false))
    (if (not _bsuccess)
      (return "Error" (`KismetStringLibrary.Concat_StrStr` "Widget \"" _array_element "\" is not found."))))
  (return "Complete" ""))