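; Shiden scenario command that shows the player up to five options and stores the selected index in a variable.
; Pre-processing fills the options, switches the widget to options-only or text-plus-options mode, and sets selection input.
; Processing waits each tick for a selection, writes it to a user, local or system variable (other kinds error), then restores window and input modes.
; Preview mirrors the window change, setting options only for the current command.
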(fn `CallSetOptions`
  (params (Command :type "ShidenCommand Structure (by ref)") (Widget :type "ShidenWidget Object Reference"))
  (bind (_commandname _presetname _arg1 _arg2 _arg3 _arg4 _arg5) (break `ShidenCommand` Command))
  (`ShidenWidget.SetOptions` Widget (`|MakeArray` _arg1 _arg2 _arg3 _arg4 _arg5)))

(fn `ChangeWindowMode`
  (params (Command :type "ShidenCommand Structure") (Widget :type "ShidenWidget Object Reference"))
  (bind _output_get (set `self.PreviousWindowMode` (`ShidenWidget.GetWindowMode` Widget)))
  (if (or (`|EnumEquality` _output_get) (== (`.Arg8` (break `ShidenCommand` Command)) "true"))
    (`ShidenWidget.ChangeWindowMode` Widget "Options" true)
    (else
      (`ShidenWidget.ChangeWindowMode` Widget "TextAndOptions" true))))

(fn `PreProcessCommmand`
  (params (ProcessName :type String) (Command :type "ShidenCommand Structure") (Widget :type "ShidenWidget Object Reference") (ScenarioManager :type "ShidenScenarioManagerInterface Interface (by ref)") (HookedObject :type "Object Object Reference"))
  (returns (Status :type "EShidenPreProcessStatus Enum") (ErrorMessage :type String))
  (`self.CallSetOptions` Command Widget)
  (`self.ChangeWindowMode` Command Widget)
  (`ShidenWidget.SetInputModeSelectOption` Widget)
  (return "Completed" ""))

(fn `PreviewCommmand`
  (params (Command :type "ShidenCommand Structure (by ref)") (Widget :type "ShidenWidget Object Reference") (ScenarioManager :type "ShidenScenarioManagerInterface Interface (by ref)") (bIsCurrentCommand :type Boolean))
  (returns (Status :type "EShidenPreviewStatus Enum") (ErrorMessage :type String))
  (`self.ChangeWindowMode` Command Widget)
  (if bIsCurrentCommand
    (`self.CallSetOptions` Command Widget)
    (return "Completed" "")
    (else
      (return "Completed" ""))))

(fn `ProcessCommmand`
  (params (ProcessName :type String) (Command :type "ShidenCommand Structure") (Widget :type "ShidenWidget Object Reference") (ScenarioManager :type "ShidenScenarioManagerInterface Interface (by ref)") (DeltaTime :type "Float (single-precision)") (HookedObject :type "Object Object Reference"))
  (returns (Status :type "EShidenProcessStatus Enum") (BreakReason :type String) (NextScenarioName :type String) (ErrorMessage :type String))
  (bind (_commandname _presetname _arg1 _arg2 _arg3 _arg4 _arg5 _arg6 _arg7) (break `ShidenCommand` Command))
  (bind _result (`ShidenWidget.GetSelectedOption` Widget))
  (bind _widget (`local.Widget`))
  (bind (_result_2 _bsuccess) (`ShidenVariableFunctionLibrary.ConvertToVariableKind` _arg6))
  (if (!= _result -1)
    (if _bsuccess
      (switch `EShidenVariableKind` _result_2
        (:`UserVariable`
          (`ShidenVariableFunctionLibrary.AddUserInteger` _arg7 _result)
          (`ShidenWidget.ChangeWindowMode` _widget (`self.PreviousWindowMode`) true :!label _label)
          (`ShidenWidget.SetInputModeGameAndUI` _widget)
          (return "Next" "" "" ""))
        (:`LocalVariable`
          (`ShidenVariableFunctionLibrary.AddLocalInteger` "Default" _arg7 _result)
          (goto _label))
        (:`SystemVariable`
          (`ShidenVariableFunctionLibrary.AddSystemInteger` _arg7 _result)
          (goto _label))
        (:`PredefinedSystemVariable`
          _)))
    (return "Error" "" "" (`KismetStringLibrary.Concat_StrStr` "Variable kind \"" _arg6 "\" is invalid"))
    (else
      (return "DelayUntilNextTick" "" "" ""))))