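; Shiden scenario command that stops a named parallel scenario process.
; PreProcessCommand reads the command arguments and requests cancellation with the given reason, either immediately or when that process's current command ends, erroring on any other timing.
; ProcessCommand optionally waits for completion, delaying each tick while the process remains in the subsystem's ScenarioProgressStack, then moves to the next command.
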(fn `PreProcessCommand`
  (params (ProcessName :type String) (Command :type "ShidenCommand Structure") (Widget :type "ShidenWidget Object Reference") (ScenarioManager :type "ShidenScenarioManagerInterface Interface (by ref)") (CallerObject :type "Object Object Reference"))
  (returns (Status :type "EShidenPreProcessStatus Enum") (ErrorMessage :type String))
  (bind (_processname _reason _stoptiming) (`|GetCommandArguments` "/Shiden/Commands/DA_ShidenPrimaryCommandDefinitions.DA_ShidenPrimaryCommandDefinitions" "StopParallelProcess" Command))
  (switch `string` _stoptiming
    (:`Default`
      (return "Error" "Invalid Cancel Type"))
    (:`Immediately`
      (`ShidenScenarioFunctionLibrary.RequestCancelScenario` _processname _reason "Immediately"))
    (:`OnCurrentCommandEnd`
      (`ShidenScenarioFunctionLibrary.RequestCancelScenario` _processname _reason "OnCurrentCommandEnd")))
  (return "Complete" ""))

(fn `ProcessCommand`
  (params (ProcessName :type String) (Command :type "ShidenCommand Structure") (Widget :type "ShidenWidget Object Reference") (ScenarioManager :type "ShidenScenarioManagerInterface Interface (by ref)") (DeltaTime :type "Float (single-precision)") (CallerObject :type "Object Object Reference"))
  (returns (Status :type "EShidenProcessStatus Enum") (BreakReason :type String) (NextScenarioName :type String) (ErrorMessage :type String))
  (bind (_processname _reason _stoptiming _waitforcompletion) (`|GetCommandArguments` "/Shiden/Commands/DA_ShidenPrimaryCommandDefinitions.DA_ShidenPrimaryCommandDefinitions" "StopParallelProcess" Command))
  (if (== _waitforcompletion "true")
    (if (`.ReturnValue` (`BlueprintMapLibrary.Map_Find` (`ShidenSubsystem.ScenarioProgressStack` (subsystem `ShidenSubsystem`)) _processname))
      (return "DelayUntilNextTick" "" "" "")
      (else
        _)))
  (return "Next" "" "" ""))