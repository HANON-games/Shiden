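; Shiden scenario command that sets a texture parameter on the material of a named Image or Retainer Box in the widget.
; Process and preview load the texture from Arg4 and share ChangeTextureParameter to apply it.
; Processing also saves the path as a scenario property under an escaped "type::target::parameter" key.
; InitFromSaveData parses that key to reapply the texture, but returns after the first saved entry.
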(fn `ChangeTextureParameter`
  (params (Command :type "ShidenCommand Structure (by ref)") (Widget :type "ShidenWidget Object Reference") (Texture :type "Texture Object Reference"))
  (returns (Success :type Boolean) (ErrorMessage :type String))
  (bind (_commandname _presetname _arg1 _arg2 _arg3) (break `ShidenCommand` Command))
  (bind (_value _returnvalue) (`BlueprintMapLibrary.Map_Find` (`ShidenWidget.GetRetainerBoxes` Widget) _arg2))
  (bind (_value_2 _returnvalue_2) (`BlueprintMapLibrary.Map_Find` (`ShidenWidget.GetImages` Widget) (`.Arg2` (break `ShidenCommand` Command))))
  (switch `string` _arg1
    (:`Image`
      (if _returnvalue_2
        (`MaterialInstanceDynamic.SetTextureParameterValue` (`WidgetBlueprintLibrary.GetDynamicMaterial` (`Image.Brush` _value_2)) (`KismetStringLibrary.Conv_StringToName` _arg3) Texture)
        (else
          (return false "Image  not found"))))
    (:`RetainerBox`
      (if _returnvalue
        (`MaterialInstanceDynamic.SetTextureParameterValue` (`RetainerBox.GetEffectMaterial` _value) (`KismetStringLibrary.Conv_StringToName` _arg3) Texture)
        (else
          (return false "RetainerBox  not found")))))
  (return true ""))

(fn `GetAssetPaths`
  (params (Command :type "ShidenCommand Structure"))
  (returns (AssetObjectPaths :type "Set of String"))
  (return (`|MakeSet` (`.Arg4` (break `ShidenCommand` Command)))))

(fn `InitFromSaveData`
  (params (ScenarioProperties :type "Map of String to String (by ref)") (Widget :type "ShidenWidget Object Reference") (ScenarioManager :type "ShidenScenarioManagerInterface Interface (by ref)"))
  (returns (Status :type "EShidenInitFromSaveDataStatus Enum") (ErrorMessage :type String))
  (bind _keys (`BlueprintMapLibrary.Map_Keys` ScenarioProperties))
  (for _array_element _keys
    (bind (_asset _bsuccess) (`ShidenCoreFunctionLibrary.GetAsset` (`BlueprintMapLibrary.Map_Find` ScenarioProperties _array_element)))
    (if _bsuccess
      (bind _astexture (cast `Texture` _asset)
        (:`then`
          (bind (_targettype _targetname _parametername) (`self.ParseCurrentKey` _array_element))
          (bind (_success _errormessage) (`self.ChangeTextureParameter` (make `ShidenCommand` "ChangeMaterialTextureParameter" "" _targettype _targetname _parametername) Widget _astexture))
          (if _success
            (return "Completed" "")
            (else
              (return "Error" _errormessage))))
        (:`CastFailed`
          (return "Error" "Cannot cast to Texture")))
      (else
        (return "Completed" ""))))
  (return "Completed" ""))

(fn `MakeCurrentKey`
  (params (TargetType :type String) (TargetName :type String) (ParameterName :type String))
  (returns (ReturnValue :type String))
  (return (`KismetStringLibrary.Concat_StrStr` (`KismetStringLibrary.Replace` TargetType ":" "\\:") "::" (`KismetStringLibrary.Replace` TargetName ":" "\\:") "::" (`KismetStringLibrary.Replace` ParameterName ":" "\\:"))))

(fn `ParseCurrentKey`
  (params (Key :type String))
  (returns (TargetType :type String) (TargetName :type String) (ParameterName :type String))
  (bind (_lefts _rights) (`KismetStringLibrary.Split` Key "::"))
  (bind (_lefts_2 _rights_2) (`KismetStringLibrary.Split` _rights "::"))
  (return (`KismetStringLibrary.Replace` _lefts "\\:" ":") (`KismetStringLibrary.Replace` _lefts_2 "\\:" ":") (`KismetStringLibrary.Replace` _rights_2 "\\:" ":")))

(fn `PreviewCommmand`
  (params (Command :type "ShidenCommand Structure (by ref)") (Widget :type "ShidenWidget Object Reference") (ScenarioManager :type "ShidenScenarioManagerInterface Interface (by ref)") (bIsCurrentCommand :type Boolean))
  (returns (Status :type "EShidenPreviewStatus Enum") (ErrorMessage :type String))
  (bind (_commandname _presetname _arg1 _arg2 _arg3 _arg4) (break `ShidenCommand` Command))
  (bind (_asset _bsuccess) (`ShidenCoreFunctionLibrary.GetAsset` _arg4))
  (if _bsuccess
    (bind _astexture (cast `Texture` _asset)
      (:`then`
        (bind (_success _errormessage) (`self.ChangeTextureParameter` Command Widget _astexture))
        (if _success
          (return "Completed" "")
          (else
            (return "Error" _errormessage))))
      (:`CastFailed`
        (return "Error" "Cannot cast to Texture")))
    (else
      (return "Error" (`KismetStringLibrary.Concat_StrStr` "Asset \"" _arg4 "\" is not found")))))

(fn `ProcessCommmand`
  (params (ProcessName :type String) (Command :type "ShidenCommand Structure") (Widget :type "ShidenWidget Object Reference") (ScenarioManager :type "ShidenScenarioManagerInterface Interface (by ref)") (DeltaTime :type "Float (single-precision)") (HookedObject :type "Object Object Reference"))
  (returns (Status :type "EShidenProcessStatus Enum") (BreakReason :type String) (NextScenarioName :type String) (ErrorMessage :type String))
  (bind (_commandname _presetname _arg1 _arg2 _arg3 _arg4) (break `ShidenCommand` Command))
  (bind (_asset _bsuccess) (`ShidenCoreFunctionLibrary.GetAsset` (`.Arg4` (break `ShidenCommand` Command))))
  (if _bsuccess
    (bind _astexture (cast `Texture` _asset)
      (:`then`
        (bind (_success _errormessage) (`self.ChangeTextureParameter` Command Widget _astexture))
        (if _success
          (`ShidenCommandFunctionLibrary.RegisterCurrentScenarioProperty` (`.CommandName` (break `ShidenCommand` Command)) (`self.MakeCurrentKey` _arg1 _arg2 _arg3) _arg4)
          (return "Next" "" "" "")
          (else
            (return "Error" "" "" _errormessage))))
      (:`CastFailed`
        (return "Error" "" "" "Cast failed")))
    (else
      (return "Error" "" "" "Asset not found"))))