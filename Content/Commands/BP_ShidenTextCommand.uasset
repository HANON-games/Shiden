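; Shiden scenario command that types localized dialogue into a named text slot, with optional voice and appending to the slot's previous text.
; PreProcess finds the slot, builds the text and starts the voice; Process reveals letters over time, honoring next and skip input.
; It then waits for input, skip or auto mode, which accounts for voice length, before registering the property and writing the backlog.
; Save-data restore and editor preview set slot text directly.
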(fn `GetAssetPaths`
  (params (Command :type "ShidenCommand Structure") (CallerObject :type "Object Object Reference"))
  (returns (AssetObjectPaths :type "Set of String"))
  (bind (_commandname _presetname _arg1 _arg2 _arg3 _arg4 _arg5) (break `ShidenCommand` Command))
  (if (`KismetStringLibrary.IsEmpty` _arg5)
    (return)
    (else
      (return (`|MakeSet` _arg5)))))

(fn `GetInput`
  (params (ScenarioManager :type "ShidenScenarioManagerInterface Interface") (ScenarioWidget :type "ShidenWidget Object Reference"))
  (bind _digitalinputs (`ShidenScenarioManagerInterface.GetShidenInput` ScenarioManager))
  (`|ExecutionSequence`
    (:`then_0`
      (bind (_value _returnvalue) (`BlueprintMapLibrary.Map_Find` _digitalinputs "/Shiden/Misc/EnhancedInput/IA_ShidenNext.IA_ShidenNext"))
      (if _returnvalue
        (if _value
          (if (`self.NextButtonPress`)
            (set `self.NextButtonPressStart` false)
            (else
              (set `self.NextButtonPressStart` true)
              (set `self.NextButtonPress` true)))
          (else
            (set `self.NextButtonPressStart` false)
            (set `self.NextButtonPress` false)))))
    (:`then_1`
      (if (or (`BlueprintMapLibrary.Map_Find` _digitalinputs "/Shiden/Misc/EnhancedInput/IA_ShidenSkip.IA_ShidenSkip") (`ShidenWidget.IsSkipPressed` ScenarioWidget))
        (if (`self.SkipButtonPress`)
          (set `self.SkipButtonPressStart` false)
          (else
            (set `self.SkipButtonPressStart` true)
            (set `self.SkipButtonPress` true)))
        (else
          (set `self.SkipButtonPressStart` false)
          (set `self.SkipButtonPress` false))))))

(fn `GetText`
  (params (Command :type "ShidenCommand Structure"))
  (returns (Text :type String))
  (bind (_commandname _presetname _arg1 _arg2 _arg3 _arg4 _arg5 _arg6 _arg7 _arg8 _arg9 _arg10) (break `ShidenCommand` Command))
  (return (select `int` (`ShidenVariableFunctionLibrary.GetLanguageIndex`) :`0` _arg2 :`1` _arg7 :`2` _arg8 :`3` _arg9 :`4` _arg10)))

(fn `GetTextWidget`
  (params (SlotName :type String) (ScenarioWidget :type "ShidenWidget Object Reference"))
  (returns (TextBlock :type "RichTextBlock Object Reference") (Found :type Boolean))
  (bind _textobjects (`ShidenWidget.GetTexts` ScenarioWidget))
  (bind (_value _returnvalue) (`BlueprintMapLibrary.Map_Find` _textobjects SlotName))
  (if (`KismetStringLibrary.IsEmpty` SlotName)
    ;[1 1 1] Set text to first slot
    (bind _values (`BlueprintMapLibrary.Map_Values` _textobjects))
    (for _array_element _values
      (return _array_element true))
    (return null false)
    (else
      (return _value _returnvalue))))

(fn `InitFromSaveData`
  (params (ScenarioProperties :type "Map of String to String (by ref)") (Widget :type "ShidenWidget Object Reference") (ScenarioManager :type "ShidenScenarioManagerInterface Interface (by ref)") (CallerObject :type "Object Object Reference"))
  (returns (Status :type "EShidenInitFromSaveDataStatus Enum") (ErrorMessage :type String))
  (bind _textobjects (`ShidenWidget.GetTexts` Widget))
  (bind _keys (`BlueprintMapLibrary.Map_Keys` _textobjects))
  (for _array_element _keys
    (bind (_value _returnvalue) (`BlueprintMapLibrary.Map_Find` _textobjects _array_element))
    (if _returnvalue
      (bind _value_2 (`BlueprintMapLibrary.Map_Find` ScenarioProperties _array_element))
      (`RichTextBlock.SetText` _value (`KismetTextLibrary.Conv_StringToText` _value_2))
      (if (`KismetStringLibrary.EqualEqual_StrStr` _array_element "Name")
        (`ShidenCoreFunctionLibrary.AddBacklog` _array_element _value_2))
      (else
        (return "Error" (`KismetStringLibrary.Concat_StrStr` "Text \"" _array_element "\" is not found")))))
  (return "Completed" ""))

(fn `PreProcessCommmand`
  (params (ProcessName :type String) (Command :type "ShidenCommand Structure") (Widget :type "ShidenWidget Object Reference") (ScenarioManager :type "ShidenScenarioManagerInterface Interface (by ref)") (CallerObject :type "Object Object Reference"))
  (returns (Status :type "EShidenPreProcessStatus Enum") (ErrorMessage :type String))
  (bind (_commandname _presetname _arg1) (break `ShidenCommand` Command))
  (bind (_commandname_2 _presetname_2 _arg1_2 _arg2 _arg3 _arg4 _arg5) (break `ShidenCommand` (`local.Command`)))
  (bind (_commandname_3 _presetname_3 _arg1_3 _arg2_2 _arg3_2 _arg4_2 _arg5_2 _arg6) (break `ShidenCommand` (`local.Command`)))
  (bind (_textblock _found) (`self.GetTextWidget` _arg1 Widget))
  (if _found
    (set `self.TotalElapsedTime` 0.0)
    (set `self.CurrentText` "")
    (set `self.CurrentSlotName` (`KismetMathLibrary.SelectString` "Default" _arg1_3 (`KismetStringLibrary.IsEmpty` _arg1_3)))
    (if (== _arg6 "true")
      (bind (_arrayindex _arrayelement) (`/Engine/EditorBlueprintResources/StandardMacros.ReverseForEachLoop` (`ShidenCoreFunctionLibrary.GetBacklog`))
        (:`LoopBody`
          (if (`KismetStringLibrary.EqualEqual_StrStr` (break `ShidenBacklogItem` _arrayelement) (`self.CurrentSlotName`))
            (bind _output_get (set `self.CurrentText` (`.Text` (break `ShidenBacklogItem` _arrayelement))))
            (bind _returnvalue (`ShidenCoreFunctionLibrary.GetParsedLength` _output_get))
            (set `self.CurrentTextIndex` _returnvalue)
            (bind _output_get_2 (set `self.CurrentText` (`KismetStringLibrary.Concat_StrStr` (`self.CurrentText`) (`self.GetText` (`local.Command`))) :!label _label))
            (bind _returnvalue_2 (`ShidenCoreFunctionLibrary.GetParsedLength` _output_get_2))
            (set `self.TextLength` _returnvalue_2)
            (`ShidenWidget.ChangeWindowMode` (`local.Widget`) "Texts" true)
            ;[1 1 1] Play voice (if skip mode is enabled, should not play voice)
            (bind _digitalinputs (`ShidenScenarioManagerInterface.GetShidenInput` (`local.ScenarioManager`)))
            (if (`ShidenVariableFunctionLibrary.GetStopVoiceWhenNextDialogueStart`)
              (`ShidenScenarioManagerInterface.StopVoices` (`local.ScenarioManager`) false))
            (if (or (`KismetStringLibrary.IsEmpty` _arg5) (`BlueprintMapLibrary.Map_Find` _digitalinputs "/Shiden/Misc/EnhancedInput/IA_ShidenSkip.IA_ShidenSkip"))
              (set `self.VoiceDuration` 0.0)
              (set `self.VoiceStarted` false)
              (else
                (bind (_duration _bsuccess) (`ShidenScenarioManagerInterface.PlaySound2d` (`local.ScenarioManager`) (make `ShidenSoundInfo` 0 "Voice" _arg5 1.0 1.0 0.0 false "Linear" 0.0)))
                (if _bsuccess
                  (set `self.VoiceDuration` _duration)
                  (set `self.VoiceStarted` true)
                  (else
                    (return "Error" "Play sound 2d failed")))))
            (return "Completed" "")))
        (:`Completed`
          (set `self.CurrentTextIndex` 0 :!label _label_2)
          (goto _label)))
      (else
        (`RichTextBlock.SetText` _textblock "") ; Clear text
        (goto _label_2)))
    (else
      (return "Error" (`KismetStringLibrary.Concat_StrStr` "Text slot \"" _arg1 "\" is not found")))))

(fn `PreviewCommmand`
  (params (Command :type "ShidenCommand Structure (by ref)") (Widget :type "ShidenWidget Object Reference") (ScenarioManager :type "ShidenScenarioManagerInterface Interface (by ref)") (bIsCurrentCommand :type Boolean))
  (returns (Status :type "EShidenPreviewStatus Enum") (ErrorMessage :type String))
  (locals (temp :type "ShidenSoundInfo Structure"))
  (bind (_commandname _presetname _arg1 _arg2 _arg3 _arg4 _arg5) (break `ShidenCommand` Command))
  (bind (_commandname_2 _presetname_2 _arg1_2 _arg2_2 _arg3_2 _arg4_2 _arg5_2 _arg6) (break `ShidenCommand` (`local.Command`)))
  (bind _text (`self.GetText` (`local.Command`)))
  (if (`KismetStringLibrary.IsEmpty` _arg5)
    _
    (elif bIsCurrentCommand
      (bind (_duration _bsuccess) (`ShidenScenarioManagerInterface.PlaySound2d` ScenarioManager (make `ShidenSoundInfo` 0 "Voice" _arg5 1.0 1.0 0.0 false "Linear" 0.0)))
      (if _bsuccess
        _
        (else
          (return "Error" "Play Sound failed")))))
  (`ShidenWidget.ChangeWindowMode` (`local.Widget`) "Texts" false)
  (bind (_textblock _found) (`self.GetTextWidget` _arg1_2 (`local.Widget`)))
  (if _found
    (if (== _arg6 "true")
      (`RichTextBlock.SetText` _textblock (`KismetTextLibrary.Conv_StringToText` (`KismetStringLibrary.Concat_StrStr` (`KismetTextLibrary.Conv_TextToString` (`RichTextBlock.GetText` _textblock)) _text)))
      (else
        (`RichTextBlock.SetText` _textblock (`KismetTextLibrary.Conv_StringToText` _text))))
    (return "Completed" "")
    (else
      (return "Error" (`KismetStringLibrary.Concat_StrStr` "Text slot \"" _arg1_2 "\" is not found")))))

(fn `ProcessCommmand`
  (params (ProcessName :type String) (Command :type "ShidenCommand Structure") (Widget :type "ShidenWidget Object Reference") (ScenarioManager :type "ShidenScenarioManagerInterface Interface (by ref)") (DeltaTime :type "Float (single-precision)") (CallerObject :type "Object Object Reference"))
  (returns (Status :type "EShidenProcessStatus Enum") (BreakReason :type String) (NextScenarioName :type String) (ErrorMessage :type String))
  (bind (_commandname _presetname _arg1 _arg2 _arg3 _arg4 _arg5) (break `ShidenCommand` (`local.Command`)))
  (bind (_commandname_2 _presetname_2 _arg1_2 _arg2_2 _arg3_2 _arg4_2 _arg5_2) (break `ShidenCommand` (`local.Command`)))
  (bind (_commandname_3 _presetname_3 _arg1_3 _arg2_3 _arg3_3 _arg4_3 _arg5_3 _arg6) (break `ShidenCommand` (`local.Command`)))
  (`self.GetInput` ScenarioManager Widget)
  (set `self.TotalElapsedTime` (+ (`self.TotalElapsedTime`) DeltaTime))
  (`|ExecutionSequence`
    (:`then_0`
      (if (`ShidenSubsystem.IsPreviewMode` (subsystem `ShidenSubsystem`))
        (return "DelayUntilNextTick" "" "" "")))
    (:`then_1`
      (if (and (not (`KismetStringLibrary.IsEmpty` _arg5_2)) (not (`self.VoiceStarted`)))
        (bind (_duration _bsuccess) (`ShidenScenarioManagerInterface.PlaySound2d` (`local.ScenarioManager`) (make `ShidenSoundInfo` 0 "Voice" _arg5_2)))
        (if _bsuccess
          (set `self.VoiceDuration` _duration)
          (set `self.VoiceStarted` true)
          (else
            (return "Error" "" "" "Play sound 2d failed")))))
    (:`then_2`
      (if (!= (`self.CurrentTextIndex`) (`self.TextLength`))
        (if (or (== (`.Arg4` (break `ShidenCommand` (`local.Command`))) "true") (`self.NextButtonPressStart`))
          (set `self.CurrentTextIndex` (`self.TextLength`))
          (elif (> (`self.ElapsedTime`) (`ShidenVariableFunctionLibrary.GetSecondsToWaitForEachLetter`))
            (`/Engine/EditorBlueprintResources/StandardMacros.IncrementInt` (`self.CurrentTextIndex`)
              (:`  `
                _))
            (else
              (set `self.ElapsedTime` (+ (`self.ElapsedTime`) (`KismetMathLibrary.SelectFloat` (* (`local.DeltaTime`) (`ShidenVariableFunctionLibrary.GetSkipSpeedRate`)) (`local.DeltaTime`) (`self.SkipButtonPress`))))
              (return "DelayUntilNextTick" "" "" ""))))
        (`self.ShowText` (`local.Widget`) (`self.CurrentSlotName`) (`self.CurrentText`) (`self.CurrentTextIndex`))
        (set `self.ElapsedTime` 0.0)
        (return "DelayUntilNextTick" "" "" "")))
    (:`then_3`
      (if (or (== (`.Arg3` (break `ShidenCommand` (`local.Command`))) "false") (or (`self.NextButtonPressStart`) (and (`self.SkipButtonPress`) (`ShidenScenarioFunctionLibrary.CanSkipCommand`))) (and (`ShidenSubsystem.IsAutoTextMode` (subsystem `ShidenSubsystem`)) (and (> (`self.ElapsedTime`) (`ShidenVariableFunctionLibrary.GetWaitTimeOnAutoMode`)) (or (or (`KismetStringLibrary.IsEmpty` _arg5) (`KismetStringLibrary.EqualEqual_StrStr` _arg5)) (> (`self.TotalElapsedTime`) (+ (`self.VoiceDuration`) (`ShidenVariableFunctionLibrary.GetWaitTimeOnAutoMode`)))))))
        (`ShidenCommandFunctionLibrary.RegisterScenarioProperty` (`.CommandName` (break `ShidenCommand` (`local.Command`))) (`self.CurrentSlotName`) (`self.CurrentText`))
        (if (and (== _arg6 "true") (`KismetStringLibrary.NotEqual_StrStr` _arg1_3 "Name"))
          (bind (_arrayindex _arrayelement) (`/Engine/EditorBlueprintResources/StandardMacros.ReverseForEachLoop` (`ShidenCoreFunctionLibrary.GetBacklog`))
            (:`LoopBody`
              (if (`KismetStringLibrary.EqualEqual_StrStr` (break `ShidenBacklogItem` _arrayelement) (`self.CurrentSlotName`))
                (`ShidenCoreFunctionLibrary.UpdateBacklog` _arrayindex (`self.CurrentSlotName`) (`self.CurrentText`))
                (return "Next" "" "" "")))
            (:`Completed`
              (`ShidenCoreFunctionLibrary.AddBacklog` (`self.CurrentSlotName`) (`self.CurrentText`) :!label _label)
              (return "Next" "" "" "")))
          (else
            (goto _label)))
        (else
          (set `self.ElapsedTime` (+ (`self.ElapsedTime`) (`local.DeltaTime`)))
          (return "DelayUntilNextTick" "" "" ""))))))

(fn `ShowText`
  (params (ScenarioWidget :type "ShidenWidget Object Reference") (SlotName :type String) (text :type String) (CharacterCount :type "Integer (by ref)"))
  (bind _textblock (`self.GetTextWidget` SlotName ScenarioWidget)) ; Widget may always be found because\nwe checked widget in preprocess
  (bind _returnvalue (`ShidenCoreFunctionLibrary.GetCharactersWithParsedLength` text CharacterCount))
  (`RichTextBlock.SetText` _textblock (`KismetTextLibrary.Conv_StringToText` _returnvalue)))