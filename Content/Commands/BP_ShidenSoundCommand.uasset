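; Shiden scenario command that plays 2D BGM, SE or Voice on numbered tracks through the ScenarioManager, with volume, pitch, start time and fade options.
; BGM settings are saved as "TrackId::Field" scenario properties, replayed by InitFromSaveData and removed when the path is empty.
; An empty path is still passed on for BGM and Voice but skipped for SE.
; Preview plays SE and Voice, and applies fade duration, only for the current command.
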(fn `ConvertToAudioFaderCurve`
  (params (AudioFaderCurve :type String))
  (returns (EnumValue :type "EAudioFaderCurve Enum") (Success :type Boolean))
  (switch `string` AudioFaderCurve
    (:`Default`
      (return "Linear" false))
    (:`Linear`
      (return "Linear" true))
    (:`Logarithmic`
      (return "Logarithmic" true))
    (:`Sin (S-Curve)`
      (return "SCurve" true))
    (:`Sin (Equal Power)`
      (return "Sin" true))))

(fn `GetAssetPaths`
  (params (Command :type "ShidenCommand Structure") (CallerObject :type "Object Object Reference"))
  (returns (AssetObjectPaths :type "Set of String"))
  (return (`|MakeSet` (`.Arg3` (break `ShidenCommand` Command)))))

(fn `InitFromSaveData`
  (params (ScenarioProperties :type "Map of String to String (by ref)") (Widget :type "ShidenWidget Object Reference") (ScenarioManager :type "ShidenScenarioManagerInterface Interface (by ref)") (CallerObject :type "Object Object Reference"))
  (returns (Status :type "EShidenInitFromSaveDataStatus Enum") (ErrorMessage :type String))
  (bind _keys (`BlueprintMapLibrary.Map_Keys` ScenarioProperties))
  (for _array_element _keys
    (if (`KismetStringLibrary.EndsWith` _array_element "::Path")
      (bind (_value _returnvalue) (`BlueprintMapLibrary.Map_Find` ScenarioProperties _array_element))
      (bind _lefts (`KismetStringLibrary.Split` _array_element "::" "IgnoreCase" "FromEnd"))
      (bind (_value_2 _returnvalue_2) (`BlueprintMapLibrary.Map_Find` ScenarioProperties (`KismetStringLibrary.Concat_StrStr` _lefts "::Volume")))
      (bind (_value_3 _returnvalue_3) (`BlueprintMapLibrary.Map_Find` ScenarioProperties (`KismetStringLibrary.Concat_StrStr` _lefts "::Pitch")))
      (bind (_value_4 _returnvalue_4) (`BlueprintMapLibrary.Map_Find` ScenarioProperties (`KismetStringLibrary.Concat_StrStr` _lefts "::StartTime")))
      (if (and _returnvalue _returnvalue_2 _returnvalue_3 _returnvalue_4)
        (bind (_duration _bsuccess) (`ShidenScenarioManagerInterface.PlaySound2d` ScenarioManager (make `ShidenSoundInfo` (`KismetStringLibrary.Conv_StringToInt` _lefts) "BGM" _value (`KismetStringLibrary.Conv_StringToDouble` _value_2) (`KismetStringLibrary.Conv_StringToDouble` _value_3) (`KismetStringLibrary.Conv_StringToDouble` _value_4))))
        (if (not _bsuccess)
          (return "Error" "Play Sound 2d failed"))
        (else
          (return "Completed" "")))))
  (return "Completed" ""))

(fn `PreviewCommmand`
  (params (Command :type "ShidenCommand Structure (by ref)") (Widget :type "ShidenWidget Object Reference") (ScenarioManager :type "ShidenScenarioManagerInterface Interface (by ref)") (bIsCurrentCommand :type Boolean))
  (returns (Status :type "EShidenPreviewStatus Enum") (ErrorMessage :type String))
  (bind (_commandname _presetname _arg1 _arg2 _arg3 _arg4 _arg5 _arg6 _arg7 _arg8 _arg9 _arg10) (break `ShidenCommand` Command))
  (bind _enumvalue (foreach `EShidenSoundType` false)
    (:`LoopBody`
      (if (`KismetStringLibrary.EqualEqual_StrStr` _arg1 (`|GetEnumeratorNameAsString` _enumvalue))
        (switch `EShidenSoundType` _enumvalue
          (:`None`
            (return "Error" "Invalid SoundType"))
          (:`BGM`
            (bind _shidensoundinfo (make `ShidenSoundInfo` (`KismetStringLibrary.Conv_StringToInt` _arg2) _enumvalue _arg3 (`KismetStringLibrary.Conv_StringToDouble` _arg4) (`KismetStringLibrary.Conv_StringToDouble` _arg5) (`KismetStringLibrary.Conv_StringToDouble` _arg6) (== _arg7 "FadeOut") (`self.ConvertToAudioFaderCurve` _arg8) (`KismetMathLibrary.SelectFloat` (`KismetStringLibrary.Conv_StringToDouble` _arg9) 0.0 bIsCurrentCommand) (== _arg10 "true")))
            (bind (_duration _bsuccess) (`ShidenScenarioManagerInterface.PlaySound2d` ScenarioManager _shidensoundinfo))
            (if _bsuccess
              _
              (else
                (return "Error" "Play Sound Failed"))))
          (:`SE`
            (if bIsCurrentCommand :!label _label
              (bind (_duration_2 _bsuccess_2) (`ShidenScenarioManagerInterface.PlaySound2d` ScenarioManager _shidensoundinfo))
              (if _bsuccess_2
                _
                (else
                  (return "Error" "Play Sound Failed")))
              (else
                (return "Completed" ""))))
          (:`Voice`
            (goto _label)))
        (return "Completed" "")))
    (:`then`
      (return "Error" "Invalid SoundType"))))

(fn `ProcessCommmand`
  (params (ProcessName :type String) (Command :type "ShidenCommand Structure") (Widget :type "ShidenWidget Object Reference") (ScenarioManager :type "ShidenScenarioManagerInterface Interface (by ref)") (DeltaTime :type "Float (single-precision)") (CallerObject :type "Object Object Reference"))
  (returns (Status :type "EShidenProcessStatus Enum") (BreakReason :type String) (NextScenarioName :type String) (ErrorMessage :type String))
  (locals (SoundType :type "EShidenSoundType Enum"))
  (bind (_commandname _presetname _arg1 _arg2 _arg3 _arg4 _arg5 _arg6) (break `ShidenCommand` Command))
  (bind (_commandname_2 _presetname_2 _arg1_2 _arg2_2 _arg3_2 _arg4_2 _arg5_2 _arg6_2 _arg7 _arg8 _arg9 _arg10) (break `ShidenCommand` Command))
  (bind (_commandname_3 _presetname_3 _arg1_3 _arg2_3 _arg3_3 _arg4_3 _arg5_3 _arg6_3 _arg7_2 _arg8_2 _arg9_2 _arg10_2) (break `ShidenCommand` (`local.Command`)))
  (bind _returnvalue (`KismetStringLibrary.Conv_StringToInt` _arg2_2))
  (bind (_enumvalue _success) (`self.ConvertToAudioFaderCurve` _arg8_2))
  (if (or (`KismetStringLibrary.EqualEqual_StrStr` _arg3) (`KismetStringLibrary.IsEmpty` _arg3))
    (switch `string` _arg1
      (:`BGM`
        (`self.RemoveProperties` _commandname_2 _returnvalue)
        (set `local.SoundType` "BGM")
        (bind (_duration _bsuccess) (`ShidenScenarioManagerInterface.PlaySound2d` (`local.ScenarioManager`) (make `ShidenSoundInfo` _returnvalue (`local.SoundType`) _arg3_2 (`KismetStringLibrary.Conv_StringToDouble` _arg4_2) (`KismetStringLibrary.Conv_StringToDouble` _arg5_2) (`KismetStringLibrary.Conv_StringToDouble` _arg6_2) (== _arg7 "FadeOut") (`self.ConvertToAudioFaderCurve` _arg8) (`KismetStringLibrary.Conv_StringToDouble` _arg9) (== _arg10 "true")) :!label _label))
        (if _bsuccess
          _
          (else
            (return "Error" "" "" "Play Sound Failed"))))
      (:`SE`
        _)
      (:`Voice`
        (set `local.SoundType` "Voice")
        (goto _label)))
    (else
      (switch `string` _arg1
        (:`BGM`
          (`self.RegisterProperties` (`.CommandName` (break `ShidenCommand` Command)) (`KismetStringLibrary.Conv_StringToInt` _arg2) _arg3 _arg4 _arg5 _arg6)
          (set `local.SoundType` "BGM"))
        (:`SE`
          (set `local.SoundType` "SE"))
        (:`Voice`
          (set `local.SoundType` "Voice")))
      (if _success
        (bind (_duration_2 _bsuccess_2) (`ShidenScenarioManagerInterface.PlaySound2d` (`local.ScenarioManager`) (make `ShidenSoundInfo` (`KismetStringLibrary.Conv_StringToInt` _arg2_3) (`local.SoundType`) _arg3_3 (`KismetStringLibrary.Conv_StringToDouble` _arg4_3) (`KismetStringLibrary.Conv_StringToDouble` _arg5_3) (`KismetStringLibrary.Conv_StringToDouble` _arg6_3) (== _arg7_2 "FadeOut") _enumvalue (`KismetStringLibrary.Conv_StringToDouble` _arg9_2) (== _arg10_2 "true"))))
        (if _bsuccess_2
          _
          (else
            (return "Error" "" "" "Play Sound Failed")))
        (else
          (return "Error" "" "" (`KismetStringLibrary.Concat_StrStr` "\"" _arg8_2 "\" is Invalid Audio Fader Curve"))))))
  (return "Next" "" "" ""))

(fn `RegisterProperties`
  (params (CommandName :type String) (TrackId :type Integer) (Path :type String) (Volume :type String) (Pitch :type String) (StartTime :type String))
  (bind _returnvalue (`KismetStringLibrary.Conv_IntToString` TrackId))
  (`ShidenCommandFunctionLibrary.RegisterScenarioProperty` CommandName (`KismetStringLibrary.Concat_StrStr` _returnvalue "::Path") Path)
  (`ShidenCommandFunctionLibrary.RegisterScenarioProperty` CommandName (`KismetStringLibrary.Concat_StrStr` _returnvalue "::Volume") Volume)
  (`ShidenCommandFunctionLibrary.RegisterScenarioProperty` CommandName (`KismetStringLibrary.Concat_StrStr` _returnvalue "::Pitch") Pitch)
  (`ShidenCommandFunctionLibrary.RegisterScenarioProperty` CommandName (`KismetStringLibrary.Concat_StrStr` _returnvalue "::StartTime") StartTime))

(fn `RemoveProperties`
  (params (CommandName :type String) (TrackId :type Integer))
  (bind _returnvalue (`KismetStringLibrary.Conv_IntToString` TrackId))
  (`ShidenCommandFunctionLibrary.RemoveScenarioProperty` CommandName (`KismetStringLibrary.Concat_StrStr` _returnvalue "::Path"))
  (`ShidenCommandFunctionLibrary.RemoveScenarioProperty` CommandName (`KismetStringLibrary.Concat_StrStr` _returnvalue "::Volume"))
  (`ShidenCommandFunctionLibrary.RemoveScenarioProperty` CommandName (`KismetStringLibrary.Concat_StrStr` _returnvalue "::Pitch"))
  (`ShidenCommandFunctionLibrary.RemoveScenarioProperty` CommandName (`KismetStringLibrary.Concat_StrStr` _returnvalue "::StartTime")))