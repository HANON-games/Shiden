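; Shiden scenario command for WaitClick, which holds the scenario until the player presses the Next input or skips.
; Each tick it moves on if the command's argument and CanSkipCommand allow skipping and Skip input is active; otherwise it checks Next, delaying until triggered.
; PressNext starts true in pre-processing and tracks the last Next value, so only a fresh press advances, not one already held.
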(fn `PreProcessCommand`
  (params (ProcessName :type String) (Command :type "ShidenCommand Structure") (Widget :type "ShidenWidget Object Reference") (ScenarioManager :type "ShidenScenarioManagerInterface Interface (by ref)") (CallerObject :type "Object Object Reference"))
  (returns (Status :type "EShidenPreProcessStatus Enum") (ErrorMessage :type String))
  (set `self.PressNext` true)
  (return "Complete" ""))

(fn `ProcessCommand`
  (params (ProcessName :type String) (Command :type "ShidenCommand Structure") (Widget :type "ShidenWidget Object Reference") (ScenarioManager :type "ShidenScenarioManagerInterface Interface (by ref)") (DeltaTime :type "Float (single-precision)") (CallerObject :type "Object Object Reference"))
  (returns (Status :type "EShidenProcessStatus Enum") (BreakReason :type String) (NextScenarioName :type String) (ErrorMessage :type String))
  (if (and (`ShidenCommandFunctionLibrary.IsTrue` (`|GetCommandArguments` "/Shiden/Commands/DA_ShidenPrimaryCommandDefinitions.DA_ShidenPrimaryCommandDefinitions" "WaitClick" Command)) (`ShidenScenarioFunctionLibrary.CanSkipCommand`))
    (bind (_bvalue _bresult) (`ShidenScenarioManagerInterface.FindShidenDigitalInput` ScenarioManager "/Shiden/Misc/EnhancedInput/IA_ShidenSkip.IA_ShidenSkip"))
    (if _bresult
      (if (not _bvalue)
        (bind (_bvalue_2 _bresult_2) (`ShidenScenarioManagerInterface.FindShidenDigitalInput` ScenarioManager "/Shiden/Misc/EnhancedInput/IA_ShidenNext.IA_ShidenNext" :!label _label))
        (if _bresult_2
          (if (and (== (`self.PressNext`) false) _bvalue_2)
            _
            (else
              (set `self.PressNext` _bvalue_2)
              (return "DelayUntilNextTick" "" "" "")))
          (else
            (return "DelayUntilNextTick" "" "" ""))))
      (else
        (goto _label)))
    (else
      (goto _label)))
  (return "Next" "" "" ""))