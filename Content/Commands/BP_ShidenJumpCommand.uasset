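; BP_ShidenJumpCommand implements the Shiden scenario Jump command, which moves a process to a named tag within its current scenario.
; It gets the current scenario from the cache and scans its commands from the start for a Tag command whose argument matches the Jump's.
; On a match it sets the scenario index to that command and returns Next; otherwise it returns Error naming the missing tag.
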(fn `Find Next Index`
  (params (ProcessName :type String) (Command :type "ShidenCommand Structure (by ref)"))
  (returns (Success :type Boolean) (`Array Index` :type Integer) (ErrorMessage :type String))
  (bind _destinationtagname (`|GetCommandArguments` "/Shiden/Commands/DA_ShidenPrimaryCommandDefinitions.DA_ShidenPrimaryCommandDefinitions" "Jump" Command))
  (bind _scenarioprogress (`ShidenScenarioFunctionLibrary.PeekScenario` ProcessName))
  (bind _scenario (`ShidenScenarioFunctionLibrary.GetScenarioFromCache` (break `ShidenScenarioProgress` _scenarioprogress)))
  (for (_array_element _array_index) (`ShidenScenario.Commands` _scenario)
    (if (and (`KismetStringLibrary.EqualEqual_StrStr` (`.CommandName` (break `ShidenCommand` _array_element)) "Tag") (`KismetStringLibrary.EqualEqual_StrStr` _destinationtagname (`|GetCommandArguments` "/Shiden/Commands/DA_ShidenPrimaryCommandDefinitions.DA_ShidenPrimaryCommandDefinitions" "Tag" _array_element)))
      (return true _array_index "")))
  (return false 0 (`KismetStringLibrary.Concat_StrStr` "Tag " _destinationtagname " is not found")))

(fn `ProcessCommmand`
  (params (ProcessName :type String) (Command :type "ShidenCommand Structure") (Widget :type "ShidenWidget Object Reference") (ScenarioManager :type "ShidenScenarioManagerInterface Interface (by ref)") (DeltaTime :type "Float (single-precision)") (CallerObject :type "Object Object Reference"))
  (returns (Status :type "EShidenProcessStatus Enum") (BreakReason :type String) (NextScenarioName :type String) (ErrorMessage :type String))
  (bind (_success _array_index _errormessage) (`self.Find Next Index` ProcessName Command))
  (if _success
    (`ShidenScenarioFunctionLibrary.SetCurrentScenarioIndex` ProcessName _array_index)
    (return "Next" "" "" "")
    (else
      (return "Error" "" "" _errormessage))))