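; Shiden scenario command that fades a BGM track's volume to a target level through the ScenarioManager.
; PreProcess parses track, volume, duration and fade curve from the command arguments and starts the fade, erroring on an invalid curve name.
; Process optionally waits out the fade by accumulating DeltaTime, then records the track's volume as a "Sound" scenario property.
; Preview applies the fade instantly unless it is the current command; InitFromSaveData restores nothing.
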(fn `ConvertToAudioFaderCurve`
  (params (AudioFaderCurve :type String))
  (returns (EnumValue :type "EAudioFaderCurve Enum") (Success :type Boolean))
  (switch `string` AudioFaderCurve
    (:`Default`
      (return "Linear" false))
    (:`Linear`
      (return "Linear" true))
    (:`Logarithmic`
      (return "Logarithmic" true))
    (:`Sin (S-Curve)`
      (return "SCurve" true))
    (:`Sin (Equal Power)`
      (return "Sin" true))))

(fn `GetAssetPaths`
  (params (Command :type "ShidenCommand Structure") (CallerObject :type "Object Object Reference"))
  (returns (AssetObjectPaths :type "Set of String"))
  (return))

(fn `InitFromSaveData`
  (params (ScenarioProperties :type "Map of String to String (by ref)") (Widget :type "ShidenWidget Object Reference") (ScenarioManager :type "ShidenScenarioManagerInterface Interface (by ref)") (CallerObject :type "Object Object Reference"))
  (returns (Status :type "EShidenInitFromSaveDataStatus Enum") (ErrorMessage :type String))
  (return "Completed" ""))

(fn `PreProcessCommmand`
  (params (ProcessName :type String) (Command :type "ShidenCommand Structure") (Widget :type "ShidenWidget Object Reference") (ScenarioManager :type "ShidenScenarioManagerInterface Interface (by ref)") (CallerObject :type "Object Object Reference"))
  (returns (Status :type "EShidenPreProcessStatus Enum") (ErrorMessage :type String))
  (bind (_trackid _volume _fadefunction _fadeduration) (`|GetCommandArguments` "/Shiden/Commands/DA_ShidenPrimaryCommandDefinitions.DA_ShidenPrimaryCommandDefinitions" "AdjustBgmVolume" Command))
  (bind (_enumvalue _success) (`self.ConvertToAudioFaderCurve` _fadefunction))
  (set `self.ElaspedTime` 0.0)
  (if _success
    (bind _bsuccess (`ShidenScenarioManagerInterface.AdjustBgmVolume` ScenarioManager (`KismetStringLibrary.Conv_StringToInt` _trackid) (`KismetStringLibrary.Conv_StringToDouble` _fadeduration) (`KismetStringLibrary.Conv_StringToDouble` _volume) _enumvalue))
    (if _bsuccess
      (return "Completed" "")
      (else
        (return "Error" "Adjust BGM volume failed.")))
    (else
      (return "Error" "Fade function is invalid."))))

(fn `PreviewCommmand`
  (params (Command :type "ShidenCommand Structure (by ref)") (Widget :type "ShidenWidget Object Reference") (ScenarioManager :type "ShidenScenarioManagerInterface Interface (by ref)") (bIsCurrentCommand :type Boolean))
  (returns (Status :type "EShidenPreviewStatus Enum") (ErrorMessage :type String))
  (bind (_trackid _volume _fadefunction _fadeduration) (`|GetCommandArguments` "/Shiden/Commands/DA_ShidenPrimaryCommandDefinitions.DA_ShidenPrimaryCommandDefinitions" "AdjustBgmVolume" Command))
  (bind (_enumvalue _success) (`self.ConvertToAudioFaderCurve` _fadefunction))
  (if _success
    (bind _bsuccess (`ShidenScenarioManagerInterface.AdjustBgmVolume` ScenarioManager (`KismetStringLibrary.Conv_StringToInt` _trackid) (`KismetMathLibrary.SelectFloat` (`KismetStringLibrary.Conv_StringToDouble` _fadeduration) 0.0 bIsCurrentCommand) (`KismetStringLibrary.Conv_StringToDouble` _volume) _enumvalue))
    (if _bsuccess
      (return "Completed" "")
      (else
        (return "Error" "Adjust BGM volume failed.")))
    (else
      (return "Error" "Fade function is invalid."))))

(fn `ProcessCommmand`
  (params (ProcessName :type String) (Command :type "ShidenCommand Structure") (Widget :type "ShidenWidget Object Reference") (ScenarioManager :type "ShidenScenarioManagerInterface Interface (by ref)") (DeltaTime :type "Float (single-precision)") (CallerObject :type "Object Object Reference"))
  (returns (Status :type "EShidenProcessStatus Enum") (BreakReason :type String) (NextScenarioName :type String) (ErrorMessage :type String))
  (bind (_trackid _volume _fadefunction _fadeduration _waitforcompletion) (`|GetCommandArguments` "/Shiden/Commands/DA_ShidenPrimaryCommandDefinitions.DA_ShidenPrimaryCommandDefinitions" "AdjustBgmVolume" Command))
  (if (== _waitforcompletion "true")
    (bind _output_get (set `self.ElaspedTime` (+ DeltaTime (`self.ElaspedTime`))))
    (if (> _output_get _fadeduration)
      _
      (else
        (return "DelayUntilNextTick" "" "" ""))))
  (`ShidenCommandFunctionLibrary.RegisterScenarioProperty` "Sound" (`KismetStringLibrary.Concat_StrStr` (`KismetStringLibrary.Conv_IntToString` (`KismetStringLibrary.Conv_StringToInt` _trackid)) "::Volume") _volume)
  (return "Next" "" "" ""))