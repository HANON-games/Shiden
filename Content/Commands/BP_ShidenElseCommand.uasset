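; Shiden scenario command for Else, which moves the running process to an End if command and returns Next.
; FindEndifIndex scans the cached scenario's commands from the current index and sets the process index at the first End if.
; On encountering an If, it calls itself recursively, intending to step over nested blocks.
; A failed search returns an Error status with its message.
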(fn `FindEndifIndex`
  (params (ProcessName :type String) (ScenarioManager :type "ShidenScenarioManagerInterface Interface"))
  (returns (Success :type Boolean) (ErrorMessage :type String))
  (locals (TargetCommandNames :type "Array of String"))
  (bind _scenarioprogress (`ShidenScenarioFunctionLibrary.PeekScenario` ProcessName))
  (bind _scenario (`ShidenScenarioFunctionLibrary.GetScenarioFromCache` (break `ShidenScenarioProgress` _scenarioprogress)))
  (bind _commands (`ShidenScenario.Commands` _scenario))
  (for _index (range (`.CurrentIndex` (break `ShidenScenarioProgress` _scenarioprogress)) (`KismetArrayLibrary.Array_Length` _commands))
    (switch `string` (`.CommandName` (break `ShidenCommand` (`|GetArrayItem` _commands _index)))
      (:`EndIf`
        (`ShidenScenarioFunctionLibrary.SetCurrentScenarioIndex` (`local.ProcessName`) _index)
        (return true ""))
      (:`If`
        (bind (_success _errormessage) (`self.FindEndifIndex` (`local.ProcessName`) (`local.ScenarioManager`))) ; Change Index to EndIf
        (if _success
          (bind (_success_2 _errormessage_2) (`self.FindEndifIndex` (`local.ProcessName`) (`local.ScenarioManager`)))
          (return _success_2 _errormessage_2)
          (else
            (return false _errormessage))))))
  (return false "Not Found EndIf"))

(fn `ProcessCommmand`
  (params (ProcessName :type String) (Command :type "ShidenCommand Structure") (Widget :type "ShidenWidget Object Reference") (ScenarioManager :type "ShidenScenarioManagerInterface Interface (by ref)") (DeltaTime :type "Float (single-precision)") (HookedObject :type "Object Object Reference"))
  (returns (Status :type "EShidenProcessStatus Enum") (BreakReason :type String) (NextScenarioName :type String) (ErrorMessage :type String))
  (bind (_success _errormessage) (`self.FindEndifIndex` ProcessName ScenarioManager))
  (if _success
    (return "Next" "" "" "")
    (else
      (return "Error" "" "" _errormessage))))