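; Shiden scenario command for Loop While, which gates a loop body in a scenario on a variable comparison.
; ProcessCommand reads the command arguments, then CheckCondition type-checks the variable and evaluates it against the right-hand value.
; When false, FindEndLoopWhileIndex moves the scenario index to the matching End Loop While, recursing past nested loops.
; Invalid arguments, missing variables, type mismatches or a missing end marker return errors.
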(fn `CheckCondition`
  (params (ProcessName :type String) (Kind :type "EShidenVariableKind Enum" :default "UserVariable") (Type :type "EShidenVariableType Enum" :default "Boolean") (Key :type String) (Operator :type String) (Value :type String))
  (returns (Success :type Boolean) (ErrorMessage :type String))
  (bind (_variabletype _bbooleanvalue _stringvalue _integervalue _floatvalue _vector2value _vector3value _breturnvalue) (`ShidenVariableFunctionLibrary.FindVariable` ProcessName Kind Key))
  (if _breturnvalue
    (if (`|EnumEquality` _variabletype Type)
      (bind (_bresult _bsuccess _errormessage) (`ShidenVariableFunctionLibrary.EvaluateCondition` Type Operator _bbooleanvalue _stringvalue _integervalue _floatvalue _vector2value _vector3value (== Value "true") Value (`KismetStringLibrary.Conv_StringToInt` Value) (`KismetStringLibrary.Conv_StringToDouble` Value) (`KismetStringLibrary.Conv_StringToVector2D` Value) (`KismetStringLibrary.Conv_StringToVector` Value)))
      (if _bsuccess
        (if _bresult
          (return true "")
          (else
            (`ShidenScenarioFunctionLibrary.ToNext` (`local.ProcessName`))
            (bind (_success _errormessage_2) (`self.FindEndLoopWhileIndex` (`local.ProcessName`)))
            (if _success
              (return true "")
              (else
                (return false _errormessage_2)))))
        (else
          (return false _errormessage)))
      (else
        (return false "Variable type not match")))
    (else
      (return false "Variable not found"))))

(fn `FindEndLoopWhileIndex`
  (params (ProcessName :type String))
  (returns (Success :type Boolean) (ErrorMessage :type String))
  (locals (TargetCommandNames :type "Array of String"))
  (bind _scenarioprogress (`ShidenScenarioFunctionLibrary.PeekScenario` ProcessName))
  (bind _scenario (`ShidenScenarioFunctionLibrary.GetScenarioFromCache` (break `ShidenScenarioProgress` _scenarioprogress)))
  (bind _commands (`ShidenScenario.Commands` _scenario))
  (for _index (range (`.CurrentIndex` (break `ShidenScenarioProgress` _scenarioprogress)) (`KismetArrayLibrary.Array_Length` _commands))
    (switch `string` (`.CommandName` (break `ShidenCommand` (`|GetArrayItem` _commands _index)))
      (:`EndLoopWhile`
        (`ShidenScenarioFunctionLibrary.SetCurrentScenarioIndex` (`local.ProcessName`) _index)
        (return true ""))
      (:`LoopWhile`
        (`ShidenScenarioFunctionLibrary.ToNext` (`local.ProcessName`))
        (bind (_success _errormessage) (`self.FindEndLoopWhileIndex` (`local.ProcessName`))) ; Change Index to EndLoopWhile
        (if _success
          (`ShidenScenarioFunctionLibrary.ToNext` (`local.ProcessName`))
          (bind (_success_2 _errormessage_2) (`self.FindEndLoopWhileIndex` (`local.ProcessName`)))
          (return _success_2 _errormessage_2)
          (else
            (return false _errormessage))))))
  (return false "Not Found EndIf"))

(fn `ProcessCommand`
  (params (ProcessName :type String) (Command :type "ShidenCommand Structure") (Widget :type "ShidenWidget Object Reference") (ScenarioManager :type "ShidenScenarioManagerInterface Interface (by ref)") (DeltaTime :type "Float (single-precision)") (CallerObject :type "Object Object Reference"))
  (returns (Status :type "EShidenProcessStatus Enum") (BreakReason :type String) (NextScenarioName :type String) (ErrorMessage :type String))
  (bind (_variablekind _variabletype _variablename _operator _righthandvalue) (`|GetCommandArguments` "/Shiden/Commands/DA_ShidenPrimaryCommandDefinitions.DA_ShidenPrimaryCommandDefinitions" "LoopWhile" Command))
  (bind (_variablekind_2 _variabletype_2) (`|GetCommandArguments` "/Shiden/Commands/DA_ShidenPrimaryCommandDefinitions.DA_ShidenPrimaryCommandDefinitions" "LoopWhile" Command))
  (bind (_result _bsuccess) (`ShidenVariableFunctionLibrary.ConvertToVariableType` _variabletype_2))
  (bind (_result_2 _bsuccess_2) (`ShidenVariableFunctionLibrary.ConvertToVariableKind` _variablekind_2))
  (if _bsuccess_2
    (if _bsuccess
      (bind (_success _errormessage) (`self.CheckCondition` ProcessName _result_2 _result _variablename _operator _righthandvalue))
      (if _success
        (return "Next" "" "" "")
        (else
          (return "Error" "" "" _errormessage)))
      (else
        (return "Error" "" "" "Invalid variable type")))
    (else
      (return "Error" "" "" "Invalid variable kind"))))