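; Shiden scenario command that starts a macro scenario as a named parallel process.
; ProcessCommmand rejects "Default" or already running process names, finds the macro by ID or object path, pushes it and calls CallMacroAsParallel, returning Next immediately.
; SetMacroArguments stores up to five typed arguments as process locals, using defaults for empty values and stopping at the first unnamed one.
; GetAssetPaths is empty; a note says the scenario manager loads macro assets.
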(fn `GetAssetPaths`
  (params (Command :type "ShidenCommand Structure") (CallerObject :type "Object Object Reference"))
  (returns (AssetObjectPaths :type "Set of String"))
  (return))

(fn `ProcessCommmand`
  (params (ProcessName :type String) (Command :type "ShidenCommand Structure") (Widget :type "ShidenWidget Object Reference") (ScenarioManager :type "ShidenScenarioManagerInterface Interface (by ref)") (DeltaTime :type "Float (single-precision)") (CallerObject :type "Object Object Reference"))
  (returns (Status :type "EShidenProcessStatus Enum") (BreakReason :type String) (NextScenarioName :type String) (ErrorMessage :type String))
  (bind (_commandname _presetname _arg1) (break `ShidenCommand` Command))
  (bind (_commandname_2 _presetname_2 _arg1_2 _arg2 _arg3 _arg4 _arg5 _arg6 _arg7) (break `ShidenCommand` Command))
  (bind (_commandname_3 _presetname_3 _arg1_3 _arg2_2) (break `ShidenCommand` Command))
  (if (`KismetStringLibrary.NotEqual_StrStr` _arg1 "Default")
    (bind (_scenarioprogress _cancelinfo _bislastelement _bismacro _bsuccess) (`ShidenScenarioFunctionLibrary.PeekScenario` _arg1))
    (if _bsuccess
      (return "Error" "" "" (`KismetStringLibrary.Concat_StrStr` "Process \"" _arg1 "\" is already running"))
      (else
        (bind (_scenarioid _scenario _bsuccess_2) (`ShidenScenarioFunctionLibrary.GetScenarioByIdOrObjectPath` _arg2_2))
        (if _bsuccess_2
          (`ShidenScenarioFunctionLibrary.PushScenario` _arg1_2 _scenario)
          (`self.SetMacroArguments` _arg1_2 (`local.ScenarioManager`) _scenario _arg3 _arg4 _arg5 _arg6 _arg7)
          (`ShidenScenarioManagerInterface.CallMacroAsParallel` (`local.ScenarioManager`) _arg1_2 CallerObject)
          (return "Next" "" "" "")
          (else
            (return "Error" "" "" (`KismetStringLibrary.Concat_StrStr` "Macro \"" _arg2_2 "\" is not found."))))))
    (else
      (return "Error" "" "" "Cannot use \"Default\" as parallel process name"))))

(fn `SetMacroArguments`
  (params (ProcessName :type String) (ScenarioManager :type "ShidenScenarioManagerInterface Interface") (ShidenScenario :type "ShidenScenario Object Reference") (Arg1Value :type String) (Arg2Value :type String) (Arg3Value :type String) (Arg4Value :type String) (Arg5Value :type String))
  (bind _processname (`local.ProcessName`))
  (for _index (range 5)
    (bind _returnvalue (select `int` _index :`0` (`ShidenScenario.Arg1Name` ShidenScenario) :`1` (`ShidenScenario.Arg2Name` ShidenScenario) :`2` (`ShidenScenario.Arg3Name` ShidenScenario) :`3` (`ShidenScenario.Arg4Name` ShidenScenario) :`4` (`ShidenScenario.Arg5Name` ShidenScenario)))
    (if (not (`KismetStringLibrary.IsEmpty` _returnvalue))
      (switch `EShidenVariableType` (select `int` _index :`0` (`ShidenScenario.Arg1Type` ShidenScenario) :`1` (`ShidenScenario.Arg2Type` ShidenScenario) :`2` (`ShidenScenario.Arg3Type` ShidenScenario) :`3` (`ShidenScenario.Arg4Type` ShidenScenario) :`4` (`ShidenScenario.Arg5Type` ShidenScenario))
        (:`Boolean`
          (bind _returnvalue_2 (select `int` _index :`0` Arg1Value :`1` Arg2Value :`2` Arg3Value :`3` Arg4Value :`4` Arg5Value))
          (bind _returnvalue_3 (`KismetMathLibrary.SelectString` (select `int` _index :`0` (`ShidenScenario.Arg1DefaultValue` ShidenScenario) :`1` (`ShidenScenario.Arg2DefaultValue` ShidenScenario) :`2` (`ShidenScenario.Arg3DefaultValue` ShidenScenario) :`3` (`ShidenScenario.Arg4DefaultValue` ShidenScenario) :`4` (`ShidenScenario.Arg5DefaultValue` ShidenScenario)) _returnvalue_2 (`KismetStringLibrary.IsEmpty` _returnvalue_2)))
          (`ShidenVariableFunctionLibrary.AddLocalBoolean` _processname _returnvalue (== _returnvalue_3 "true")))
        (:`String`
          (`ShidenVariableFunctionLibrary.AddLocalString` _processname _returnvalue _returnvalue_3))
        (:`Integer`
          (`ShidenVariableFunctionLibrary.AddLocalInteger` _processname _returnvalue (`KismetStringLibrary.Conv_StringToInt` _returnvalue_3)))
        (:`Float`
          (`ShidenVariableFunctionLibrary.AddLocalFloat` _processname _returnvalue (`KismetStringLibrary.Conv_StringToDouble` _returnvalue_3)))
        (:`Vector2`
          (`ShidenVariableFunctionLibrary.AddLocalVector2` _processname _returnvalue (`KismetStringLibrary.Conv_StringToVector2D` _returnvalue_3)))
        (:`Vector3`
          (`ShidenVariableFunctionLibrary.AddLocalVector3` _processname _returnvalue (`KismetStringLibrary.Conv_StringToVector` _returnvalue_3))))
      (else
        (break))))
  (return))