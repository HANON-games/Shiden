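; Shiden scenario command that shows, changes or hides an image in a named slot of the Shiden widget with an eased fade.
; PreProcess and Preview load the slate brush and call ShowImage, which applies optional position and size overrides and starts the fade; an empty path fades to transparent.
; ProcessCommand optionally waits for the fade, then records path and color as scenario properties, which RestoreFromSaveData uses to rebuild slots from saves.
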(fn `ConvertToEasingFunc`
  (params (EasingFunc :type String))
  (returns (EnumValue :type "EEasingFunc Enum") (Success :type Boolean))
  (switch `string` EasingFunc
    (:`Default`
      (return "Linear" false))
    (:`Linear`
      (return "Linear" true))
    (:`Step`
      (return "Step" true))
    (:`Sinusoidal in`
      (return "SinusoidalIn" true))
    (:`Sinusoidal out`
      (return "SinusoidalOut" true))
    (:`Sinusoidal in out`
      (return "SinusoidalInOut" true))
    (:`Ease in`
      (return "EaseIn" true))
    (:`Ease out`
      (return "EaseOut" true))
    (:`Ease in out`
      (return "EaseInOut" true))
    (:`Expo in`
      (return "ExpoIn" true))
    (:`Expo out`
      (return "ExpoOut" true))
    (:`Expo in out`
      (return "ExpoInOut" true))
    (:`Circular in`
      (return "CircularIn" true))
    (:`Circular out`
      (return "CircularOut" true))
    (:`Circular in out`
      (return "CircularInOut" true))))

(fn `IsImagePathEmpty`
  (params (Command :type "ShidenCommand Structure (by ref)"))
  (returns (IsEmpty :type Boolean))
  (bind (_slotname _image) (`|GetCommandArguments` "/Shiden/Commands/DA_ShidenPrimaryCommandDefinitions.DA_ShidenPrimaryCommandDefinitions" "Image" Command))
  (return (or (`KismetStringLibrary.EqualEqual_StrStr` _image) (`KismetStringLibrary.IsEmpty` _image))))

(fn `PreProcessCommand`
  (params (ProcessName :type String) (Command :type "ShidenCommand Structure") (Widget :type "ShidenWidget Object Reference") (ScenarioManager :type "ShidenScenarioManagerInterface Interface (by ref)") (CallerObject :type "Object Object Reference"))
  (returns (Status :type "EShidenPreProcessStatus Enum") (ErrorMessage :type String))
  (bind (_slotname _image) (`|GetCommandArguments` "/Shiden/Commands/DA_ShidenPrimaryCommandDefinitions.DA_ShidenPrimaryCommandDefinitions" "Image" Command))
  (bind (_asset _bsuccess) (`ShidenCoreFunctionLibrary.GetOrLoadAsset` _image))
  (if (`self.IsImagePathEmpty` Command)
    _
    (elif _bsuccess
      (bind _asslate_brush_asset (cast `SlateBrushAsset` _asset)
        (:`then`
          _)
        (:`CastFailed`
          (return "Error" "Cast failed")))
      (else
        (return "Error" (`KismetStringLibrary.Concat_StrStr` "Asset " _image " is not found")))))
  (bind (_success _errormessage) (`self.ShowImage` Command Widget _asslate_brush_asset true ProcessName))
  (if _success
    (return "Complete" "")
    (else
      (return "Error" _errormessage))))

(fn `PreviewCommand`
  (params (Command :type "ShidenCommand Structure (by ref)") (Widget :type "ShidenWidget Object Reference") (ScenarioManager :type "ShidenScenarioManagerInterface Interface (by ref)") (bIsCurrentCommand :type Boolean))
  (returns (Status :type "EShidenPreviewStatus Enum") (ErrorMessage :type String))
  (bind (_asset _bsuccess) (`ShidenCoreFunctionLibrary.GetOrLoadAsset` (`.Image` (`|GetCommandArguments` "/Shiden/Commands/DA_ShidenPrimaryCommandDefinitions.DA_ShidenPrimaryCommandDefinitions" "Image" Command))))
  (if (`self.IsImagePathEmpty` Command)
    _
    (elif _bsuccess
      (bind _asslate_brush_asset (cast `SlateBrushAsset` _asset)
        (:`then`
          _)
        (:`CastFailed`
          (return "Error" "Cast Failed")))
      (else
        (return "Error" "Asset not found"))))
  (bind (_success _errormessage) (`self.ShowImage` Command Widget _asslate_brush_asset bIsCurrentCommand "Default"))
  (if _success
    (return "Complete" "")
    (else
      (return "Error" _errormessage))))

(fn `ProcessCommand`
  (params (ProcessName :type String) (Command :type "ShidenCommand Structure") (Widget :type "ShidenWidget Object Reference") (ScenarioManager :type "ShidenScenarioManagerInterface Interface (by ref)") (DeltaTime :type "Float (single-precision)") (CallerObject :type "Object Object Reference"))
  (returns (Status :type "EShidenProcessStatus Enum") (BreakReason :type String) (NextScenarioName :type String) (ErrorMessage :type String))
  (bind (_commandid _benabled _commandname) (break `ShidenCommand` Command))
  (bind (_returnvalue_r _returnvalue_g _returnvalue_b) (break `LinearColor` (`KismetMathLibrary.LinearColor_White`)))
  (bind (_slotname _image) (`|GetCommandArguments` "/Shiden/Commands/DA_ShidenPrimaryCommandDefinitions.DA_ShidenPrimaryCommandDefinitions" "Image" Command))
  (if (== (`.WaitForCompletion` (`|GetCommandArguments` "/Shiden/Commands/DA_ShidenPrimaryCommandDefinitions.DA_ShidenPrimaryCommandDefinitions" "Image" Command)) "true")
    (if (`ShidenWidget.IsImageFadeCompleted` Widget (`|GetCommandArguments` "/Shiden/Commands/DA_ShidenPrimaryCommandDefinitions.DA_ShidenPrimaryCommandDefinitions" "Image" Command))
      _
      (else
        (return "DelayUntilNextTick" "" "" ""))))
  (if (`self.IsImagePathEmpty` Command)
    (`Image.SetBrush` (`ShidenWidget.FindImage` Widget _slotname) (`WidgetBlueprintLibrary.NoResourceBrush`)))
  (`ShidenCommandFunctionLibrary.RegisterScenarioProperty` _commandname (`KismetStringLibrary.Concat_StrStr` _slotname "::Path") _image)
  (`ShidenCommandFunctionLibrary.RegisterScenarioProperty` _commandname (`KismetStringLibrary.Concat_StrStr` _slotname "::Color") (`KismetStringLibrary.Conv_ColorToString` (`KismetMathLibrary.MakeColor` _returnvalue_r _returnvalue_g _returnvalue_b (`KismetMathLibrary.SelectFloat` 0.0 1.0 (`self.IsImagePathEmpty` Command)))))
  (return "Next" "" "" ""))

(fn `RestoreFromSaveData`
  (params (ScenarioProperties :type "Map of String to String (by ref)") (Widget :type "ShidenWidget Object Reference") (ScenarioManager :type "ShidenScenarioManagerInterface Interface (by ref)") (CallerObject :type "Object Object Reference"))
  (returns (Status :type "EShidenInitFromSaveDataStatus Enum") (ErrorMessage :type String))
  (bind _keys (`BlueprintMapLibrary.Map_Keys` ScenarioProperties))
  (for _array_element _keys
    (bind (_lefts _rights) (`KismetStringLibrary.Split` _array_element "::" "IgnoreCase" "FromEnd"))
    (if (not (`KismetStringLibrary.IsEmpty` _lefts))
      (bind (_image _bresult) (`ShidenWidget.FindImage` Widget _lefts))
      (if _bresult
        (switch `string` _rights
          (:`Default`
            (return "Error" (`KismetStringLibrary.Concat_StrStr` "Key \"" _array_element "\" is invalid")))
          (:`Path`
            (bind _value (`BlueprintMapLibrary.Map_Find` ScenarioProperties _array_element))
            (if (not (or (`KismetStringLibrary.IsEmpty` _value) (`KismetStringLibrary.EqualEqual_StrStr` _value)))
              (bind (_asset _bsuccess) (`ShidenCoreFunctionLibrary.GetOrLoadAsset` _value))
              (if _bsuccess
                (bind _asslate_brush_asset (cast `SlateBrushAsset` _asset)
                  (:`then`
                    (`Image.SetBrushFromAsset` _image _asslate_brush_asset))
                  (:`CastFailed`
                    (return "Error" (`KismetStringLibrary.Concat_StrStr` "Asset \"" _value "\" is not SlateBrushAsset"))))
                (else
                  (return "Error" (`KismetStringLibrary.Concat_StrStr` "Asset \"" _value "\" is not found"))))))
          (:`Color`
            (bind (_outconvertedcolor _outisvalid) (`KismetStringLibrary.Conv_StringToColor` _value))
            (if _outisvalid
              (`Image.SetColorAndOpacity` _image _outconvertedcolor)
              (else
                (return "Error" (`KismetStringLibrary.Concat_StrStr` "Value \"" _value "\" is invalid")))))
          (:`Position`
            (bind (_outconvertedvector2d _outisvalid_2) (`KismetStringLibrary.Conv_StringToVector2D` _value))
            (if _outisvalid_2
              (`CanvasPanelSlot.SetPosition` (`WidgetLayoutLibrary.SlotAsCanvasSlot` _image) _outconvertedvector2d)
              (else
                (return "Error" (`KismetStringLibrary.Concat_StrStr` "Value \"" _value "\" is invalid")))))
          (:`Size`
            (bind (_outconvertedvector2d_2 _outisvalid_3) (`KismetStringLibrary.Conv_StringToVector2D` _value))
            (if _outisvalid_3
              (`CanvasPanelSlot.SetSize` (`WidgetLayoutLibrary.SlotAsCanvasSlot` _image) _outconvertedvector2d_2)
              (else
                (return "Error" (`KismetStringLibrary.Concat_StrStr` "Value \"" _value "\" is invalid")))))
          (:`SizeToContent`
            (if (== _value "true")
              (bind _returnvalue (`WidgetLayoutLibrary.SlotAsCanvasSlot` _image))
              (set `CanvasPanelSlot.bAutoSize` true _returnvalue)
              (else
                (set `CanvasPanelSlot.bAutoSize` false _returnvalue)))))
        (else
          (return "Error" (`KismetStringLibrary.Concat_StrStr` "Image \"" _lefts "\" is not found"))))
      (else
        (return "Error" (`KismetStringLibrary.Concat_StrStr` "Key \"" _array_element "\" is invalid")))))
  (return "Complete" ""))

(fn `ShowImage`
  (params (Command :type "ShidenCommand Structure") (Widget :type "ShidenWidget Object Reference") (SlateBrushAsset :type "SlateBrushAsset Object Reference") (Animate :type Boolean) (OwnerProcessName :type String))
  (returns (Success :type Boolean) (ErrorMessage :type String))
  (locals (ImageSlotName :type String))
  (bind (_slotname _image _overwriteposition _overwritesize _overwritesizetocontent _fadefunction) (`|GetCommandArguments` "/Shiden/Commands/DA_ShidenPrimaryCommandDefinitions.DA_ShidenPrimaryCommandDefinitions" "Image" (`local.Command`)))
  (bind (_slotname_2 _image_2 _overwriteposition_2) (`|GetCommandArguments` "/Shiden/Commands/DA_ShidenPrimaryCommandDefinitions.DA_ShidenPrimaryCommandDefinitions" "Image" (`local.Command`)))
  (bind (_slotname_3 _image_3 _overwriteposition_3 _overwritesize_2) (`|GetCommandArguments` "/Shiden/Commands/DA_ShidenPrimaryCommandDefinitions.DA_ShidenPrimaryCommandDefinitions" "Image" (`local.Command`)))
  (bind (_slotname_4 _image_4 _overwriteposition_4 _overwritesize_3 _overwritesizetocontent_2) (`|GetCommandArguments` "/Shiden/Commands/DA_ShidenPrimaryCommandDefinitions.DA_ShidenPrimaryCommandDefinitions" "Image" (`local.Command`)))
  (bind (_slotname_5 _image_5 _overwriteposition_5 _overwritesize_4 _overwritesizetocontent_3 _fadefunction_2 _fadeduration _steps _blendexp) (`|GetCommandArguments` "/Shiden/Commands/DA_ShidenPrimaryCommandDefinitions.DA_ShidenPrimaryCommandDefinitions" "Image" (`local.Command`)))
  (bind (_enumvalue _success) (`self.ConvertToEasingFunc` _fadefunction))
  (bind _returnvalue (`KismetStringLibrary.Conv_StringToInt` _steps))
  (bind _returnvalue_2 (`KismetStringLibrary.Conv_StringToDouble` _blendexp))
  (bind _returnvalue_3 (`KismetMathLibrary.SelectFloat` (`KismetStringLibrary.Conv_StringToDouble` (`.FadeDuration` (`|GetCommandArguments` "/Shiden/Commands/DA_ShidenPrimaryCommandDefinitions.DA_ShidenPrimaryCommandDefinitions" "Image" (`local.Command`)))) 0.0 (`local.Animate`)))
  (bind _output_get (set `local.ImageSlotName` (`|GetCommandArguments` "/Shiden/Commands/DA_ShidenPrimaryCommandDefinitions.DA_ShidenPrimaryCommandDefinitions" "Image" Command)))
  (bind (_image_6 _bresult) (`ShidenWidget.FindImage` Widget _output_get))
  (if _bresult
    (if (not (`self.IsImagePathEmpty` (`local.Command`)))
      (if (not (`KismetStringLibrary.IsEmpty` _overwriteposition_2))
        (bind _returnvalue_4 (`WidgetLayoutLibrary.SlotAsCanvasSlot` _image_6))
        (`CanvasPanelSlot.SetPosition` _returnvalue_4 (`KismetStringLibrary.Conv_StringToVector2D` _overwriteposition_2))
        (`ShidenCommandFunctionLibrary.RegisterScenarioProperty` (`.CommandName` (break `ShidenCommand` (`local.Command`))) (`KismetStringLibrary.Concat_StrStr` (`local.ImageSlotName`) "::Position") _overwriteposition_2))
      (if (not (`KismetStringLibrary.IsEmpty` _overwritesize_2))
        (`CanvasPanelSlot.SetSize` _returnvalue_4 (`KismetStringLibrary.Conv_StringToVector2D` _overwritesize_2))
        (`ShidenCommandFunctionLibrary.RegisterScenarioProperty` (`.CommandName` (break `ShidenCommand` (`local.Command`))) (`KismetStringLibrary.Concat_StrStr` (`local.ImageSlotName`) "::Size") _overwritesize_2))
      (if (not (`KismetStringLibrary.IsEmpty` _overwritesizetocontent_2))
        (set `CanvasPanelSlot.bAutoSize` (== _overwritesizetocontent_2 "true") _returnvalue_4)
        (`ShidenCommandFunctionLibrary.RegisterScenarioProperty` (`.CommandName` (break `ShidenCommand` (`local.Command`))) (`KismetStringLibrary.Concat_StrStr` (`local.ImageSlotName`) "::SizeToContent") _overwritesizetocontent_2)))
    (if _success
      (if (or (`KismetStringLibrary.EqualEqual_StrStr` _image) (`KismetStringLibrary.IsEmpty` _image))
        (bind (_success_2 _errormessage) (`ShidenWidget.StartImageFade` (`local.Widget`) (`local.ImageSlotName`) _image_6 _enumvalue _returnvalue_3 true true _returnvalue_2 _returnvalue (`local.OwnerProcessName`)))
        (return _success_2 _errormessage)
        (else
          (`Image.SetBrushFromAsset` _image_6 (`local.SlateBrushAsset`))
          (bind (_success_3 _errormessage_2) (`ShidenWidget.StartImageFade` (`local.Widget`) (`local.ImageSlotName`) _image_6 _enumvalue _returnvalue_3 true false _returnvalue_2 _returnvalue (`local.OwnerProcessName`)))
          (return _success_3 _errormessage_2)))
      (else
        (return false (`KismetStringLibrary.Concat_StrStr` "Easing func \"" _fadefunction "\" is invalid"))))
    (else
      (return false (`KismetStringLibrary.Concat_StrStr` "Image slot \"" (`local.ImageSlotName`) "\" is not found")))))