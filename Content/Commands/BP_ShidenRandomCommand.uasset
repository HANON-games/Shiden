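; Shiden scenario command "Random" that stores a random number in a scenario variable.
; SetRandomValue reads the kind, type, name and min/max arguments from the primary command definitions, then adds an Integer or Float variable with a value in that range.
; ProcessCommmand writes under the running process and moves to Next, while PreviewCommmand writes under "Default" and completes.
; An invalid kind, unsupported type or failed add returns an error.
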(fn `PreviewCommmand`
  (params (Command :type "ShidenCommand Structure (by ref)") (Widget :type "ShidenWidget Object Reference") (ScenarioManager :type "ShidenScenarioManagerInterface Interface (by ref)") (bIsCurrentCommand :type Boolean))
  (returns (Status :type "EShidenPreviewStatus Enum") (ErrorMessage :type String))
  (bind (_success _errormessage) (`self.SetRandomValue` "Default" Command))
  (if _success
    (return "Completed" "")
    (else
      (return "Error" _errormessage))))

(fn `ProcessCommmand`
  (params (ProcessName :type String) (Command :type "ShidenCommand Structure") (Widget :type "ShidenWidget Object Reference") (ScenarioManager :type "ShidenScenarioManagerInterface Interface (by ref)") (DeltaTime :type "Float (single-precision)") (CallerObject :type "Object Object Reference"))
  (returns (Status :type "EShidenProcessStatus Enum") (BreakReason :type String) (NextScenarioName :type String) (ErrorMessage :type String))
  (bind (_success _errormessage) (`self.SetRandomValue` ProcessName Command))
  (if _success
    (return "Next" "" "" "")
    (else
      (return "Error" "" "" _errormessage))))

(fn `SetRandomValue`
  (params (ProcessName :type String) (Command :type "ShidenCommand Structure (by ref)"))
  (returns (Success :type Boolean) (ErrorMessage :type String))
  (bind (_variablekind _variabletype _destinationvariablename _min _max) (`|GetCommandArguments` "/Shiden/Commands/DA_ShidenPrimaryCommandDefinitions.DA_ShidenPrimaryCommandDefinitions" "Random" Command))
  (bind (_result _bsuccess) (`ShidenVariableFunctionLibrary.ConvertToVariableKind` _variablekind))
  (if _bsuccess
    (switch `string` _variabletype
      (:`Default`
        (return false "Invalid number type"))
      (:`Integer`
        (bind (_bsuccess_2 _errormessage) (`ShidenVariableFunctionLibrary.AddVariable` ProcessName _result "Integer" _destinationvariablename false "" (`KismetMathLibrary.RandomIntegerInRange` (`KismetStringLibrary.Conv_StringToInt` _min) (`KismetStringLibrary.Conv_StringToInt` _max))))
        (return _bsuccess_2 _errormessage))
      (:`Float`
        (bind (_bsuccess_3 _errormessage_2) (`ShidenVariableFunctionLibrary.AddVariable` ProcessName _result "Float" _destinationvariablename false "" 0 (`KismetMathLibrary.RandomFloatInRange` (`KismetStringLibrary.Conv_StringToDouble` _min) (`KismetStringLibrary.Conv_StringToDouble` _max))))
        (return _bsuccess_3 _errormessage_2)))
    (else
      (return false "Invalid Type"))))