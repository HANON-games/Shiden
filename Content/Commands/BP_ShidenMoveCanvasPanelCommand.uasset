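; Shiden scenario command MoveCanvasPanel, which eases a named canvas panel slot to a new position and size and can override its Z order.
; Pre-process sets Z order and starts the move, either absolute or added to any pending move's target or the current slot value.
; Process optionally waits for completion, then registers the destinations as scenario properties, which InitFromSaveData reapplies.
; Preview runs the same move, with zero duration for non-current commands.
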(fn `ConvertToEasingFunc`
  (params (EasingFunc :type String))
  (returns (EnumValue :type "EEasingFunc Enum") (Success :type Boolean))
  (switch `string` EasingFunc
    (:`Default`
      (return "Linear" false))
    (:`Linear`
      (return "Linear" true))
    (:`Step`
      (return "Step" true))
    (:`Sinusoidal in`
      (return "SinusoidalIn" true))
    (:`Sinusoidal out`
      (return "SinusoidalOut" true))
    (:`Sinusoidal in out`
      (return "SinusoidalInOut" true))
    (:`Ease in`
      (return "EaseIn" true))
    (:`Ease out`
      (return "EaseOut" true))
    (:`Ease in out`
      (return "EaseInOut" true))
    (:`Expo in`
      (return "ExpoIn" true))
    (:`Expo out`
      (return "ExpoOut" true))
    (:`Expo in out`
      (return "ExpoInOut" true))
    (:`Circular in`
      (return "CircularIn" true))
    (:`Circular out`
      (return "CircularOut" true))
    (:`Circular in out`
      (return "CircularInOut" true))))

(fn `InitFromSaveData`
  (params (ScenarioProperties :type "Map of String to String (by ref)") (Widget :type "ShidenWidget Object Reference") (ScenarioManager :type "ShidenScenarioManagerInterface Interface (by ref)") (CallerObject :type "Object Object Reference"))
  (returns (Status :type "EShidenInitFromSaveDataStatus Enum") (ErrorMessage :type String))
  (bind _keys (`BlueprintMapLibrary.Map_Keys` ScenarioProperties))
  (for _array_element _keys
    (bind (_lefts _rights) (`KismetStringLibrary.Split` _array_element "::" "IgnoreCase" "FromEnd"))
    (bind (_canvaspanel _bresult) (`ShidenWidget.FindCanvasPanel` Widget _lefts))
    (if _bresult
      (switch `string` _rights
        (:`Position`
          (bind _value (`BlueprintMapLibrary.Map_Find` ScenarioProperties _array_element))
          (bind (_outconvertedvector2d _outisvalid) (`KismetStringLibrary.Conv_StringToVector2D` _value))
          (if _outisvalid
            (bind _returnvalue (`WidgetLayoutLibrary.SlotAsCanvasSlot` _canvaspanel))
            (`CanvasPanelSlot.SetPosition` _returnvalue _outconvertedvector2d)
            (else
              (return "Error" (`KismetStringLibrary.Concat_StrStr` "Value \"" _value "\" is invalid")))))
        (:`Size`
          (bind (_outconvertedvector2d_2 _outisvalid_2) (`KismetStringLibrary.Conv_StringToVector2D` _value))
          (if _outisvalid_2
            (`CanvasPanelSlot.SetSize` _returnvalue _outconvertedvector2d_2)
            (else
              (return "Error" (`KismetStringLibrary.Concat_StrStr` "Value \"" _value "\" is invalid")))))
        (:`ZOrder`
          (`CanvasPanelSlot.SetZOrder` _returnvalue (`KismetStringLibrary.Conv_StringToInt` _value))))
      (else
        (return "Error" (`KismetStringLibrary.Concat_StrStr` "Canvas panel slot \"" _lefts "\" is not found")))))
  (return "Completed" ""))

(fn `OverwriteZOrder`
  (params (ShidenCommand :type "ShidenCommand Structure (by ref)") (Widget :type "ShidenWidget Object Reference") (RegisterCurrentProperty :type Boolean))
  (returns (Success :type Boolean) (ErrorMessage :type String))
  (bind (_panelname _easingfunction _duration _changetype _overwriteposition _overwritesize _overwritezorder) (`|GetCommandArguments` "/Shiden/Commands/DA_ShidenPrimaryCommandDefinitions.DA_ShidenPrimaryCommandDefinitions" "MoveCanvasPanel" ShidenCommand))
  (bind (_canvaspanel _bresult) (`ShidenWidget.FindCanvasPanel` Widget _panelname))
  (if (not (`KismetStringLibrary.IsEmpty` _overwritezorder))
    (if _bresult
      (`CanvasPanelSlot.SetZOrder` (`WidgetLayoutLibrary.SlotAsCanvasSlot` _canvaspanel) (`KismetStringLibrary.Conv_StringToInt` _overwritezorder))
      (if RegisterCurrentProperty
        (`ShidenCommandFunctionLibrary.RegisterScenarioProperty` (`.CommandName` (break `ShidenCommand` ShidenCommand)) (`KismetStringLibrary.Concat_StrStr` _panelname "::ZOrder") _overwritezorder)
        (return true "")
        (else
          (return true "")))
      (else
        (return false (`KismetStringLibrary.Concat_StrStr` "Canvas panel slot \"" _panelname "\" is not found"))))
    (else
      (return true ""))))

(fn `PreProcessCommmand`
  (params (ProcessName :type String) (Command :type "ShidenCommand Structure") (Widget :type "ShidenWidget Object Reference") (ScenarioManager :type "ShidenScenarioManagerInterface Interface (by ref)") (CallerObject :type "Object Object Reference"))
  (returns (Status :type "EShidenPreProcessStatus Enum") (ErrorMessage :type String))
  (bind (_success _errormessage) (`self.OverwriteZOrder` Command Widget true))
  (if _success
    (bind (_success_2 _errormessage_2) (`self.StartMoveSlot` Command Widget ProcessName))
    (if _success_2
      (return "Completed" "")
      (else
        (return "Error" _errormessage_2)))
    (else
      (return "Error" _errormessage))))

(fn `PreviewCommmand`
  (params (Command :type "ShidenCommand Structure (by ref)") (Widget :type "ShidenWidget Object Reference") (ScenarioManager :type "ShidenScenarioManagerInterface Interface (by ref)") (bIsCurrentCommand :type Boolean))
  (returns (Status :type "EShidenPreviewStatus Enum") (ErrorMessage :type String))
  (bind (_success _errormessage) (`self.OverwriteZOrder` Command Widget))
  (if _success
    (if bIsCurrentCommand
      (bind (_success_2 _errormessage_2) (`self.StartMoveSlot` Command Widget "Default"))
      (if _success_2
        _
        (else
          (return "Error" _errormessage_2)))
      (else
        (`BlueprintMapLibrary.Map_Add` (`.Args` (break `ShidenCommand` Command)) "Duration" "0.0")
        (bind (_success_3 _errormessage_3) (`self.StartMoveSlot` Command Widget "Default"))
        (if _success_3
          _
          (else
            (return "Error" _errormessage_3)))))
    (return "Completed" "")
    (else
      (return "Error" _errormessage))))

(fn `ProcessCommmand`
  (params (ProcessName :type String) (Command :type "ShidenCommand Structure") (Widget :type "ShidenWidget Object Reference") (ScenarioManager :type "ShidenScenarioManagerInterface Interface (by ref)") (DeltaTime :type "Float (single-precision)") (CallerObject :type "Object Object Reference"))
  (returns (Status :type "EShidenProcessStatus Enum") (BreakReason :type String) (NextScenarioName :type String) (ErrorMessage :type String))
  (bind (_panelname _easingfunction _duration _changetype _overwriteposition _overwritesize _overwritezorder _steps _blendexp _waitforcompletion) (`|GetCommandArguments` "/Shiden/Commands/DA_ShidenPrimaryCommandDefinitions.DA_ShidenPrimaryCommandDefinitions" "MoveCanvasPanel" Command))
  (if (`KismetStringLibrary.EqualEqual_StrStr` _waitforcompletion "true")
    (if (`ShidenWidget.IsCanvasPanelMoveCompleted` Widget _panelname)
      _
      (else
        (return "DelayUntilNextTick" "" "" ""))))
  (if (not (`KismetStringLibrary.IsEmpty` _overwriteposition))
    (`ShidenCommandFunctionLibrary.RegisterScenarioProperty` (`.CommandName` (break `ShidenCommand` Command)) (`KismetStringLibrary.Concat_StrStr` _panelname "::Position") (`KismetStringLibrary.Conv_Vector2dToString` (`self.DestinationPosition`))))
  (if (not (`KismetStringLibrary.IsEmpty` _overwritesize))
    (`ShidenCommandFunctionLibrary.RegisterScenarioProperty` (`.CommandName` (break `ShidenCommand` Command)) (`KismetStringLibrary.Concat_StrStr` _panelname "::Size") (`KismetStringLibrary.Conv_Vector2dToString` (`self.DestinationSize`))))
  (return "Next" "" "" ""))

(fn `SelectVector2D`
  (params (A :type "Vector2D Structure") (B :type "Vector2D Structure") (PickA :type Boolean))
  (returns (ReturnValue :type "Vector2D Structure"))
  (if PickA
    (return A)
    (else
      (return B))))

(fn `StartMoveSlot`
  (params (Command :type "ShidenCommand Structure (by ref)") (Widget :type "ShidenWidget Object Reference") (OwnerProcessName :type String))
  (returns (Success :type Boolean) (ErrorMessage :type String))
  (bind (_panelname _easingfunction _duration _changetype _overwriteposition _overwritesize _overwritezorder _steps _blendexp) (`|GetCommandArguments` "/Shiden/Commands/DA_ShidenPrimaryCommandDefinitions.DA_ShidenPrimaryCommandDefinitions" "MoveCanvasPanel" Command))
  (bind (_value _bsuccess) (`ShidenWidget.FindCanvasPanelMoveParams` Widget _panelname))
  (bind _outconvertedvector2d (`KismetStringLibrary.Conv_StringToVector2D` _overwritesize))
  (bind _outconvertedvector2d_2 (`KismetStringLibrary.Conv_StringToVector2D` _overwriteposition))
  (bind _returnvalue (`KismetStringLibrary.EqualEqual_StrStr` _changetype "AddToCurrent"))
  (bind (_enumvalue _success) (`self.ConvertToEasingFunc` _easingfunction))
  (bind _panelname_2 (`|GetCommandArguments` "/Shiden/Commands/DA_ShidenPrimaryCommandDefinitions.DA_ShidenPrimaryCommandDefinitions" "MoveCanvasPanel" (`local.Command`)))
  (bind (_target _moveduration _movefunction _easingalpha _bchangeposition _startposition _endposition _bchangesize _startsize _endsize) (break `ShidenCanvasPanelMoveParams` _value))
  (bind (_canvaspanel _bresult) (`ShidenWidget.FindCanvasPanel` Widget _panelname_2))
  (bind _returnvalue_2 (`WidgetLayoutLibrary.SlotAsCanvasSlot` (`ShidenWidget.FindCanvasPanel` (`local.Widget`) _panelname)))
  (bind _returnvalue_3 (not (`KismetStringLibrary.IsEmpty` _overwritesize)))
  (bind _returnvalue_4 (not (`KismetStringLibrary.IsEmpty` _overwriteposition)))
  (bind _returnvalue_5 (`self.SelectVector2D` (+ _outconvertedvector2d_2 (`self.SelectVector2D` _endposition (`CanvasPanelSlot.GetPosition` _returnvalue_2) (and _bsuccess _bchangeposition))) _outconvertedvector2d_2 _returnvalue))
  (bind _returnvalue_6 (`self.SelectVector2D` (+ _outconvertedvector2d (`self.SelectVector2D` _endsize (`CanvasPanelSlot.GetSize` _returnvalue_2) (and _bsuccess _bchangesize))) _outconvertedvector2d _returnvalue))
  (if _success
    (if _bresult
      (bind (_success_2 _errormessage) (`ShidenWidget.StartCanvasPanelMove` Widget _panelname_2 _canvaspanel _enumvalue (`KismetStringLibrary.Conv_StringToDouble` _duration) _returnvalue_4 _returnvalue_5 _returnvalue_3 _returnvalue_6 (`KismetStringLibrary.Conv_StringToDouble` _blendexp) (`KismetStringLibrary.Conv_StringToInt` _steps) OwnerProcessName))
      (if _success_2
        (set `self.ChangePosition` _returnvalue_4)
        (set `self.DestinationPosition` _returnvalue_5)
        (set `self.ChangeSize` _returnvalue_3)
        (set `self.DestinationSize` _returnvalue_6)
        (return true "")
        (else
          (return false _errormessage)))
      (else
        (return false (`KismetStringLibrary.Concat_StrStr` "Canvas panel slot \"" _panelname_2 "\" is not found"))))
    (else
      (return false "Invalid ease func"))))