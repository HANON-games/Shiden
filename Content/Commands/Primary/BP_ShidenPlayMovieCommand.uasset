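; Shiden scenario command that plays a movie on the widget and holds the command until it ends.
; PreProcessCommand starts playback from the command arguments (media source path, pause-menu permission, Z-orders) and reports an error if it fails.
; ProcessCommand polls for movie end each update, then collapses the movie and, if pausing was allowed, reapplies the current window mode.
; The media path is exposed through GetAssetPaths; save restore and preview are no-ops.
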(fn `GetAssetPaths`
  (params (Command :type "ShidenCommand Structure"))
  (returns (AssetObjectPaths :type "Set of String"))
  (return (`|MakeSet` Command_Arg1)))

(fn `InitFromSaveData`
  (params (KeyValueMap :type "Map of String to String") (Widget :type "/Shiden/Core/WBP_ShidenWidgetBase Object Reference") (ScenarioManager :type "/Shiden/Core/BP_ShidenScenarioManager Object Reference"))
  (returns (Success :type "/Shiden/Commands/Core/E_ShidenInitFromSaveDataStatus Enum") (ErrorMessage :type String))
  (return "NewEnumerator0" ""))

(fn `PreProcessCommand`
  (params (ProcessName :type String) (Command :type "ShidenCommand Structure") (Widget :type "/Shiden/Core/WBP_ShidenWidgetBase Object Reference") (ScenarioManager :type "/Shiden/Core/BP_ShidenScenarioManager Object Reference") (HookedObject :type "Object Object Reference"))
  (returns (Status :type "/Shiden/Commands/Core/E_ShidenPreProcessStatus Enum") (ErrorMessage :type String))
  (bind _success (`/Shiden/Core/WBP_ShidenWidgetBase.PlayMovie` (`local.Widget`) Command_Arg1 (== Command_Arg2 "true") (`KismetStringLibrary.Conv_StringToInt` Command_Arg3) (`KismetStringLibrary.Conv_StringToInt` Command_Arg4)))
  (if _success
    (return "NewEnumerator0" "")
    (else
      (return "NewEnumerator2" "Playing movie failed"))))

(fn `PreviewCommand`
  (params (Command :type "ShidenCommand Structure") (Widget :type "/Shiden/Core/WBP_ShidenWidgetBase Object Reference") (IsCurrentCommand :type Boolean))
  (returns (Status :type "/Shiden/Commands/Core/E_ShidenPreviewStatus Enum") (SoundInfo :type "/Shiden/Commands/Primary/F_ShidenSoundInfo Structure") (ErrorMessage :type String))
  (return "NewEnumerator0" (struct) ""))

(fn `ProcessCommand`
  (params (ProcessName :type String) (Command :type "ShidenCommand Structure") (Widget :type "/Shiden/Core/WBP_ShidenWidgetBase Object Reference") (ScenarioManager :type "/Shiden/Core/BP_ShidenScenarioManager Object Reference") (DeltaTime :type "Float (double-precision)") (HookedObject :type "Object Object Reference"))
  (returns (Status :type "/Shiden/Commands/Core/E_ShidenProcessStatus Enum") (BreakReason :type String) (NextScenarioName :type String) (ErrorMessage :type String))
  (bind _result (`/Shiden/Core/WBP_ShidenWidgetBase.IsMovieEnd` Widget))
  (if _result
    (`/Shiden/Core/WBP_ShidenWidgetBase.CollapseMovie` Widget)
    (`/Shiden/Core/WBP_ShidenWidgetBase.CollapseMovie` (`local.Widget`))
    (if (== (`.Arg2` (break `ShidenCommand` Command)) "true")
      (`/Shiden/Core/WBP_ShidenWidgetBase.ChangeWindowMode` Widget (`self.CurrentWindowMode`) false)
      (`/Shiden/Core/WBP_ShidenWidgetBase.ChangeWindowMode` (`local.Widget`) (`self.CurrentWindowMode`) false))
    (return "NewEnumerator3" "" "" "")
    (else
      (return "NewEnumerator4" "" "" ""))))