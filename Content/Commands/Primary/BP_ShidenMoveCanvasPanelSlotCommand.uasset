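; Shiden scenario command that moves and resizes a named canvas panel slot with a chosen easing function, optionally setting its Z order.
; PreProcess sets Z order and starts the tween, with targets either absolute or added to the current or in-flight destination.
; Process optionally waits for the move to end, then registers position and size as scenario properties, which InitFromSaveData restores.
; Preview zeroes the duration for non-current commands.
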(fn `ConvertToEasingFunc`
  (params (EasingFunc :type String))
  (returns (EnumValue :type "EEasingFunc Enum") (Success :type Boolean))
  (switch `string` EasingFunc
    (:`Default`
      (return "Linear" false))
    (:`Linear`
      (return "Linear" true))
    (:`Step`
      (return "Step" true))
    (:`Sinusoidal in`
      (return "SinusoidalIn" true))
    (:`Sinusoidal out`
      (return "SinusoidalOut" true))
    (:`Sinusoidal in out`
      (return "SinusoidalInOut" true))
    (:`Ease in`
      (return "EaseIn" true))
    (:`Ease out`
      (return "EaseOut" true))
    (:`Ease in out`
      (return "EaseInOut" true))
    (:`Expo in`
      (return "ExpoIn" true))
    (:`Expo out`
      (return "ExpoOut" true))
    (:`Expo in out`
      (return "ExpoInOut" true))
    (:`Circular in`
      (return "CircularIn" true))
    (:`Circular out`
      (return "CircularOut" true))
    (:`Circular in out`
      (return "CircularInOut" true))))

(fn `GetAssetPaths`
  (params (Command :type "ShidenCommand Structure"))
  (returns (AssetObjectPaths :type "Set of String"))
  (return))

(fn `InitFromSaveData`
  (params (KeyValueMap :type "Map of String to String") (Widget :type "/Shiden/Core/WBP_ShidenWidgetBase Object Reference") (ScenarioManager :type "/Shiden/Core/BP_ShidenScenarioManager Object Reference"))
  (returns (Success :type "/Shiden/Commands/Core/E_ShidenInitFromSaveDataStatus Enum") (ErrorMessage :type String))
  (bind _keys (`BlueprintMapLibrary.Map_Keys` KeyValueMap))
  (for _array_element _keys
    (bind (_lefts _rights) (`KismetStringLibrary.Split` _array_element "::" "IgnoreCase" "FromEnd"))
    (bind (_value _returnvalue) (`BlueprintMapLibrary.Map_Find` (`/Shiden/Core/WBP_ShidenWidgetBase.GetCanvasPanelSlots` Widget) _lefts))
    (if _returnvalue
      (switch `string` _rights
        (:`Position`
          (bind _value_2 (`BlueprintMapLibrary.Map_Find` KeyValueMap _array_element))
          (bind (_outconvertedvector2d _outisvalid) (`KismetStringLibrary.Conv_StringToVector2D` _value_2))
          (if _outisvalid
            (bind _returnvalue_2 (`WidgetLayoutLibrary.SlotAsCanvasSlot` _value))
            (`CanvasPanelSlot.SetPosition` _returnvalue_2 _outconvertedvector2d)
            (else
              (return "NewEnumerator2" (`KismetStringLibrary.Concat_StrStr` "Value \"" _value_2 "\" is invalid")))))
        (:`Size`
          (bind (_outconvertedvector2d_2 _outisvalid_2) (`KismetStringLibrary.Conv_StringToVector2D` _value_2))
          (if _outisvalid_2
            (`CanvasPanelSlot.SetSize` _returnvalue_2 _outconvertedvector2d_2)
            (else
              (return "NewEnumerator2" (`KismetStringLibrary.Concat_StrStr` "Value \"" _value_2 "\" is invalid")))))
        (:`ZOrder`
          (`CanvasPanelSlot.SetZOrder` _returnvalue_2 (`KismetStringLibrary.Conv_StringToInt` _value_2))))
      (else
        (return "NewEnumerator2" (`KismetStringLibrary.Concat_StrStr` "Canvas panel slot \"" _lefts "\" is not found")))))
  (return "NewEnumerator0" ""))

(fn `OverwriteZOrder`
  (params (ShidenCommand :type "ShidenCommand Structure (by ref)") (Widget :type "/Shiden/Core/WBP_ShidenWidgetBase Object Reference") (RegisterCurrentProperty :type Boolean))
  (returns (Success :type Boolean) (ErrorMessage :type String))
  (bind (_commandname _presetname _arg1 _arg2 _arg3 _arg4 _arg5 _arg6 _arg7) (break `ShidenCommand` ShidenCommand))
  (bind (_value _returnvalue) (`BlueprintMapLibrary.Map_Find` (`/Shiden/Core/WBP_ShidenWidgetBase.GetCanvasPanelSlots` Widget) _arg1))
  (if (not (`KismetStringLibrary.IsEmpty` _arg7))
    (if _returnvalue
      (`CanvasPanelSlot.SetZOrder` (`WidgetLayoutLibrary.SlotAsCanvasSlot` _value) (`KismetStringLibrary.Conv_StringToInt` _arg7))
      (if RegisterCurrentProperty
        (`ShidenCommandFunctionLibrary.RegisterCurrentScenarioProperty` (`.CommandName` (break `ShidenCommand` ShidenCommand)) (`KismetStringLibrary.Concat_StrStr` _arg1 "::ZOrder") _arg7)
        (return true "")
        (else
          (return true "")))
      (else
        (return false (`KismetStringLibrary.Concat_StrStr` "Canvas panel slot \"" _arg1 "\" is not found"))))
    (else
      (return true ""))))

(fn `PreProcessCommand`
  (params (ProcessName :type String) (Command :type "ShidenCommand Structure") (Widget :type "/Shiden/Core/WBP_ShidenWidgetBase Object Reference") (ScenarioManager :type "/Shiden/Core/BP_ShidenScenarioManager Object Reference") (HookedObject :type "Object Object Reference"))
  (returns (Status :type "/Shiden/Commands/Core/E_ShidenPreProcessStatus Enum") (ErrorMessage :type String))
  (bind (_success _errormessage) (`self.OverwriteZOrder` Command Widget true))
  (if _success
    (bind (_success_2 _errormessage_2) (`self.StartMoveSlot` Command Widget ProcessName))
    (if _success_2
      (return "NewEnumerator0" "")
      (else
        (return "NewEnumerator2" _errormessage_2)))
    (else
      (return "NewEnumerator2" _errormessage))))

(fn `PreviewCommand`
  (params (Command :type "ShidenCommand Structure") (Widget :type "/Shiden/Core/WBP_ShidenWidgetBase Object Reference") (IsCurrentCommand :type Boolean))
  (returns (Status :type "/Shiden/Commands/Core/E_ShidenPreviewStatus Enum") (SoundInfo :type "/Shiden/Commands/Primary/F_ShidenSoundInfo Structure") (ErrorMessage :type String))
  (bind (_success _errormessage) (`self.OverwriteZOrder` Command Widget))
  (if _success
    (if IsCurrentCommand
      (bind (_success_2 _errormessage_2) (`self.StartMoveSlot` Command (`local.Widget`) "Default"))
      (if _success_2
        _
        (else
          (return "NewEnumerator2" (struct) _errormessage_2)))
      (else
        (bind _structout (setmembers `ShidenCommand` :`StructRef` Command :`Arg3` "0.0")) ; Override dulation
        (bind (_success_3 _errormessage_3) (`self.StartMoveSlot` _structout (`local.Widget`) "Default"))
        (if _success_3
          _
          (else
            (return "NewEnumerator2" (struct) _errormessage_3)))))
    (return "NewEnumerator0" (struct) "")
    (else
      (return "NewEnumerator2" (struct) _errormessage))))

(fn `ProcessCommand`
  (params (ProcessName :type String) (Command :type "ShidenCommand Structure") (Widget :type "/Shiden/Core/WBP_ShidenWidgetBase Object Reference") (ScenarioManager :type "/Shiden/Core/BP_ShidenScenarioManager Object Reference") (DeltaTime :type "Float (double-precision)") (HookedObject :type "Object Object Reference"))
  (returns (Status :type "/Shiden/Commands/Core/E_ShidenProcessStatus Enum") (BreakReason :type String) (NextScenarioName :type String) (ErrorMessage :type String))
  (bind (_commandname _presetname _arg1 _arg2 _arg3 _arg4 _arg5 _arg6 _arg7 _arg8 _arg9 _arg10) (break `ShidenCommand` Command))
  (if (`KismetStringLibrary.EqualEqual_StrStr` _arg10 "true")
    (bind _result (`/Shiden/Core/WBP_ShidenWidgetBase.IsMoveEnd` (`local.Widget`) _arg1))
    (if _result
      _
      (else
        (return "NewEnumerator4" "" "" ""))))
  (if (not (`KismetStringLibrary.IsEmpty` _arg5))
    (`ShidenCommandFunctionLibrary.RegisterCurrentScenarioProperty` (`.CommandName` (break `ShidenCommand` (`local.Command`))) (`KismetStringLibrary.Concat_StrStr` _arg1 "::Position") (`KismetStringLibrary.Conv_Vector2dToString` (`self.DestinationPosition`))))
  (if (not (`KismetStringLibrary.IsEmpty` _arg6))
    (`ShidenCommandFunctionLibrary.RegisterCurrentScenarioProperty` (`.CommandName` (break `ShidenCommand` (`local.Command`))) (`KismetStringLibrary.Concat_StrStr` _arg1 "::Size") (`KismetStringLibrary.Conv_Vector2dToString` (`self.DestinationSize`))))
  (return "NewEnumerator3" "" "" ""))

(fn `SelectVector2D`
  (params (A :type "Vector2D Structure") (B :type "Vector2D Structure") (PickA :type Boolean))
  (returns (ReturnValue :type "Vector2D Structure"))
  (if PickA
    (return A)
    (else
      (return B))))

(fn `StartMoveSlot`
  (params (Command :type "ShidenCommand Structure (by ref)") (Widget :type "/Shiden/Core/WBP_ShidenWidgetBase Object Reference") (OwnerProcessName :type String))
  (returns (Success :type Boolean) (ErrorMessage :type String))
  (bind (_commandname _presetname _arg1 _arg2 _arg3 _arg4 _arg5 _arg6 _arg7 _arg8 _arg9) (break `ShidenCommand` Command))
  (bind (_commandname_2 _presetname_2 _arg1_2) (break `ShidenCommand` (`local.Command`)))
  (bind (_value _returnvalue) (`BlueprintMapLibrary.Map_Find` (`/Shiden/Core/WBP_ShidenWidgetBase.CanvasPanelSlotMoveParams` Widget) _arg1))
  (bind _outconvertedvector2d (`KismetStringLibrary.Conv_StringToVector2D` _arg6))
  (bind _outconvertedvector2d_2 (`KismetStringLibrary.Conv_StringToVector2D` _arg5))
  (bind _returnvalue_2 (`KismetStringLibrary.EqualEqual_StrStr` _arg4 "AddToCurrent"))
  (bind (_enumvalue _success) (`self.ConvertToEasingFunc` _arg2))
  (bind (_targetslot _movedulation _movefunction _easingalpha _changeposition _startposition _destinarionposition _changesize _startsize _destinationsize) (break `/Shiden/Commands/Primary/F_ShidenCanvasPanelSlotMoveParams` _value))
  (bind _returnvalue_3 (`WidgetLayoutLibrary.SlotAsCanvasSlot` (`BlueprintMapLibrary.Map_Find` (`/Shiden/Core/WBP_ShidenWidgetBase.GetCanvasPanelSlots` Widget) _arg1)))
  (bind _returnvalue_4 (not (`KismetStringLibrary.IsEmpty` _arg6)))
  (bind _returnvalue_5 (not (`KismetStringLibrary.IsEmpty` _arg5)))
  (bind (_value_2 _returnvalue_6) (`BlueprintMapLibrary.Map_Find` (`/Shiden/Core/WBP_ShidenWidgetBase.GetCanvasPanelSlots` Widget) _arg1_2))
  (bind _returnvalue_7 (`self.SelectVector2D` (+ _outconvertedvector2d_2 (`self.SelectVector2D` _destinarionposition (`CanvasPanelSlot.GetPosition` _returnvalue_3) (and _returnvalue _changeposition))) _outconvertedvector2d_2 _returnvalue_2))
  (bind _returnvalue_8 (`self.SelectVector2D` (+ _outconvertedvector2d (`self.SelectVector2D` _destinationsize (`CanvasPanelSlot.GetSize` _returnvalue_3) (and _returnvalue _changesize))) _outconvertedvector2d _returnvalue_2))
  (if _success
    (if _returnvalue_6
      (bind (_success_2 _errormessage) (`/Shiden/Core/WBP_ShidenWidgetBase.StartCanvasPanelSlotMove` Widget _arg1_2 _value_2 (`KismetStringLibrary.Conv_StringToDouble` _arg3) _enumvalue _returnvalue_5 _returnvalue_7 _returnvalue_4 _returnvalue_8 (`KismetStringLibrary.Conv_StringToDouble` _arg9) (`KismetStringLibrary.Conv_StringToInt` _arg8) OwnerProcessName))
      (if _success_2
        (set `self.ChangePosition` _returnvalue_5)
        (set `self.DestinationPosition` _returnvalue_7)
        (set `self.ChangeSize` _returnvalue_4)
        (set `self.DestinationSize` _returnvalue_8)
        (return true "")
        (else
          (return false _errormessage)))
      (else
        (return false (`KismetStringLibrary.Concat_StrStr` "Canvas panel slot \"" _arg1_2 "\" is not found"))))
    (else
      (return false "Invalid ease func"))))