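; Shiden scenario command that plays a named animation on the scenario widget, using command arguments for timing, loops, play mode and speed.
; PreProcess, and Preview for the current command, start playback; an optional wait flag binds the finished event so ProcessCommand holds until it fires.
; On completion it registers the animation name as a scenario property, letting InitFromSaveData restore state by playing saved animations from their end time.
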(event `Bind to Animation Finished`
  (params (Widget :type "UserWidget Object Reference") (Animation :type "WidgetAnimation Object Reference"))
  (`UserWidget.BindToAnimationFinished` Widget Animation (delegate `OnAnimationFinished`)))

(event `OnAnimationFinished`
  (set `self.IsAnimationEnd` true))

(fn `ConvertToPlayMode`
  (params (PlayMode :type String))
  (returns (Result :type "EUMGSequencePlayMode Enum") (Success :type Boolean))
  (switch `string` PlayMode
    (:`Default`
      (return "Forward" false))
    (:`Forward`
      (return "Forward" true))
    (:`Reverse`
      (return "Reverse" true))
    (:`Ping Pong`
      (return "PingPong" true))))

(fn `GetAssetPaths`
  (params (Command :type "ShidenCommand Structure"))
  (returns (AssetObjectPaths :type "Set of String"))
  (return))

(fn `InitFromSaveData`
  (params (KeyValueMap :type "Map of String to String") (Widget :type "/Shiden/Core/WBP_ShidenWidgetBase Object Reference") (ScenarioManager :type "/Shiden/Core/BP_ShidenScenarioManager Object Reference"))
  (returns (Success :type "/Shiden/Commands/Core/E_ShidenInitFromSaveDataStatus Enum") (ErrorMessage :type String))
  (bind _keys (`BlueprintMapLibrary.Map_Keys` KeyValueMap))
  (for _array_element _keys
    (bind (_value _returnvalue) (`BlueprintMapLibrary.Map_Find` (`/Shiden/Core/WBP_ShidenWidgetBase.GetAnimations` Widget) _array_element))
    (if _returnvalue
      (`UserWidget.PlayAnimation` Widget _value (`WidgetAnimation.GetEndTime` _value) 1 "Forward" 1.0 false)
      (else
        (return "NewEnumerator2" (`KismetStringLibrary.Concat_StrStr` "Animation \"" _array_element "\" is not found")))))
  (return "NewEnumerator0" ""))

(fn `PreProcessCommand`
  (params (ProcessName :type String) (Command :type "ShidenCommand Structure") (Widget :type "/Shiden/Core/WBP_ShidenWidgetBase Object Reference") (ScenarioManager :type "/Shiden/Core/BP_ShidenScenarioManager Object Reference") (HookedObject :type "Object Object Reference"))
  (returns (Status :type "/Shiden/Commands/Core/E_ShidenPreProcessStatus Enum") (ErrorMessage :type String))
  (bind _result (`self.StartAnimation` Command Widget))
  (if _result
    (return "NewEnumerator0" "")
    (else
      (return "NewEnumerator2" "Animation not found"))))

(fn `PreviewCommand`
  (params (Command :type "ShidenCommand Structure") (Widget :type "/Shiden/Core/WBP_ShidenWidgetBase Object Reference") (IsCurrentCommand :type Boolean))
  (returns (Status :type "/Shiden/Commands/Core/E_ShidenPreviewStatus Enum") (SoundInfo :type "/Shiden/Commands/Primary/F_ShidenSoundInfo Structure") (ErrorMessage :type String))
  (if IsCurrentCommand
    (bind _result (`self.StartAnimation` Command Widget))
    (if _result
      (return "NewEnumerator0" (struct) "")
      (else
        (return "NewEnumerator2" (struct) "Animation not found")))
    (else
      (return "NewEnumerator0" (struct) ""))))

(fn `ProcessCommand`
  (params (ProcessName :type String) (Command :type "ShidenCommand Structure") (Widget :type "/Shiden/Core/WBP_ShidenWidgetBase Object Reference") (ScenarioManager :type "/Shiden/Core/BP_ShidenScenarioManager Object Reference") (DeltaTime :type "Float (double-precision)") (HookedObject :type "Object Object Reference"))
  (returns (Status :type "/Shiden/Commands/Core/E_ShidenProcessStatus Enum") (BreakReason :type String) (NextScenarioName :type String) (ErrorMessage :type String))
  (bind (_commandname _presetname _arg1) (break `ShidenCommand` (`local.Command`)))
  (if (`self.IsAnimationEnd`)
    (`ShidenCommandFunctionLibrary.RegisterCurrentScenarioProperty` _commandname _arg1 "EMPTY")
    (return "NewEnumerator3" "" "" "")
    (else
      (return "NewEnumerator4" "" "" ""))))

(fn `StartAnimation`
  (params (Command :type "ShidenCommand Structure (by ref)") (ScenarioWidget :type "/Shiden/Core/WBP_ShidenWidgetBase Object Reference"))
  (returns (Result :type Boolean))
  (bind (_commandname _presetname _arg1 _arg2 _arg3 _arg4 _arg5 _arg6 _arg7) (break `ShidenCommand` Command))
  (bind (_result _success) (`self.ConvertToPlayMode` _arg4))
  (bind (_value _returnvalue) (`BlueprintMapLibrary.Map_Find` (`/Shiden/Core/WBP_ShidenWidgetBase.GetAnimations` ScenarioWidget) _arg1))
  (if _returnvalue
    (switch `string` _arg7
      (:`Default`
        (set `self.IsAnimationEnd` true :!label _label))
      (:`true`
        (set `self.IsAnimationEnd` false)
        (`self.Bind to Animation Finished` (`local.ScenarioWidget`) _value))
      (:`false`
        (goto _label)))
    (if _success
      (`UserWidget.PlayAnimation` (`local.ScenarioWidget`) _value (`KismetStringLibrary.Conv_StringToDouble` _arg2) (`KismetStringLibrary.Conv_StringToInt` _arg3) _result (`KismetStringLibrary.Conv_StringToDouble` _arg5) (== _arg6 "true"))
      (return true)
      (else
        (return false)))
    (else
      (return false))))