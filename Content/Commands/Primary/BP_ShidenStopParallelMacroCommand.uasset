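; Shiden scenario command that stops a parallel macro by requesting cancellation of the named process.
; PreProcessCommand sends the request with a reason, either immediately or when the current command ends, and errors on any other cancel type.
; When the ensure-cancel argument is true, ProcessCommand returns a different status while that process remains in the subsystem's ScenarioProgressStack, apparently holding until it clears.
; Preview, save-data restore and asset-path hooks do no work.
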(fn `GetAssetPaths`
  (params (Command :type "ShidenCommand Structure"))
  (returns (AssetObjectPaths :type "Set of String"))
  (return))

(fn `InitFromSaveData`
  (params (KeyValueMap :type "Map of String to String") (Widget :type "/Shiden/Core/WBP_ShidenWidgetBase Object Reference") (ScenarioManager :type "/Shiden/Core/BP_ShidenScenarioManager Object Reference"))
  (returns (Success :type "/Shiden/Commands/Core/E_ShidenInitFromSaveDataStatus Enum") (ErrorMessage :type String))
  (return "NewEnumerator0" ""))

(fn `PreProcessCommand`
  (params (ProcessName :type String) (Command :type "ShidenCommand Structure") (Widget :type "/Shiden/Core/WBP_ShidenWidgetBase Object Reference") (ScenarioManager :type "/Shiden/Core/BP_ShidenScenarioManager Object Reference") (HookedObject :type "Object Object Reference"))
  (returns (Status :type "/Shiden/Commands/Core/E_ShidenPreProcessStatus Enum") (ErrorMessage :type String))
  (switch `string` Command_Arg3
    (:`Default`
      (return "NewEnumerator2" "Invalid Cancel Type"))
    (:`Immediately`
      (`ShidenScenarioFunctionLibrary.RequestCancelScenario` Command_Arg1 Command_Arg2 "Immediately"))
    (:`OnCurrentCommandEnd`
      (`ShidenScenarioFunctionLibrary.RequestCancelScenario` Command_Arg1 Command_Arg2 "OnCurrentCommandEnd")))
  (return "NewEnumerator0" ""))

(fn `PreviewCommand`
  (params (Command :type "ShidenCommand Structure") (Widget :type "/Shiden/Core/WBP_ShidenWidgetBase Object Reference") (IsCurrentCommand :type Boolean))
  (returns (Status :type "/Shiden/Commands/Core/E_ShidenPreviewStatus Enum") (SoundInfo :type "/Shiden/Commands/Primary/F_ShidenSoundInfo Structure") (ErrorMessage :type String))
  (return "NewEnumerator0" (struct) ""))

(fn `ProcessCommand`
  (params (ProcessName :type String) (Command :type "ShidenCommand Structure") (Widget :type "/Shiden/Core/WBP_ShidenWidgetBase Object Reference") (ScenarioManager :type "/Shiden/Core/BP_ShidenScenarioManager Object Reference") (DeltaTime :type "Float (double-precision)") (HookedObject :type "Object Object Reference"))
  (returns (Status :type "/Shiden/Commands/Core/E_ShidenProcessStatus Enum") (BreakReason :type String) (NextScenarioName :type String) (ErrorMessage :type String))
  (if (== Command_Arg4 "true")
    (if (`.ReturnValue` (`BlueprintMapLibrary.Map_Find` (`ShidenSubsystem.ScenarioProgressStack` (subsystem `ShidenSubsystem`)) Command_Arg1))
      (return "NewEnumerator4" "" "" "")
      (else
        _)))
  (return "NewEnumerator3" "" "" ""))