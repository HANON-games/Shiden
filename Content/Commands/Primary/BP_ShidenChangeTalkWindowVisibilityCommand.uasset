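; Shiden scenario command that shows or hides the talk window according to its "true"/"false" argument.
; Processing and preview share SetVisibility, which switches the widget's window mode only when moving into or out of the hidden mode, registering the change as a current property.
; InitFromSaveData restores the mode from the saved ChangeTalkWindowVisibility value without re-registering it, and reports when that value is missing.
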(fn `GetAssetPaths`
  (params (Command :type "ShidenCommand Structure"))
  (returns (AssetObjectPaths :type "Set of String"))
  (return))

(fn `InitFromSaveData`
  (params (KeyValueMap :type "Map of String to String") (Widget :type "/Shiden/Core/WBP_ShidenWidgetBase Object Reference") (ScenarioManager :type "/Shiden/Core/BP_ShidenScenarioManager Object Reference"))
  (returns (Success :type "/Shiden/Commands/Core/E_ShidenInitFromSaveDataStatus Enum") (ErrorMessage :type String))
  (bind (_value _returnvalue) (`BlueprintMapLibrary.Map_Find` KeyValueMap "ChangeTalkWindowVisibility"))
  (if _returnvalue
    (switch `string` _value
      (:`Default`
        (`/Shiden/Core/WBP_ShidenWidgetBase.ChangeWindowMode` Widget "NewEnumerator3" false :!label _label))
      (:`true`
        (`/Shiden/Core/WBP_ShidenWidgetBase.ChangeWindowMode` Widget "NewEnumerator0" false))
      (:`false`
        (goto _label)))
    (return "NewEnumerator0" "")
    (else
      (return "NewEnumerator2" "Value not found"))))

(fn `PreProcessCommand`
  (params (ProcessName :type String) (Command :type "ShidenCommand Structure") (Widget :type "/Shiden/Core/WBP_ShidenWidgetBase Object Reference") (ScenarioManager :type "/Shiden/Core/BP_ShidenScenarioManager Object Reference") (HookedObject :type "Object Object Reference"))
  (returns (Status :type "/Shiden/Commands/Core/E_ShidenPreProcessStatus Enum") (ErrorMessage :type String))
  (return "NewEnumerator0" ""))

(fn `PreviewCommand`
  (params (Command :type "ShidenCommand Structure") (Widget :type "/Shiden/Core/WBP_ShidenWidgetBase Object Reference") (IsCurrentCommand :type Boolean))
  (returns (Status :type "/Shiden/Commands/Core/E_ShidenPreviewStatus Enum") (SoundInfo :type "/Shiden/Commands/Primary/F_ShidenSoundInfo Structure") (ErrorMessage :type String))
  (`self.SetVisibility` Command_Arg1 Widget)
  (return "NewEnumerator0" (struct) ""))

(fn `ProcessCommand`
  (params (ProcessName :type String) (Command :type "ShidenCommand Structure") (Widget :type "/Shiden/Core/WBP_ShidenWidgetBase Object Reference") (ScenarioManager :type "/Shiden/Core/BP_ShidenScenarioManager Object Reference") (DeltaTime :type "Float (double-precision)") (HookedObject :type "Object Object Reference"))
  (returns (Status :type "/Shiden/Commands/Core/E_ShidenProcessStatus Enum") (BreakReason :type String) (NextScenarioName :type String) (ErrorMessage :type String))
  (`self.SetVisibility` Command_Arg1 Widget)
  (return "NewEnumerator3" "" "" ""))

(fn `SetVisibility`
  (params (Visible :type String) (Widget :type "/Shiden/Core/WBP_ShidenWidgetBase Object Reference"))
  (if (and (== Visible "true") (`|EnumEquality` (`/Shiden/Core/WBP_ShidenWidgetBase.GetWIndowMode` Widget) "NewEnumerator3"))
    (`/Shiden/Core/WBP_ShidenWidgetBase.ChangeWindowMode` Widget "NewEnumerator0" true)
    (elif (and (== Visible "false") (`|EnumInequality` (`/Shiden/Core/WBP_ShidenWidgetBase.GetWIndowMode` Widget) "NewEnumerator3"))
      (`/Shiden/Core/WBP_ShidenWidgetBase.ChangeWindowMode` Widget "NewEnumerator3" true)))
  (return))