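; Shiden scenario command that calls a function on the scenario widget, chosen by name at runtime from the command's first argument.
; ProcessCommand appends the remaining arguments into one parameter string, passes it to CallFunctionByName on the Widget, then returns a fixed status without waiting.
; Asset gathering, save-data init, pre-process and preview are stubs, so the call happens only during processing.
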(fn `GetAssetPaths`
  (params (Command :type "ShidenCommand Structure"))
  (returns (AssetObjectPaths :type "Set of String"))
  (return))

(fn `InitFromSaveData`
  (params (KeyValueMap :type "Map of String to String") (Widget :type "/Shiden/Core/WBP_ShidenWidgetBase Object Reference") (ScenarioManager :type "/Shiden/Core/BP_ShidenScenarioManager Object Reference"))
  (returns (Success :type "/Shiden/Commands/Core/E_ShidenInitFromSaveDataStatus Enum") (ErrorMessage :type String))
  (return "NewEnumerator0" ""))

(fn `PreProcessCommand`
  (params (ProcessName :type String) (Command :type "ShidenCommand Structure") (Widget :type "/Shiden/Core/WBP_ShidenWidgetBase Object Reference") (ScenarioManager :type "/Shiden/Core/BP_ShidenScenarioManager Object Reference") (HookedObject :type "Object Object Reference"))
  (returns (Status :type "/Shiden/Commands/Core/E_ShidenPreProcessStatus Enum") (ErrorMessage :type String))
  (return "NewEnumerator0" ""))

(fn `PreviewCommand`
  (params (Command :type "ShidenCommand Structure") (Widget :type "/Shiden/Core/WBP_ShidenWidgetBase Object Reference") (IsCurrentCommand :type Boolean))
  (returns (Status :type "/Shiden/Commands/Core/E_ShidenPreviewStatus Enum") (SoundInfo :type "/Shiden/Commands/Primary/F_ShidenSoundInfo Structure") (ErrorMessage :type String))
  (return "NewEnumerator0" (struct) ""))

(fn `ProcessCommand`
  (params (ProcessName :type String) (Command :type "ShidenCommand Structure") (Widget :type "/Shiden/Core/WBP_ShidenWidgetBase Object Reference") (ScenarioManager :type "/Shiden/Core/BP_ShidenScenarioManager Object Reference") (DeltaTime :type "Float (double-precision)") (HookedObject :type "Object Object Reference"))
  (returns (Status :type "/Shiden/Commands/Core/E_ShidenProcessStatus Enum") (BreakReason :type String) (NextScenarioName :type String) (ErrorMessage :type String))
  (bind (_commandname _presetname _arg1 _arg2 _arg3 _arg4 _arg5 _arg6 _arg7 _arg8 _arg9 _arg10) (break `ShidenCommand` Command))
  (`ShidenCoreFunctionLibrary.CallFunctionByName` Widget _arg1 (`KismetStringLibrary.Concat_StrStr` _arg2 " " _arg3 " " _arg4 " " _arg5 " " _arg6 " " _arg7 " " _arg8 " " _arg9 " " _arg10))
  (return "NewEnumerator3" "" "" ""))