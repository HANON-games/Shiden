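; Shiden scenario command that, as its name indicates, holds a scenario until a variable meets a condition.
; ProcessCommand reads the variable kind, type, key, operator and comparison value from the command arguments, then looks up the variable.
; EvaluateCondition compares it against the string argument converted to each supported type, and the result selects the returned status.
; Invalid arguments, missing variables, type mismatches and evaluation failures return error messages; the other overrides are empty stubs.
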(fn `GetAssetPaths`
  (params (Command :type "ShidenCommand Structure"))
  (returns (AssetObjectPaths :type "Set of String"))
  (return))

(fn `InitFromSaveData`
  (params (KeyValueMap :type "Map of String to String") (Widget :type "/Shiden/Core/WBP_ShidenWidgetBase Object Reference") (ScenarioManager :type "/Shiden/Core/BP_ShidenScenarioManager Object Reference"))
  (returns (Success :type "/Shiden/Commands/Core/E_ShidenInitFromSaveDataStatus Enum") (ErrorMessage :type String))
  (return "NewEnumerator0" ""))

(fn `PreProcessCommand`
  (params (ProcessName :type String) (Command :type "ShidenCommand Structure") (Widget :type "/Shiden/Core/WBP_ShidenWidgetBase Object Reference") (ScenarioManager :type "/Shiden/Core/BP_ShidenScenarioManager Object Reference") (HookedObject :type "Object Object Reference"))
  (returns (Status :type "/Shiden/Commands/Core/E_ShidenPreProcessStatus Enum") (ErrorMessage :type String))
  (return "NewEnumerator0" ""))

(fn `PreviewCommand`
  (params (Command :type "ShidenCommand Structure") (Widget :type "/Shiden/Core/WBP_ShidenWidgetBase Object Reference") (IsCurrentCommand :type Boolean))
  (returns (Status :type "/Shiden/Commands/Core/E_ShidenPreviewStatus Enum") (SoundInfo :type "/Shiden/Commands/Primary/F_ShidenSoundInfo Structure") (ErrorMessage :type String))
  (return "NewEnumerator0" (struct) ""))

(fn `ProcessCommand`
  (params (ProcessName :type String) (Command :type "ShidenCommand Structure") (Widget :type "/Shiden/Core/WBP_ShidenWidgetBase Object Reference") (ScenarioManager :type "/Shiden/Core/BP_ShidenScenarioManager Object Reference") (DeltaTime :type "Float (double-precision)") (HookedObject :type "Object Object Reference"))
  (returns (Status :type "/Shiden/Commands/Core/E_ShidenProcessStatus Enum") (BreakReason :type String) (NextScenarioName :type String) (ErrorMessage :type String))
  (locals (TempBoolean :type Boolean))
  (bind (_commandname _presetname _arg1 _arg2 _arg3 _arg4 _arg5) (break `ShidenCommand` Command))
  (bind (_result _bsuccess) (`ShidenVariableFunctionLibrary.ConvertToVariableType` _arg2))
  (bind (_result_2 _bsuccess_2) (`ShidenVariableFunctionLibrary.ConvertToVariableKind` _arg1))
  (if _bsuccess_2
    (bind (_variabletype _bbooleanvalue _stringvalue _integervalue _floatvalue _vector2value _vector3value _breturnvalue) (`ShidenVariableFunctionLibrary.FindVariable` ProcessName _result_2 _arg3))
    (if _breturnvalue
      (if _bsuccess
        (if (`|EnumEquality` _variabletype _result)
          (bind (_bresult _bsuccess_3 _errormessage) (`ShidenVariableFunctionLibrary.EvaluateCondition` _result _arg4 _bbooleanvalue _stringvalue _integervalue _floatvalue _vector2value _vector3value (== _arg5 "true") _arg5 (`KismetStringLibrary.Conv_StringToInt` _arg5) (`KismetStringLibrary.Conv_StringToDouble` _arg5) (`KismetStringLibrary.Conv_StringToVector2D` _arg5) (`KismetStringLibrary.Conv_StringToVector` _arg5)))
          (if _bsuccess_3
            (if _bresult
              (return "NewEnumerator3" "" "" "")
              (else
                (return "NewEnumerator4" "" "" "")))
            (else
              (return "NewEnumerator2" "" "" _errormessage)))
          (else
            (return "NewEnumerator2" "" "" "Variable type not match")))
        (else
          (return "NewEnumerator2" "" "" "Invalid variable type")))
      (else
        (return "NewEnumerator2" "" "" "Variable not found")))
    (else
      (return "NewEnumerator2" "" "" "Invalid variable kind"))))