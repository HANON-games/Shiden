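; Shiden scenario command that eases a scalar material parameter on a named widget Image or RetainerBox.
; PreProcessCommand starts the change through the widget, setting an absolute value or adding to any tracked end value, else the current one.
; ProcessCommand optionally waits for completion, then registers the end value as a scenario property under an escaped type::target::parameter key.
; Save restore replays those keys with zero duration, as does preview for non-current commands.
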(fn `ConvertToEasingFunc`
  (params (EasingFunc :type String))
  (returns (EnumValue :type "EEasingFunc Enum") (Success :type Boolean))
  (switch `string` EasingFunc
    (:`Default`
      (return "Linear" false))
    (:`Linear`
      (return "Linear" true))
    (:`Step`
      (return "Step" true))
    (:`Sinusoidal in`
      (return "SinusoidalIn" true))
    (:`Sinusoidal out`
      (return "SinusoidalOut" true))
    (:`Sinusoidal in out`
      (return "SinusoidalInOut" true))
    (:`Ease in`
      (return "EaseIn" true))
    (:`Ease out`
      (return "EaseOut" true))
    (:`Ease in out`
      (return "EaseInOut" true))
    (:`Expo in`
      (return "ExpoIn" true))
    (:`Expo out`
      (return "ExpoOut" true))
    (:`Expo in out`
      (return "ExpoInOut" true))
    (:`Circular in`
      (return "CircularIn" true))
    (:`Circular out`
      (return "CircularOut" true))
    (:`Circular in out`
      (return "CircularInOut" true))))

(fn `GetAssetPaths`
  (params (Command :type "ShidenCommand Structure"))
  (returns (AssetObjectPaths :type "Set of String"))
  (return))

(fn `GetEndValueFromImageMaterial Params`
  (params (Widget :type "/Shiden/Core/WBP_ShidenWidgetBase Object Reference") (Command :type "ShidenCommand Structure (by ref)"))
  (returns (EndValue :type "Float (double-precision)") (Found :type Boolean))
  (bind (_commandname _presetname _arg1 _arg2 _arg3) (break `ShidenCommand` Command))
  (bind (_value _returnvalue) (`BlueprintMapLibrary.Map_Find` (`/Shiden/Core/WBP_ShidenWidgetBase.ImageMaterialParams` Widget) (`/Shiden/Core/WBP_ShidenWidgetBase.MakeMaterialParamsKey` Widget _arg2 _arg3)))
  (return (`.EndValue_36_3B4C2D63463609B909999B8B58DFE59C` (break `/Shiden/Commands/Primary/F_ShidenImageMaterialScalarParams` _value)) _returnvalue))

(fn `GetEndValueFromRetainerMaterial Params`
  (params (Widget :type "/Shiden/Core/WBP_ShidenWidgetBase Object Reference") (Command :type "ShidenCommand Structure (by ref)"))
  (returns (EndValue :type "Float (double-precision)") (Found :type Boolean))
  (bind (_commandname _presetname _arg1 _arg2 _arg3) (break `ShidenCommand` Command))
  (bind (_value _returnvalue) (`BlueprintMapLibrary.Map_Find` (`/Shiden/Core/WBP_ShidenWidgetBase.RetainerMaterialParams` Widget) (`/Shiden/Core/WBP_ShidenWidgetBase.MakeMaterialParamsKey` Widget _arg2 _arg3)))
  (return (`.EndValue_36_3B4C2D63463609B909999B8B58DFE59C` (break `/Shiden/Commands/Primary/F_ShidenRetainerMaterialScalarParams` _value)) _returnvalue))

(fn `InitFromSaveData`
  (params (KeyValueMap :type "Map of String to String") (Widget :type "/Shiden/Core/WBP_ShidenWidgetBase Object Reference") (ScenarioManager :type "/Shiden/Core/BP_ShidenScenarioManager Object Reference"))
  (returns (Success :type "/Shiden/Commands/Core/E_ShidenInitFromSaveDataStatus Enum") (ErrorMessage :type String))
  (bind _keys (`BlueprintMapLibrary.Map_Keys` KeyValueMap))
  (for _array_element _keys
    (bind (_targettype _targetname _parametername) (`self.ParseCurrentKey` _array_element))
    (bind (_success _errormessage) (`self.StartChangeParameter` (make `ShidenCommand` "ChangeMaterialScalarParameter" "" _targettype _targetname _parametername "Linear" "0.0" "AbsoluteValue" (`BlueprintMapLibrary.Map_Find` KeyValueMap _array_element)) Widget "Default"))
    (if (not _success)
      (return "NewEnumerator2" _errormessage)))
  (return "NewEnumerator0" ""))

(fn `MakeCurrentKey`
  (params (TargetType :type String) (TargetName :type String) (ParameterName :type String))
  (returns (ReturnValue :type String))
  (return (`KismetStringLibrary.Concat_StrStr` (`KismetStringLibrary.Replace` TargetType ":" "\\:") "::" (`KismetStringLibrary.Replace` TargetName ":" "\\:") "::" (`KismetStringLibrary.Replace` ParameterName ":" "\\:"))))

(fn `ParseCurrentKey`
  (params (Key :type String))
  (returns (TargetType :type String) (TargetName :type String) (ParameterName :type String))
  (bind (_lefts _rights) (`KismetStringLibrary.Split` Key "::"))
  (bind (_lefts_2 _rights_2) (`KismetStringLibrary.Split` _rights "::"))
  (return (`KismetStringLibrary.Replace` _lefts "\\:" ":") (`KismetStringLibrary.Replace` _lefts_2 "\\:" ":") (`KismetStringLibrary.Replace` _rights_2 "\\:" ":")))

(fn `PreProcessCommand`
  (params (ProcessName :type String) (Command :type "ShidenCommand Structure") (Widget :type "/Shiden/Core/WBP_ShidenWidgetBase Object Reference") (ScenarioManager :type "/Shiden/Core/BP_ShidenScenarioManager Object Reference") (HookedObject :type "Object Object Reference"))
  (returns (Status :type "/Shiden/Commands/Core/E_ShidenPreProcessStatus Enum") (ErrorMessage :type String))
  (bind (_success _errormessage) (`self.StartChangeParameter` Command Widget ProcessName))
  (if _success
    (return "NewEnumerator0" "")
    (else
      (return "NewEnumerator2" _errormessage))))

(fn `PreviewCommand`
  (params (Command :type "ShidenCommand Structure") (Widget :type "/Shiden/Core/WBP_ShidenWidgetBase Object Reference") (IsCurrentCommand :type Boolean))
  (returns (Status :type "/Shiden/Commands/Core/E_ShidenPreviewStatus Enum") (SoundInfo :type "/Shiden/Commands/Primary/F_ShidenSoundInfo Structure") (ErrorMessage :type String))
  (if IsCurrentCommand
    (bind (_success _errormessage) (`self.StartChangeParameter` Command Widget "Default"))
    (if _success
      (return "NewEnumerator0" (struct) "")
      (else
        (return "NewEnumerator2" (struct) _errormessage)))
    (else
      (bind _structout (setmembers `ShidenCommand` :`StructRef` Command :`Arg5` "0.0")) ; Override dulation
      (bind (_success_2 _errormessage_2) (`self.StartChangeParameter` _structout Widget "Default"))
      (if _success_2
        (return "NewEnumerator0" (struct) "")
        (else
          (return "NewEnumerator2" (struct) _errormessage_2))))))

(fn `ProcessCommand`
  (params (ProcessName :type String) (Command :type "ShidenCommand Structure") (Widget :type "/Shiden/Core/WBP_ShidenWidgetBase Object Reference") (ScenarioManager :type "/Shiden/Core/BP_ShidenScenarioManager Object Reference") (DeltaTime :type "Float (double-precision)") (HookedObject :type "Object Object Reference"))
  (returns (Status :type "/Shiden/Commands/Core/E_ShidenProcessStatus Enum") (BreakReason :type String) (NextScenarioName :type String) (ErrorMessage :type String))
  (bind (_commandname _presetname _arg1 _arg2 _arg3 _arg4 _arg5 _arg6 _arg7 _arg8 _arg9 _arg10) (break `ShidenCommand` Command))
  (if (`KismetStringLibrary.EqualEqual_StrStr` _arg10 "true")
    (if (`KismetStringLibrary.EqualEqual_StrStr` _arg1 "RetainerBox")
      (bind _result (`/Shiden/Core/WBP_ShidenWidgetBase.IsRetainerParameterChangeEnd` Widget _arg2 _arg3))
      (if _result
        _
        (else
          (return "NewEnumerator4" "" "" "")))
      (else
        (bind _result_2 (`/Shiden/Core/WBP_ShidenWidgetBase.IsImageParameterChangeEnd` Widget _arg2 _arg3))
        (if _result_2
          _
          (else
            (return "NewEnumerator4" "" "" ""))))))
  (`ShidenCommandFunctionLibrary.RegisterCurrentScenarioProperty` (`.CommandName` (break `ShidenCommand` (`local.Command`))) (`self.MakeCurrentKey` _arg1 _arg2 _arg3) (`KismetStringLibrary.Conv_DoubleToString` (`self.EndValue`)))
  (return "NewEnumerator3" "" "" ""))

(fn `Start Image Material Change`
  (params (Command :type "ShidenCommand Structure (by ref)") (Widget :type "/Shiden/Core/WBP_ShidenWidgetBase Object Reference") (Image :type "Image Object Reference") (EasingFunction :type "EEasingFunc Enum" :default "Linear") (OwnerProcessName :type String))
  (returns (Success :type Boolean) (ErrorMessage :type String))
  (bind (_commandname _presetname _arg1 _arg2 _arg3) (break `ShidenCommand` Command))
  (bind (_endvalue _found) (`self.GetEndValueFromImageMaterial Params` Widget Command))
  (bind (_commandname_2 _presetname_2 _arg1_2 _arg2_2 _arg3_2 _arg4 _arg5 _arg6 _arg7 _arg8 _arg9) (break `ShidenCommand` (`local.Command`)))
  (bind (_commandname_3 _presetname_3 _arg1_3 _arg2_3 _arg3_3 _arg4_2 _arg5_2 _arg6_2 _arg7_2) (break `ShidenCommand` (`local.Command`)))
  (bind _returnvalue (`KismetStringLibrary.Conv_StringToDouble` _arg7_2))
  (bind _returnvalue_2 (`MaterialInstanceDynamic.K2_GetScalarParameterValue` (`WidgetBlueprintLibrary.GetDynamicMaterial` (`Image.Brush` (`BlueprintMapLibrary.Map_Find` (`/Shiden/Core/WBP_ShidenWidgetBase.GetImages` (`local.Widget`)) _arg2))) (`KismetStringLibrary.Conv_StringToName` _arg3)))
  (bind _returnvalue_3 (`KismetMathLibrary.SelectFloat` (+ _returnvalue (`KismetMathLibrary.SelectFloat` _endvalue _returnvalue_2 _found)) _returnvalue (`KismetStringLibrary.EqualEqual_StrStr` _arg6_2 "AddToCurrent")))
  (bind (_success _errormessage) (`/Shiden/Core/WBP_ShidenWidgetBase.StartImageMaterialScalarChange` (`local.Widget`) _arg2_2 (`local.Image`) (`KismetStringLibrary.Conv_StringToName` _arg3_2) (`local.EasingFunction`) (`KismetStringLibrary.Conv_StringToDouble` _arg5) _returnvalue_3 (`KismetStringLibrary.Conv_StringToDouble` _arg9) (`KismetStringLibrary.Conv_StringToInt` _arg8) (`local.OwnerProcessName`)))
  (if _success
    (set `self.EndValue` _returnvalue_3)
    (return true "")
    (else
      (return false _errormessage))))

(fn `StartChangeParameter`
  (params (Command :type "ShidenCommand Structure (by ref)") (Widget :type "/Shiden/Core/WBP_ShidenWidgetBase Object Reference") (OwnerProcessName :type String))
  (returns (Success :type Boolean) (ErrorMessage :type String))
  (bind (_commandname _presetname _arg1 _arg2) (break `ShidenCommand` Command))
  (bind (_value _returnvalue) (`BlueprintMapLibrary.Map_Find` (`/Shiden/Core/WBP_ShidenWidgetBase.GetImages` (`local.Widget`)) _arg2))
  (bind (_enumvalue _success) (`self.ConvertToEasingFunc` (`.Arg4` (break `ShidenCommand` (`local.Command`)))))
  (bind (_enumvalue_2 _success_2) (`self.ConvertToEasingFunc` (`.Arg4` (break `ShidenCommand` (`local.Command`)))))
  (bind (_value_2 _returnvalue_2) (`BlueprintMapLibrary.Map_Find` (`/Shiden/Core/WBP_ShidenWidgetBase.GetRetainerBoxes` (`local.Widget`)) (`.Arg2` (break `ShidenCommand` (`local.Command`)))))
  (if (== _arg1 "RetainerBox")
    (if _returnvalue_2
      (if _success_2
        (bind (_success_3 _errormessage) (`self.StartRetainerMaterialChange` Command (`local.Widget`) _value_2 _enumvalue_2 (`local.OwnerProcessName`)))
        (return _success_3 _errormessage)
        (else
          (return false "Invalid ease func")))
      (else
        (return false "Retainer Box not found")))
    (elif _returnvalue
      (if _success
        (bind (_success_4 _errormessage_2) (`self.Start Image Material Change` (`local.Command`) (`local.Widget`) _value _enumvalue (`local.OwnerProcessName`)))
        (return _success_4 _errormessage_2)
        (else
          (return false "Invalid ease func")))
      (else
        (return false "Image not found")))))

(fn `StartRetainerMaterialChange`
  (params (Command :type "ShidenCommand Structure (by ref)") (Widget :type "/Shiden/Core/WBP_ShidenWidgetBase Object Reference") (RetainerBox :type "RetainerBox Object Reference") (EasingFunction :type "EEasingFunc Enum" :default "Linear") (`Owner Process Name` :type String))
  (returns (Success :type Boolean) (ErrorMessage :type String))
  (bind (_commandname _presetname _arg1 _arg2 _arg3) (break `ShidenCommand` Command))
  (bind (_endvalue _found) (`self.GetEndValueFromRetainerMaterial Params` Widget Command))
  (bind (_commandname_2 _presetname_2 _arg1_2 _arg2_2 _arg3_2 _arg4 _arg5 _arg6 _arg7 _arg8 _arg9) (break `ShidenCommand` (`local.Command`)))
  (bind (_commandname_3 _presetname_3 _arg1_3 _arg2_3 _arg3_3 _arg4_2 _arg5_2 _arg6_2 _arg7_2) (break `ShidenCommand` (`local.Command`)))
  (bind _returnvalue (`KismetStringLibrary.Conv_StringToDouble` _arg7_2))
  (bind _returnvalue_2 (`MaterialInstanceDynamic.K2_GetScalarParameterValue` (`RetainerBox.GetEffectMaterial` (`BlueprintMapLibrary.Map_Find` (`/Shiden/Core/WBP_ShidenWidgetBase.GetRetainerBoxes` (`local.Widget`)) _arg2)) (`KismetStringLibrary.Conv_StringToName` _arg3)))
  (bind _returnvalue_3 (`KismetMathLibrary.SelectFloat` (+ _returnvalue (`KismetMathLibrary.SelectFloat` _endvalue _returnvalue_2 _found)) _returnvalue (`KismetStringLibrary.EqualEqual_StrStr` _arg6_2 "AddToCurrent")))
  (bind (_success _errormessage) (`/Shiden/Core/WBP_ShidenWidgetBase.StartRetainerMaterialScalarChange` (`local.Widget`) _arg2_2 (`local.RetainerBox`) (`KismetStringLibrary.Conv_StringToName` _arg3_2) (`local.EasingFunction`) (`KismetStringLibrary.Conv_StringToDouble` _arg5) _returnvalue_3 (`KismetStringLibrary.Conv_StringToDouble` _arg9) (`KismetStringLibrary.Conv_StringToInt` _arg8) (`local.Owner Process Name`)))
  (if _success
    (set `self.EndValue` _returnvalue_3)
    (return true "")
    (else
      (return false _errormessage))))