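; Shiden scenario command that implements Jump, moving a running scenario process to a named Tag command.
; It looks up the process's current scenario in the cache and scans its commands for a Tag whose first argument matches the Jump argument.
; A match sets the current scenario index to that position; otherwise it returns a tag-not-found error.
; The other command hooks, such as preview, preprocess and save restore, are placeholders.
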(fn `FindNextIndex`
  (params (ProcessName :type String) (Command :type "ShidenCommand Structure (by ref)") (ScenarioManager :type "/Shiden/Core/BP_ShidenScenarioManager Object Reference"))
  (returns (Success :type Boolean) (`Array Index` :type Integer) (ErrorMessage :type String))
  (bind (_commandname _presetname _arg1) (break `ShidenCommand` Command))
  (bind _scenarioprogress (`ShidenScenarioFunctionLibrary.PeekScenario` ProcessName))
  (bind _scenario (`ShidenInternalFunctionLibrary.GetScenarioFromCache` (break `ShidenScenarioProgress` _scenarioprogress)))
  (for (_array_element _array_index) (`ShidenScenario.Commands` _scenario)
    (bind (_commandname_2 _presetname_2 _arg1_2) (break `ShidenCommand` _array_element))
    (if (and (`KismetStringLibrary.EqualEqual_StrStr` _commandname_2 "Tag") (`KismetStringLibrary.EqualEqual_StrStr` _arg1_2 _arg1))
      (return true _array_index "")))
  (return false 0 (`KismetStringLibrary.Concat_StrStr` "Tag " _arg1 " is not found")))

(fn `GetAssetPaths`
  (params (Command :type "ShidenCommand Structure"))
  (returns (AssetObjectPaths :type "Set of String"))
  (return))

(fn `InitFromSaveData`
  (params (KeyValueMap :type "Map of String to String") (Widget :type "/Shiden/Core/WBP_ShidenWidgetBase Object Reference") (ScenarioManager :type "/Shiden/Core/BP_ShidenScenarioManager Object Reference"))
  (returns (Success :type "/Shiden/Commands/Core/E_ShidenInitFromSaveDataStatus Enum") (ErrorMessage :type String))
  (return "NewEnumerator0" ""))

(fn `PreProcessCommand`
  (params (ProcessName :type String) (Command :type "ShidenCommand Structure") (Widget :type "/Shiden/Core/WBP_ShidenWidgetBase Object Reference") (ScenarioManager :type "/Shiden/Core/BP_ShidenScenarioManager Object Reference") (HookedObject :type "Object Object Reference"))
  (returns (Status :type "/Shiden/Commands/Core/E_ShidenPreProcessStatus Enum") (ErrorMessage :type String))
  (return "NewEnumerator0" ""))

(fn `PreviewCommand`
  (params (Command :type "ShidenCommand Structure") (Widget :type "/Shiden/Core/WBP_ShidenWidgetBase Object Reference") (IsCurrentCommand :type Boolean))
  (returns (Status :type "/Shiden/Commands/Core/E_ShidenPreviewStatus Enum") (SoundInfo :type "/Shiden/Commands/Primary/F_ShidenSoundInfo Structure") (ErrorMessage :type String))
  (return "NewEnumerator0" (struct) ""))

(fn `ProcessCommand`
  (params (ProcessName :type String) (Command :type "ShidenCommand Structure") (Widget :type "/Shiden/Core/WBP_ShidenWidgetBase Object Reference") (ScenarioManager :type "/Shiden/Core/BP_ShidenScenarioManager Object Reference") (DeltaTime :type "Float (double-precision)") (HookedObject :type "Object Object Reference"))
  (returns (Status :type "/Shiden/Commands/Core/E_ShidenProcessStatus Enum") (BreakReason :type String) (NextScenarioName :type String) (ErrorMessage :type String))
  (bind (_success _array_index _errormessage) (`self.FindNextIndex` ProcessName Command ScenarioManager))
  (if _success
    (`ShidenScenarioFunctionLibrary.SetCurrentScenarioIndex` (`local.ProcessName`) _array_index)
    (return "NewEnumerator3" "" "" "")
    (else
      (return "NewEnumerator2" "" "" _errormessage))))