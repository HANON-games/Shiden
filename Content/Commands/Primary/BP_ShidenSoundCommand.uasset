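; Shiden scenario command that plays BGM, SE or Voice through the ScenarioManager, parsing track, path, playback and fade settings from command args.
; Only BGM registers scenario properties per track, which InitFromSaveData replays on load.
; An empty or "None" path clears BGM properties and is still forwarded for BGM and Voice, while SE skips it.
; Preview builds the same sound info, zeroing fade duration for non-current commands.
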(fn `ConvertToAudioFaderCurve`
  (params (AudioFaderCurve :type String))
  (returns (EnumValue :type "EAudioFaderCurve Enum") (Success :type Boolean))
  (switch `string` AudioFaderCurve
    (:`Default`
      (return "Linear" false))
    (:`Linear`
      (return "Linear" true))
    (:`Logarithmic`
      (return "Logarithmic" true))
    (:`Sin (S-Curve)`
      (return "SCurve" true))
    (:`Sin (Equal Power)`
      (return "Sin" true))))

(fn `GetAssetPaths`
  (params (Command :type "ShidenCommand Structure"))
  (returns (AssetObjectPaths :type "Set of String"))
  (return (`|MakeSet` Command_Arg3)))

(fn `InitFromSaveData`
  (params (KeyValueMap :type "Map of String to String") (Widget :type "/Shiden/Core/WBP_ShidenWidgetBase Object Reference") (ScenarioManager :type "/Shiden/Core/BP_ShidenScenarioManager Object Reference"))
  (returns (Success :type "/Shiden/Commands/Core/E_ShidenInitFromSaveDataStatus Enum") (ErrorMessage :type String))
  (bind _keys (`BlueprintMapLibrary.Map_Keys` KeyValueMap))
  (for _array_element _keys
    (if (`KismetStringLibrary.EndsWith` _array_element "::Path")
      (bind (_value _returnvalue) (`BlueprintMapLibrary.Map_Find` KeyValueMap _array_element))
      (bind _lefts (`KismetStringLibrary.Split` _array_element "::" "IgnoreCase" "FromEnd"))
      (bind (_value_2 _returnvalue_2) (`BlueprintMapLibrary.Map_Find` KeyValueMap (`KismetStringLibrary.Concat_StrStr` _lefts "::Volume")))
      (bind (_value_3 _returnvalue_3) (`BlueprintMapLibrary.Map_Find` KeyValueMap (`KismetStringLibrary.Concat_StrStr` _lefts "::Pitch")))
      (bind (_value_4 _returnvalue_4) (`BlueprintMapLibrary.Map_Find` KeyValueMap (`KismetStringLibrary.Concat_StrStr` _lefts "::StartTime")))
      (if (and _returnvalue _returnvalue_2 _returnvalue_3 _returnvalue_4)
        (bind _success (`/Shiden/Core/BP_ShidenScenarioManager.PlaySound2d` ScenarioManager (make `/Shiden/Commands/Primary/F_ShidenSoundInfo` (`KismetStringLibrary.Conv_StringToInt` _lefts) "NewEnumerator1" _value (`KismetStringLibrary.Conv_StringToDouble` _value_2) (`KismetStringLibrary.Conv_StringToDouble` _value_3) (`KismetStringLibrary.Conv_StringToDouble` _value_4))))
        (if (not _success)
          (return "NewEnumerator2" "Play Sound 2d failed"))
        (else
          (return "NewEnumerator0" "")))))
  (return "NewEnumerator0" ""))

(fn `PreProcessCommand`
  (params (ProcessName :type String) (Command :type "ShidenCommand Structure") (Widget :type "/Shiden/Core/WBP_ShidenWidgetBase Object Reference") (ScenarioManager :type "/Shiden/Core/BP_ShidenScenarioManager Object Reference") (HookedObject :type "Object Object Reference"))
  (returns (Status :type "/Shiden/Commands/Core/E_ShidenPreProcessStatus Enum") (ErrorMessage :type String))
  (return "NewEnumerator0" ""))

(fn `PreviewCommand`
  (params (Command :type "ShidenCommand Structure") (Widget :type "/Shiden/Core/WBP_ShidenWidgetBase Object Reference") (IsCurrentCommand :type Boolean))
  (returns (Status :type "/Shiden/Commands/Core/E_ShidenPreviewStatus Enum") (SoundInfo :type "/Shiden/Commands/Primary/F_ShidenSoundInfo Structure") (ErrorMessage :type String))
  (bind _enumvalue (foreach `/Shiden/Commands/Primary/E_ShidenSoundType` false)
    (:`LoopBody`
      (if (`KismetStringLibrary.EqualEqual_StrStr` Command_Arg1 (`|GetEnumeratorNameAsString` _enumvalue))
        (return "NewEnumerator0" (make `/Shiden/Commands/Primary/F_ShidenSoundInfo` (`KismetStringLibrary.Conv_StringToInt` Command_Arg2) _enumvalue Command_Arg3 (`KismetStringLibrary.Conv_StringToDouble` Command_Arg4) (`KismetStringLibrary.Conv_StringToDouble` Command_Arg5) (`KismetStringLibrary.Conv_StringToDouble` Command_Arg6) (== Command_Arg7 "FadeOut") (`self.ConvertToAudioFaderCurve` Command_Arg8) (`KismetMathLibrary.SelectFloat` (`KismetStringLibrary.Conv_StringToDouble` Command_Arg9) 0.0 IsCurrentCommand) (== Command_Arg10 "true")) "")))
    (:`then`
      (return "NewEnumerator2" (struct) "Invalid SoundType"))))

(fn `ProcessCommand`
  (params (ProcessName :type String) (Command :type "ShidenCommand Structure") (Widget :type "/Shiden/Core/WBP_ShidenWidgetBase Object Reference") (ScenarioManager :type "/Shiden/Core/BP_ShidenScenarioManager Object Reference") (DeltaTime :type "Float (double-precision)") (HookedObject :type "Object Object Reference"))
  (returns (Status :type "/Shiden/Commands/Core/E_ShidenProcessStatus Enum") (BreakReason :type String) (NextScenarioName :type String) (ErrorMessage :type String))
  (locals (SoundType :type "/Shiden/Commands/Primary/E_ShidenSoundType Enum"))
  (bind (_commandname _presetname _arg1 _arg2 _arg3 _arg4 _arg5 _arg6) (break `ShidenCommand` Command))
  (bind (_commandname_2 _presetname_2 _arg1_2 _arg2_2 _arg3_2 _arg4_2 _arg5_2 _arg6_2 _arg7 _arg8 _arg9 _arg10) (break `ShidenCommand` Command))
  (bind (_commandname_3 _presetname_3 _arg1_3 _arg2_3 _arg3_3 _arg4_3 _arg5_3 _arg6_3 _arg7_2 _arg8_2 _arg9_2 _arg10_2) (break `ShidenCommand` (`local.Command`)))
  (bind _returnvalue (`KismetStringLibrary.Conv_StringToInt` _arg2_2))
  (bind (_enumvalue _success) (`self.ConvertToAudioFaderCurve` _arg8_2))
  (if (or (`KismetStringLibrary.EqualEqual_StrStr` _arg3) (`KismetStringLibrary.IsEmpty` _arg3))
    (switch `string` _arg1
      (:`BGM`
        (`self.RemoveProperties` _commandname_2 _returnvalue)
        (set `local.SoundType` "NewEnumerator1")
        (bind _success_2 (`/Shiden/Core/BP_ShidenScenarioManager.PlaySound2d` (`local.ScenarioManager`) (make `/Shiden/Commands/Primary/F_ShidenSoundInfo` _returnvalue (`local.SoundType`) _arg3_2 (`KismetStringLibrary.Conv_StringToDouble` _arg4_2) (`KismetStringLibrary.Conv_StringToDouble` _arg5_2) (`KismetStringLibrary.Conv_StringToDouble` _arg6_2) (== _arg7 "FadeOut") (`self.ConvertToAudioFaderCurve` _arg8) (`KismetStringLibrary.Conv_StringToDouble` _arg9) (== _arg10 "true")) :!label _label))
        (if _success_2
          _
          (else
            (return "NewEnumerator2" "" "" "Play Sound Failed"))))
      (:`SE`
        _)
      (:`Voice`
        (set `local.SoundType` "NewEnumerator3")
        (goto _label)))
    (else
      (switch `string` _arg1
        (:`BGM`
          (`self.RegisterProperties` (`.CommandName` (break `ShidenCommand` (`local.Command`))) (`KismetStringLibrary.Conv_StringToInt` _arg2) _arg3 _arg4 _arg5 _arg6)
          (set `local.SoundType` "NewEnumerator1"))
        (:`SE`
          (set `local.SoundType` "NewEnumerator2"))
        (:`Voice`
          (set `local.SoundType` "NewEnumerator3")))
      (if _success
        (`/Shiden/Core/BP_ShidenScenarioManager.PlaySound2d` ScenarioManager (make `/Shiden/Commands/Primary/F_ShidenSoundInfo` (`KismetStringLibrary.Conv_StringToInt` _arg2_3) (`local.SoundType`) _arg3_3 (`KismetStringLibrary.Conv_StringToDouble` _arg4_3) (`KismetStringLibrary.Conv_StringToDouble` _arg5_3) (`KismetStringLibrary.Conv_StringToDouble` _arg6_3) (== _arg7_2 "FadeOut") _enumvalue (`KismetStringLibrary.Conv_StringToDouble` _arg9_2) (== _arg10_2 "true")))
        (bind _success_3 (`/Shiden/Core/BP_ShidenScenarioManager.PlaySound2d` (`local.ScenarioManager`) (make `/Shiden/Commands/Primary/F_ShidenSoundInfo` (`KismetStringLibrary.Conv_StringToInt` _arg2_3) (`local.SoundType`) _arg3_3 (`KismetStringLibrary.Conv_StringToDouble` _arg4_3) (`KismetStringLibrary.Conv_StringToDouble` _arg5_3) (`KismetStringLibrary.Conv_StringToDouble` _arg6_3) (== _arg7_2 "FadeOut") _enumvalue (`KismetStringLibrary.Conv_StringToDouble` _arg9_2) (== _arg10_2 "true"))))
        (if _success_3
          _
          (else
            (return "NewEnumerator2" "" "" "Play Sound Failed")))
        (else
          (return "NewEnumerator2" "" "" (`KismetStringLibrary.Concat_StrStr` "\"" _arg8_2 "\" is Invalid Audio Fader Curve"))))))
  (return "NewEnumerator3" "" "" ""))

(fn `RegisterProperties`
  (params (CommandName :type String) (TrackId :type Integer) (Path :type String) (Volume :type String) (Pitch :type String) (StartTime :type String))
  (bind _returnvalue (`KismetStringLibrary.Conv_IntToString` TrackId))
  (`ShidenCommandFunctionLibrary.RegisterCurrentScenarioProperty` CommandName (`KismetStringLibrary.Concat_StrStr` _returnvalue "::Path") Path)
  (`ShidenCommandFunctionLibrary.RegisterCurrentScenarioProperty` CommandName (`KismetStringLibrary.Concat_StrStr` _returnvalue "::Volume") Volume)
  (`ShidenCommandFunctionLibrary.RegisterCurrentScenarioProperty` CommandName (`KismetStringLibrary.Concat_StrStr` _returnvalue "::Pitch") Pitch)
  (`ShidenCommandFunctionLibrary.RegisterCurrentScenarioProperty` CommandName (`KismetStringLibrary.Concat_StrStr` _returnvalue "::StartTime") StartTime))

(fn `RemoveProperties`
  (params (CommandName :type String) (TrackId :type Integer))
  (bind _returnvalue (`KismetStringLibrary.Conv_IntToString` TrackId))
  (`ShidenCommandFunctionLibrary.RemoveCurrentScenarioProperty` CommandName (`KismetStringLibrary.Concat_StrStr` _returnvalue "::Path"))
  (`ShidenCommandFunctionLibrary.RemoveCurrentScenarioProperty` CommandName (`KismetStringLibrary.Concat_StrStr` _returnvalue "::Volume"))
  (`ShidenCommandFunctionLibrary.RemoveCurrentScenarioProperty` CommandName (`KismetStringLibrary.Concat_StrStr` _returnvalue "::Pitch"))
  (`ShidenCommandFunctionLibrary.RemoveCurrentScenarioProperty` CommandName (`KismetStringLibrary.Concat_StrStr` _returnvalue "::StartTime")))