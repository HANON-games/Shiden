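; Shiden scenario command that starts a macro scenario as a parallel process under a given name.
; ProcessCommand rejects the name "Default", already running processes and missing macros, then pushes the scenario and calls CallMacroAsParallel on the scenario manager.
; SetMacroArguments writes up to five typed arguments as process-local variables, using defaults for empty values and stopping at the first unnamed slot.
; The other command hooks are stubs.
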(fn `GetAssetPaths`
  (params (Command :type "ShidenCommand Structure"))
  (returns (AssetObjectPaths :type "Set of String"))
  (return))

(fn `InitFromSaveData`
  (params (KeyValueMap :type "Map of String to String") (Widget :type "/Shiden/Core/WBP_ShidenWidgetBase Object Reference") (ScenarioManager :type "/Shiden/Core/BP_ShidenScenarioManager Object Reference"))
  (returns (Success :type "/Shiden/Commands/Core/E_ShidenInitFromSaveDataStatus Enum") (ErrorMessage :type String))
  (return "NewEnumerator0" ""))

(fn `PreProcessCommand`
  (params (ProcessName :type String) (Command :type "ShidenCommand Structure") (Widget :type "/Shiden/Core/WBP_ShidenWidgetBase Object Reference") (ScenarioManager :type "/Shiden/Core/BP_ShidenScenarioManager Object Reference") (HookedObject :type "Object Object Reference"))
  (returns (Status :type "/Shiden/Commands/Core/E_ShidenPreProcessStatus Enum") (ErrorMessage :type String))
  (return "NewEnumerator0" ""))

(fn `PreviewCommand`
  (params (Command :type "ShidenCommand Structure") (Widget :type "/Shiden/Core/WBP_ShidenWidgetBase Object Reference") (IsCurrentCommand :type Boolean))
  (returns (Status :type "/Shiden/Commands/Core/E_ShidenPreviewStatus Enum") (SoundInfo :type "/Shiden/Commands/Primary/F_ShidenSoundInfo Structure") (ErrorMessage :type String))
  (return "NewEnumerator0" (struct) ""))

(fn `ProcessCommand`
  (params (ProcessName :type String) (Command :type "ShidenCommand Structure") (Widget :type "/Shiden/Core/WBP_ShidenWidgetBase Object Reference") (ScenarioManager :type "/Shiden/Core/BP_ShidenScenarioManager Object Reference") (DeltaTime :type "Float (double-precision)") (HookedObject :type "Object Object Reference"))
  (returns (Status :type "/Shiden/Commands/Core/E_ShidenProcessStatus Enum") (BreakReason :type String) (NextScenarioName :type String) (ErrorMessage :type String))
  (locals (NewLocalVar :type String))
  (if (`KismetStringLibrary.NotEqual_StrStr` Command_Arg1 "Default")
    (bind (_scenarioprogress _cancelinfo _bislastelement _bismacro _bsuccess) (`ShidenScenarioFunctionLibrary.PeekScenario` Command_Arg1))
    (if _bsuccess
      (return "NewEnumerator2" "" "" (`KismetStringLibrary.Concat_StrStr` "Process \"" Command_Arg1 "\" is already running"))
      (else
        (bind (_scenarioid _scenario _succeeded) (`/Shiden/Libraries/BP_ShidenInternalFunctionLibrary.GetScenarioByIdOrObjectPath` Command_Arg2 (`local.ScenarioManager`)))
        (if _succeeded
          (`ShidenScenarioFunctionLibrary.PushScenario` Command_Arg1 _scenario)
          (`self.SetMacroArguments` Command_Arg1 (`local.ScenarioManager`) _scenario Command_Arg3 Command_Arg4 Command_Arg5 Command_Arg6 Command_Arg7)
          (`/Shiden/Core/BP_ShidenScenarioManager.CallMacroAsParallel` (`local.ScenarioManager`) Command_Arg1 Widget HookedObject)
          (return "NewEnumerator3" "" "" "")
          (else
            (return "NewEnumerator2" "" "" (`KismetStringLibrary.Concat_StrStr` "Macro \"" Command_Arg2 "\" is not found."))))))
    (else
      (return "NewEnumerator2" "" "" "Cannot use \"Default\" as parallel process name"))))

(fn `SetMacroArguments`
  (params (ProcessName :type String) (ScenarioManager :type "/Shiden/Core/BP_ShidenScenarioManager Object Reference") (ShidenScenario :type "ShidenScenario Object Reference") (Arg1Value :type String) (Arg2Value :type String) (Arg3Value :type String) (Arg4Value :type String) (Arg5Value :type String))
  (bind _processname (`local.ProcessName`))
  (for _index (range 5)
    (bind _returnvalue (select `int` _index :`0` (`ShidenScenario.Arg1Name` ShidenScenario) :`1` (`ShidenScenario.Arg2Name` ShidenScenario) :`2` (`ShidenScenario.Arg3Name` ShidenScenario) :`3` (`ShidenScenario.Arg4Name` ShidenScenario) :`4` (`ShidenScenario.Arg5Name` ShidenScenario)))
    (if (not (`KismetStringLibrary.IsEmpty` _returnvalue))
      (switch `EShidenVariableType` (select `int` _index :`0` (`ShidenScenario.Arg1Type` ShidenScenario) :`1` (`ShidenScenario.Arg2Type` ShidenScenario) :`2` (`ShidenScenario.Arg3Type` ShidenScenario) :`3` (`ShidenScenario.Arg4Type` ShidenScenario) :`4` (`ShidenScenario.Arg5Type` ShidenScenario))
        (:`Boolean`
          (bind _returnvalue_2 (select `int` _index :`0` Arg1Value :`1` Arg2Value :`2` Arg3Value :`3` Arg4Value :`4` Arg5Value))
          (bind _returnvalue_3 (`KismetMathLibrary.SelectString` (select `int` _index :`0` (`ShidenScenario.Arg1DefaultValue` ShidenScenario) :`1` (`ShidenScenario.Arg2DefaultValue` ShidenScenario) :`2` (`ShidenScenario.Arg3DefaultValue` ShidenScenario) :`3` (`ShidenScenario.Arg4DefaultValue` ShidenScenario) :`4` (`ShidenScenario.Arg5DefaultValue` ShidenScenario)) _returnvalue_2 (`KismetStringLibrary.IsEmpty` _returnvalue_2)))
          (`ShidenVariableFunctionLibrary.AddLocalBoolean` _processname _returnvalue (== _returnvalue_3 "true")))
        (:`String`
          (`ShidenVariableFunctionLibrary.AddLocalString` _processname _returnvalue _returnvalue_3))
        (:`Integer`
          (`ShidenVariableFunctionLibrary.AddLocalInteger` _processname _returnvalue (`KismetStringLibrary.Conv_StringToInt` _returnvalue_3)))
        (:`Float`
          (`ShidenVariableFunctionLibrary.AddLocalFloat` _processname _returnvalue (`KismetStringLibrary.Conv_StringToDouble` _returnvalue_3)))
        (:`Vector2`
          (`ShidenVariableFunctionLibrary.AddLocalVector2` _processname _returnvalue (`KismetStringLibrary.Conv_StringToVector2D` _returnvalue_3)))
        (:`Vector3`
          (`ShidenVariableFunctionLibrary.AddLocalVector3` _processname _returnvalue (`KismetStringLibrary.Conv_StringToVector` _returnvalue_3))))
      (else
        (break))))
  (return))