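; Shiden scenario command that types localized dialogue into a named text slot, with optional voice.
; PreProcess resolves the slot, appends to backlog text or starts fresh, and starts voice.
; Process reveals parsed characters on a timer, sped up by skip, then advances on input, skip, no-wait or auto mode after voice.
; Finished text is registered as a scenario property and written to backlog; save restore and editor preview are supported.
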(fn `GetAssetPaths`
  (params (Command :type "ShidenCommand Structure"))
  (returns (AssetObjectPaths :type "Set of String"))
  (if (`KismetStringLibrary.IsEmpty` Command_Arg5)
    (return)
    (else
      (return (`|MakeSet` Command_Arg5)))))

(fn `GetInput`
  (params (ScenarioManager :type "/Shiden/Core/BP_ShidenScenarioManager Object Reference") (ScenarioWidget :type "/Shiden/Core/WBP_ShidenWidgetBase Object Reference"))
  (locals (InputAction :type "InputAction Object Reference" :default "/Script/EnhancedInput.InputAction'/Shiden/Misc/EnhancedInput/IA_ShidenTalkNext.IA_ShidenTalkNext'") (SkipAction :type "InputAction Object Reference" :default "/Script/EnhancedInput.InputAction'/Shiden/Misc/EnhancedInput/IA_ShidenTalkSkip.IA_ShidenTalkSkip'"))
  (bind _digitalinputs (`/Shiden/Core/BP_ShidenScenarioManager.GetShidenInput` ScenarioManager))
  (`|ExecutionSequence`
    (:`then_0`
      (bind (_value _returnvalue) (`BlueprintMapLibrary.Map_Find` _digitalinputs (`KismetSystemLibrary.GetDisplayName` (`local.InputAction`))))
      (if _returnvalue
        (if _value
          (if (`self.TalkButtonPress`)
            (set `self.TalkButtonPressStart` false)
            (else
              (set `self.TalkButtonPressStart` true)
              (set `self.TalkButtonPress` true)))
          (else
            (set `self.TalkButtonPressStart` false)
            (set `self.TalkButtonPress` false)))))
    (:`then_1`
      (if (or (`BlueprintMapLibrary.Map_Find` _digitalinputs (`KismetSystemLibrary.GetDisplayName` (`local.SkipAction`))) (`/Shiden/Core/WBP_ShidenWidgetBase.PressSkipButton` ScenarioWidget))
        (if (`self.SkipButtonPress`)
          (set `self.SkipButtonPressStart` false)
          (else
            (set `self.SkipButtonPressStart` true)
            (set `self.SkipButtonPress` true)))
        (else
          (set `self.SkipButtonPressStart` false)
          (set `self.SkipButtonPress` false))))))

(fn `GetText`
  (params (Command :type "ShidenCommand Structure") (LanguageIndex :type Integer))
  (returns (Text :type String))
  (bind (_commandname _presetname _arg1 _arg2 _arg3 _arg4 _arg5 _arg6 _arg7 _arg8 _arg9 _arg10) (break `ShidenCommand` Command))
  (return (select `int` LanguageIndex :`0` _arg2 :`1` _arg7 :`2` _arg8 :`3` _arg9 :`4` _arg10)))

(fn `GetTextWidget`
  (params (SlotName :type String) (ScenarioWidget :type "/Shiden/Core/WBP_ShidenWidgetBase Object Reference"))
  (returns (TextBlock :type "RichTextBlock Object Reference") (Found :type Boolean))
  (bind _textobjects (`/Shiden/Core/WBP_ShidenWidgetBase.GetTexts` ScenarioWidget))
  (bind (_value _returnvalue) (`BlueprintMapLibrary.Map_Find` _textobjects SlotName))
  (if (`KismetStringLibrary.IsEmpty` SlotName)
    ;[1 1 1] Set text to first slot
    (bind _values (`BlueprintMapLibrary.Map_Values` _textobjects))
    (for _array_element _values
      (return _array_element true))
    (return null false)
    (else
      (return _value _returnvalue))))

(fn `InitFromSaveData`
  (params (KeyValueMap :type "Map of String to String") (Widget :type "/Shiden/Core/WBP_ShidenWidgetBase Object Reference") (ScenarioManager :type "/Shiden/Core/BP_ShidenScenarioManager Object Reference"))
  (returns (Success :type "/Shiden/Commands/Core/E_ShidenInitFromSaveDataStatus Enum") (ErrorMessage :type String))
  (bind _textobjects (`/Shiden/Core/WBP_ShidenWidgetBase.GetTexts` Widget))
  (bind _keys (`BlueprintMapLibrary.Map_Keys` _textobjects))
  (for _array_element _keys
    (bind (_value _returnvalue) (`BlueprintMapLibrary.Map_Find` _textobjects _array_element))
    (if _returnvalue
      (bind _value_2 (`BlueprintMapLibrary.Map_Find` KeyValueMap _array_element))
      (`RichTextBlock.SetText` _value (`KismetTextLibrary.Conv_StringToText` _value_2))
      (if (`KismetStringLibrary.EqualEqual_StrStr` _array_element "Name")
        (`ShidenCoreFunctionLibrary.AddBacklog` _array_element _value_2))
      (else
        (return "NewEnumerator2" (`KismetStringLibrary.Concat_StrStr` "Text \"" _array_element "\" is not found")))))
  (return "NewEnumerator0" ""))

(fn `PreProcessCommand`
  (params (ProcessName :type String) (Command :type "ShidenCommand Structure") (Widget :type "/Shiden/Core/WBP_ShidenWidgetBase Object Reference") (ScenarioManager :type "/Shiden/Core/BP_ShidenScenarioManager Object Reference") (HookedObject :type "Object Object Reference"))
  (returns (Status :type "/Shiden/Commands/Core/E_ShidenPreProcessStatus Enum") (ErrorMessage :type String))
  (locals (VariableMap :type "Map of String to String") (SkipAction :type "InputAction Object Reference" :default "/Script/EnhancedInput.InputAction'/Shiden/Misc/EnhancedInput/IA_ShidenTalkSkip.IA_ShidenTalkSkip'"))
  (bind (_commandname _presetname _arg1) (break `ShidenCommand` Command))
  (bind (_commandname_2 _presetname_2 _arg1_2 _arg2 _arg3 _arg4 _arg5) (break `ShidenCommand` (`local.Command`)))
  (bind (_commandname_3 _presetname_3 _arg1_3 _arg2_2 _arg3_2 _arg4_2 _arg5_2 _arg6) (break `ShidenCommand` (`local.Command`)))
  (bind (_textblock _found) (`self.GetTextWidget` _arg1 Widget))
  (if _found
    (set `self.TotalElapsedTime` 0.0)
    (set `self.CurrentText` "")
    (set `self.CurrentSlotName` (`KismetMathLibrary.SelectString` "Default" _arg1_3 (`KismetStringLibrary.IsEmpty` _arg1_3)))
    (if (== _arg6 "true")
      (bind (_arrayindex _arrayelement) (`/Engine/EditorBlueprintResources/StandardMacros.ReverseForEachLoop` (`ShidenCoreFunctionLibrary.GetBacklog`))
        (:`LoopBody`
          (if (`KismetStringLibrary.EqualEqual_StrStr` (break `ShidenBacklogItem` _arrayelement) (`self.CurrentSlotName`))
            (bind _output_get (set `self.CurrentText` (`.Text` (break `ShidenBacklogItem` _arrayelement))))
            (bind _returnvalue (`ShidenCoreFunctionLibrary.GetParsedLength` _output_get))
            (set `self.CurrentTextIndex` _returnvalue)
            (bind _output_get_2 (set `self.CurrentText` (`KismetStringLibrary.Concat_StrStr` (`self.CurrentText`) (`self.GetText` (`local.Command`) (`.LanguageIndex` (break `ShidenPredefinedSystemVariable` (`ShidenSubsystem.PredefinedSystemVariable` (subsystem `ShidenSubsystem`)))))) :!label _label))
            (bind _returnvalue_2 (`ShidenCoreFunctionLibrary.GetParsedLength` _output_get_2))
            (set `self.TextLength` _returnvalue_2)
            (`/Shiden/Core/WBP_ShidenWidgetBase.ChangeWindowMode` (`local.Widget`) "NewEnumerator0" true)
            ;[1 1 1] Play voice (if skip mode is enabled, should not play voice)
            (bind _digitalinputs (`/Shiden/Core/BP_ShidenScenarioManager.GetShidenInput` (`local.ScenarioManager`)))
            (if (`.bStopVoiceWhenNextDialogueStart` (break `ShidenPredefinedSystemVariable` (`ShidenSubsystem.PredefinedSystemVariable` (subsystem `ShidenSubsystem`))))
              (`/Shiden/Core/BP_ShidenScenarioManager.StopVoiceAuto2d` (`local.ScenarioManager`)))
            (if (or (`KismetStringLibrary.IsEmpty` _arg5) (`BlueprintMapLibrary.Map_Find` _digitalinputs (`KismetSystemLibrary.GetDisplayName` (`local.SkipAction`))))
              (set `self.VoiceDuration` 0.0)
              (set `self.VoiceStarted` false)
              (else
                (bind (_success _duration) (`/Shiden/Core/BP_ShidenScenarioManager.PlaySound2d` (`local.ScenarioManager`) (make `/Shiden/Commands/Primary/F_ShidenSoundInfo` 0 "NewEnumerator3" _arg5 1.0 1.0)))
                (if _success
                  (set `self.VoiceDuration` _duration)
                  (set `self.VoiceStarted` true)
                  (else
                    (return "NewEnumerator2" "Play sound 2d failed")))))
            (return "NewEnumerator0" "")))
        (:`Completed`
          (set `self.CurrentTextIndex` 0 :!label _label_2)
          (goto _label)))
      (else
        (`RichTextBlock.SetText` _textblock "") ; Clear text
        (goto _label_2)))
    (else
      (return "NewEnumerator2" (`KismetStringLibrary.Concat_StrStr` "Text slot \"" _arg1 "\" is not found")))))

(fn `PreviewCommand`
  (params (Command :type "ShidenCommand Structure") (Widget :type "/Shiden/Core/WBP_ShidenWidgetBase Object Reference") (IsCurrentCommand :type Boolean))
  (returns (Status :type "/Shiden/Commands/Core/E_ShidenPreviewStatus Enum") (SoundInfo :type "/Shiden/Commands/Primary/F_ShidenSoundInfo Structure") (ErrorMessage :type String))
  (locals (temp :type "/Shiden/Commands/Primary/F_ShidenSoundInfo Structure"))
  (bind (_commandname _presetname _arg1 _arg2 _arg3 _arg4 _arg5) (break `ShidenCommand` Command))
  (bind (_commandname_2 _presetname_2 _arg1_2 _arg2_2 _arg3_2 _arg4_2 _arg5_2 _arg6) (break `ShidenCommand` (`local.Command`)))
  (bind _text (`self.GetText` Command (`.LanguageIndex` (break `ShidenPredefinedSystemVariable` (`ShidenSubsystem.PredefinedSystemVariable` (subsystem `ShidenSubsystem`))))))
  (if (not (`KismetStringLibrary.IsEmpty` _arg5))
    (set `local.temp` (make `/Shiden/Commands/Primary/F_ShidenSoundInfo` 0 "NewEnumerator3" _arg5 1.0 1.0)))
  (`/Shiden/Core/WBP_ShidenWidgetBase.ChangeWindowMode` (`local.Widget`) "NewEnumerator0" false)
  (bind (_textblock _found) (`self.GetTextWidget` _arg1_2 (`local.Widget`)))
  (if _found
    (if (== _arg6 "true")
      (`RichTextBlock.SetText` _textblock (`KismetTextLibrary.Conv_StringToText` (`KismetStringLibrary.Concat_StrStr` (`KismetTextLibrary.Conv_TextToString` (`RichTextBlock.GetText` _textblock)) _text)))
      (else
        (`RichTextBlock.SetText` _textblock (`KismetTextLibrary.Conv_StringToText` _text))))
    (return "NewEnumerator0" (`local.temp`) "")
    (else
      (return "NewEnumerator2" (struct) (`KismetStringLibrary.Concat_StrStr` "Text slot \"" _arg1_2 "\" is not found")))))

(fn `ProcessCommand`
  (params (ProcessName :type String) (Command :type "ShidenCommand Structure") (Widget :type "/Shiden/Core/WBP_ShidenWidgetBase Object Reference") (ScenarioManager :type "/Shiden/Core/BP_ShidenScenarioManager Object Reference") (DeltaTime :type "Float (double-precision)") (HookedObject :type "Object Object Reference"))
  (returns (Status :type "/Shiden/Commands/Core/E_ShidenProcessStatus Enum") (BreakReason :type String) (NextScenarioName :type String) (ErrorMessage :type String))
  (bind (_commandname _presetname _arg1 _arg2 _arg3 _arg4 _arg5) (break `ShidenCommand` (`local.Command`)))
  (bind (_commandname_2 _presetname_2 _arg1_2 _arg2_2 _arg3_2 _arg4_2 _arg5_2) (break `ShidenCommand` (`local.Command`)))
  (bind (_commandname_3 _presetname_3 _arg1_3 _arg2_3 _arg3_3 _arg4_3 _arg5_3 _arg6) (break `ShidenCommand` (`local.Command`)))
  (bind (_skipspeedrate _voicevolumerate _sevolumerate _bgmvolumerate _bshowmousecursorwhenstarting _languageindex _secondstowaitforeachletter _waittimeonautomode) (break `ShidenPredefinedSystemVariable` (`ShidenSubsystem.PredefinedSystemVariable` (subsystem `ShidenSubsystem`))))
  (bind (_skipspeedrate_2 _voicevolumerate_2 _sevolumerate_2 _bgmvolumerate_2 _bshowmousecursorwhenstarting_2 _languageindex_2 _secondstowaitforeachletter_2) (break `ShidenPredefinedSystemVariable` (`ShidenSubsystem.PredefinedSystemVariable` (subsystem `ShidenSubsystem`))))
  (`self.GetInput` (`local.ScenarioManager`) (`local.Widget`))
  (set `self.TotalElapsedTime` (+ (`self.TotalElapsedTime`) (`local.DeltaTime`)))
  (`|ExecutionSequence`
    (:`then_0`
      (if (`ShidenSubsystem.IsPreviewMode` (subsystem `ShidenSubsystem`))
        (return "NewEnumerator4" "" "" "")))
    (:`then_1`
      (if (and (not (`KismetStringLibrary.IsEmpty` _arg5_2)) (not (`self.VoiceStarted`)))
        (bind (_success _duration) (`/Shiden/Core/BP_ShidenScenarioManager.PlaySound2d` (`local.ScenarioManager`) (make `/Shiden/Commands/Primary/F_ShidenSoundInfo` 0 "NewEnumerator3" _arg5_2)))
        (if _success
          (set `self.VoiceDuration` _duration)
          (set `self.VoiceStarted` true)
          (else
            (return "NewEnumerator2" "" "" "Play sound 2d failed")))))
    (:`then_2`
      (if (!= (`self.CurrentTextIndex`) (`self.TextLength`))
        (if (or (== (`.Arg4` (break `ShidenCommand` (`local.Command`))) "true") (`self.TalkButtonPressStart`))
          (set `self.CurrentTextIndex` (`self.TextLength`))
          (elif (> (`self.ElapsedTime`) _secondstowaitforeachletter_2)
            (`/Engine/EditorBlueprintResources/StandardMacros.IncrementInt` (`self.CurrentTextIndex`)
              (:`  `
                _))
            (else
              (set `self.ElapsedTime` (+ (`self.ElapsedTime`) (`KismetMathLibrary.SelectFloat` (* (`local.DeltaTime`) _skipspeedrate_2) (`local.DeltaTime`) (`self.SkipButtonPress`))))
              (return "NewEnumerator4" "" "" ""))))
        (`self.ShowText` (`local.Widget`) (`self.CurrentSlotName`) (`self.CurrentText`) (`self.CurrentTextIndex`))
        (set `self.ElapsedTime` 0.0)
        (return "NewEnumerator4" "" "" "")))
    (:`then_3`
      (if (or (== (`.Arg3` (break `ShidenCommand` (`local.Command`))) "false") (or (`self.TalkButtonPressStart`) (and (`self.SkipButtonPress`) (`ShidenScenarioFunctionLibrary.CanSkipCommand`))) (and (`ShidenSubsystem.IsAutoTextMode` (subsystem `ShidenSubsystem`)) (and (> (`self.ElapsedTime`) _waittimeonautomode) (or (or (`KismetStringLibrary.IsEmpty` _arg5) (`KismetStringLibrary.EqualEqual_StrStr` _arg5)) (> (`self.TotalElapsedTime`) (+ (`self.VoiceDuration`) _waittimeonautomode))))))
        (`ShidenCommandFunctionLibrary.RegisterCurrentScenarioProperty` (`.CommandName` (break `ShidenCommand` (`local.Command`))) (`self.CurrentSlotName`) (`self.CurrentText`))
        (if (and (== _arg6 "true") (`KismetStringLibrary.NotEqual_StrStr` _arg1_3 "Name"))
          (bind (_arrayindex _arrayelement) (`/Engine/EditorBlueprintResources/StandardMacros.ReverseForEachLoop` (`ShidenCoreFunctionLibrary.GetBacklog`))
            (:`LoopBody`
              (if (`KismetStringLibrary.EqualEqual_StrStr` (break `ShidenBacklogItem` _arrayelement) (`self.CurrentSlotName`))
                (`ShidenCoreFunctionLibrary.UpdateBacklog` _arrayindex (`self.CurrentSlotName`) (`self.CurrentText`))
                (return "NewEnumerator3" "" "" "")))
            (:`Completed`
              (`ShidenCoreFunctionLibrary.AddBacklog` (`self.CurrentSlotName`) (`self.CurrentText`) :!label _label)
              (return "NewEnumerator3" "" "" "")))
          (else
            (goto _label)))
        (else
          (set `self.ElapsedTime` (+ (`self.ElapsedTime`) (`local.DeltaTime`)))
          (return "NewEnumerator4" "" "" ""))))))

(fn `ShowText`
  (params (ScenarioWidget :type "/Shiden/Core/WBP_ShidenWidgetBase Object Reference") (SlotName :type String) (text :type String) (CharacterCount :type "Integer (by ref)"))
  (bind _textblock (`self.GetTextWidget` SlotName ScenarioWidget)) ; Widget may always be found because\nwe checked widget in preprocess
  (bind _returnvalue (`ShidenCoreFunctionLibrary.GetCharactersWithParsedLength` text CharacterCount))
  (`RichTextBlock.SetText` _textblock (`KismetTextLibrary.Conv_StringToText` _returnvalue)))