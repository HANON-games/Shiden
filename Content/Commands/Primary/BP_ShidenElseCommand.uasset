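; Shiden scenario command for Else, which skips the rest of the branch when executed by moving the process to an End if.
; ProcessCommand calls FindEndifIndex, which scans the cached scenario's commands from the current index and sets the index at the End if it finds.
; The search calls itself recursively on a nested If and reports an error when no End if is found.
; Preprocess, preview, save-data init and asset-path functions hold no logic.
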(fn `FindEndifIndex`
  (params (ProcessName :type String) (ScenarioManager :type "/Shiden/Core/BP_ShidenScenarioManager Object Reference"))
  (returns (Success :type Boolean) (ErrorMessage :type String))
  (locals (TargetCommandNames :type "Array of String"))
  (bind _scenarioprogress (`ShidenScenarioFunctionLibrary.PeekScenario` ProcessName))
  (bind _scenario (`ShidenInternalFunctionLibrary.GetScenarioFromCache` (break `ShidenScenarioProgress` _scenarioprogress)))
  (bind _commands (`ShidenScenario.Commands` _scenario))
  (for _index (range (`.CurrentIndex` (break `ShidenScenarioProgress` _scenarioprogress)) (`KismetArrayLibrary.Array_Length` _commands))
    (switch `string` (`.CommandName` (break `ShidenCommand` (`|GetArrayItem` _commands _index)))
      (:`EndIf`
        (`ShidenScenarioFunctionLibrary.SetCurrentScenarioIndex` (`local.ProcessName`) _index)
        (return true ""))
      (:`If`
        (bind (_success _errormessage) (`self.FindEndifIndex` (`local.ProcessName`) (`local.ScenarioManager`))) ; Change Index to EndIf
        (if _success
          (bind (_success_2 _errormessage_2) (`self.FindEndifIndex` (`local.ProcessName`) (`local.ScenarioManager`)))
          (return _success_2 _errormessage_2)
          (else
            (return false _errormessage))))))
  (return false "Not Found EndIf"))

(fn `GetAssetPaths`
  (params (Command :type "ShidenCommand Structure"))
  (returns (AssetObjectPaths :type "Set of String"))
  (return))

(fn `InitFromSaveData`
  (params (KeyValueMap :type "Map of String to String") (Widget :type "/Shiden/Core/WBP_ShidenWidgetBase Object Reference") (ScenarioManager :type "/Shiden/Core/BP_ShidenScenarioManager Object Reference"))
  (returns (Success :type "/Shiden/Commands/Core/E_ShidenInitFromSaveDataStatus Enum") (ErrorMessage :type String))
  (return "NewEnumerator0" ""))

(fn `PreProcessCommand`
  (params (ProcessName :type String) (Command :type "ShidenCommand Structure") (Widget :type "/Shiden/Core/WBP_ShidenWidgetBase Object Reference") (ScenarioManager :type "/Shiden/Core/BP_ShidenScenarioManager Object Reference") (HookedObject :type "Object Object Reference"))
  (returns (Status :type "/Shiden/Commands/Core/E_ShidenPreProcessStatus Enum") (ErrorMessage :type String))
  (return "NewEnumerator0" ""))

(fn `PreviewCommand`
  (params (Command :type "ShidenCommand Structure") (Widget :type "/Shiden/Core/WBP_ShidenWidgetBase Object Reference") (IsCurrentCommand :type Boolean))
  (returns (Status :type "/Shiden/Commands/Core/E_ShidenPreviewStatus Enum") (SoundInfo :type "/Shiden/Commands/Primary/F_ShidenSoundInfo Structure") (ErrorMessage :type String))
  (return "NewEnumerator0" (struct) ""))

(fn `ProcessCommand`
  (params (ProcessName :type String) (Command :type "ShidenCommand Structure") (Widget :type "/Shiden/Core/WBP_ShidenWidgetBase Object Reference") (ScenarioManager :type "/Shiden/Core/BP_ShidenScenarioManager Object Reference") (DeltaTime :type "Float (double-precision)") (HookedObject :type "Object Object Reference"))
  (returns (Status :type "/Shiden/Commands/Core/E_ShidenProcessStatus Enum") (BreakReason :type String) (NextScenarioName :type String) (ErrorMessage :type String))
  (bind (_success _errormessage) (`self.FindEndifIndex` ProcessName ScenarioManager))
  (if _success
    (return "NewEnumerator3" "" "" "")
    (else
      (return "NewEnumerator2" "" "" _errormessage))))