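; Shiden scenario command that shows or clears a SlateBrushAsset image in a named widget slot, with an eased fade.
; PreProcessCommand and PreviewCommand load the asset and call ShowImage, which applies optional canvas layout and starts the fade; non-current previews skip animation.
; ProcessCommand optionally waits for the fade, then records path and color as scenario properties.
; InitFromSaveData restores slots from saved "Slot::Property" keys, reporting invalid entries as errors.
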(fn `ConvertToEasingFunc`
  (params (EasingFunc :type String))
  (returns (EnumValue :type "EEasingFunc Enum") (Success :type Boolean))
  (switch `string` EasingFunc
    (:`Default`
      (return "Linear" false))
    (:`Linear`
      (return "Linear" true))
    (:`Step`
      (return "Step" true))
    (:`Sinusoidal in`
      (return "SinusoidalIn" true))
    (:`Sinusoidal out`
      (return "SinusoidalOut" true))
    (:`Sinusoidal in out`
      (return "SinusoidalInOut" true))
    (:`Ease in`
      (return "EaseIn" true))
    (:`Ease out`
      (return "EaseOut" true))
    (:`Ease in out`
      (return "EaseInOut" true))
    (:`Expo in`
      (return "ExpoIn" true))
    (:`Expo out`
      (return "ExpoOut" true))
    (:`Expo in out`
      (return "ExpoInOut" true))
    (:`Circular in`
      (return "CircularIn" true))
    (:`Circular out`
      (return "CircularOut" true))
    (:`Circular in out`
      (return "CircularInOut" true))))

(fn `GetAssetPaths`
  (params (Command :type "ShidenCommand Structure"))
  (returns (AssetObjectPaths :type "Set of String"))
  (return (`|MakeSet` Command_Arg2)))

(fn `InitFromSaveData`
  (params (KeyValueMap :type "Map of String to String") (Widget :type "/Shiden/Core/WBP_ShidenWidgetBase Object Reference") (ScenarioManager :type "/Shiden/Core/BP_ShidenScenarioManager Object Reference"))
  (returns (Success :type "/Shiden/Commands/Core/E_ShidenInitFromSaveDataStatus Enum") (ErrorMessage :type String))
  (bind _keys (`BlueprintMapLibrary.Map_Keys` KeyValueMap))
  (for _array_element _keys
    (bind (_lefts _rights) (`KismetStringLibrary.Split` _array_element "::" "IgnoreCase" "FromEnd"))
    (if (not (`KismetStringLibrary.IsEmpty` _lefts))
      (bind (_value _returnvalue) (`BlueprintMapLibrary.Map_Find` (`/Shiden/Core/WBP_ShidenWidgetBase.GetImages` Widget) _lefts))
      (if _returnvalue
        (switch `string` _rights
          (:`Default`
            (return "NewEnumerator2" (`KismetStringLibrary.Concat_StrStr` "Key \"" _array_element "\" is invalid")))
          (:`Path`
            (bind _value_2 (`BlueprintMapLibrary.Map_Find` KeyValueMap _array_element))
            (if (not (or (`KismetStringLibrary.IsEmpty` _value_2) (`KismetStringLibrary.EqualEqual_StrStr` _value_2)))
              (bind (_asset _bsuccess) (`ShidenCoreFunctionLibrary.GetAsset` _value_2))
              (if _bsuccess
                (bind _asslate_brush_asset (cast `SlateBrushAsset` _asset)
                  (:`then`
                    (`Image.SetBrushFromAsset` _value _asslate_brush_asset))
                  (:`CastFailed`
                    (return "NewEnumerator2" (`KismetStringLibrary.Concat_StrStr` "Asset \"" _value_2 "\" is not SlateBrushAsset"))))
                (else
                  (return "NewEnumerator2" (`KismetStringLibrary.Concat_StrStr` "Asset \"" _value_2 "\" is not found"))))))
          (:`Color`
            (bind (_outconvertedcolor _outisvalid) (`KismetStringLibrary.Conv_StringToColor` _value_2))
            (if _outisvalid
              (`Image.SetColorAndOpacity` _value _outconvertedcolor)
              (else
                (return "NewEnumerator2" (`KismetStringLibrary.Concat_StrStr` "Value \"" _value_2 "\" is invalid")))))
          (:`Position`
            (bind (_outconvertedvector2d _outisvalid_2) (`KismetStringLibrary.Conv_StringToVector2D` _value_2))
            (if _outisvalid_2
              (`CanvasPanelSlot.SetPosition` (`WidgetLayoutLibrary.SlotAsCanvasSlot` _value) _outconvertedvector2d)
              (else
                (return "NewEnumerator2" (`KismetStringLibrary.Concat_StrStr` "Value \"" _value_2 "\" is invalid")))))
          (:`Size`
            (bind (_outconvertedvector2d_2 _outisvalid_3) (`KismetStringLibrary.Conv_StringToVector2D` _value_2))
            (if _outisvalid_3
              (`CanvasPanelSlot.SetSize` (`WidgetLayoutLibrary.SlotAsCanvasSlot` _value) _outconvertedvector2d_2)
              (else
                (return "NewEnumerator2" (`KismetStringLibrary.Concat_StrStr` "Value \"" _value_2 "\" is invalid")))))
          (:`SizeToContent`
            (if (== _value_2 "true")
              (bind _returnvalue_2 (`WidgetLayoutLibrary.SlotAsCanvasSlot` _value))
              (set `CanvasPanelSlot.bAutoSize` true _returnvalue_2)
              (else
                (set `CanvasPanelSlot.bAutoSize` false _returnvalue_2)))))
        (else
          (return "NewEnumerator2" (`KismetStringLibrary.Concat_StrStr` "Image \"" _lefts "\" is not found"))))
      (else
        (return "NewEnumerator2" (`KismetStringLibrary.Concat_StrStr` "Key \"" _array_element "\" is invalid")))))
  (return "NewEnumerator0" ""))

(fn `IsImagePathEmpty`
  (params (Command :type "ShidenCommand Structure (by ref)"))
  (returns (IsEmpty :type Boolean))
  (bind (_commandname _presetname _arg1 _arg2) (break `ShidenCommand` Command))
  (return (or (`KismetStringLibrary.EqualEqual_StrStr` _arg2) (`KismetStringLibrary.IsEmpty` _arg2))))

(fn `PreProcessCommand`
  (params (ProcessName :type String) (Command :type "ShidenCommand Structure") (Widget :type "/Shiden/Core/WBP_ShidenWidgetBase Object Reference") (ScenarioManager :type "/Shiden/Core/BP_ShidenScenarioManager Object Reference") (HookedObject :type "Object Object Reference"))
  (returns (Status :type "/Shiden/Commands/Core/E_ShidenPreProcessStatus Enum") (ErrorMessage :type String))
  (bind (_commandname _presetname _arg1 _arg2) (break `ShidenCommand` Command))
  (bind (_asset _bsuccess) (`ShidenCoreFunctionLibrary.GetAsset` _arg2))
  (if (`self.IsImagePathEmpty` Command)
    _
    (elif _bsuccess
      (bind _asslate_brush_asset (cast `SlateBrushAsset` _asset)
        (:`then`
          _)
        (:`CastFailed`
          (return "NewEnumerator2" "Cast failed")))
      (else
        (return "NewEnumerator2" (`KismetStringLibrary.Concat_StrStr` "Asset " _arg2 " is not found")))))
  (bind (_success _errormessage) (`self.ShowImage` Command Widget _asslate_brush_asset true (`local.ProcessName`)))
  (if _success
    (return "NewEnumerator0" "")
    (else
      (return "NewEnumerator2" _errormessage))))

(fn `PreviewCommand`
  (params (Command :type "ShidenCommand Structure") (Widget :type "/Shiden/Core/WBP_ShidenWidgetBase Object Reference") (IsCurrentCommand :type Boolean))
  (returns (Status :type "/Shiden/Commands/Core/E_ShidenPreviewStatus Enum") (SoundInfo :type "/Shiden/Commands/Primary/F_ShidenSoundInfo Structure") (ErrorMessage :type String))
  (bind (_asset _bsuccess) (`ShidenCoreFunctionLibrary.GetAsset` (`.Arg2` (break `ShidenCommand` Command))))
  (if (`self.IsImagePathEmpty` Command)
    _
    (elif _bsuccess
      (bind _asslate_brush_asset (cast `SlateBrushAsset` _asset)
        (:`then`
          _)
        (:`CastFailed`
          (return "NewEnumerator2" (struct) "Cast Failed")))
      (else
        (return "NewEnumerator2" (struct) "Asset not found"))))
  (bind (_success _errormessage) (`self.ShowImage` Command null _asslate_brush_asset IsCurrentCommand "Default"))
  (if _success
    (return "NewEnumerator0" (struct) "")
    (else
      (return "NewEnumerator2" (struct) _errormessage))))

(fn `ProcessCommand`
  (params (ProcessName :type String) (Command :type "ShidenCommand Structure") (Widget :type "/Shiden/Core/WBP_ShidenWidgetBase Object Reference") (ScenarioManager :type "/Shiden/Core/BP_ShidenScenarioManager Object Reference") (DeltaTime :type "Float (double-precision)") (HookedObject :type "Object Object Reference"))
  (returns (Status :type "/Shiden/Commands/Core/E_ShidenProcessStatus Enum") (BreakReason :type String) (NextScenarioName :type String) (ErrorMessage :type String))
  (bind (_returnvalue_r _returnvalue_g _returnvalue_b) (break `LinearColor` (`KismetMathLibrary.LinearColor_White`)))
  (bind (_commandname _presetname _arg1 _arg2) (break `ShidenCommand` (`local.Command`)))
  (bind _commandname_2 (break `ShidenCommand` (`local.Command`)))
  (if (== (`.Arg10` (break `ShidenCommand` Command)) "true")
    (bind _result (`/Shiden/Core/WBP_ShidenWidgetBase.IsImageFadeEnd` Widget (`.Arg1` (break `ShidenCommand` Command))))
    (if _result
      _
      (else
        (return "NewEnumerator4" "" "" ""))))
  (if (`self.IsImagePathEmpty` Command)
    (`Image.SetBrush` (`BlueprintMapLibrary.Map_Find` (`/Shiden/Core/WBP_ShidenWidgetBase.GetImages` Widget) _arg1) (`WidgetBlueprintLibrary.NoResourceBrush`)))
  (`ShidenCommandFunctionLibrary.RegisterCurrentScenarioProperty` _commandname_2 (`KismetStringLibrary.Concat_StrStr` _arg1 "::Path") _arg2)
  (`ShidenCommandFunctionLibrary.RegisterCurrentScenarioProperty` _commandname_2 (`KismetStringLibrary.Concat_StrStr` _arg1 "::Color") (`KismetStringLibrary.Conv_ColorToString` (`KismetMathLibrary.MakeColor` _returnvalue_r _returnvalue_g _returnvalue_b (`KismetMathLibrary.SelectFloat` 0.0 1.0 (`self.IsImagePathEmpty` Command)))))
  (return "NewEnumerator3" "" "" ""))

(fn `ShowImage`
  (params (Command :type "ShidenCommand Structure") (Widget :type "/Shiden/Core/WBP_ShidenWidgetBase Object Reference") (SlateBrushAsset :type "SlateBrushAsset Object Reference") (Animate :type Boolean) (OwnerProcessName :type String))
  (returns (Success :type Boolean) (ErrorMessage :type String))
  (locals (ImageSlotName :type String))
  (bind (_commandname _presetname _arg1 _arg2 _arg3 _arg4 _arg5 _arg6) (break `ShidenCommand` (`local.Command`)))
  (bind (_commandname_2 _presetname_2 _arg1_2 _arg2_2 _arg3_2) (break `ShidenCommand` (`local.Command`)))
  (bind (_commandname_3 _presetname_3 _arg1_3 _arg2_3 _arg3_3 _arg4_2) (break `ShidenCommand` (`local.Command`)))
  (bind (_commandname_4 _presetname_4 _arg1_4 _arg2_4 _arg3_4 _arg4_3 _arg5_2) (break `ShidenCommand` (`local.Command`)))
  (bind (_commandname_5 _presetname_5 _arg1_5 _arg2_5 _arg3_5 _arg4_4 _arg5_3 _arg6_2 _arg7 _arg8 _arg9) (break `ShidenCommand` (`local.Command`)))
  (bind (_enumvalue _success) (`self.ConvertToEasingFunc` _arg6))
  (bind _returnvalue (`KismetStringLibrary.Conv_StringToInt` _arg8))
  (bind _returnvalue_2 (`KismetStringLibrary.Conv_StringToDouble` _arg9))
  (bind _returnvalue_3 (`KismetMathLibrary.SelectFloat` (`KismetStringLibrary.Conv_StringToDouble` (`.Arg7` (break `ShidenCommand` (`local.Command`)))) 0.0 (`local.Animate`)))
  (bind _output_get (set `local.ImageSlotName` (`.Arg1` (break `ShidenCommand` Command))))
  (bind (_value _returnvalue_4) (`BlueprintMapLibrary.Map_Find` (`/Shiden/Core/WBP_ShidenWidgetBase.GetImages` Widget) _output_get))
  (if _returnvalue_4
    (if (not (`self.IsImagePathEmpty` (`local.Command`)))
      (if (not (`KismetStringLibrary.IsEmpty` _arg3_2))
        (bind _returnvalue_5 (`WidgetLayoutLibrary.SlotAsCanvasSlot` _value))
        (`CanvasPanelSlot.SetPosition` _returnvalue_5 (`KismetStringLibrary.Conv_StringToVector2D` _arg3_2))
        (`ShidenCommandFunctionLibrary.RegisterCurrentScenarioProperty` (`.CommandName` (break `ShidenCommand` (`local.Command`))) (`KismetStringLibrary.Concat_StrStr` (`local.ImageSlotName`) "::Position") _arg3_2))
      (if (not (`KismetStringLibrary.IsEmpty` _arg4_2))
        (`CanvasPanelSlot.SetSize` _returnvalue_5 (`KismetStringLibrary.Conv_StringToVector2D` _arg4_2))
        (`ShidenCommandFunctionLibrary.RegisterCurrentScenarioProperty` (`.CommandName` (break `ShidenCommand` (`local.Command`))) (`KismetStringLibrary.Concat_StrStr` (`local.ImageSlotName`) "::Size") _arg4_2))
      (if (not (`KismetStringLibrary.IsEmpty` _arg5_2))
        (set `CanvasPanelSlot.bAutoSize` (== _arg5_2 "true") _returnvalue_5)
        (`ShidenCommandFunctionLibrary.RegisterCurrentScenarioProperty` (`.CommandName` (break `ShidenCommand` (`local.Command`))) (`KismetStringLibrary.Concat_StrStr` (`local.ImageSlotName`) "::SizeToContent") _arg5_2)))
    (if _success
      (if (or (`KismetStringLibrary.EqualEqual_StrStr` _arg2) (`KismetStringLibrary.IsEmpty` _arg2))
        (bind (_success_2 _errormessage) (`/Shiden/Core/WBP_ShidenWidgetBase.StartImageFade` (`local.Widget`) (`local.ImageSlotName`) _value _returnvalue_3 true true _enumvalue _returnvalue_2 _returnvalue (`local.OwnerProcessName`)))
        (return _success_2 _errormessage)
        (else
          (`Image.SetBrushFromAsset` _value (`local.SlateBrushAsset`))
          (bind (_success_3 _errormessage_2) (`/Shiden/Core/WBP_ShidenWidgetBase.StartImageFade` (`local.Widget`) (`local.ImageSlotName`) _value _returnvalue_3 true false _enumvalue _returnvalue_2 _returnvalue (`local.OwnerProcessName`)))
          (return _success_3 _errormessage_2)))
      (else
        (return false (`KismetStringLibrary.Concat_StrStr` "Easing func \"" _arg6 "\" is invalid"))))
    (else
      (return false (`KismetStringLibrary.Concat_StrStr` "Image slot \"" (`local.ImageSlotName`) "\" is not found")))))