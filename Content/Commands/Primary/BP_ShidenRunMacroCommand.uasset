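; Shiden scenario command that runs another scenario as a macro, found by ID or object path.
; Up to five arguments become typed local variables, falling back to scenario defaults when empty.
; Processing pushes the macro onto the scenario stack and resets its index to -1.
; Preview runs macro-callable commands inline, skips If blocks without evaluating them, carries background music info out, then pops the scenario.
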(fn `GetAssetPaths`
  (params (Command :type "ShidenCommand Structure"))
  (returns (AssetObjectPaths :type "Set of String"))
  (return))

(fn `InitFromSaveData`
  (params (KeyValueMap :type "Map of String to String") (Widget :type "/Shiden/Core/WBP_ShidenWidgetBase Object Reference") (ScenarioManager :type "/Shiden/Core/BP_ShidenScenarioManager Object Reference"))
  (returns (Success :type "/Shiden/Commands/Core/E_ShidenInitFromSaveDataStatus Enum") (ErrorMessage :type String))
  (return "NewEnumerator0" ""))

(fn `PreProcessCommand`
  (params (ProcessName :type String) (Command :type "ShidenCommand Structure") (Widget :type "/Shiden/Core/WBP_ShidenWidgetBase Object Reference") (ScenarioManager :type "/Shiden/Core/BP_ShidenScenarioManager Object Reference") (HookedObject :type "Object Object Reference"))
  (returns (Status :type "/Shiden/Commands/Core/E_ShidenPreProcessStatus Enum") (ErrorMessage :type String))
  (return "NewEnumerator0" ""))

(fn `PreviewCommand`
  (params (Command :type "ShidenCommand Structure") (Widget :type "/Shiden/Core/WBP_ShidenWidgetBase Object Reference") (IsCurrentCommand :type Boolean))
  (returns (Status :type "/Shiden/Commands/Core/E_ShidenPreviewStatus Enum") (SoundInfo :type "/Shiden/Commands/Primary/F_ShidenSoundInfo Structure") (ErrorMessage :type String))
  (locals (IsInIfBracket :type Boolean) (CurrentBgm :type "/Shiden/Commands/Primary/F_ShidenSoundInfo Structure"))
  (bind (_scenarioid _scenario _succeeded) (`/Shiden/Libraries/BP_ShidenInternalFunctionLibrary.GetScenarioByIdOrObjectPath` Command_Arg1 Widget))
  (if _succeeded
    (`ShidenCoreFunctionLibrary.PushScenario` "Default" _scenario)
    (`self.SetMacroArguments` "Default" Widget _scenario Command_Arg2 Command_Arg3 Command_Arg4 Command_Arg5 Command_Arg6)
    (set `local.IsInIfBracket` false)
    (for (_array_element _array_index) (`ShidenScenario.Commands` _scenario)
      (bind _constructedcommand (`/Shiden/Libraries/BP_ShidenInternalFunctionLibrary.ConstructCommand` "Default" _array_element (`local.Widget`)))
      (bind (_commandname _presetname _arg1 _arg2 _arg3 _arg4 _arg5 _arg6 _arg7 _arg8 _arg9 _arg10 _commandid _benabled) (break `ShidenCommand` _constructedcommand))
      (if _benabled
        (switch `string` _commandname
          (:`Default`
            (bind (_value _returnvalue) (`BlueprintMapLibrary.Map_Find` (`ShidenSubsystem.CommandDefinitionCache` (subsystem `ShidenSubsystem`)) _commandname))
            (if _returnvalue
              (bind (_note _fontcolor _itemnormalcolor _itemhoveredcolor _itempressedcolor _bcancallinmacro _commandblueprint) (break `ShidenCommandDefinition` _value))
              (if _bcancallinmacro
                (if (not (`local.IsInIfBracket`))
                  (bind _object (`/Shiden/Libraries/BP_ShidenInternalFunctionLibrary.GetCommandFromCache` self "Default" _commandblueprint (`local.Widget`)))
                  (bind (_status _soundinfo _errormessage) (message `/Shiden/Commands/Core/BI_ShidenCommandInterface.PreviewCommand` _object _constructedcommand (`local.Widget`) (`local.IsCurrentCommand`)))
                  (if (`|EnumEquality` _status "NewEnumerator0")
                    (if (`|EnumEquality` (`.Type_2_74D6FA3248579A2E767D94B94718E88D` (break `/Shiden/Commands/Primary/F_ShidenSoundInfo` _soundinfo)) "NewEnumerator1")
                      (set `local.CurrentBgm` _soundinfo))
                    (else
                      (return "NewEnumerator2" (struct) (`/Shiden/Libraries/BP_ShidenInternalFunctionLibrary.MakeErrorMessage` _scenarioid _array_index _commandname _errormessage (`local.Widget`))))))
                (else
                  (return "NewEnumerator2" (struct) (`/Shiden/Libraries/BP_ShidenInternalFunctionLibrary.MakeErrorMessage` _scenarioid _array_index _commandname "this command cannot call in macro" (`local.Widget`)))))
              (else
                (return "NewEnumerator2" (struct) (`/Shiden/Libraries/BP_ShidenInternalFunctionLibrary.MakeErrorMessage` _scenarioid _array_index _commandname "command definition not found" (`local.Widget`))))))
          (:`If`
            (set `local.IsInIfBracket` true :!label _label))
          (:`ElseIf`
            (goto _label))
          (:`Else`
            (goto _label))
          (:`EndIf`
            (set `local.IsInIfBracket` false)))))
    (`ShidenCoreFunctionLibrary.PopScenario` "Default")
    (return "NewEnumerator0" (`local.CurrentBgm`) "")
    (else
      (return "NewEnumerator2" (struct) (`KismetStringLibrary.Concat_StrStr` "Macro \"" Command_Arg1 "\" was not found")))))

(fn `ProcessCommand`
  (params (ProcessName :type String) (Command :type "ShidenCommand Structure") (Widget :type "/Shiden/Core/WBP_ShidenWidgetBase Object Reference") (ScenarioManager :type "/Shiden/Core/BP_ShidenScenarioManager Object Reference") (DeltaTime :type "Float (double-precision)") (HookedObject :type "Object Object Reference"))
  (returns (Status :type "/Shiden/Commands/Core/E_ShidenProcessStatus Enum") (BreakReason :type String) (NextScenarioName :type String) (ErrorMessage :type String))
  (bind (_scenarioid _scenario _succeeded) (`/Shiden/Libraries/BP_ShidenInternalFunctionLibrary.GetScenarioByIdOrObjectPath` Command_Arg1 ScenarioManager))
  (if _succeeded
    (`ShidenCoreFunctionLibrary.PushScenario` ProcessName _scenario)
    (`ShidenCoreFunctionLibrary.SetCurrentScenarioIndex` ProcessName -1)
    (`self.SetMacroArguments` ProcessName ScenarioManager _scenario Command_Arg2 Command_Arg3 Command_Arg4 Command_Arg5 Command_Arg6)
    (return "NewEnumerator3" "" "" "")
    (else
      (return "NewEnumerator2" "" "" (`KismetStringLibrary.Concat_StrStr` "Macro \"" Command_Arg1 "\" is not found.")))))

(fn `SetMacroArguments`
  (params (ProcessName :type String) (WorldContext :type "Object Object Reference") (ShidenScenario :type "ShidenScenario Object Reference") (Arg1Value :type String) (Arg2Value :type String) (Arg3Value :type String) (Arg4Value :type String) (Arg5Value :type String))
  (bind _processname (`local.ProcessName`))
  (for _index (range 5)
    (bind _returnvalue (select `int` _index :`0` (`ShidenScenario.Arg1Name` ShidenScenario) :`1` (`ShidenScenario.Arg2Name` ShidenScenario) :`2` (`ShidenScenario.Arg3Name` ShidenScenario) :`3` (`ShidenScenario.Arg4Name` ShidenScenario) :`4` (`ShidenScenario.Arg5Name` ShidenScenario)))
    (if (not (`KismetStringLibrary.IsEmpty` _returnvalue))
      (switch `EShidenVariableType` (select `int` _index :`0` (`ShidenScenario.Arg1Type` ShidenScenario) :`1` (`ShidenScenario.Arg2Type` ShidenScenario) :`2` (`ShidenScenario.Arg3Type` ShidenScenario) :`3` (`ShidenScenario.Arg4Type` ShidenScenario) :`4` (`ShidenScenario.Arg5Type` ShidenScenario))
        (:`Boolean`
          (bind _returnvalue_2 (select `int` _index :`0` Arg1Value :`1` Arg2Value :`2` Arg3Value :`3` Arg4Value :`4` Arg5Value))
          (bind _returnvalue_3 (`KismetMathLibrary.SelectString` (select `int` _index :`0` (`ShidenScenario.Arg1DefaultValue` ShidenScenario) :`1` (`ShidenScenario.Arg2DefaultValue` ShidenScenario) :`2` (`ShidenScenario.Arg3DefaultValue` ShidenScenario) :`3` (`ShidenScenario.Arg4DefaultValue` ShidenScenario) :`4` (`ShidenScenario.Arg5DefaultValue` ShidenScenario)) _returnvalue_2 (`KismetStringLibrary.IsEmpty` _returnvalue_2)))
          (`ShidenVariableFunctionLibrary.AddLocalBoolean` _processname _returnvalue (== _returnvalue_3 "true")))
        (:`String`
          (`ShidenVariableFunctionLibrary.AddLocalString` _processname _returnvalue _returnvalue_3))
        (:`Integer`
          (`ShidenVariableFunctionLibrary.AddLocalInteger` _processname _returnvalue (`KismetStringLibrary.Conv_StringToInt` _returnvalue_3)))
        (:`Float`
          (`ShidenVariableFunctionLibrary.AddLocalFloat` _processname _returnvalue (`KismetStringLibrary.Conv_StringToDouble` _returnvalue_3)))
        (:`Vector2`
          (`ShidenVariableFunctionLibrary.AddLocalVector2` _processname _returnvalue (`KismetStringLibrary.Conv_StringToVector2D` _returnvalue_3)))
        (:`Vector3`
          (`ShidenVariableFunctionLibrary.AddLocalVector3` _processname _returnvalue (`KismetStringLibrary.Conv_StringToVector` _returnvalue_3))))
      (else
        (break))))
  (return))