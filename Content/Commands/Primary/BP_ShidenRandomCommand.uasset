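; BP_ShidenRandomCommand is a Shiden scenario command that stores a random integer or float in a scenario variable.
; SetRandomValue reads the variable kind, number type, key and range from the command arguments, then writes the result through AddVariable, rejecting invalid kinds or types.
; ProcessCommand runs it under the current process name and PreviewCommand under "Default", both passing on any error.
; The asset-path, save-data and pre-process hooks do no work.
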(fn `GetAssetPaths`
  (params (Command :type "ShidenCommand Structure"))
  (returns (AssetObjectPaths :type "Set of String"))
  (return))

(fn `InitFromSaveData`
  (params (KeyValueMap :type "Map of String to String") (Widget :type "/Shiden/Core/WBP_ShidenWidgetBase Object Reference") (ScenarioManager :type "/Shiden/Core/BP_ShidenScenarioManager Object Reference"))
  (returns (Success :type "/Shiden/Commands/Core/E_ShidenInitFromSaveDataStatus Enum") (ErrorMessage :type String))
  (return "NewEnumerator0" ""))

(fn `PreProcessCommand`
  (params (ProcessName :type String) (Command :type "ShidenCommand Structure") (Widget :type "/Shiden/Core/WBP_ShidenWidgetBase Object Reference") (ScenarioManager :type "/Shiden/Core/BP_ShidenScenarioManager Object Reference") (HookedObject :type "Object Object Reference"))
  (returns (Status :type "/Shiden/Commands/Core/E_ShidenPreProcessStatus Enum") (ErrorMessage :type String))
  (return "NewEnumerator0" ""))

(fn `PreviewCommand`
  (params (Command :type "ShidenCommand Structure") (Widget :type "/Shiden/Core/WBP_ShidenWidgetBase Object Reference") (IsCurrentCommand :type Boolean))
  (returns (Status :type "/Shiden/Commands/Core/E_ShidenPreviewStatus Enum") (SoundInfo :type "/Shiden/Commands/Primary/F_ShidenSoundInfo Structure") (ErrorMessage :type String))
  (bind (_success _errormessage) (`self.SetRandomValue` "Default" Command Widget))
  (if _success
    (return "NewEnumerator0" (struct) "")
    (else
      (return "NewEnumerator2" (struct) _errormessage))))

(fn `ProcessCommand`
  (params (ProcessName :type String) (Command :type "ShidenCommand Structure") (Widget :type "/Shiden/Core/WBP_ShidenWidgetBase Object Reference") (ScenarioManager :type "/Shiden/Core/BP_ShidenScenarioManager Object Reference") (DeltaTime :type "Float (double-precision)") (HookedObject :type "Object Object Reference"))
  (returns (Status :type "/Shiden/Commands/Core/E_ShidenProcessStatus Enum") (BreakReason :type String) (NextScenarioName :type String) (ErrorMessage :type String))
  (bind (_success _errormessage) (`self.SetRandomValue` ProcessName Command ScenarioManager))
  (if _success
    (return "NewEnumerator3" "" "" "")
    (else
      (return "NewEnumerator2" "" "" _errormessage))))

(fn `SetRandomValue`
  (params (ProcessName :type String) (Command :type "ShidenCommand Structure (by ref)") (WorldContext :type "Object Object Reference"))
  (returns (Success :type Boolean) (ErrorMessage :type String))
  (bind (_commandname _presetname _arg1 _arg2 _arg3 _arg4 _arg5) (break `ShidenCommand` Command))
  (bind (_result _bsuccess) (`ShidenVariableFunctionLibrary.ConvertToVariableKind` _arg1))
  (if _bsuccess
    (switch `string` _arg2
      (:`Default`
        (return false "Invalid number type"))
      (:`Integer`
        (bind (_bsuccess_2 _errormessage) (`ShidenVariableFunctionLibrary.AddVariable` ProcessName _result "Integer" _arg3 false "" (`KismetMathLibrary.RandomIntegerInRange` (`KismetStringLibrary.Conv_StringToInt` _arg4) (`KismetStringLibrary.Conv_StringToInt` _arg5))))
        (return _bsuccess_2 _errormessage))
      (:`Float`
        (bind (_bsuccess_3 _errormessage_2) (`ShidenVariableFunctionLibrary.AddVariable` ProcessName _result "Float" _arg3 false "" 0 (`KismetMathLibrary.RandomFloatInRange` (`KismetStringLibrary.Conv_StringToDouble` _arg4) (`KismetStringLibrary.Conv_StringToDouble` _arg5))))
        (return _bsuccess_3 _errormessage_2)))
    (else
      (return false "Invalid Type"))))