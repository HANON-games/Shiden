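; Shiden scenario command that applies a compound assignment operator (+=, -=, *=, /=, %=) to a stored scenario variable.
; CalculationVariable finds the target, takes a literal or second-variable operand, checks types, and writes back the result.
; Per-type Calc helpers handle integers, floats and vectors (no modulo for vectors), while strings always append and Booleans are rejected.
; ProcessCommand and PreviewCommand share this routine, with preview using the "Default" process.
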(event `AddFloat`
  (params (VariableKind :type String) (Key :type String) (NewParam :type String)))

(fn `CalcFloat`
  (params (Operator :type String) (A :type "Float (double-precision)") (B :type "Float (double-precision)"))
  (returns (ReturnValue :type "Float (double-precision)") (Success :type Boolean))
  (switch `string` Operator
    (:`Default`
      (return 0.0 false))
    (:`+=`
      (return (+ A B) true))
    (:`-=`
      (return (- A B) true))
    (:`*=`
      (return (* A B) true))
    (:`/=`
      (return (/ A B) true))
    (:`%=`
      (return (mod A B) true))))

(fn `CalcInteger`
  (params (A :type Integer) (B :type Integer) (operator :type String))
  (returns (ReturnValue :type Integer) (Success :type Boolean))
  (switch `string` operator
    (:`Default`
      (return 0 false))
    (:`+=`
      (return (+ A B) true))
    (:`-=`
      (return (- A B) true))
    (:`*=`
      (return (* A B) true))
    (:`/=`
      (return (/ A B) true))
    (:`%=`
      (return (mod A B) true))))

(fn `CalculationVariable`
  (params (ProcessName :type String) (Command :type "ShidenCommand Structure") (WorldContext :type "Object Object Reference"))
  (returns (Success :type Boolean) (ErrorMessage :type String))
  (locals (IsRVariable :type Boolean))
  (bind (_commandname _presetname _arg1 _arg2 _arg3 _arg4 _arg5) (break `ShidenCommand` Command))
  (bind (_result _bsuccess) (`ShidenVariableFunctionLibrary.ConvertToVariableKind` _arg1))
  (bind (_result_2 _bsuccess_2) (`ShidenVariableFunctionLibrary.ConvertToVariableType` _arg2))
  (bind (_result_3 _bsuccess_3) (`ShidenVariableFunctionLibrary.ConvertToVariableKind` _arg2))
  (if _bsuccess
    (bind (_variabletype _bbooleanvalue _stringvalue _integervalue _floatvalue _vector2value _vector3value _breturnvalue) (`ShidenVariableFunctionLibrary.FindVariable` ProcessName _result _arg3))
    (if _breturnvalue
      (if _bsuccess_2
        (if (`|EnumEquality` _result_2 _variabletype)
          (set `local.IsRVariable` false)
          (else
            (return false "Variable type is not match")))
        (elif (or (and (`|EnumEquality` _variabletype "Boolean") (`KismetStringLibrary.EqualEqual_StrStr` _arg4 "+=")) (and (or (`|EnumEquality` _variabletype "Boolean") (`|EnumEquality` _variabletype "Boolean")) (`KismetStringLibrary.NotEqual_StrStr` _arg4 "%=")))
          (if _bsuccess_3
            (bind (_variabletype_2 _bbooleanvalue_2 _stringvalue_2 _integervalue_2 _floatvalue_2 _vector2value_2 _vector3value_2 _breturnvalue_2) (`ShidenVariableFunctionLibrary.FindVariable` (`local.ProcessName`) _result_3 _arg5))
            (if _breturnvalue_2
              (if (`|EnumEquality` _variabletype _variabletype_2)
                (set `local.IsRVariable` true)
                (else
                  (return false "Variable type is not match")))
              (else
                (return false "Variable not found")))
            (else
              (return false "Invalid variable type")))
          (else
            (return false "Invalid operator"))))
      (switch `EShidenVariableType` _variabletype
        (:`Boolean`
          (return false "Boolean is not supported"))
        (:`String`
          (bind (_bsuccess_4 _errormessage) (`ShidenVariableFunctionLibrary.AddVariable` (`local.ProcessName`) _result _variabletype _arg3 false (`KismetStringLibrary.Concat_StrStr` _stringvalue (`KismetMathLibrary.SelectString` _stringvalue_2 _arg5 (`local.IsRVariable`)))))
          (return _bsuccess_4 _errormessage))
        (:`Integer`
          (bind (_returnvalue _success) (`self.CalcInteger` _integervalue (`KismetMathLibrary.SelectInt` _integervalue_2 (`KismetStringLibrary.Conv_StringToInt` _arg5) (`local.IsRVariable`)) _arg4))
          (if _success
            (bind (_bsuccess_5 _errormessage_2) (`ShidenVariableFunctionLibrary.AddVariable` (`local.ProcessName`) _result _variabletype _arg3 false "" _returnvalue))
            (return _bsuccess_5 _errormessage_2)
            (else
              (return false "Calculation failed"))))
        (:`Float`
          (bind (_returnvalue_2 _success_2) (`self.CalcFloat` _arg4 _floatvalue (`KismetMathLibrary.SelectFloat` _floatvalue_2 (`KismetStringLibrary.Conv_StringToDouble` _arg5) (`local.IsRVariable`))))
          (if _success_2
            (bind (_bsuccess_6 _errormessage_3) (`ShidenVariableFunctionLibrary.AddVariable` (`local.ProcessName`) _result _variabletype _arg3 false "" 0 _returnvalue_2))
            (return _bsuccess_6 _errormessage_3)
            (else
              (return false "Calculation failed"))))
        (:`Vector2`
          (bind (_returnvalue_3 _success_3) (`self.CalcVector2` _arg4 _vector2value (select `bool` (`local.IsRVariable`) :`false` (`KismetStringLibrary.Conv_StringToVector2D` _arg5) :`true` _vector2value_2)))
          (if _success_3
            (bind (_bsuccess_7 _errormessage_4) (`ShidenVariableFunctionLibrary.AddVariable` (`local.ProcessName`) _result _variabletype _arg3 false "" 0 0.0 _returnvalue_3))
            (return _bsuccess_7 _errormessage_4)
            (else
              (return false "Calculation failed"))))
        (:`Vector3`
          (bind (_returnvalue_4 _success_4) (`self.CalcVector3` _arg4 _vector3value (`KismetMathLibrary.SelectVector` _vector3value_2 (`KismetStringLibrary.Conv_StringToVector` _arg5) (`local.IsRVariable`))))
          (if _success_4
            (bind (_bsuccess_8 _errormessage_5) (`ShidenVariableFunctionLibrary.AddVariable` (`local.ProcessName`) _result _variabletype _arg3 false "" 0 0.0 (0.0 0.0) _returnvalue_4))
            (return _bsuccess_8 _errormessage_5)
            (else
              (return false "Calculation failed")))))
      (else
        (return false "Variable not found")))
    (else
      (return false "Invalid variable kind"))))

(fn `CalcVector2`
  (params (Operator :type String) (A :type "Vector2D Structure") (B :type "Vector2D Structure"))
  (returns (ReturnValue :type "Vector2D Structure") (Success :type Boolean))
  (switch `string` Operator
    (:`Default`
      (return (0.0 0.0) false))
    (:`+=`
      (return (+ A B) true))
    (:`-=`
      (return (- A B) true))
    (:`*=`
      (return (* A B) true))
    (:`/=`
      (return (/ A B) true))))

(fn `CalcVector3`
  (params (Operator :type String) (A :type "Vector Structure") (B :type "Vector Structure"))
  (returns (ReturnValue :type "Vector Structure") (Success :type Boolean))
  (switch `string` Operator
    (:`Default`
      (return (0.0 0.0 0.0) false))
    (:`+=`
      (return (+ A B) true))
    (:`-=`
      (return (- A B) true))
    (:`*=`
      (return (* A B) true))
    (:`/=`
      (return (/ A B) true))))

(fn `GetAssetPaths`
  (params (Command :type "ShidenCommand Structure"))
  (returns (AssetObjectPaths :type "Set of String"))
  (return))

(fn `InitFromSaveData`
  (params (KeyValueMap :type "Map of String to String") (Widget :type "/Shiden/Core/WBP_ShidenWidgetBase Object Reference") (ScenarioManager :type "/Shiden/Core/BP_ShidenScenarioManager Object Reference"))
  (returns (Success :type "/Shiden/Commands/Core/E_ShidenInitFromSaveDataStatus Enum") (ErrorMessage :type String))
  (return "NewEnumerator0" ""))

(fn `PreProcessCommand`
  (params (ProcessName :type String) (Command :type "ShidenCommand Structure") (Widget :type "/Shiden/Core/WBP_ShidenWidgetBase Object Reference") (ScenarioManager :type "/Shiden/Core/BP_ShidenScenarioManager Object Reference") (HookedObject :type "Object Object Reference"))
  (returns (Status :type "/Shiden/Commands/Core/E_ShidenPreProcessStatus Enum") (ErrorMessage :type String))
  (return "NewEnumerator0" ""))

(fn `PreviewCommand`
  (params (Command :type "ShidenCommand Structure") (Widget :type "/Shiden/Core/WBP_ShidenWidgetBase Object Reference") (IsCurrentCommand :type Boolean))
  (returns (Status :type "/Shiden/Commands/Core/E_ShidenPreviewStatus Enum") (SoundInfo :type "/Shiden/Commands/Primary/F_ShidenSoundInfo Structure") (ErrorMessage :type String))
  (bind (_success _errormessage) (`self.CalculationVariable` "Default" Command Widget))
  (if _success
    (return "NewEnumerator0" (struct) "")
    (else
      (return "NewEnumerator2" (struct) _errormessage))))

(fn `ProcessCommand`
  (params (ProcessName :type String) (Command :type "ShidenCommand Structure") (Widget :type "/Shiden/Core/WBP_ShidenWidgetBase Object Reference") (ScenarioManager :type "/Shiden/Core/BP_ShidenScenarioManager Object Reference") (DeltaTime :type "Float (double-precision)") (HookedObject :type "Object Object Reference"))
  (returns (Status :type "/Shiden/Commands/Core/E_ShidenProcessStatus Enum") (BreakReason :type String) (NextScenarioName :type String) (ErrorMessage :type String))
  (bind (_success _errormessage) (`self.CalculationVariable` ProcessName Command ScenarioManager))
  (if _success
    (return "NewEnumerator3" "" "" "")
    (else
      (return "NewEnumerator2" "" "" _errormessage))))