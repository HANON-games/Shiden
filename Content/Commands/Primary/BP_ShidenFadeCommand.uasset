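; Shiden scenario command that fades a named screen layer in or out with a chosen color, easing and Z-order.
; PreProcessCommand converts arguments and starts the fade on the widget; ProcessCommand optionally waits for completion, then registers color, with alpha marking fade-out, and Z-order as scenario properties.
; InitFromSaveData re-applies saved opaque fades instantly, always on the "Default" layer.
; Preview plays the current command normally and others with zero duration.
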(fn `ConvertToEasingFunc`
  (params (EasingFunc :type String))
  (returns (EnumValue :type "EEasingFunc Enum") (Success :type Boolean))
  (switch `string` EasingFunc
    (:`Default`
      (return "Linear" false))
    (:`Linear`
      (return "Linear" true))
    (:`Step`
      (return "Step" true))
    (:`Sinusoidal in`
      (return "SinusoidalIn" true))
    (:`Sinusoidal out`
      (return "SinusoidalOut" true))
    (:`Sinusoidal in out`
      (return "SinusoidalInOut" true))
    (:`Ease in`
      (return "EaseIn" true))
    (:`Ease out`
      (return "EaseOut" true))
    (:`Ease in out`
      (return "EaseInOut" true))
    (:`Expo in`
      (return "ExpoIn" true))
    (:`Expo out`
      (return "ExpoOut" true))
    (:`Expo in out`
      (return "ExpoInOut" true))
    (:`Circular in`
      (return "CircularIn" true))
    (:`Circular out`
      (return "CircularOut" true))
    (:`Circular in out`
      (return "CircularInOut" true))))

(fn `GetAssetPaths`
  (params (Command :type "ShidenCommand Structure"))
  (returns (AssetObjectPaths :type "Set of String"))
  (return))

(fn `GetFadeInfo`
  (params (FadeType :type String))
  (returns (IsFadeOut :type Boolean))
  (switch `string` FadeType
    (:`FadeOut`
      (return true))
    (:`FadeIn`
      (return false))))

(fn `InitFromSaveData`
  (params (KeyValueMap :type "Map of String to String") (Widget :type "/Shiden/Core/WBP_ShidenWidgetBase Object Reference") (ScenarioManager :type "/Shiden/Core/BP_ShidenScenarioManager Object Reference"))
  (returns (Success :type "/Shiden/Commands/Core/E_ShidenInitFromSaveDataStatus Enum") (ErrorMessage :type String))
  (bind _keys (`BlueprintMapLibrary.Map_Keys` KeyValueMap))
  (for _array_element _keys
    (bind (_lefts _rights) (`KismetStringLibrary.Split` _array_element "::"))
    (if (`KismetStringLibrary.EqualEqual_StrStr` _rights "Color")
      (bind (_value _returnvalue) (`BlueprintMapLibrary.Map_Find` KeyValueMap _array_element))
      (if _returnvalue
        (bind (_outconvertedcolor _outisvalid) (`KismetStringLibrary.Conv_StringToColor` _value))
        (if _outisvalid
          (if (== (`.A` (`KismetMathLibrary.BreakColor` _outconvertedcolor)) 1.0)
            (bind (_success _errormessage) (`self.Start Fade` (make `ShidenCommand` "Fade" "" "Default" "FadeOut" "0.0" "Linear" _value "2" "2.0" "true" (`BlueprintMapLibrary.Map_Find` KeyValueMap (`KismetStringLibrary.Concat_StrStr` _lefts "::ZOrder"))) Widget "Default"))
            (if (not _success)
              (return "NewEnumerator2" _errormessage)))
          (else
            (return "NewEnumerator2" (`KismetStringLibrary.Concat_StrStr` "BrushColor \"" _value "\" is invalid"))))
        (else
          (return "NewEnumerator2" "Value not found")))))
  (return "NewEnumerator0" ""))

(fn `PreProcessCommand`
  (params (ProcessName :type String) (Command :type "ShidenCommand Structure") (Widget :type "/Shiden/Core/WBP_ShidenWidgetBase Object Reference") (ScenarioManager :type "/Shiden/Core/BP_ShidenScenarioManager Object Reference") (HookedObject :type "Object Object Reference"))
  (returns (Status :type "/Shiden/Commands/Core/E_ShidenPreProcessStatus Enum") (ErrorMessage :type String))
  (bind (_success _errormessage) (`self.Start Fade` Command Widget ProcessName))
  (if _success
    (return "NewEnumerator0" "")
    (else
      (return "NewEnumerator2" _errormessage))))

(fn `PreviewCommand`
  (params (Command :type "ShidenCommand Structure") (Widget :type "/Shiden/Core/WBP_ShidenWidgetBase Object Reference") (IsCurrentCommand :type Boolean))
  (returns (Status :type "/Shiden/Commands/Core/E_ShidenPreviewStatus Enum") (SoundInfo :type "/Shiden/Commands/Primary/F_ShidenSoundInfo Structure") (ErrorMessage :type String))
  (if IsCurrentCommand
    (bind (_success _errormessage) (`self.Start Fade` Command Widget "Default"))
    (if _success
      (return "NewEnumerator0" (struct) "")
      (else
        (return "NewEnumerator2" (struct) _errormessage)))
    (else
      (bind _structout (setmembers `ShidenCommand` :`StructRef` Command :`Arg3` "0.0")) ; Override dulation
      (bind (_success_2 _errormessage_2) (`self.Start Fade` _structout Widget "Default"))
      (if _success_2
        (return "NewEnumerator0" (struct) "")
        (else
          (return "NewEnumerator2" (struct) _errormessage_2))))))

(fn `ProcessCommand`
  (params (ProcessName :type String) (Command :type "ShidenCommand Structure") (Widget :type "/Shiden/Core/WBP_ShidenWidgetBase Object Reference") (ScenarioManager :type "/Shiden/Core/BP_ShidenScenarioManager Object Reference") (DeltaTime :type "Float (double-precision)") (HookedObject :type "Object Object Reference"))
  (returns (Status :type "/Shiden/Commands/Core/E_ShidenProcessStatus Enum") (BreakReason :type String) (NextScenarioName :type String) (ErrorMessage :type String))
  (bind (_commandname _presetname _arg1 _arg2 _arg3 _arg4 _arg5 _arg6 _arg7 _arg8 _arg9) (break `ShidenCommand` Command))
  (bind _commandname_2 (break `ShidenCommand` (`local.Command`)))
  (bind _outconvertedcolor (`KismetStringLibrary.Conv_StringToColor` _arg5))
  (if (`KismetStringLibrary.EqualEqual_StrStr` _arg8 "true")
    (bind _result (`/Shiden/Core/WBP_ShidenWidgetBase.IsFadeEnd` Widget _arg1))
    (if _result
      _
      (else
        (return "NewEnumerator4" "" "" ""))))
  (`ShidenCommandFunctionLibrary.RegisterCurrentScenarioProperty` _commandname_2 (`KismetStringLibrary.Concat_StrStr` _arg1 "::Color") (`KismetStringLibrary.Conv_ColorToString` (`KismetMathLibrary.MakeColor` (break `LinearColor` _outconvertedcolor) (`.G` (break `LinearColor` _outconvertedcolor)) (`.B` (break `LinearColor` _outconvertedcolor)) (`KismetMathLibrary.SelectFloat` 1.0 0.0 (`self.GetFadeInfo` _arg2)))))
  (`ShidenCommandFunctionLibrary.RegisterCurrentScenarioProperty` _commandname_2 (`KismetStringLibrary.Concat_StrStr` _arg1 "::ZOrder") _arg9)
  (return "NewEnumerator3" "" "" ""))

(fn `Start Fade`
  (params (Command :type "ShidenCommand Structure (by ref)") (Widget :type "/Shiden/Core/WBP_ShidenWidgetBase Object Reference") (OwnerProcessName :type String))
  (returns (Success :type Boolean) (ErrorMessage :type String))
  (locals (NewLocalVar :type "LinearColor Structure"))
  (bind (_commandname _presetname _arg1 _arg2 _arg3 _arg4 _arg5 _arg6 _arg7 _arg8 _arg9) (break `ShidenCommand` Command))
  (bind (_enumvalue _success) (`self.ConvertToEasingFunc` _arg4))
  (if _success
    (bind (_success_2 _errormessage) (`/Shiden/Core/WBP_ShidenWidgetBase.StartFade` Widget _arg1 _enumvalue (`KismetStringLibrary.Conv_StringToDouble` _arg3) (`KismetStringLibrary.Conv_StringToColor` _arg5) (`self.GetFadeInfo` _arg2) (`KismetStringLibrary.Conv_StringToDouble` _arg7) (`KismetStringLibrary.Conv_StringToInt` _arg6) OwnerProcessName (`KismetStringLibrary.Conv_StringToInt` _arg9)))
    (return _success_2 _errormessage)
    (else
      (return false "Invalid ease func"))))