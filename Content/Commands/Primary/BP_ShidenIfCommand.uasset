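; Shiden scenario command for "If": tests a stored variable against a value and moves the scenario index to the matching branch.
; ProcessCommand parses the arguments for CheckCondition, which looks up the variable, verifies its type and evaluates the operator.
; On false, it scans forward to Else if, Else or End if, recursively checking each Else if.
; Nested If blocks are skipped via recursive FindEndifIndex.
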(fn `CheckCondition`
  (params (ProcessName :type String) (Kind :type "EShidenVariableKind Enum" :default "UserVariable") (Type :type "EShidenVariableType Enum" :default "Boolean") (Key :type String) (Operator :type String) (Value :type String) (ScenarioManager :type "/Shiden/Core/BP_ShidenScenarioManager Object Reference"))
  (returns (Success :type Boolean) (ErrorMessage :type String))
  (bind (_variabletype _bbooleanvalue _stringvalue _integervalue _floatvalue _vector2value _vector3value _breturnvalue) (`ShidenVariableFunctionLibrary.FindVariable` ProcessName Kind Key))
  (if _breturnvalue
    (if (`|EnumEquality` _variabletype Type)
      (bind (_bresult _bsuccess _errormessage) (`ShidenVariableFunctionLibrary.EvaluateCondition` Type Operator _bbooleanvalue _stringvalue _integervalue _floatvalue _vector2value _vector3value (== Value "true") Value (`KismetStringLibrary.Conv_StringToInt` Value) (`KismetStringLibrary.Conv_StringToDouble` Value) (`KismetStringLibrary.Conv_StringToVector2D` Value) (`KismetStringLibrary.Conv_StringToVector` Value)))
      (if _bsuccess
        (if _bresult
          (return true "")
          (else
            (`ShidenScenarioFunctionLibrary.ToNext` (`local.ProcessName`))
            (bind (_success _commandname _index _errormessage_2) (`self.FindNextIfOrElseIfOrElseOrEndif` (`local.ProcessName`) (`local.ScenarioManager`) :!label _label))
            (if _success
              (`ShidenScenarioFunctionLibrary.SetCurrentScenarioIndex` (`local.ProcessName`) _index)
              (switch `string` _commandname
                (:`If`
                  (`ShidenScenarioFunctionLibrary.ToNext` (`local.ProcessName`))
                  (bind (_success_2 _errormessage_3) (`self.FindEndifIndex` (`local.ProcessName`) (`local.ScenarioManager`)))
                  (if _success_2
                    (`ShidenScenarioFunctionLibrary.ToNext` (`local.ProcessName`))
                    (goto _label)
                    (else
                      (return false _errormessage_3))))
                (:`ElseIf`
                  (bind _scenarioprogress (`ShidenScenarioFunctionLibrary.PeekScenario` (`local.ProcessName`)))
                  (bind _scenario (`ShidenScenarioFunctionLibrary.GetScenarioFromCache` (break `ShidenScenarioProgress` _scenarioprogress)))
                  (bind _constructedcommand (`/Shiden/Libraries/BP_ShidenInternalFunctionLibrary.ConstructCommand` (`local.ProcessName`) (`|GetArrayItem` (`ShidenScenario.Commands` _scenario) (`.CurrentIndex` (break `ShidenScenarioProgress` _scenarioprogress))) (`local.ScenarioManager`))) ; Construct ElseIf command
                  (bind (_result _bsuccess_2) (`ShidenVariableFunctionLibrary.ConvertToVariableKind` (`.Arg1` (break `ShidenCommand` _constructedcommand))))
                  (if _bsuccess_2
                    (bind (_result_2 _bsuccess_3) (`ShidenVariableFunctionLibrary.ConvertToVariableType` (`.Arg2` (break `ShidenCommand` _constructedcommand))))
                    (if _bsuccess_3
                      (bind (_success_3 _errormessage_4) (`self.CheckCondition` (`local.ProcessName`) _result _result_2 (`.Arg3` (break `ShidenCommand` _constructedcommand)) (`.Arg4` (break `ShidenCommand` _constructedcommand)) (`.Arg5` (break `ShidenCommand` _constructedcommand)) (`local.ScenarioManager`)))
                      (return _success_3 _errormessage_4)
                      (else
                        (return false "Invalid variable type")))
                    (else
                      (return false "Invalid variable kind"))))
                (:`Else`
                  _)
                (:`EndIf`
                  _))
              (return true "")
              (else
                (return false _errormessage_2)))))
        (else
          (return false _errormessage)))
      (else
        (return false "Variable type not match")))
    (else
      (return false "Variable not found"))))

(fn `FindEndifIndex`
  (params (ProcessName :type String) (ScenarioManager :type "/Shiden/Core/BP_ShidenScenarioManager Object Reference"))
  (returns (Success :type Boolean) (ErrorMessage :type String))
  (locals (TargetCommandNames :type "Array of String"))
  (bind _scenarioprogress (`ShidenScenarioFunctionLibrary.PeekScenario` ProcessName))
  (bind _scenario (`ShidenScenarioFunctionLibrary.GetScenarioFromCache` (break `ShidenScenarioProgress` _scenarioprogress)))
  (bind _commands (`ShidenScenario.Commands` _scenario))
  (for _index (range (`.CurrentIndex` (break `ShidenScenarioProgress` _scenarioprogress)) (`KismetArrayLibrary.Array_Length` _commands))
    (switch `string` (`.CommandName` (break `ShidenCommand` (`|GetArrayItem` _commands _index)))
      (:`EndIf`
        (`ShidenScenarioFunctionLibrary.SetCurrentScenarioIndex` (`local.ProcessName`) _index)
        (return true ""))
      (:`If`
        (bind _success (`self.FindEndifIndex` (`local.ProcessName`) (`local.ScenarioManager`))) ; Change Index to EndIf
        (if _success
          (bind (_success_2 _errormessage) (`self.FindEndifIndex` (`local.ProcessName`) (`local.ScenarioManager`)))
          (return _success_2 _errormessage)
          (else
            (return false ""))))))
  (return false "Not Found EndIf"))

(fn `FindNextIfOrElseIfOrElseOrEndif`
  (params (ProcessName :type String) (ScenarioManager :type "/Shiden/Core/BP_ShidenScenarioManager Object Reference"))
  (returns (Success :type Boolean) (CommandName :type String) (Index :type Integer) (ErrorMessage :type String))
  (bind _scenarioprogress (`ShidenScenarioFunctionLibrary.PeekScenario` ProcessName))
  (bind _scenario (`ShidenScenarioFunctionLibrary.GetScenarioFromCache` (break `ShidenScenarioProgress` _scenarioprogress)))
  (bind _commands (`ShidenScenario.Commands` _scenario))
  (for _index (range (`.CurrentIndex` (break `ShidenScenarioProgress` _scenarioprogress)) (`KismetArrayLibrary.Array_Length` _commands))
    (bind _commandname (break `ShidenCommand` (`|GetArrayItem` _commands _index)))
    (switch `string` _commandname
      (:`ElseIf`
        _)
      (:`Else`
        _)
      (:`EndIf`
        _)
      (:`If`
        _))
    (return true _commandname _index ""))
  (return false "" -1 "Not Found Else, ElseIf, EndIf"))

(fn `GetAssetPaths`
  (params (Command :type "ShidenCommand Structure"))
  (returns (AssetObjectPaths :type "Set of String"))
  (return))

(fn `InitFromSaveData`
  (params (KeyValueMap :type "Map of String to String") (Widget :type "/Shiden/Core/WBP_ShidenWidgetBase Object Reference") (ScenarioManager :type "/Shiden/Core/BP_ShidenScenarioManager Object Reference"))
  (returns (Success :type "/Shiden/Commands/Core/E_ShidenInitFromSaveDataStatus Enum") (ErrorMessage :type String))
  (return "NewEnumerator0" ""))

(fn `PreProcessCommand`
  (params (ProcessName :type String) (Command :type "ShidenCommand Structure") (Widget :type "/Shiden/Core/WBP_ShidenWidgetBase Object Reference") (ScenarioManager :type "/Shiden/Core/BP_ShidenScenarioManager Object Reference") (HookedObject :type "Object Object Reference"))
  (returns (Status :type "/Shiden/Commands/Core/E_ShidenPreProcessStatus Enum") (ErrorMessage :type String))
  (return "NewEnumerator0" ""))

(fn `PreviewCommand`
  (params (Command :type "ShidenCommand Structure") (Widget :type "/Shiden/Core/WBP_ShidenWidgetBase Object Reference") (IsCurrentCommand :type Boolean))
  (returns (Status :type "/Shiden/Commands/Core/E_ShidenPreviewStatus Enum") (SoundInfo :type "/Shiden/Commands/Primary/F_ShidenSoundInfo Structure") (ErrorMessage :type String))
  (return "NewEnumerator0" (struct) ""))

(fn `ProcessCommand`
  (params (ProcessName :type String) (Command :type "ShidenCommand Structure") (Widget :type "/Shiden/Core/WBP_ShidenWidgetBase Object Reference") (ScenarioManager :type "/Shiden/Core/BP_ShidenScenarioManager Object Reference") (DeltaTime :type "Float (double-precision)") (HookedObject :type "Object Object Reference"))
  (returns (Status :type "/Shiden/Commands/Core/E_ShidenProcessStatus Enum") (BreakReason :type String) (NextScenarioName :type String) (ErrorMessage :type String))
  (locals (TempBoolean :type Boolean) (StartIndex :type Integer :default 0))
  (bind (_result _bsuccess) (`ShidenVariableFunctionLibrary.ConvertToVariableType` Command_Arg2))
  (bind (_result_2 _bsuccess_2) (`ShidenVariableFunctionLibrary.ConvertToVariableKind` Command_Arg1))
  (if _bsuccess_2
    (if _bsuccess
      (bind (_success _errormessage) (`self.CheckCondition` ProcessName _result_2 _result Command_Arg3 Command_Arg4 Command_Arg5 ScenarioManager))
      (if _success
        (return "NewEnumerator3" "" "" "")
        (else
          (return "NewEnumerator2" "" "" _errormessage)))
      (else
        (return "NewEnumerator2" "" "" "Invalid variable type")))
    (else
      (return "NewEnumerator2" "" "" "Invalid variable kind"))))