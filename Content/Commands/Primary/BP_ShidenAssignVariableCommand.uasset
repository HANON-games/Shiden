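; Shiden scenario command that assigns a typed variable from its arguments (kind, type, key, value).
; SetVariables checks the key and kind, validates and converts the value text for boolean, string, integer, float or 2D/3D vector, then calls AddVariable.
; PreviewCommand runs it under the "Default" process and ProcessCommand under the given one, both returning failures as error messages.
; A branch for copying another variable's value exists but never runs.
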(fn `GetAssetPaths`
  (params (Command :type "ShidenCommand Structure"))
  (returns (AssetObjectPaths :type "Set of String"))
  (return))

(fn `InitFromSaveData`
  (params (KeyValueMap :type "Map of String to String") (Widget :type "/Shiden/Core/WBP_ShidenWidgetBase Object Reference") (ScenarioManager :type "/Shiden/Core/BP_ShidenScenarioManager Object Reference"))
  (returns (Success :type "/Shiden/Commands/Core/E_ShidenInitFromSaveDataStatus Enum") (ErrorMessage :type String))
  (return "NewEnumerator0" ""))

(fn `PreProcessCommand`
  (params (ProcessName :type String) (Command :type "ShidenCommand Structure") (Widget :type "/Shiden/Core/WBP_ShidenWidgetBase Object Reference") (ScenarioManager :type "/Shiden/Core/BP_ShidenScenarioManager Object Reference") (HookedObject :type "Object Object Reference"))
  (returns (Status :type "/Shiden/Commands/Core/E_ShidenPreProcessStatus Enum") (ErrorMessage :type String))
  (return "NewEnumerator0" ""))

(fn `PreviewCommand`
  (params (Command :type "ShidenCommand Structure") (Widget :type "/Shiden/Core/WBP_ShidenWidgetBase Object Reference") (IsCurrentCommand :type Boolean))
  (returns (Status :type "/Shiden/Commands/Core/E_ShidenPreviewStatus Enum") (SoundInfo :type "/Shiden/Commands/Primary/F_ShidenSoundInfo Structure") (ErrorMessage :type String))
  (bind (_success _errormessage) (`self.SetVariables` "Default" Command))
  (if _success
    (return "NewEnumerator0" (struct) "")
    (else
      (return "NewEnumerator2" (struct) _errormessage))))

(fn `ProcessCommand`
  (params (ProcessName :type String) (Command :type "ShidenCommand Structure") (Widget :type "/Shiden/Core/WBP_ShidenWidgetBase Object Reference") (ScenarioManager :type "/Shiden/Core/BP_ShidenScenarioManager Object Reference") (DeltaTime :type "Float (double-precision)") (HookedObject :type "Object Object Reference"))
  (returns (Status :type "/Shiden/Commands/Core/E_ShidenProcessStatus Enum") (BreakReason :type String) (NextScenarioName :type String) (ErrorMessage :type String))
  (bind (_success _errormessage) (`self.SetVariables` ProcessName Command))
  (if _success
    (return "NewEnumerator3" "" "" "")
    (else
      (return "NewEnumerator2" "" "" _errormessage))))

(fn `SetVariables`
  (params (ProcessName :type String) (Command :type "ShidenCommand Structure"))
  (returns (Success :type Boolean) (ErrorMessage :type String))
  (bind (_commandname _presetname _arg1 _arg2 _arg3 _arg4) (break `ShidenCommand` Command))
  (bind (_outconvertedvector2d _outisvalid) (`KismetStringLibrary.Conv_StringToVector2D` _arg4))
  (bind (_outconvertedvector _outisvalid_2) (`KismetStringLibrary.Conv_StringToVector` _arg4))
  (bind (_result _bsuccess) (`ShidenVariableFunctionLibrary.ConvertToVariableKind` _arg1))
  (bind (_result_2 _bsuccess_2) (`ShidenVariableFunctionLibrary.ConvertToVariableType` _arg2))
  (if (not (`KismetStringLibrary.Contains` _arg3 " "))
    (if _bsuccess
      (switch `EShidenVariableType` _result_2
        (:`Boolean`
          (if (or (== _arg4 "true") (== _arg4 "false"))
            (bind (_bsuccess_3 _errormessage) (`ShidenVariableFunctionLibrary.AddVariable` (`local.ProcessName`) _result _result_2 _arg3 (== _arg4 "true")))
            (return _bsuccess_3 _errormessage)
            (else
              (return false "Invalid boolean"))))
        (:`String`
          (bind (_bsuccess_4 _errormessage_2) (`ShidenVariableFunctionLibrary.AddVariable` (`local.ProcessName`) _result _result_2 _arg3 false _arg4))
          (return _bsuccess_4 _errormessage_2))
        (:`Integer`
          (if (`KismetStringLibrary.IsNumeric` _arg4)
            (bind (_bsuccess_5 _errormessage_3) (`ShidenVariableFunctionLibrary.AddVariable` (`local.ProcessName`) _result _result_2 _arg3 false "" (`KismetStringLibrary.Conv_StringToInt` _arg4)))
            (return _bsuccess_5 _errormessage_3)
            (else
              (return false "Invalid Integer"))))
        (:`Float`
          (if (`KismetStringLibrary.IsNumeric` _arg4)
            (bind (_bsuccess_6 _errormessage_4) (`ShidenVariableFunctionLibrary.AddVariable` (`local.ProcessName`) _result _result_2 _arg3 false "" 0 (`KismetStringLibrary.Conv_StringToDouble` _arg4)))
            (return _bsuccess_6 _errormessage_4)
            (else
              (return false "Invalid float"))))
        (:`Vector2`
          (if _outisvalid
            (bind (_bsuccess_7 _errormessage_5) (`ShidenVariableFunctionLibrary.AddVariable` (`local.ProcessName`) _result _result_2 _arg3 false "" 0 0.0 _outconvertedvector2d))
            (return _bsuccess_7 _errormessage_5)
            (else
              (return false "Invalid Vector2"))))
        (:`Vector3`
          (if _outisvalid_2
            (bind (_bsuccess_8 _errormessage_6) (`ShidenVariableFunctionLibrary.AddVariable` (`local.ProcessName`) _result _result_2 _arg3 false "" 0 0.0 (0.0 0.0) _outconvertedvector))
            (return _bsuccess_8 _errormessage_6)
            (else
              (return false "Invalid vector3")))))
      (else
        (return false "Invalid variable kind")))
    (else
      (return false "Whitespace cannot be used for key."))))