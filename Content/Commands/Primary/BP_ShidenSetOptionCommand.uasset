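; Shiden scenario command that shows up to five choice options to the player and records the selected one.
; Pre-processing fills the widget's options, saves and switches the window mode, and enables choice input.
; Processing waits for a selection, writes its index to a user, local or system integer variable, then restores window and input modes.
; Preview applies the window mode and shows options only for the current command.
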(fn `CallSetOptions`
  (params (Command :type "ShidenCommand Structure (by ref)") (Widget :type "/Shiden/Core/WBP_ShidenWidgetBase Object Reference"))
  (bind (_commandname _presetname _arg1 _arg2 _arg3 _arg4 _arg5) (break `ShidenCommand` Command))
  (`/Shiden/Core/WBP_ShidenWidgetBase.SetOptions` Widget (`|MakeArray` _arg1 _arg2 _arg3 _arg4 _arg5)))

(fn `ChangeWindowMode`
  (params (Command :type "ShidenCommand Structure") (Widget :type "/Shiden/Core/WBP_ShidenWidgetBase Object Reference"))
  (bind _output_get (set `self.PreviousWindowMode` (`/Shiden/Core/WBP_ShidenWidgetBase.GetWIndowMode` Widget)))
  (if (or (`|EnumEquality` _output_get "NewEnumerator3") (== (`.Arg8` (break `ShidenCommand` Command)) "true"))
    (`/Shiden/Core/WBP_ShidenWidgetBase.ChangeWindowMode` Widget "NewEnumerator1" true)
    (else
      (`/Shiden/Core/WBP_ShidenWidgetBase.ChangeWindowMode` Widget "NewEnumerator2" true))))

(fn `GetAssetPaths`
  (params (Command :type "ShidenCommand Structure"))
  (returns (AssetObjectPaths :type "Set of String"))
  (return))

(fn `InitFromSaveData`
  (params (KeyValueMap :type "Map of String to String") (Widget :type "/Shiden/Core/WBP_ShidenWidgetBase Object Reference") (ScenarioManager :type "/Shiden/Core/BP_ShidenScenarioManager Object Reference"))
  (returns (Success :type "/Shiden/Commands/Core/E_ShidenInitFromSaveDataStatus Enum") (ErrorMessage :type String))
  (return "NewEnumerator0" ""))

(fn `PreProcessCommand`
  (params (ProcessName :type String) (Command :type "ShidenCommand Structure") (Widget :type "/Shiden/Core/WBP_ShidenWidgetBase Object Reference") (ScenarioManager :type "/Shiden/Core/BP_ShidenScenarioManager Object Reference") (HookedObject :type "Object Object Reference"))
  (returns (Status :type "/Shiden/Commands/Core/E_ShidenPreProcessStatus Enum") (ErrorMessage :type String))
  (`self.CallSetOptions` Command Widget)
  (`self.ChangeWindowMode` Command Widget)
  (`/Shiden/Core/WBP_ShidenWidgetBase.SetChoiceInputMode` Widget)
  (return "NewEnumerator0" ""))

(fn `PreviewCommand`
  (params (Command :type "ShidenCommand Structure") (Widget :type "/Shiden/Core/WBP_ShidenWidgetBase Object Reference") (IsCurrentCommand :type Boolean))
  (returns (Status :type "/Shiden/Commands/Core/E_ShidenPreviewStatus Enum") (SoundInfo :type "/Shiden/Commands/Primary/F_ShidenSoundInfo Structure") (ErrorMessage :type String))
  (`self.ChangeWindowMode` Command Widget)
  (if IsCurrentCommand
    (`self.CallSetOptions` Command Widget)
    (return "NewEnumerator0" (struct) "")
    (else
      (return "NewEnumerator0" (struct) ""))))

(fn `ProcessCommand`
  (params (ProcessName :type String) (Command :type "ShidenCommand Structure") (Widget :type "/Shiden/Core/WBP_ShidenWidgetBase Object Reference") (ScenarioManager :type "/Shiden/Core/BP_ShidenScenarioManager Object Reference") (DeltaTime :type "Float (double-precision)") (HookedObject :type "Object Object Reference"))
  (returns (Status :type "/Shiden/Commands/Core/E_ShidenProcessStatus Enum") (BreakReason :type String) (NextScenarioName :type String) (ErrorMessage :type String))
  (bind (_commandname _presetname _arg1 _arg2 _arg3 _arg4 _arg5 _arg6 _arg7) (break `ShidenCommand` Command))
  (bind _widget (`local.Widget`))
  (bind (_result _bsuccess) (`ShidenVariableFunctionLibrary.ConvertToVariableKind` _arg6))
  (bind _result_2 (`/Shiden/Core/WBP_ShidenWidgetBase.GetSelectedOption` Widget))
  (if (!= _result_2 -1)
    (if _bsuccess
      (switch `EShidenVariableKind` _result
        (:`UserVariable`
          (`ShidenVariableFunctionLibrary.AddUserInteger` _arg7 _result_2)
          (`/Shiden/Core/WBP_ShidenWidgetBase.ChangeWindowMode` _widget (`self.PreviousWindowMode`) true :!label _label)
          (`/Shiden/Core/WBP_ShidenWidgetBase.SetInputModeGameAndUI` _widget)
          (return "NewEnumerator3" "" "" ""))
        (:`LocalVariable`
          (`ShidenVariableFunctionLibrary.AddLocalInteger` ProcessName _arg7 _result_2)
          (goto _label))
        (:`SystemVariable`
          (`ShidenVariableFunctionLibrary.AddSystemInteger` _arg7 _result_2)
          (goto _label))
        (:`PredefinedSystemVariable`
          _)))
    (return "NewEnumerator2" "" "" (`KismetStringLibrary.Concat_StrStr` "Variable kind \"" _arg6 "\" is invalid"))
    (else
      (return "NewEnumerator4" "" "" ""))))