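; Shiden scenario command that sets a texture parameter on the material of a named Image or Retainer Box in the widget.
; Process and preview load the texture from Arg4 and share ChangeTextureParameter; processing also registers the path as a scenario property.
; Its key joins target type, name and parameter with "::", escaping colons.
; InitFromSaveData parses saved keys to reapply textures, but returns after the first entry.
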(fn `ChangeTextureParameter`
  (params (Command :type "ShidenCommand Structure (by ref)") (Widget :type "/Shiden/Core/WBP_ShidenWidgetBase Object Reference") (Texture :type "Texture Object Reference"))
  (returns (Success :type Boolean) (ErrorMessage :type String))
  (bind (_commandname _presetname _arg1 _arg2 _arg3) (break `ShidenCommand` Command))
  (bind (_value _returnvalue) (`BlueprintMapLibrary.Map_Find` (`/Shiden/Core/WBP_ShidenWidgetBase.GetRetainerBoxes` Widget) _arg2))
  (bind (_value_2 _returnvalue_2) (`BlueprintMapLibrary.Map_Find` (`/Shiden/Core/WBP_ShidenWidgetBase.GetImages` Widget) (`.Arg2` (break `ShidenCommand` Command))))
  (switch `string` _arg1
    (:`Image`
      (if _returnvalue_2
        (`MaterialInstanceDynamic.SetTextureParameterValue` (`WidgetBlueprintLibrary.GetDynamicMaterial` (`Image.Brush` _value_2)) (`KismetStringLibrary.Conv_StringToName` _arg3) Texture)
        (else
          (return false "Image  not found"))))
    (:`RetainerBox`
      (if _returnvalue
        (`MaterialInstanceDynamic.SetTextureParameterValue` (`RetainerBox.GetEffectMaterial` _value) (`KismetStringLibrary.Conv_StringToName` _arg3) Texture)
        (else
          (return false "RetainerBox  not found")))))
  (return true ""))

(fn `GetAssetPaths`
  (params (Command :type "ShidenCommand Structure"))
  (returns (AssetObjectPaths :type "Set of String"))
  (return (`|MakeSet` Command_Arg4)))

(fn `InitFromSaveData`
  (params (KeyValueMap :type "Map of String to String") (Widget :type "/Shiden/Core/WBP_ShidenWidgetBase Object Reference") (ScenarioManager :type "/Shiden/Core/BP_ShidenScenarioManager Object Reference"))
  (returns (Success :type "/Shiden/Commands/Core/E_ShidenInitFromSaveDataStatus Enum") (ErrorMessage :type String))
  (bind _keys (`BlueprintMapLibrary.Map_Keys` KeyValueMap))
  (for _array_element _keys
    (bind _value (`BlueprintMapLibrary.Map_Find` KeyValueMap _array_element))
    (bind (_asset _bsuccess) (`ShidenCoreFunctionLibrary.GetAsset` _value))
    (if _bsuccess
      (bind _astexture (cast `Texture` _asset)
        (:`then`
          (bind (_targettype _targetname _parametername) (`self.ParseCurrentKey` _array_element))
          (bind (_success _errormessage) (`self.ChangeTextureParameter` (make `ShidenCommand` "ChangeMaterialTextureParameter" "" _targettype _targetname _parametername) Widget _astexture))
          (if _success
            (return "NewEnumerator0" "")
            (else
              (return "NewEnumerator2" _errormessage))))
        (:`CastFailed`
          (return "NewEnumerator2" "Cannot cast to Texture")))
      (else
        (return "NewEnumerator2" (`KismetStringLibrary.Concat_StrStr` "Asset \"" _value "\" is not found")))))
  (return "NewEnumerator0" ""))

(fn `MakeCurrentKey`
  (params (TargetType :type String) (TargetName :type String) (ParameterName :type String))
  (returns (ReturnValue :type String))
  (return (`KismetStringLibrary.Concat_StrStr` (`KismetStringLibrary.Replace` TargetType ":" "\\:") "::" (`KismetStringLibrary.Replace` TargetName ":" "\\:") "::" (`KismetStringLibrary.Replace` ParameterName ":" "\\:"))))

(fn `ParseCurrentKey`
  (params (Key :type String))
  (returns (TargetType :type String) (TargetName :type String) (ParameterName :type String))
  (bind (_lefts _rights) (`KismetStringLibrary.Split` Key "::"))
  (bind (_lefts_2 _rights_2) (`KismetStringLibrary.Split` _rights "::"))
  (return (`KismetStringLibrary.Replace` _lefts "\\:" ":") (`KismetStringLibrary.Replace` _lefts_2 "\\:" ":") (`KismetStringLibrary.Replace` _rights_2 "\\:" ":")))

(fn `PreProcessCommand`
  (params (ProcessName :type String) (Command :type "ShidenCommand Structure") (Widget :type "/Shiden/Core/WBP_ShidenWidgetBase Object Reference") (ScenarioManager :type "/Shiden/Core/BP_ShidenScenarioManager Object Reference") (HookedObject :type "Object Object Reference"))
  (returns (Status :type "/Shiden/Commands/Core/E_ShidenPreProcessStatus Enum") (ErrorMessage :type String))
  (return "NewEnumerator0" ""))

(fn `PreviewCommand`
  (params (Command :type "ShidenCommand Structure") (Widget :type "/Shiden/Core/WBP_ShidenWidgetBase Object Reference") (IsCurrentCommand :type Boolean))
  (returns (Status :type "/Shiden/Commands/Core/E_ShidenPreviewStatus Enum") (SoundInfo :type "/Shiden/Commands/Primary/F_ShidenSoundInfo Structure") (ErrorMessage :type String))
  (bind (_commandname _presetname _arg1 _arg2 _arg3 _arg4) (break `ShidenCommand` Command))
  (bind (_asset _bsuccess) (`ShidenCoreFunctionLibrary.GetAsset` _arg4))
  (if _bsuccess
    (bind _astexture (cast `Texture` _asset)
      (:`then`
        (bind (_success _errormessage) (`self.ChangeTextureParameter` (`local.Command`) (`local.Widget`) _astexture))
        (if _success
          (return "NewEnumerator0" (struct) "")
          (else
            (return "NewEnumerator2" (struct) _errormessage))))
      (:`CastFailed`
        (return "NewEnumerator2" (struct) "Cannot cast to Texture")))
    (else
      (return "NewEnumerator2" (struct) (`KismetStringLibrary.Concat_StrStr` "Asset \"" _arg4 "\" is not found")))))

(fn `ProcessCommand`
  (params (ProcessName :type String) (Command :type "ShidenCommand Structure") (Widget :type "/Shiden/Core/WBP_ShidenWidgetBase Object Reference") (ScenarioManager :type "/Shiden/Core/BP_ShidenScenarioManager Object Reference") (DeltaTime :type "Float (double-precision)") (HookedObject :type "Object Object Reference"))
  (returns (Status :type "/Shiden/Commands/Core/E_ShidenProcessStatus Enum") (BreakReason :type String) (NextScenarioName :type String) (ErrorMessage :type String))
  (bind (_commandname _presetname _arg1 _arg2 _arg3 _arg4) (break `ShidenCommand` (`local.Command`)))
  (bind (_asset _bsuccess) (`ShidenCoreFunctionLibrary.GetAsset` (`.Arg4` (break `ShidenCommand` Command))))
  (if _bsuccess
    (bind _astexture (cast `Texture` _asset)
      (:`then`
        (bind (_success _errormessage) (`self.ChangeTextureParameter` Command Widget _astexture))
        (if _success
          (`ShidenCommandFunctionLibrary.RegisterCurrentScenarioProperty` (`.CommandName` (break `ShidenCommand` (`local.Command`))) (`self.MakeCurrentKey` _arg1 _arg2 _arg3) _arg4)
          (return "NewEnumerator3" "" "" "")
          (else
            (return "NewEnumerator2" "" "" _errormessage))))
      (:`CastFailed`
        (return "NewEnumerator2" "" "" "Cast failed")))
    (else
      (return "NewEnumerator2" "" "" "Asset not found"))))