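; Shiden scenario command that implements If branching by comparing a stored variable against an argument value.
; ProcessCommmand parses variable kind and type, then CheckCondition finds the variable and evaluates it, returning errors on failure.
; A false condition moves the scenario index to the next branch, recursively evaluating Else if or stopping at Else or End if.
; Nested If blocks are skipped through recursive FindEndifIndex scans.
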(fn `CheckCondition`
  (params (ProcessName :type String) (Kind :type "EShidenVariableKind Enum" :default "UserVariable") (Type :type "EShidenVariableType Enum" :default "Boolean") (Key :type String) (Operator :type String) (Value :type String) (ScenarioManager :type "ShidenScenarioManagerInterface Interface"))
  (returns (Success :type Boolean) (ErrorMessage :type String))
  (bind (_variabletype _bbooleanvalue _stringvalue _integervalue _floatvalue _vector2value _vector3value _breturnvalue) (`ShidenVariableFunctionLibrary.FindVariable` ProcessName Kind Key))
  (if _breturnvalue
    (if (`|EnumEquality` _variabletype Type)
      (bind (_bresult _bsuccess _errormessage) (`ShidenVariableFunctionLibrary.EvaluateCondition` Type Operator _bbooleanvalue _stringvalue _integervalue _floatvalue _vector2value _vector3value (== Value "true") Value (`KismetStringLibrary.Conv_StringToInt` Value) (`KismetStringLibrary.Conv_StringToDouble` Value) (`KismetStringLibrary.Conv_StringToVector2D` Value) (`KismetStringLibrary.Conv_StringToVector` Value)))
      (if _bsuccess
        (if _bresult
          (return true "")
          (else
            (`ShidenScenarioFunctionLibrary.ToNext` (`local.ProcessName`))
            (bind (_success _commandname _index _errormessage_2) (`self.Find Next if or Else if or Else or Endif` (`local.ProcessName`) :!label _label))
            (if _success
              (`ShidenScenarioFunctionLibrary.SetCurrentScenarioIndex` (`local.ProcessName`) _index)
              (switch `string` _commandname
                (:`If`
                  (`ShidenScenarioFunctionLibrary.ToNext` (`local.ProcessName`))
                  (bind (_success_2 _errormessage_3) (`self.FindEndifIndex` (`local.ProcessName`) (`local.ScenarioManager`)))
                  (if _success_2
                    (`ShidenScenarioFunctionLibrary.ToNext` (`local.ProcessName`))
                    (goto _label)
                    (else
                      (return false _errormessage_3))))
                (:`ElseIf`
                  (bind _scenarioprogress (`ShidenScenarioFunctionLibrary.PeekScenario` (`local.ProcessName`)))
                  (bind _scenario (`ShidenScenarioFunctionLibrary.GetScenarioFromCache` (break `ShidenScenarioProgress` _scenarioprogress)))
                  (bind _command (`ShidenScenarioFunctionLibrary.ConstructCommand` (`local.ProcessName`) (`|GetArrayItem` (`ShidenScenario.Commands` _scenario) (`.CurrentIndex` (break `ShidenScenarioProgress` _scenarioprogress))))) ; Construct ElseIf command
                  (bind (_result _bsuccess_2) (`ShidenVariableFunctionLibrary.ConvertToVariableKind` (`.Arg1` (break `ShidenCommand` _command))))
                  (if _bsuccess_2
                    (bind (_result_2 _bsuccess_3) (`ShidenVariableFunctionLibrary.ConvertToVariableType` (`.Arg2` (break `ShidenCommand` _command))))
                    (if _bsuccess_3
                      (bind (_success_3 _errormessage_4) (`self.CheckCondition` (`local.ProcessName`) _result _result_2 (`.Arg3` (break `ShidenCommand` _command)) (`.Arg4` (break `ShidenCommand` _command)) (`.Arg5` (break `ShidenCommand` _command)) (`local.ScenarioManager`)))
                      (return _success_3 _errormessage_4)
                      (else
                        (return false "Invalid variable type")))
                    (else
                      (return false "Invalid variable kind"))))
                (:`Else`
                  _)
                (:`EndIf`
                  _))
              (return true "")
              (else
                (return false _errormessage_2)))))
        (else
          (return false _errormessage)))
      (else
        (return false "Variable type not match")))
    (else
      (return false "Variable not found"))))

(fn `Find Next if or Else if or Else or Endif`
  (params (ProcessName :type String))
  (returns (Success :type Boolean) (CommandName :type String) (Index :type Integer) (ErrorMessage :type String))
  (bind _scenarioprogress (`ShidenScenarioFunctionLibrary.PeekScenario` ProcessName))
  (bind _scenario (`ShidenScenarioFunctionLibrary.GetScenarioFromCache` (break `ShidenScenarioProgress` _scenarioprogress)))
  (bind _commands (`ShidenScenario.Commands` _scenario))
  (for _index (range (`.CurrentIndex` (break `ShidenScenarioProgress` _scenarioprogress)) (`KismetArrayLibrary.Array_Length` _commands))
    (bind _commandname (break `ShidenCommand` (`|GetArrayItem` _commands _index)))
    (switch `string` _commandname
      (:`ElseIf`
        _)
      (:`Else`
        _)
      (:`EndIf`
        _)
      (:`If`
        _))
    (return true _commandname _index ""))
  (return false "" -1 "Not Found Else, ElseIf, EndIf"))

(fn `FindEndifIndex`
  (params (ProcessName :type String) (ScenarioManager :type "ShidenScenarioManagerInterface Interface"))
  (returns (Success :type Boolean) (ErrorMessage :type String))
  (locals (TargetCommandNames :type "Array of String"))
  (bind _scenarioprogress (`ShidenScenarioFunctionLibrary.PeekScenario` ProcessName))
  (bind _scenario (`ShidenScenarioFunctionLibrary.GetScenarioFromCache` (break `ShidenScenarioProgress` _scenarioprogress)))
  (bind _commands (`ShidenScenario.Commands` _scenario))
  (for _index (range (`.CurrentIndex` (break `ShidenScenarioProgress` _scenarioprogress)) (`KismetArrayLibrary.Array_Length` _commands))
    (switch `string` (`.CommandName` (break `ShidenCommand` (`|GetArrayItem` _commands _index)))
      (:`EndIf`
        (`ShidenScenarioFunctionLibrary.SetCurrentScenarioIndex` (`local.ProcessName`) _index)
        (return true ""))
      (:`If`
        (bind _success (`self.FindEndifIndex` (`local.ProcessName`) (`local.ScenarioManager`))) ; Change Index to EndIf
        (if _success
          (bind (_success_2 _errormessage) (`self.FindEndifIndex` (`local.ProcessName`) (`local.ScenarioManager`)))
          (return _success_2 _errormessage)
          (else
            (return false ""))))))
  (return false "Not Found EndIf"))

(fn `ProcessCommmand`
  (params (ProcessName :type String) (Command :type "ShidenCommand Structure") (Widget :type "ShidenWidget Object Reference") (ScenarioManager :type "ShidenScenarioManagerInterface Interface (by ref)") (DeltaTime :type "Float (single-precision)") (HookedObject :type "Object Object Reference"))
  (returns (Status :type "EShidenProcessStatus Enum") (BreakReason :type String) (NextScenarioName :type String) (ErrorMessage :type String))
  (bind (_commandname _presetname _arg1 _arg2) (break `ShidenCommand` Command))
  (bind (_commandname_2 _presetname_2 _arg1_2 _arg2_2 _arg3 _arg4 _arg5) (break `ShidenCommand` Command))
  (bind (_result _bsuccess) (`ShidenVariableFunctionLibrary.ConvertToVariableType` _arg2))
  (bind (_result_2 _bsuccess_2) (`ShidenVariableFunctionLibrary.ConvertToVariableKind` _arg1))
  (if _bsuccess_2
    (if _bsuccess
      (bind (_success _errormessage) (`self.CheckCondition` ProcessName _result_2 _result _arg3 _arg4 _arg5 ScenarioManager))
      (if _success
        (return "Next" "" "" "")
        (else
          (return "Error" "" "" _errormessage)))
      (else
        (return "Error" "" "" "Invalid variable type")))
    (else
      (return "Error" "" "" "Invalid variable kind"))))