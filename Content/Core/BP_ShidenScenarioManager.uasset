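; Scenario manager actor for the Shiden system, serving the scenario widget with audio, input, force feedback and parallel macro execution.
; PlaySound2d loads sounds by path, caching BGM and voice components per track for fades, replacement and stopping, while SE plays uncached.
; Input actions toggle the text layer and open the media pause menu; app deactivation can trigger an auto-save.
; Spawned parallel process managers run macros and are destroyed with it, alongside stopping BGM and voices.
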(event `self.ReceiveBeginPlay`
  (`self.EnableInput` (`GameplayStatics.GetPlayerController` 0)))

(event `EnhancedInput|/Shiden/Misc/EnhancedInput/IA_ShidenToggleTextLayerVisibility`
  (params (ActionValue :type Boolean) (ElapsedSeconds :type "Float (double-precision)") (TriggeredSeconds :type "Float (double-precision)") (InputAction :type "InputAction Object Reference" :default "/Shiden/Misc/EnhancedInput/IA_ShidenToggleTextLayerVisibility.IA_ShidenToggleTextLayerVisibility"))
  (bind _textbaselayer (`ShidenWidget.TextBaseLayer` (`self.ScenarioWidget`)))
  (:`Started`
    (if (`ShidenWidget.IsMenuOpen` (`self.ScenarioWidget`))
      _
      (elif (`Widget.IsVisible` _textbaselayer)
        (if (`self.IsTextLayerVisible`)
          (`Widget.SetVisibility` _textbaselayer "Collapsed"))
        (else
          (`Widget.SetVisibility` _textbaselayer "SelfHitTestInvisible"))))))

(event `self.ReceiveDestroyed`
  (for _array_element (`self.ParallelProcessManagers`)
    (`/Engine/EditorBlueprintResources/StandardMacros.IsValid` _array_element
      (:`Is Valid`
        (`self.K2_DestroyActor` _array_element))))
  (bind _keys (`BlueprintMapLibrary.Map_Keys` (`self.BgmComponentCaches`)))
  (for _array_element_2 _keys
    (`self.StopSound2d` _array_element_2 "BGM"))
  (bind _keys_2 (`BlueprintMapLibrary.Map_Keys` (`self.VoiceComponentCaches`)))
  (for _array_element_3 _keys_2
    (`self.StopSound2d` _array_element_3 "Voice")))

(event `ShidenScenarioManagerInterface.SetScenarioWidget`
  (params (Widget :type "ShidenWidget Object Reference"))
  (set `self.ScenarioWidget` Widget))

(event `ShidenScenarioManagerInterface.CallMacroAsParallel`
  (params (NewProcessName :type String) (CallerObject :type "Object Object Reference"))
  (bind _returnvalue (`|SpawnActorFromClass` "/Shiden/Core/BP_ShidenParallelProcessManager.BP_ShidenParallelProcessManager_C" (`KismetMathLibrary.MakeTransform` (0.0 0.0 0.0)) "Undefined" "MultiplyWithRoot" null null))
  (`/Shiden/Core/BP_ShidenParallelProcessManager.StartProcessingMacro` _returnvalue NewProcessName (`self.ScenarioWidget`) self CallerObject)
  (`KismetArrayLibrary.Array_Add` (`self.ParallelProcessManagers`) _returnvalue))

(event `ShidenScenarioManagerInterface.StopVoices`
  (bind _keys (`BlueprintMapLibrary.Map_Keys` (`self.VoiceSoundInfo`)))
  (for _array_element _keys
    (`self.StopSound2d` _array_element "Voice")))

(event `ShidenScenarioManagerInterface.StopSound2d`
  (params (TrackId :type Integer) (Type :type "EShidenSoundType Enum" :default "BGM"))
  (bind _returnvalue (select `EShidenSoundType` Type :`BGM` (`self.BgmComponentCaches`) :`Voice` (`self.VoiceComponentCaches`)))
  (bind (_value _returnvalue_2) (`BlueprintMapLibrary.Map_Find` _returnvalue TrackId))
  (if (or (`|EnumEquality` Type "BGM") (`|EnumEquality` Type "Voice"))
    (if _returnvalue_2
      (`/Engine/EditorBlueprintResources/StandardMacros.IsValid` _value
        (:`Is Valid`
          (`ActorComponent.SetActive` _value false false)
          (`BlueprintMapLibrary.Map_Remove` _returnvalue TrackId)
          (if (`|EnumEquality` Type "Voice")
            (`BlueprintMapLibrary.Map_Remove` (`self.VoiceSoundInfo`) TrackId)))))))

(event `ShidenScenarioManagerInterface.Destroy`
  (`self.K2_DestroyActor`))

(event `EnhancedInput|/Shiden/Misc/EnhancedInput/IA_ShidenOpenMediaPauseMenu`
  (params (ActionValue :type Boolean) (ElapsedSeconds :type "Float (double-precision)") (TriggeredSeconds :type "Float (double-precision)") (InputAction :type "InputAction Object Reference" :default "/Shiden/Misc/EnhancedInput/IA_ShidenOpenMediaPauseMenu.IA_ShidenOpenMediaPauseMenu"))
  (:`Started`
    (`ShidenWidget.OpenMediaPauseMenu` (`self.ScenarioWidget`))))

(event `self.ApplicationLifecycle.ApplicationWillDeactivateDelegate`
  (if (`.bAutoSaveOnMobileAppWillDeactivate` (defaults `ShidenProjectConfig` "/Script/ShidenCore.ShidenProjectConfig"))
    (bind _resulttexture (`ShidenWidget.CaptureScreenToTexture2D` (`self.ScenarioWidget`)))
    (`ShidenCoreFunctionLibrary.SaveUserData` "AutoSave" _resulttexture)
    (`ShidenCoreFunctionLibrary.SaveSystemData`)))

(fn `AdjustBgmVolume`
  (params (TrackId :type Integer) (VolumeDuration :type "Float (single-precision)") (VolumeLevel :type "Float (single-precision)") (FadeCurve :type "EAudioFaderCurve Enum" :default "Linear"))
  (returns (bSuccess :type Boolean))
  (bind (_value _returnvalue) (`BlueprintMapLibrary.Map_Find` (`self.BgmComponentCaches`) TrackId))
  (if _returnvalue
    (`AudioComponent.AdjustVolume` _value VolumeDuration (* VolumeLevel (`ShidenVariableFunctionLibrary.GetBgmVolumeRate`)) FadeCurve)
    (return true)
    (else
      (return false))))

(fn `FindShidenDigitalInput`
  (params (InputAction :type "InputAction Object Reference"))
  (returns (bValue :type Boolean) (bResult :type Boolean))
  (bind (_value _returnvalue) (`BlueprintMapLibrary.Map_Find` (`|MakeMap` "/Shiden/Misc/EnhancedInput/IA_ShidenLoad.IA_ShidenLoad" (`|GetInputActionValue`) "/Shiden/Misc/EnhancedInput/IA_ShidenNext.IA_ShidenNext" (`|GetInputActionValue`) "/Shiden/Misc/EnhancedInput/IA_ShidenToggleTextLayerVisibility.IA_ShidenToggleTextLayerVisibility" (`|GetInputActionValue`) "/Shiden/Misc/EnhancedInput/IA_ShidenOpenMediaPauseMenu.IA_ShidenOpenMediaPauseMenu" (`|GetInputActionValue`) "/Shiden/Misc/EnhancedInput/IA_ShidenSave.IA_ShidenSave" (`|GetInputActionValue`) "/Shiden/Misc/EnhancedInput/IA_ShidenSkip.IA_ShidenSkip" (`|GetInputActionValue`) :!type "InputAction Object Reference") InputAction))
  (return _value _returnvalue))

(fn `IsTextLayerVisible`
  (returns (ReturnValue :type Boolean))
  (locals (Children :type "Array of Widget Object Reference"))
  (bind _textlayer (`ShidenWidget.TextLayer` (`self.ScenarioWidget`)))
  (if (`Widget.IsVisible` _textlayer)
    (bind _output_get (set `local.Children` (`PanelWidget.GetAllChildren` _textlayer)))
    (for _array_element _output_get
      (if (`Widget.IsVisible` _array_element)
        (return true)))
    (return false)
    (else
      (return false))))

(fn `PlayBgmOrVoice`
  (params (SoundInfo :type "ShidenSoundInfo Structure") (Sound :type "SoundBase Object Reference"))
  (bind (_trackid _type) (break `ShidenSoundInfo` (`local.SoundInfo`)))
  (bind (_trackid_2 _type_2 _soundpath _startvolumemultiplier _endvolumemultiplier) (break `ShidenSoundInfo` (`local.SoundInfo`)))
  (bind (_trackid_3 _type_3 _soundpath_2 _startvolumemultiplier_2 _endvolumemultiplier_2 _pitchmultiplier _starttime _audiofadercurve _fadeduration) (break `ShidenSoundInfo` (`local.SoundInfo`)))
  (bind (_trackid_4 _type_4) (break `ShidenSoundInfo` (`local.SoundInfo`)))
  (bind (_trackid_5 _type_5 _soundpath_3 _startvolumemultiplier_3 _endvolumemultiplier_3) (break `ShidenSoundInfo` (`local.SoundInfo`)))
  (bind (_trackid_6 _type_6) (break `ShidenSoundInfo` (`local.SoundInfo`)))
  (bind (_trackid_7 _type_7 _soundpath_4 _startvolumemultiplier_4 _endvolumemultiplier_4 _pitchmultiplier_2 _starttime_2 _audiofadercurve_2 _fadeduration_2) (break `ShidenSoundInfo` (`local.SoundInfo`)))
  (bind (_trackid_8 _type_8 _soundpath_5 _startvolumemultiplier_5 _endvolumemultiplier_5 _pitchmultiplier_3 _starttime_3 _audiofadercurve_3 _fadeduration_3) (break `ShidenSoundInfo` (`local.SoundInfo`)))
  (bind _returnvalue (select `EShidenSoundType` _type_6 :`BGM` (`ShidenVariableFunctionLibrary.GetBgmVolumeRate`) :`SE` (`ShidenVariableFunctionLibrary.GetSeVolumeRate`) :`Voice` (`ShidenVariableFunctionLibrary.GetVoiceVolumeRate`)))
  (bind _returnvalue_2 (select `EShidenSoundType` _type_7 :`BGM` (`self.BgmComponentCaches`) :`Voice` (`self.VoiceComponentCaches`)))
  (bind (_value _returnvalue_3) (`BlueprintMapLibrary.Map_Find` _returnvalue_2 _trackid_7))
  (bind _returnvalue_4 (`KismetStringLibrary.NotEqual_StrStr` (`KismetSystemLibrary.GetPathName` (`AudioComponent.Sound` _value)) (`KismetSystemLibrary.GetPathName` (`local.Sound`))))
  (if (or (`|EnumEquality` _type_6 "BGM") (`|EnumEquality` _type_6 "Voice"))
    (if (== _endvolumemultiplier 0.0)
      (if _returnvalue_3
        (`/Engine/EditorBlueprintResources/StandardMacros.IsValid` _value
          (:`Is Valid`
            (if _returnvalue_4
              (`self.StopSound2d` _trackid_7 _type_7)
              (bind _returnvalue_5 (`GameplayStatics.SpawnSound2D` (`local.Sound`) (* _returnvalue _startvolumemultiplier_3) _pitchmultiplier_2 _starttime_2 null :!label _label))
              (`AudioComponent.FadeOut` _returnvalue_5 _fadeduration_2 0.0 _audiofadercurve_2)
              (else
                (`AudioComponent.FadeOut` (`BlueprintMapLibrary.Map_Find` _returnvalue_2 (`.TrackId` (break `ShidenSoundInfo` (`local.SoundInfo`)))) _fadeduration 0.0 _audiofadercurve)
                (`BlueprintMapLibrary.Map_Remove` _returnvalue_2 _trackid)
                (if (`|EnumEquality` _type "Voice")
                  (`BlueprintMapLibrary.Map_Remove` (`self.VoiceSoundInfo`) _trackid)))))
          (:`Is Not Valid`
            (goto _label)))
        (else
          (goto _label)))
      (else
        (if (== _startvolumemultiplier 0.0)
          (`self.StopSound2d` _trackid_2 _type_2)
          (bind _returnvalue_6 (`GameplayStatics.CreateSound2D` (`local.Sound`) (* _returnvalue _endvolumemultiplier_3) _pitchmultiplier 0.0 null))
          (`AudioComponent.FadeIn` _returnvalue_6 _fadeduration 1.0 _starttime _audiofadercurve)
          (`BlueprintMapLibrary.Map_Add` _returnvalue_2 _trackid _returnvalue_6)
          (elif _returnvalue_3
            (`/Engine/EditorBlueprintResources/StandardMacros.IsValid` _value
              (:`Is Valid`
                (if _returnvalue_4
                  (`self.StopSound2d` _trackid_2 _type_2)
                  (bind _returnvalue_7 (`GameplayStatics.SpawnSound2D` (`local.Sound`) _startvolumemultiplier_5 _pitchmultiplier_3 _starttime_3 null :!label _label_2))
                  (`AudioComponent.AdjustVolume` _returnvalue_7 _fadeduration_3 _endvolumemultiplier_5 _audiofadercurve_3)
                  (`BlueprintMapLibrary.Map_Add` _returnvalue_2 _trackid_4 _returnvalue_7)
                  (else
                    (`AudioComponent.AdjustVolume` _value _fadeduration_3 _endvolumemultiplier_5 _audiofadercurve_3))))
              (:`Is Not Valid`
                (goto _label_2)))
            (else
              (goto _label_2))))
        (if (`|EnumEquality` _type_4 "Voice")
          (`BlueprintMapLibrary.Map_Add` (`self.VoiceSoundInfo`) _trackid_4 (`local.SoundInfo`)))))))

(fn `PlayForceFeedback`
  (params (ForceFeedbackEffectPath :type String))
  (returns (bSuccess :type Boolean))
  (bind (_asset _bsuccess) (`ShidenCoreFunctionLibrary.GetOrLoadAsset` ForceFeedbackEffectPath))
  (if _bsuccess
    (bind _asforce_feedback_effect (cast `ForceFeedbackEffect` _asset)
      (:`then`
        (`PlayerController.K2_ClientPlayForceFeedback` (`GameplayStatics.GetPlayerController` 0) _asforce_feedback_effect "None" false false false)
        (return true))
      (:`CastFailed`
        _)))
  (return false))

(fn `PlaySound2d`
  (params (SoundInfo :type "ShidenSoundInfo Structure"))
  (returns (Duration :type "Float (single-precision)") (bSuccess :type Boolean))
  (locals (SoundDuration :type "Float (single-precision)"))
  (bind (_trackid _type _soundpath _startvolumemultiplier _endvolumemultiplier _pitchmultiplier _starttime _audiofadercurve _fadeduration) (break `ShidenSoundInfo` SoundInfo))
  (bind (_trackid_2 _type_2) (break `ShidenSoundInfo` SoundInfo))
  (bind (_trackid_3 _type_3 _soundpath_2 _startvolumemultiplier_2 _endvolumemultiplier_2 _pitchmultiplier_2 _starttime_2 _audiofadercurve_2) (break `ShidenSoundInfo` SoundInfo))
  (bind (_trackid_4 _type_4 _soundpath_3 _startvolumemultiplier_3 _endvolumemultiplier_3 _pitchmultiplier_3 _starttime_3 _audiofadercurve_3 _fadeduration_2) (break `ShidenSoundInfo` (`local.SoundInfo`)))
  (bind (_value _returnvalue) (`BlueprintMapLibrary.Map_Find` (`self.VoiceComponentCaches`) _trackid_2))
  (bind (_value_2 _returnvalue_2) (`BlueprintMapLibrary.Map_Find` (`self.BgmComponentCaches`) _trackid_2))
  (bind (_asset _bsuccess) (`ShidenCoreFunctionLibrary.GetOrLoadAsset` _soundpath_2))
  (bind _returnvalue_3 (`KismetMathLibrary.SelectFloat` _fadeduration 0.0 (== _endvolumemultiplier 0.0)))
  (bind _returnvalue_4 (* (`ShidenVariableFunctionLibrary.GetSeVolumeRate`) _endvolumemultiplier_3))
  (if (`KismetStringLibrary.IsEmpty` _soundpath)
    (switch `EShidenSoundType` _type_2
      (:`BGM`
        (if _returnvalue_2
          (`AudioComponent.FadeOut` _value_2 _returnvalue_3 0.0 _audiofadercurve_2)
          (`BlueprintMapLibrary.Map_Remove` (`self.BgmComponentCaches`) _trackid_2))
        (return 0.0 true))
      (:`Voice`
        (if _returnvalue
          (`AudioComponent.FadeOut` _value _returnvalue_3 0.0 _audiofadercurve_2)
          (`BlueprintMapLibrary.Map_Remove` (`self.VoiceComponentCaches`) _trackid_2))
        (return 0.0 true)))
    (else
      (if _bsuccess
        (bind _assound_base (cast `SoundBase` _asset)
          (:`then`
            (set `local.SoundDuration` (`SoundBase.Duration` _assound_base))
            (switch `EShidenSoundType` _type_4
              (:`BGM`
                (`self.PlayBgmOrVoice` (`local.SoundInfo`) _assound_base :!label _label))
              (:`SE`
                (if (== _endvolumemultiplier_3 0.0)
                  (bind _returnvalue_5 (`GameplayStatics.SpawnSound2D` _assound_base (* (`ShidenVariableFunctionLibrary.GetSeVolumeRate`) _startvolumemultiplier_3) _pitchmultiplier_3 _starttime_3 null))
                  (`AudioComponent.FadeOut` _returnvalue_5 _fadeduration_2 0.0 _audiofadercurve_3)
                  (elif (== _startvolumemultiplier_3 0.0)
                    (bind _returnvalue_6 (`GameplayStatics.CreateSound2D` _assound_base _returnvalue_4 _pitchmultiplier_3 0.0 null))
                    (`AudioComponent.FadeIn` _returnvalue_6 _fadeduration_2 1.0 _starttime_3 _audiofadercurve_3)
                    (else
                      (bind _returnvalue_7 (`GameplayStatics.SpawnSound2D` _assound_base (* (`ShidenVariableFunctionLibrary.GetSeVolumeRate`) _startvolumemultiplier_3) _pitchmultiplier_3 _starttime_3 null))
                      (`AudioComponent.AdjustVolume` _returnvalue_7 _fadeduration_2 _returnvalue_4 _audiofadercurve_3)))))
              (:`Voice`
                (goto _label)))
            (return (`local.SoundDuration`) true))
          (:`CastFailed`
            _)))
      (return 0.0 false))))

(fn `UserConstructionScript`)