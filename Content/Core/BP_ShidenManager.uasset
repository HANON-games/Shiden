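; Manager actor for the Shiden scenario system, handling audio, scenario input, parallel macros and force feedback around a ScenarioWidget.
; PlaySound loads and type-checks sounds, then fades or adjusts them, tracking BGM and voice by track ID and SE in an array.
; Input toggles the text layer and opens the media pause menu, while CallMacroasParallel spawns process-manager actors, cleaned up on destruction.
; App deactivation optionally auto-saves with a screenshot thumbnail.
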(event `self.ReceiveBeginPlay`
  (`self.EnableInput` (`GameplayStatics.GetPlayerController` 0)))

(event `EnhancedInput|/Shiden/Misc/EnhancedInput/IA_ShidenToggleTextLayerVisibility`
  (params (ActionValue :type Boolean) (ElapsedSeconds :type "Float (double-precision)") (TriggeredSeconds :type "Float (double-precision)") (InputAction :type "InputAction Object Reference" :default "/Shiden/Misc/EnhancedInput/IA_ShidenToggleTextLayerVisibility.IA_ShidenToggleTextLayerVisibility"))
  (bind _textbaselayer (`ShidenWidget.TextBaseLayer` (`self.ScenarioWidget`)))
  (:`Started`
    (if (`ShidenWidget.IsMenuOpen` (`self.ScenarioWidget`))
      _
      (elif (`Widget.IsVisible` _textbaselayer)
        (if (`self.IsTextLayerVisible`)
          (`Widget.SetVisibility` _textbaselayer "Collapsed"))
        (else
          (`Widget.SetVisibility` _textbaselayer "SelfHitTestInvisible"))))))

(event `self.ReceiveDestroyed`
  (`|ExecutionSequence`
    (:`then_0`
      (for _array_element (`self.ParallelProcessManagers`)
        (`/Engine/EditorBlueprintResources/StandardMacros.IsValid` _array_element
          (:`Is Valid`
            (`self.K2_DestroyActor` _array_element)))))
    (:`then_1`
      (bind _keys (`BlueprintMapLibrary.Map_Keys` (`self.BgmComponents`)))
      (for _array_element_2 _keys
        (`self.StopSound` _array_element_2 "BGM")))
    (:`then_2`
      (bind _keys_2 (`BlueprintMapLibrary.Map_Keys` (`self.VoiceComponents`)))
      (for _array_element_3 _keys_2
        (`self.StopSound` _array_element_3 "Voice")))
    (:`then_3`
      (for _array_element_4 (`self.SeComponents`)
        (`ActorComponent.SetActive` _array_element_4 false false))
      (`KismetArrayLibrary.Array_Clear` (`self.SeComponents`)))))

(event `ShidenManagerInterface.Initialize`
  (params (Widget :type "ShidenWidget Object Reference"))
  (set `self.ScenarioWidget` Widget))

(event `ShidenManagerInterface.CallMacroAsParallel`
  (params (NewProcessName :type String) (CallerObject :type "Object Object Reference"))
  (bind _returnvalue (`|SpawnActorFromClass` "/Shiden/Core/BP_ShidenParallelProcessManager.BP_ShidenParallelProcessManager_C" (`KismetMathLibrary.MakeTransform` (0.0 0.0 0.0)) "Undefined" "MultiplyWithRoot" null null))
  (`/Shiden/Core/BP_ShidenParallelProcessManager.StartProcessingMacro` _returnvalue NewProcessName (`self.ScenarioWidget`) self CallerObject)
  (`KismetArrayLibrary.Array_Add` (`self.ParallelProcessManagers`) _returnvalue))

(event `ShidenManagerInterface.StopVoices`
  (bind _keys (`BlueprintMapLibrary.Map_Keys` (`self.VoiceComponents`)))
  (for _array_element _keys
    (`self.StopSound` _array_element "Voice")))

(event `ShidenManagerInterface.StopSound`
  (params (TrackId :type Integer) (Type :type "EShidenSoundType Enum" :default "BGM"))
  (bind _returnvalue (select `EShidenSoundType` Type :`BGM` (`self.BgmComponents`) :`Voice` (`self.VoiceComponents`)))
  (bind (_value _returnvalue_2) (`BlueprintMapLibrary.Map_Find` _returnvalue TrackId))
  (if (`|EnumInequality` Type "SE")
    (if _returnvalue_2
      (`/Engine/EditorBlueprintResources/StandardMacros.IsValid` _value
        (:`Is Valid`
          (`ActorComponent.SetActive` _value false false)
          (`BlueprintMapLibrary.Map_Remove` _returnvalue TrackId))))))

(event `ShidenManagerInterface.Destroy`
  (`self.K2_DestroyActor`))

(event `EnhancedInput|/Shiden/Misc/EnhancedInput/IA_ShidenOpenMediaPauseMenu`
  (params (ActionValue :type Boolean) (ElapsedSeconds :type "Float (double-precision)") (TriggeredSeconds :type "Float (double-precision)") (InputAction :type "InputAction Object Reference" :default "/Shiden/Misc/EnhancedInput/IA_ShidenOpenMediaPauseMenu.IA_ShidenOpenMediaPauseMenu"))
  (:`Started`
    (`ShidenWidget.OpenMediaPauseMenu` (`self.ScenarioWidget`))))

(event `self.ApplicationLifecycle.ApplicationWillDeactivateDelegate`
  (if (`.bAutoSaveOnMobileAppWillDeactivate` (defaults `ShidenProjectConfig` "/Script/ShidenCore.ShidenProjectConfig"))
    (bind _resulttexture (`ShidenWidget.CaptureScreenToTexture2D` (`self.ScenarioWidget`)))
    (`ShidenSaveFunctionLibrary.SaveUserData` "AutoSave" _resulttexture)
    (`ShidenSaveFunctionLibrary.SaveSystemData`)))

(event `OnBgmFinished`
  (`self.RemoveSound` "BGM"))

(event `OnSeFinished`
  (`self.RemoveSound` "SE"))

(event `OnVoiceFinished`
  (`self.RemoveSound` "Voice"))

(event `ShidenManagerInterface.PauseAllSounds`
  (params (bPause :type Boolean))
  (`|ExecutionSequence`
    (:`then_0`
      (bind _values (`BlueprintMapLibrary.Map_Values` (`self.BgmComponents`)))
      (for _array_element _values
        (`AudioComponent.SetPaused` _array_element bPause)))
    (:`then_1`
      (for _array_element_2 (`self.SeComponents`)
        (`AudioComponent.SetPaused` _array_element_2 bPause)))
    (:`then_2`
      (bind _values_2 (`BlueprintMapLibrary.Map_Values` (`self.VoiceComponents`)))
      (for _array_element_3 _values_2
        (`AudioComponent.SetPaused` _array_element_3 bPause)))))

(fn `AdjustBgmVolume`
  (params (TrackId :type Integer) (VolumeDuration :type "Float (single-precision)") (VolumeLevel :type "Float (single-precision)") (FadeCurve :type "EAudioFaderCurve Enum" :default "Linear"))
  (bind (_value _returnvalue) (`BlueprintMapLibrary.Map_Find` (`self.BgmComponents`) TrackId))
  (if _returnvalue
    (`AudioComponent.AdjustVolume` _value VolumeDuration VolumeLevel FadeCurve)
    (return)
    (else
      (return))))

(fn `FindShidenDigitalInput`
  (params (InputAction :type "InputAction Object Reference"))
  (returns (bValue :type Boolean) (bResult :type Boolean))
  (bind (_value _returnvalue) (`BlueprintMapLibrary.Map_Find` (`|MakeMap` "/Shiden/Misc/EnhancedInput/IA_ShidenLoad.IA_ShidenLoad" (`|GetInputActionValue`) "/Shiden/Misc/EnhancedInput/IA_ShidenNext.IA_ShidenNext" (`|GetInputActionValue`) "/Shiden/Misc/EnhancedInput/IA_ShidenToggleTextLayerVisibility.IA_ShidenToggleTextLayerVisibility" (`|GetInputActionValue`) "/Shiden/Misc/EnhancedInput/IA_ShidenOpenMediaPauseMenu.IA_ShidenOpenMediaPauseMenu" (`|GetInputActionValue`) "/Shiden/Misc/EnhancedInput/IA_ShidenSave.IA_ShidenSave" (`|GetInputActionValue`) "/Shiden/Misc/EnhancedInput/IA_ShidenSkip.IA_ShidenSkip" (`|GetInputActionValue`) :!type "InputAction Object Reference") InputAction))
  (return _value _returnvalue))

(fn `IsTextLayerVisible`
  (returns (ReturnValue :type Boolean))
  (locals (Children :type "Array of Widget Object Reference"))
  (bind _textlayer (`ShidenWidget.TextLayer` (`self.ScenarioWidget`)))
  (if (`Widget.IsVisible` _textlayer)
    (bind _output_get (set `local.Children` (`PanelWidget.GetAllChildren` _textlayer)))
    (for _array_element _output_get
      (if (`Widget.IsVisible` _array_element)
        (return true)))
    (return false)
    (else
      (return false))))

(fn `Play Se`
  (params (SoundInfo :type "ShidenSoundInfo Structure (by ref)") (Sound :type "SoundBase Object Reference") (RegisterSound :type Boolean :default true))
  (bind ((`Type` _type) (`SoundPath` _soundpath) (`StartVolumeMultiplier` _startvolumemultiplier) (`EndVolumeMultiplier` _endvolumemultiplier) (`PitchMultiplier` _pitchmultiplier) (`StartTime` _starttime) (`AudioFaderCurve` _audiofadercurve) (`FadeDuration` _fadeduration)) (break `ShidenSoundInfo` SoundInfo))
  (if (`|EnumEquality` _type "SE")
    (if (== _endvolumemultiplier 0.0)
      (bind _returnvalue (`GameplayStatics.SpawnSound2D` Sound _startvolumemultiplier _pitchmultiplier _starttime null))
      (if (`local.RegisterSound`)
        (`self.RegisterSound` (`local.SoundInfo`) _returnvalue))
      (`AudioComponent.FadeOut` _returnvalue _fadeduration 0.0 _audiofadercurve)
      (elif (== _startvolumemultiplier 0.0)
        (bind _returnvalue_2 (`GameplayStatics.CreateSound2D` Sound _endvolumemultiplier _pitchmultiplier 0.0 null))
        (if (`local.RegisterSound`)
          (`self.RegisterSound` (`local.SoundInfo`) _returnvalue_2))
        (`AudioComponent.FadeIn` _returnvalue_2 _fadeduration 1.0 _starttime _audiofadercurve)
        (else
          (bind _returnvalue_3 (`GameplayStatics.SpawnSound2D` Sound _startvolumemultiplier _pitchmultiplier _starttime null))
          (if (`local.RegisterSound`)
            (`self.RegisterSound` (`local.SoundInfo`) _returnvalue_3))
          (`AudioComponent.AdjustVolume` _returnvalue_3 _fadeduration _endvolumemultiplier _audiofadercurve))))))

(fn `PlayBgmOrVoice`
  (params (SoundInfo :type "ShidenSoundInfo Structure") (Sound :type "SoundBase Object Reference") (RegisterSound :type Boolean :default true))
  (bind ((`TrackId` _trackid) (`Type` _type) (`StartVolumeMultiplier` _startvolumemultiplier) (`PitchMultiplier` _pitchmultiplier) (`StartTime` _starttime) (`AudioFaderCurve` _audiofadercurve) (`FadeDuration` _fadeduration)) (break `ShidenSoundInfo` (`local.SoundInfo`)))
  (bind (_trackid_2 _type_2 _soundpath _startvolumemultiplier_2 _endvolumemultiplier) (break `ShidenSoundInfo` (`local.SoundInfo`)))
  (bind ((`EndVolumeMultiplier` _endvolumemultiplier_2) (`PitchMultiplier` _pitchmultiplier_2) (`StartTime` _starttime_2) (`AudioFaderCurve` _audiofadercurve_2) (`FadeDuration` _fadeduration_2)) (break `ShidenSoundInfo` (`local.SoundInfo`)))
  (bind ((`TrackId` _trackid_3) (`Type` _type_3)) (break `ShidenSoundInfo` (`local.SoundInfo`)))
  (bind ((`StartVolumeMultiplier` _startvolumemultiplier_3) (`EndVolumeMultiplier` _endvolumemultiplier_3) (`PitchMultiplier` _pitchmultiplier_3) (`StartTime` _starttime_3) (`AudioFaderCurve` _audiofadercurve_3) (`FadeDuration` _fadeduration_3)) (break `ShidenSoundInfo` (`local.SoundInfo`)))
  (bind _returnvalue (select `EShidenSoundType` _type_3 :`BGM` (`self.BgmComponents`) :`Voice` (`self.VoiceComponents`)))
  (bind _value (`BlueprintMapLibrary.Map_Find` _returnvalue (`.TrackId` (break `ShidenSoundInfo` (`local.SoundInfo`)))))
  (bind (_value_2 _returnvalue_2) (`BlueprintMapLibrary.Map_Find` (select `EShidenSoundType` _type_2 :`BGM` (`self.BgmComponents`) :`Voice` (`self.VoiceComponents`)) _trackid_2))
  (bind (_value_3 _returnvalue_3) (`BlueprintMapLibrary.Map_Find` _returnvalue _trackid_3))
  (if (`|EnumInequality` (`.Type` (break `ShidenSoundInfo` (`local.SoundInfo`))) "SE")
    (if (== _endvolumemultiplier 0.0)
      (if _returnvalue_3
        (`/Engine/EditorBlueprintResources/StandardMacros.IsValid` _value_3
          (:`Is Valid`
            (if (`KismetStringLibrary.NotEqual_StrStr` (`KismetSystemLibrary.GetPathName` (`AudioComponent.Sound` _value_3)) (`KismetSystemLibrary.GetPathName` (`local.Sound`)))
              (`self.StopSound` _trackid _type)
              (bind _returnvalue_4 (`GameplayStatics.SpawnSound2D` (`local.Sound`) _startvolumemultiplier _pitchmultiplier _starttime null :!label _label))
              (if (`local.RegisterSound`)
                (`self.RegisterSound` (`local.SoundInfo`) _returnvalue_4))
              (`AudioComponent.FadeOut` _returnvalue_4 _fadeduration 0.0 _audiofadercurve)
              (else
                (if (`local.RegisterSound`)
                  (`self.RegisterSound` (`local.SoundInfo`) _value))
                (`AudioComponent.FadeOut` _value _fadeduration_2 0.0 _audiofadercurve_2))))
          (:`Is Not Valid`
            (goto _label)))
        (else
          (goto _label)))
      (elif (== _startvolumemultiplier_2 0.0)
        (`self.StopSound` _trackid_2 _type_2)
        (bind _returnvalue_5 (`GameplayStatics.CreateSound2D` (`local.Sound`) _endvolumemultiplier_2 _pitchmultiplier_2 0.0 null))
        (if (`local.RegisterSound`)
          (`self.RegisterSound` (`local.SoundInfo`) _returnvalue_5))
        (`AudioComponent.FadeIn` _returnvalue_5 _fadeduration_2 1.0 _starttime_2 _audiofadercurve_2)
        (elif _returnvalue_2
          (`/Engine/EditorBlueprintResources/StandardMacros.IsValid` _value_2
            (:`Is Valid`
              (if (`KismetStringLibrary.NotEqual_StrStr` (`KismetSystemLibrary.GetPathName` (`AudioComponent.Sound` _value_2)) (`KismetSystemLibrary.GetPathName` (`local.Sound`)))
                (`self.StopSound` _trackid_2 _type_2)
                (bind _returnvalue_6 (`GameplayStatics.SpawnSound2D` (`local.Sound`) _startvolumemultiplier_3 _pitchmultiplier_3 _starttime_3 null :!label _label_2))
                (if (`local.RegisterSound`)
                  (`self.RegisterSound` (`local.SoundInfo`) _returnvalue_6))
                (`AudioComponent.AdjustVolume` _returnvalue_6 _fadeduration_3 _endvolumemultiplier_3 _audiofadercurve_3)
                (else
                  (if (`local.RegisterSound`)
                    (`self.RegisterSound` (`local.SoundInfo`) _value_2))
                  (`AudioComponent.AdjustVolume` _value_2 _fadeduration_3 _endvolumemultiplier_3 _audiofadercurve_3))))
            (:`Is Not Valid`
              (goto _label_2)))
          (else
            (goto _label_2)))))))

(fn `PlayForceFeedback`
  (params (ForceFeedbackEffectPath :type String))
  (returns (bSuccess :type Boolean))
  (bind (_asset _bsuccess) (`ShidenCoreFunctionLibrary.GetOrLoadAsset` ForceFeedbackEffectPath))
  (if _bsuccess
    (bind _asforce_feedback_effect (cast `ForceFeedbackEffect` _asset)
      (:`then`
        (`PlayerController.K2_ClientPlayForceFeedback` (`GameplayStatics.GetPlayerController` 0) _asforce_feedback_effect "None" false false false)
        (return true))
      (:`CastFailed`
        _)))
  (return false))

(fn `PlaySound`
  (params (SoundInfo :type "ShidenSoundInfo Structure") (bRegisterSound :type Boolean))
  (returns (Duration :type "Float (single-precision)") (bSuccess :type Boolean))
  (locals (SoundDuration :type "Float (single-precision)"))
  (bind ((`Type` _type) (`SoundPath` _soundpath) (`EndVolumeMultiplier` _endvolumemultiplier) (`FadeDuration` _fadeduration)) (break `ShidenSoundInfo` SoundInfo))
  (bind (_trackid _type_2) (break `ShidenSoundInfo` SoundInfo))
  (bind ((`Type` _type_3) (`SoundPath` _soundpath_2) (`AudioFaderCurve` _audiofadercurve)) (break `ShidenSoundInfo` SoundInfo))
  (bind _soundinfo (`local.SoundInfo`))
  (bind (_value _returnvalue) (`BlueprintMapLibrary.Map_Find` (`self.VoiceComponents`) _trackid))
  (bind (_value_2 _returnvalue_2) (`BlueprintMapLibrary.Map_Find` (`self.BgmComponents`) _trackid))
  (bind (_asset _bsuccess) (`ShidenCoreFunctionLibrary.GetOrLoadAsset` _soundpath_2))
  (bind _returnvalue_3 (`KismetMathLibrary.SelectFloat` _fadeduration 0.0 (== _endvolumemultiplier 0.0)))
  (if (and bRegisterSound (`KismetStringLibrary.IsEmpty` _soundpath))
    (switch `EShidenSoundType` _type_2
      (:`BGM`
        (if _returnvalue_2
          (`AudioComponent.FadeOut` _value_2 _returnvalue_3 0.0 _audiofadercurve)
          (`BlueprintMapLibrary.Map_Remove` (`self.BgmComponents`) _trackid))
        (return 0.0 true))
      (:`SE`
        (return 0.0 false))
      (:`Voice`
        (if _returnvalue
          (`AudioComponent.FadeOut` _value _returnvalue_3 0.0 _audiofadercurve)
          (`BlueprintMapLibrary.Map_Remove` (`self.VoiceComponents`) _trackid))
        (return 0.0 true)))
    (else
      (if _bsuccess
        (bind _assound_base (cast `SoundBase` _asset)
          (:`then`
            (bind (_soundtype _bsuccess_2) (`ShidenCoreFunctionLibrary.GetSoundTypeFromSoundBase` _assound_base))
            (if (and (`|EnumEquality` _type _soundtype) _bsuccess_2)
              (set `local.SoundDuration` (`SoundBase.Duration` _assound_base))
              (switch `EShidenSoundType` (`.Type` (break `ShidenSoundInfo` (`local.SoundInfo`)))
                (:`BGM`
                  (`self.PlayBgmOrVoice` _soundinfo _assound_base bRegisterSound :!label _label))
                (:`SE`
                  (`self.Play Se` _soundinfo _assound_base bRegisterSound))
                (:`Voice`
                  (goto _label)))
              (return (`local.SoundDuration`) true)
              (else
                (return 0.0 false))))
          (:`CastFailed`
            _)))
      (return 0.0 false))))

(fn `RegisterSound`
  (params (SoundInfo :type "ShidenSoundInfo Structure (by ref)") (AudioComponent :type "AudioComponent Object Reference (by ref)"))
  (bind ((`TrackId` _trackid) (`Type` _type)) (break `ShidenSoundInfo` SoundInfo))
  (if (`|EnumEquality` _type "SE")
    (`KismetArrayLibrary.Array_Add` (`self.SeComponents`) AudioComponent)
    (else
      (`BlueprintMapLibrary.Map_Add` (select `EShidenSoundType` _type :`BGM` (`self.BgmComponents`) :`Voice` (`self.VoiceComponents`)) _trackid AudioComponent)))
  (switch `EShidenSoundType` _type
    (:`BGM`
      (add `AudioComponent.OnAudioFinished` AudioComponent (`|CreateDelegate` :!event `OnBgmFinished`)))
    (:`SE`
      (add `AudioComponent.OnAudioFinished` AudioComponent (`|CreateDelegate` :!event `OnSeFinished`)))
    (:`Voice`
      (add `AudioComponent.OnAudioFinished` AudioComponent (`|CreateDelegate` :!event `OnVoiceFinished`)))))

(fn `RemoveSound`
  (params (SoundType :type "EShidenSoundType Enum" :default "BGM"))
  (bind _secomponents (`self.SeComponents`))
  (bind _returnvalue (select `EShidenSoundType` SoundType :`BGM` (`self.BgmComponents`) :`Voice` (`self.VoiceComponents`)))
  (if (`|EnumEquality` SoundType "SE")
    (for (_array_element _array_index) _secomponents
      (`/Engine/EditorBlueprintResources/StandardMacros.IsValid` _array_element
        (:`Is Valid`
          (if (`|EnumEquality` (`AudioComponent.GetPlayState` _array_element) "Stopped")
            (`KismetArrayLibrary.Array_Remove` _secomponents _array_index :!label _label)))
        (:`Is Not Valid`
          (goto _label))))
    (else
      (bind _values (`BlueprintMapLibrary.Map_Values` _returnvalue))
      (for (_array_element_2 _array_index_2) _values
        (`/Engine/EditorBlueprintResources/StandardMacros.IsValid` _array_element_2
          (:`Is Valid`
            (if (`|EnumEquality` (`AudioComponent.GetPlayState` _array_element_2) "Stopped")
              (`BlueprintMapLibrary.Map_Remove` _returnvalue _array_index_2 :!label _label_2)))
          (:`Is Not Valid`
            (goto _label_2)))))))

(fn `UserConstructionScript`)