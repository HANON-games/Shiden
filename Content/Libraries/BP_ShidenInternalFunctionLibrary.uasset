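; Internal function library for the Shiden scenario system that resolves commands, looks up scenarios and preloads the assets a scenario needs.
; ConstructCommand fills empty arguments from project-config presets, then substitutes variables.
; LoadScenarioAssetsPaths asks each enabled command object for its asset paths, recursing into macro scenarios.
; LoadScenarioAssets loads those paths into the subsystem's AssetCache, returning errors with scenario ID and index.
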(fn `ConstructCommand`
  (params (ProcessName :type String :default "Default") (OriginalCommand :type "ShidenCommand Structure (by ref)"))
  (returns (ConstructedCommand :type "ShidenCommand Structure"))
  (bind (_commandname _presetname _arg1 _arg2 _arg3 _arg4 _arg5 _arg6 _arg7 _arg8 _arg9 _arg10 _commandid _benabled) (break `ShidenCommand` OriginalCommand))
  (if (not (`KismetStringLibrary.IsEmpty` _presetname))
    (for _array_element (`.Presets` (defaults `ShidenProjectConfig` "/Script/ShidenCore.ShidenProjectConfig"))
      (bind (_commandname_2 _presetname_2 _arg1_2 _arg2_2 _arg3_2 _arg4_2 _arg5_2 _arg6_2 _arg7_2 _arg8_2 _arg9_2 _arg10_2) (break `ShidenPreset` _array_element))
      (if (and (`KismetStringLibrary.EqualEqual_StrStr` _commandname _commandname_2) (`KismetStringLibrary.EqualEqual_StrStr` _presetname _presetname_2))
        (for _index (range 10)
          (switch `int` _index
            (:`0`
              (bind _returnvalue (select `int` _index :`0` _arg1 :`1` _arg2 :`2` _arg3 :`3` _arg4 :`4` _arg5 :`5` _arg6 :`6` _arg7 :`7` _arg8 :`8` _arg9 :`9` _arg10))
              (bind _returnvalue_2 (`KismetMathLibrary.SelectString` (select `int` _index :`0` _arg1_2 :`1` _arg2_2 :`2` _arg3_2 :`3` _arg4_2 :`4` _arg5_2 :`5` _arg6_2 :`6` _arg7_2 :`7` _arg8_2 :`8` _arg9_2 :`9` _arg10_2) _returnvalue (`KismetStringLibrary.IsEmpty` _returnvalue)))
              (bind _structout (setmembers `ShidenCommand` :`StructRef` (make `ShidenCommand` _commandname _presetname "" "" "" "" "" "" "" "" "" "" _commandid _benabled) :`Arg1` _returnvalue_2)))
            (:`1`
              (bind _structout_2 (setmembers `ShidenCommand` :`StructRef` _structout :`Arg2` _returnvalue_2)))
            (:`2`
              (bind _structout_3 (setmembers `ShidenCommand` :`StructRef` _structout_2 :`Arg3` _returnvalue_2)))
            (:`3`
              (bind _structout_4 (setmembers `ShidenCommand` :`StructRef` _structout_3 :`Arg4` _returnvalue_2)))
            (:`4`
              (bind _structout_5 (setmembers `ShidenCommand` :`StructRef` _structout_4 :`Arg5` _returnvalue_2)))
            (:`5`
              (bind _structout_6 (setmembers `ShidenCommand` :`StructRef` _structout_5 :`Arg6` _returnvalue_2)))
            (:`6`
              (bind _structout_7 (setmembers `ShidenCommand` :`StructRef` _structout_6 :`Arg7` _returnvalue_2)))
            (:`7`
              (bind _structout_8 (setmembers `ShidenCommand` :`StructRef` _structout_7 :`Arg8` _returnvalue_2)))
            (:`8`
              (bind _structout_9 (setmembers `ShidenCommand` :`StructRef` _structout_8 :`Arg9` _returnvalue_2)))
            (:`9`
              (bind _structout_10 (setmembers `ShidenCommand` :`StructRef` _structout_9 :`Arg10` _returnvalue_2)))))
        (bind _returnvalue_3 (`ShidenVariableFunctionLibrary.ReplaceAllTextWithVariable` ProcessName _structout_10))
        (return _returnvalue_3))))
  (bind _returnvalue_4 (`ShidenVariableFunctionLibrary.ReplaceAllTextWithVariable` ProcessName OriginalCommand))
  (return _returnvalue_4))

(fn `GetCommandFromCache`
  (params (Outer :type "Object Object Reference") (ProcessName :type String :default "Default") (CommandSoftObjectPath :type "SoftObjectPath Structure"))
  (returns (Object :type "Object Object Reference") (Sccess :type Boolean))
  (locals (Key :type String))
  (bind (_value _returnvalue) (`BlueprintMapLibrary.Map_Find` (`ShidenSubsystem.CommandCache` (subsystem `ShidenSubsystem`)) (`local.Key`)))
  (set `local.Key` (`KismetStringLibrary.Concat_StrStr` ProcessName "::" (`KismetSystemLibrary.BreakSoftObjectPath` CommandSoftObjectPath)))
  (if _returnvalue
    (`/Engine/EditorBlueprintResources/StandardMacros.IsValid` _value
      (:`Is Valid`
        (return _value true))
      (:`Is Not Valid`
        _)))
  (bind (_shidencommandobject _sccess) (`self.GetCommandOld` Outer CommandSoftObjectPath))
  (if _sccess
    (`BlueprintMapLibrary.Map_Add` (`ShidenSubsystem.CommandCache` (subsystem `ShidenSubsystem`)) (`local.Key`) _shidencommandobject)
    (return _shidencommandobject true)
    (else
      (return null false))))

(fn `GetCommandOld`
  (params (Outer :type "Object Object Reference") (CommandSoftObjectPath :type "SoftObjectPath Structure"))
  (returns (ShidenCommandObject :type "ShidenCommandObject Object Reference") (Sccess :type Boolean))
  (bind _returnvalue (`ShidenCoreFunctionLibrary.ConstructBlueprintClassFromSoftObjectPath` CommandSoftObjectPath))
  (bind _returnvalue_2 (`|GenericCreateObject` Outer _returnvalue))
  (if (`KismetSystemLibrary.DoesImplementInterface` _returnvalue_2 "/Shiden/Commands/Core/BI_ShidenCommandInterface.BI_ShidenCommandInterface_C")
    (bind _asshiden_command_object (cast `ShidenCommandObject` _returnvalue_2)
      (:`then`
        (return _asshiden_command_object true))
      (:`CastFailed`
        _)))
  (return null false))

(fn `GetScenarioByIdOrObjectPath`
  (params (ScenarioIdOrObjectPath :type String))
  (returns (ScenarioId :type "Guid Structure") (Scenario :type "ShidenScenario Object Reference") (Succeeded :type Boolean))
  (bind (_outguid _success) (`KismetGuidLibrary.Parse_StringToGuid` ScenarioIdOrObjectPath))
  (bind _scenariopaths (defaults `ShidenProjectConfig` "/Script/ShidenCore.ShidenProjectConfig"))
  (if _success
    (bind (_scenario _bsuccess) (`ShidenScenarioFunctionLibrary.GetScenarioFromCache` _outguid))
    (return _outguid _scenario _bsuccess)
    (else
      (bind _keys (`BlueprintMapLibrary.Map_Keys` _scenariopaths))
      (for _array_element _keys
        (if (`KismetStringLibrary.EqualEqual_StrStr` ScenarioIdOrObjectPath (`BlueprintMapLibrary.Map_Find` _scenariopaths _array_element))
          (bind (_scenario_2 _bsuccess_2) (`ShidenScenarioFunctionLibrary.GetScenarioFromCache` _array_element))
          (return _array_element _scenario_2 _bsuccess_2)))
      (return (struct) null false))))

(fn `GetScenarioByPackagePath`
  (params (PackagePath :type String))
  (returns (Scenario :type "ShidenScenario Object Reference") (Succeeded :type Boolean))
  (bind _returnvalue (`AssetRegistry.GetAssetByObjectPath` (`AssetRegistryHelpers.GetAssetRegistry`) (`self.MakeObjectPathFromPackagePath` PackagePath) false))
  (bind _asshiden_scenario (cast `ShidenScenario` (`AssetRegistryHelpers.GetAsset` _returnvalue))
    (:`then`
      (return _asshiden_scenario true))
    (:`CastFailed`
      (return null false))))

(fn `LoadScenarioAssets`
  (params (Outer :type "Object Object Reference"))
  (returns (Succeeded :type Boolean) (ErrorMessage :type String) (ErrorScenarioId :type "Guid Structure") (ErrorIndex :type Integer))
  (bind _scenarioprogress (`ShidenScenarioFunctionLibrary.PeekScenario` "Default"))
  (bind (_scenario _bsuccess) (`ShidenScenarioFunctionLibrary.GetScenarioFromCache` (break `ShidenScenarioProgress` _scenarioprogress)))
  (if _bsuccess
    (`BlueprintMapLibrary.Map_Clear` (`ShidenSubsystem.AssetCache` (subsystem `ShidenSubsystem`)))
    (bind (_assetpaths _succeeded _errormessage _errorscenarioid _errorindex) (`self.LoadScenarioAssetsPaths` Outer _scenario))
    (if _succeeded
      (for _array_element _assetpaths
        (bind _returnvalue (`AssetRegistry.GetAssetByObjectPath` (`AssetRegistryHelpers.GetAssetRegistry`) (`KismetStringLibrary.Conv_StringToName` (`.ObjectPath` (break `ShidenLoadingAssetInfo` _array_element))) false))
        (bind _returnvalue_2 (`AssetRegistryHelpers.GetAsset` _returnvalue))
        (`/Engine/EditorBlueprintResources/StandardMacros.IsValid` _returnvalue_2
          (:`Is Valid`
            (`BlueprintMapLibrary.Map_Add` (`ShidenSubsystem.AssetCache` (subsystem `ShidenSubsystem`)) (`.ObjectPath` (break `ShidenLoadingAssetInfo` _array_element)) _returnvalue_2))
          (:`Is Not Valid`
            (return false (`KismetStringLibrary.Concat_StrStr` "Load Asset Failed: " (`.ObjectPath` (break `ShidenLoadingAssetInfo` _array_element))) (break `ShidenScenarioProgress` _scenarioprogress) (break `ShidenLoadingAssetInfo` _array_element)))))
      (return true "" (struct) 0)
      (else
        (return false _errormessage _errorscenarioid _errorindex)))
    (else
      (return false (`KismetStringLibrary.Concat_StrStr` "Load scenario failed: " (`BlueprintMapLibrary.Map_Find` (defaults `ShidenProjectConfig` "/Script/ShidenCore.ShidenProjectConfig") (break `ShidenScenarioProgress` _scenarioprogress))) (break `ShidenScenarioProgress` _scenarioprogress) -1))))

(fn `LoadScenarioAssetsPaths`
  (params (Outer :type "Object Object Reference") (ScenarioDataAsset :type "ShidenScenario Object Reference"))
  (returns (AssetPaths :type "Array of ShidenLoadingAssetInfo Structure") (Succeeded :type Boolean) (ErrorMessage :type String) (ErrorScenarioId :type "Guid Structure") (ErrorIndex :type Integer))
  (locals (ScenarioAssetPaths :type "Array of ShidenLoadingAssetInfo Structure"))
  (bind _commanddefinitioncache (`ShidenSubsystem.CommandDefinitionCache` (subsystem `ShidenSubsystem`)))
  (for (_array_element _array_index) (`ShidenScenario.Commands` ScenarioDataAsset)
    (bind _constructedcommand (`self.ConstructCommand` "Default" _array_element))
    (bind (_commandname _presetname _arg1 _arg2 _arg3 _arg4 _arg5 _arg6 _arg7 _arg8 _arg9 _arg10 _commandid _benabled) (break `ShidenCommand` _constructedcommand))
    (if _benabled
      (switch `string` _commandname
        (:`Default`
          (if (`BlueprintMapLibrary.Map_IsEmpty` _commanddefinitioncache)
            (`ShidenCoreFunctionLibrary.InitCommandDefinitions`))
          (bind (_shidencommandobject _sccess) (`self.GetCommandOld` Outer (`.CommandBlueprint` (break `ShidenCommandDefinition` (`BlueprintMapLibrary.Map_Find` _commanddefinitioncache _commandname)))))
          (if _sccess
            (bind _assetobjectpaths (message `/Shiden/Commands/Core/BI_ShidenCommandInterface.GetAssetPaths` _shidencommandobject _constructedcommand))
            (`BlueprintSetLibrary.Set_Remove` _assetobjectpaths) ; Remove Empty
            (bind _result (`BlueprintSetLibrary.Set_ToArray` _assetobjectpaths))
            (for _array_element_2 _result
              (`KismetArrayLibrary.Array_AddUnique` (`local.ScenarioAssetPaths`) (make `ShidenLoadingAssetInfo` _array_index _array_element_2)))
            (else
              (return _ false (`KismetStringLibrary.Concat_StrStr` "Get Command \"" _commandname "\" Failed. Please check project config and command definitions.") (`ShidenScenario.ScenarioId` ScenarioDataAsset) _array_index))))
        (:`RunMacro`
          (if (not (`KismetStringLibrary.IsEmpty` _arg1))
            (bind (_scenarioid _scenario _succeeded) (`self.GetScenarioByIdOrObjectPath` _arg1))
            (if _succeeded
              (bind (_assetpaths _succeeded_2 _errormessage _errorscenarioid _errorindex) (`self.LoadScenarioAssetsPaths` (`local.Outer`) _scenario))
              (if _succeeded_2
                (for _array_element_3 _assetpaths
                  (`KismetArrayLibrary.Array_AddUnique` (`local.ScenarioAssetPaths`) _array_element_3))
                (else
                  (return _ false _errormessage _errorscenarioid _errorindex)))
              (else
                (return _ false (`KismetStringLibrary.Concat_StrStr` "Load scenario failed: " _arg1) (`ShidenScenario.ScenarioId` ScenarioDataAsset) _array_index)))))
        (:`RunMacroAsParallel`
          (if (not (or (`KismetStringLibrary.IsEmpty` _arg1) (`KismetStringLibrary.IsEmpty` _arg2)))
            (bind (_scenarioid_2 _scenario_2 _succeeded_3) (`self.GetScenarioByIdOrObjectPath` _arg2))
            (if _succeeded_3
              (bind (_assetpaths_2 _succeeded_4 _errormessage_2 _errorscenarioid_2 _errorindex_2) (`self.LoadScenarioAssetsPaths` (`local.Outer`) _scenario_2))
              (if _succeeded_4
                (for _array_element_4 _assetpaths_2
                  (`KismetArrayLibrary.Array_AddUnique` (`local.ScenarioAssetPaths`) _array_element_4))
                (else
                  (return _ false _errormessage_2 _errorscenarioid_2 _errorindex_2)))
              (else
                (return _ false (`KismetStringLibrary.Concat_StrStr` "Load scenario failed: " _arg2) (`ShidenScenario.ScenarioId` ScenarioDataAsset) _array_index))))))))
  (return (`local.ScenarioAssetPaths`) true "" (struct) 0))

(fn `MakeErrorMessage`
  (params (ScenarioId :type "Guid Structure") (Index :type Integer) (CommandName :type String) (ErrorMessage :type String))
  (returns (Message :type String))
  (return (`KismetStringLibrary.Concat_StrStr` "[" (`KismetStringLibrary.Split` (`.RightS` (`KismetStringLibrary.Split` (`BlueprintMapLibrary.Map_Find` (defaults `ShidenProjectConfig` "/Script/ShidenCore.ShidenProjectConfig") ScenarioId) "/" "IgnoreCase" "FromEnd")) "." "IgnoreCase" "FromEnd") (`KismetMathLibrary.SelectString` "" (`KismetStringLibrary.Concat_StrStr` ":" (`KismetStringLibrary.Conv_IntToString` (+ Index 1))) (== Index -1)) "] " (`KismetMathLibrary.SelectString` "" (`KismetStringLibrary.Concat_StrStr` CommandName ": ") (`KismetStringLibrary.IsEmpty` CommandName)) ErrorMessage)))

(fn `MakeObjectPathFromPackagePath`
  (params (PackagePath :type String))
  (returns (ObjectPath :type Name))
  (return (`KismetStringLibrary.Conv_StringToName` (`KismetStringLibrary.Concat_StrStr` PackagePath "." (`.RightS` (`KismetStringLibrary.Split` PackagePath "/" "IgnoreCase" "FromEnd"))))))

(fn `PushScenarioByDataAsset`
  (params (ProcessName :type String :default "Default") (ScenarioDataAsset :type "ShidenScenario Object Reference"))
  (`BlueprintMapLibrary.Map_Add` (`ShidenSubsystem.ScenarioCache` (subsystem `ShidenSubsystem`)) (`ShidenScenario.ScenarioId` ScenarioDataAsset) ScenarioDataAsset)
  (`ShidenScenarioFunctionLibrary.PushScenario` ProcessName ScenarioDataAsset)
  (return))